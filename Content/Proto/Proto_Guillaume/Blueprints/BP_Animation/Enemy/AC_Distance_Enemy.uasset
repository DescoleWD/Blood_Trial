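; Actor component that runs the attack of a ranged enemy character, covering spell casts and melee hits.
; Its attack event is gated by a CanAttaque flag and plays the first attack montage on the owner's mesh.
; Montage notifies open or close the attack window, make a Distance owner cast its spell, or trigger a socket-to-socket sphere trace that damages pawns, ignoring Enemy-tagged actors.
; TriggerSimpleHit is empty, its box-trace logic disconnected.
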(event Custom|Attaque_Enemy_Distance
  (if (Variables|Default|GetCanAttaque)
    (Variables|Default|SetCanAttaque false)
    (if true
      (bind _notifyname (Animation|Montage|PlayMontage (Variables|/Script/Engine.Character|GetMesh (Variables|Default|GetOwner)) (Utilities|Array|Get(acopy) (Variables|Default|GetAnimationAttaque_V1)))
        (:OnCompleted
          (Variables|Default|SetCanAttaque true))
        (:OnNotifyBegin
          (switch name _notifyname
            (:Hit
              (CallFunction|TriggerComplexeHit))
            (:CanCombo
              (Variables|Default|SetCanAttaque true))
            (:Recovery
              (Variables|Default|SetCanAttaque false))
            (:Cast_Spell_D
              (bind _asdistance (Utilities|Casting|CastToDistance (Variables|Default|GetOwner)))
              (Default|CastSpell _asdistance))))))))

(event EventBeginPlay
  (bind _ascharacter (Utilities|Casting|CastToCharacter (Components|GetOwner)))
  (Variables|Default|SetOwner _ascharacter))

(fn TriggerSimpleHit)

(fn TriggerComplexeHit
  (bind _asenemy_true (Utilities|Casting|CastToEnemy_True (Variables|Default|GetOwner)))
  (bind _outactors (Actor|GetAllActorswithTag "Enemy"))
  (bind (_outhit _returnvalue) (Collision|SphereTraceForObjects (Transformation|GetSocketLocation (Variables|/Script/Engine.Character|GetMesh _asenemy_true) "SocketMelee_Start") (Transformation|GetSocketLocation (Variables|/Script/Engine.Character|GetMesh _asenemy_true) "SocketMelee_End") 1e+02 (Utilities|Array|MakeArray "ObjectTypeQuery3") false _outactors "None"))
  (if _returnvalue
    (if (Variables|/Script/Engine.Actor|GetbCanBeDamaged (.HitActor (Collision|BreakHitResult _outhit)))
      (CallFunction|Damage _asenemy_true (Variables|Default|GetEnemyDamage) (.HitActor (Collision|BreakHitResult _outhit))))))