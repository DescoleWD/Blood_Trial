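; Prototype blood wave attack actor that damages the first damageable non-player it detects, then destroys itself.
; When its static mesh begins an overlap, it runs a stationary capsule trace for pawns and physics bodies, ignoring actors tagged Player.
; Damage comes from the BloodWaveDamage value returned by GetInst.
; Debug drawing and prints remain active, and movement is not handled in these graphs.
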(event OnComponentBeginOverlap(StaticMesh)
  (params (OverlappedComponent :type Primitive%20Component%20Object%20Reference) (OtherActor :type Actor%20Object%20Reference) (OtherComp :type Primitive%20Component%20Object%20Reference) (OtherBodyIndex :type Integer) (bFromSweep :type Boolean) (SweepResult :type Hit%20Result%20Structure%20%28by%20ref%29))
  (bind _returnvalue (Transformation|GetWorldLocation OverlappedComponent))
  (bind _outactors (Actor|GetAllActorswithTag "Player"))
  (bind (_outhit _returnvalue_2) (Class|KismetSystemLibrary|CapsuleTraceSingleforObjects _returnvalue _returnvalue 1e+02 1e+02 (Utilities|Array|MakeArray "ObjectTypeQuery3" "ObjectTypeQuery4") false _outactors "ForDuration" true))
  (Development|PrintText (Utilities|Text|FormatText "BlockingHit={in1} 
returnValue={in2}  
InitialOverlap={in3} 
ImpactPoint={6} 
HitActor={10}" (.bBlockingHit (Collision|BreakHitResult _outhit)) _returnvalue_2 (.bInitialOverlap (Collision|BreakHitResult _outhit)) 0 (.HitActor (Collision|BreakHitResult _outhit))))
  ;[1 0 0.113] Zone de merde
  (if _returnvalue_2
    (if (Variables|/Script/Engine.Actor|GetbCanBeDamaged (.HitActor (Collision|BreakHitResult _outhit)))
      (Game|Damage|ApplyDamage (.HitActor (Collision|BreakHitResult _outhit)) (Variables|/Game/Proto/Main/Blueprint/BloodTrial_GameInstance.BloodTrial_GameInstance_C|GetBloodWave_Damage (CallFunction|GetInst)) 0 0)
      (Actor|DestroyActor)
      (Development|PrintString "Hello" true true "(R=1.000000,G=0.000000,B=0.010551,A=1.000000)"))))

(event Collision|EventHit
  (params (MyComp :type Primitive%20Component%20Object%20Reference) (Other :type Actor%20Object%20Reference) (OtherComp :type Primitive%20Component%20Object%20Reference) (bSelfMoved :type Boolean) (HitLocation :type Vector :default "0, 0, 0") (HitNormal :type Vector :default "0, 0, 0") (NormalImpulse :type Vector :default "0, 0, 0") (Hit :type Hit%20Result%20Structure%20%28by%20ref%29)))

(fn ConstructionScript)