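; Actor component that runs an NPC's branching dialogue from a data table through the NPC_Dialogue widget.
; Each line advance reads its row, redirects it by quest status or conditions, then updates text and spawns response buttons.
; Rows can also message the owner for shop, quest, trainer or goodbye events, camera transitions, actor activation and animation, or play sounds.
; Return lines are saved via the game mode and restored on BeginPlay.
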(event Custom|BeginDialogue
  (params (NPC%20Dialogue :type Data%20Table%20Object%20Reference) (NPC%20Name :type Text))
  ;[1 1 1] Setup Dialogue
  (Variables|Default|SetNPC%20Dialogue%20DT NPC%20Dialogue)
  (bind _returnvalue (UserInterface|CreateWidget "/Game/FlexibleCombatSystem/Widgets/NPC/NPC_Dialogue.NPC_Dialogue_C"))
  (Default|UpdateName _returnvalue NPC%20Name)
  (UserInterface|Viewport|AddtoViewport _returnvalue 0)
  (bind _output_get (Variables|Default|SetWB%20Dialogue _returnvalue))
  (Variables|/Game/FlexibleCombatSystem/Widgets/NPC/NPC_Dialogue.NPC_Dialogue_C|SetDialogueComponent _output_get self)
  (EventDispatchers|BindEventtoNextDialogueLine _output_get (delegate Custom|RunDialogue))
  (bind _output_get_2 (Variables|Default|SetDialogueLine (Variables|Default|GetStoredStartLine)))
  (CallFunction|RunDialogue _output_get_2 "NewEnumerator6"))

(event Custom|RunDialogue
  (params (Dialogue%20Line :type Integer) (Trigger%20Event :type E_DialogueEvents%20Enum :default "NewEnumerator6"))
  (bind _dialoguelineinfo (Variables|Default|GetDialogueLineInfo))
  (bind (_storedialoguelinereturnnumber _dialoguelinereturnnumber) (Utilities|Struct|BreakS_DialogueInfo _dialoguelineinfo))
  ;[1 1 1] Run Dialogue - Runs Everytime Dialogue Widget Triggers Through Click
  (bind _midtransition (CallFunction|CameraTransitionUnderway))
  (if (not _midtransition)
    (Variables|Default|SetDialogueLine Dialogue%20Line)
    (Variables|Default|SetTrigger%20Event Trigger%20Event)
    (CallFunction|PassDialogueInfo)
    (CallFunction|ConditionAdjustments)
    (CallFunction|UpdateDialogueLine)
    (CallFunction|AddResponses)
    (CallFunction|CameraTransition)
    (CallFunction|TriggerEvent)
    (CallFunction|ActivateActor)
    (CallFunction|PlaySound&Animation)
    ;;[1 1 1] Update New Dialogue Start Point
    (if _storedialoguelinereturnnumber
      (Variables|Default|SetStoredStartLine _dialoguelinereturnnumber)
      (CallFunction|DialogueWorthSaving))))

(event EventBeginPlay
  ;[1 1 1] Load Save Data
  (CallFunction|LoadSaveData))

(fn UpdateDialogueLine
  (bind _outrownames (DataTable|GetDataTableRowNames (Variables|Default|GetNPC%20Dialogue%20DT)))
  (bind _returnvalue (Utilities|GetDataTableRow (Variables|Default|GetNPC%20Dialogue%20DT) (Utilities|Array|Get(acopy) _outrownames (- (Variables|Default|GetDialogueLine) 1)))
    (:then
      (bind _output_get (Variables|Default|SetDialogueLineInfo _returnvalue))
      (Default|UpdateText (Variables|Default|GetWB%20Dialogue) (.DialogueLine (Utilities|Struct|BreakS_DialogueInfo _output_get)) (.NextDialogueLine (Utilities|Struct|BreakS_DialogueInfo _output_get)) (.TriggerEvent (Utilities|Struct|BreakS_DialogueInfo _output_get))))))

(fn AddResponses
  (bind _dialoguelineinfo (Variables|Default|GetDialogueLineInfo))
  (bind _reponses (Utilities|Struct|BreakS_DialogueInfo _dialoguelineinfo))
  (Widget|Panel|ClearChildren (Variables|/Game/FlexibleCombatSystem/Widgets/NPC/NPC_ResponseBox.NPC_ResponseBox_C|GetResponseList (Variables|/Game/FlexibleCombatSystem/Widgets/NPC/NPC_Dialogue.NPC_Dialogue_C|GetNPC_ResponseBox (Variables|Default|GetWB%20Dialogue))))
  (bind _output_get (Variables|/Game/FlexibleCombatSystem/Widgets/NPC/NPC_Dialogue.NPC_Dialogue_C|SetResponsesAvailable (Variables|Default|GetWB%20Dialogue) (> (Utilities|Array|Length _reponses) 0)))
  (if _output_get
    (for _array_element _reponses
      (bind _returnvalue (UserInterface|CreateWidget "/Game/FlexibleCombatSystem/Widgets/NPC/NPC_DialogueResponse.NPC_DialogueResponse_C" 0 (.Response (Utilities|Struct|BreakS_DialogueResponses _array_element)) (.NextDialogueLine (Utilities|Struct|BreakS_DialogueResponses _array_element)) (.TriggerEvent (Utilities|Struct|BreakS_DialogueResponses _array_element)) (Variables|Default|GetWB%20Dialogue)))
      (Class|VerticalBox|AddChildtoVerticalBox (Variables|/Game/FlexibleCombatSystem/Widgets/NPC/NPC_ResponseBox.NPC_ResponseBox_C|GetResponseList (Variables|/Game/FlexibleCombatSystem/Widgets/NPC/NPC_Dialogue.NPC_Dialogue_C|GetNPC_ResponseBox (Variables|Default|GetWB%20Dialogue))) _returnvalue)
      ;[1 1 1] If Actor Should Activate & Quest Valid, Activate With Quest
      (if (and (Utilities|Enum|Equal(Enum) (.TriggerEvent (Utilities|Struct|BreakS_DialogueResponses _array_element)) "NewEnumerator1") (!= (Utilities|Struct|BreakS_DialogueInfo (Variables|Default|GetDialogueLineInfo)) 0))
        (Variables|Default|SetQuestActivatedActor true)
        (Class|INPC|PassActorActivateNo(Message) (Components|GetOwner) (.ActivateActorFalse0 (Utilities|Struct|BreakS_DialogueInfo (Variables|Default|GetDialogueLineInfo))))))))

(fn TriggerEvent
  (bind _returnvalue (Components|GetOwner))
  (switch Utilities|FlowControl|Switch|SwitchonE_DialogueEvents (Variables|Default|GetTrigger%20Event)
    (:NewEnumerator2
      (Class|INPC|BeginTrading(Message) _returnvalue))
    (:NewEnumerator0
      (Class|INPC|EndConversation(Message) _returnvalue))
    (:NewEnumerator1
      (Class|INPC|TriggerQuest(Message) _returnvalue))
    (:NewEnumerator3
      (Class|INPC|BeginTraining(Message) _returnvalue)))
  (Widget|RemovefromParent (Variables|Default|GetWB%20Dialogue)))

(fn PlaySound&Animation
  (bind _dialoguelineinfo (Variables|Default|GetDialogueLineInfo))
  (bind (_soundtoplay _animationtoplay) (Utilities|Struct|BreakS_DialogueInfo _dialoguelineinfo))
  (Utilities|IsValid _soundtoplay
    (:Is%20Valid
      (Audio|PlaySound2D _soundtoplay 1.0 1.0 0.0 0 0))
    (:Is%20Not%20Valid
      _))
  (Utilities|IsValid _animationtoplay
    (:Is%20Valid
      (Class|INPC|PlayAnimation(Message) (Components|GetOwner) _animationtoplay))))

(fn ActivateActor
  (bind _dialoguelineinfo (Variables|Default|GetDialogueLineInfo))
  (bind _activateactorfalse0 (Utilities|Struct|BreakS_DialogueInfo _dialoguelineinfo))
  ;[1 1 1] Only Activate Actor IF - (Activate Actor Not 0) & (Camera Not Mid Transition) & (Quest Not Activating It)
  (if (Math|Boolean|ORBoolean (== _activateactorfalse0 0) (Variables|Default|GetMidCameraTransition) (Variables|Default|GetQuestActivatedActor))
    (Variables|Default|SetQuestActivatedActor false)
    (else
      (Class|INPC|ActivateActor(Message) (Components|GetOwner) _activateactorfalse0))))

(fn ConditionAdjustments
  (bind _returnvalue (Components|GetOwner))
  (bind _questcompletedialogueline (Variables|Condition|GetQuestCompleteDialogueLine))
  (bind _queststarteddialogueline (Variables|Condition|GetQuestStartedDialogueLine))
  (bind _questcomponent (Variables|Default|GetQuestComponent))
  (bind _returnvalue_2 (Actor|GetComponentbyClass _returnvalue "/Game/FlexibleCombatSystem/Blueprints/Components/QuestComponent.QuestComponent_C"))
  ;[1 1 1] Trigger Event Gets Updated After Line. IF Dialogue = First Line Use
  (if (Utilities|Enum|Equal(Enum) (Utilities|Struct|BreakS_DialogueInfo (Variables|Default|GetDialogueLineInfo)) "NewEnumerator1")
    ;[1 1 1] If Conditions Not Met Change Dialogue
    (if (Variables|/Game/FlexibleCombatSystem/Blueprints/Components/QuestComponent.QuestComponent_C|GetQuestConditionsMet (Variables|Default|GetQuestComponent))
      (if (or (Variables|/Game/FlexibleCombatSystem/Blueprints/Components/QuestComponent.QuestComponent_C|GetQuestAccepted _returnvalue_2) (Variables|/Game/FlexibleCombatSystem/Blueprints/Components/QuestComponent.QuestComponent_C|GetQuestCompleted _returnvalue_2)) :!label _label
        (CallFunction|DialogueWorthSaving)
        ;[1 1 1] Change Dialogue Based Upon Quest Status
        (if (Variables|/Game/FlexibleCombatSystem/Blueprints/Components/QuestComponent.QuestComponent_C|GetQuestCompleted _questcomponent)
          (if (== _questcompletedialogueline 0)
            _
            (else
              (Variables|Default|SetDialogueLine _questcompletedialogueline)))
          (Variables|/Game/FlexibleCombatSystem/Blueprints/Components/QuestComponent.QuestComponent_C|SetQuestCompleted _questcomponent false)
          (elif (Variables|/Game/FlexibleCombatSystem/Blueprints/Components/QuestComponent.QuestComponent_C|GetQuestAccepted _questcomponent)
            (if (not (== _queststarteddialogueline 0))
              (Variables|Default|SetDialogueLine _queststarteddialogueline)))))
      (else
        (Variables|Default|SetDialogueLine (Variables|Condition|GetQuestConditionFailed))))
    (else
      (goto _label))))

(fn DialogueWorthSaving
  (Class|IGameMode|DialogueComponentSaving(Message) (Game|GetGameMode) (Components|GetOwner)))

(fn LoadSaveData
  (bind _returnvalue (SaveGame|LoadGamefromSlot "save1"))
  (bind _asbp_save_game (Utilities|Casting|CastToBP_SaveGame _returnvalue))
  (for _array_element (Variables|/Game/FlexibleCombatSystem/Blueprints/BP_SaveGame.BP_SaveGame_C|GetDialogueSaveData _asbp_save_game)
    (if (Utilities|Enum|Equal(Enum) (Utilities|GetObjectName (Components|GetOwner)) (.QuestGiverName (Utilities|Struct|BreakS_DialogueSaveData _array_element)))
      (Variables|Default|SetStoredStartLine (.StoredStartLine (Utilities|Struct|BreakS_DialogueSaveData _array_element)))
      (Variables|Condition|SetQuestStartedDialogueLine (.QuestStartedLine (Utilities|Struct|BreakS_DialogueSaveData _array_element)))
      (Variables|Condition|SetQuestCompleteDialogueLine (.QuestCompleteLine (Utilities|Struct|BreakS_DialogueSaveData _array_element)))))
  (return))

(fn PassDialogueInfo
  ;[1 1 1] Quest Component Ref
  (bind _output_get (Variables|Default|SetQuestComponent (Actor|GetComponentbyClass (Components|GetOwner) "/Game/FlexibleCombatSystem/Blueprints/Components/QuestComponent.QuestComponent_C")))
  (Variables|Default|SetQuest%20Conditions (Variables|/Game/FlexibleCombatSystem/Blueprints/Components/QuestComponent.QuestComponent_C|GetQuestConditions _output_get))
  ;[1 1 1] Generating Dialogue Line
  (bind _outrownames (DataTable|GetDataTableRowNames (Variables|Default|GetNPC%20Dialogue%20DT)))
  (bind _returnvalue (Utilities|GetDataTableRow (Variables|Default|GetNPC%20Dialogue%20DT) (Utilities|Array|Get(acopy) _outrownames (- (Variables|Default|GetDialogueLine) 1)))
    (:then
      (bind _output_get_2 (Variables|Default|SetDialogueLineInfo _returnvalue))
      ;[1 1 1] Setting Dialogue Variables
      (Variables|Default|SetActivate%20Camera%20Transition (.ActivateCameraTransitionFalse0 (Utilities|Struct|BreakS_DialogueInfo _output_get_2)))
      (Variables|Condition|SetQuestStartedDialogueLine (.DialogueLineQuestStarted (Utilities|Struct|BreakS_DialogueInfo _output_get_2)))
      (Variables|Condition|SetQuestCompleteDialogueLine (.DialogueLineQuestCompleted (Utilities|Struct|BreakS_DialogueInfo _output_get_2)))
      (Variables|Condition|SetQuestConditionFailed (.DialogueLineQuestConditionsFailed (Utilities|Struct|BreakS_DialogueInfo _output_get_2))))))

(fn CameraTransition
  (bind _activate_camera_transition (Variables|Default|GetActivate%20Camera%20Transition))
  (if (not (== _activate_camera_transition 0))
    (Class|INPC|TransitionCamera(Message) (Components|GetOwner) (- _activate_camera_transition 1))
    (Variables|Default|SetMidCameraTransition true)))

(fn CameraTransitionUnderway
  (if (Variables|Default|GetMidCameraTransition)
    (Class|INPC|TransitionCamera(Message) (Components|GetOwner) (- (Variables|Default|GetActivate%20Camera%20Transition) 1))
    (return true)
    (else
      (return false))))

(fn PlaySound&Animationn)