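; Prototype Blueprint function library of gameplay helpers for montage checks, damage randomisation and chain-lightning effects.
; SpawnLightning sphere-traces pawns around an actor and chains beam emitters between successive hits via Source/Target parameters, but its point-damage call is unreachable.
; RandomMinMaxValue rolls between three-quarters and full damage.
; Slot, quest, button and animation-passing functions are empty stubs, and ScreenPosition returns zero on every branch.
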(fn GetSlotNumber
  (params (InventoryComponent :type %20Object%20Reference) (Item%20Type :type Byte :default 0)))

(fn IsPlayingMontage
  (params (Mesh :type Skeletal%20Mesh%20Component%20Object%20Reference) (Montage :type Anim%20Montage%20Object%20Reference))
  (bind _returnvalue (Components|SkeletalMesh|GetAnimInstance Mesh))
  (Utilities|IsValid _returnvalue
    (:Is%20Valid
      (return (Animation|Montage|MontageIsPlaying _returnvalue Montage)))
    (:Is%20Not%20Valid
      (return false))))

(fn ScreenPosition
  (bind _returnvalue (Class|WidgetLayoutLibrary|GetMousePositiononViewport))
  (bind _returnvalue_2 (Settings|GetGameUserSettings))
  (if (> (.x _returnvalue) (Math|Conversions|ToFloat(Integer) (/ (.x (Class|GameUserSettings|GetScreenResolution _returnvalue_2)) 5)))
    (if (> (.y _returnvalue) (Math|Conversions|ToFloat(Integer) (/ (.y (Class|GameUserSettings|GetScreenResolution _returnvalue_2)) 4)))
      (return 0)
      (else
        (return 0)))
    (elif (> (.y _returnvalue) (Math|Conversions|ToFloat(Integer) (/ (.y (Class|GameUserSettings|GetScreenResolution _returnvalue_2)) 4)))
      (return 0)
      (else
        (return 0)))))

(fn IsQuestActor
  (params (PlayerController :type Object%20Object%20Reference) (Quantity :type Integer) (Quest%20ID :type Text)))

(fn SpawnLightning
  (params (Actor :type Actor%20Object%20Reference) (HitActor :type Object%20Object%20Reference) (CriticalHit :type Boolean) (BaseDamage :type Float%20%28double-precision%29) (DamageCauser :type Actor%20Object%20Reference))
  (bind _returnvalue (Transformation|GetActorLocation Actor))
  (bind _outhits (Collision|MultiSphereTraceForObjects 0 _returnvalue _returnvalue 3.5e+02 (Utilities|Array|MakeArray "ObjectTypeQuery3") false (Utilities|Array|MakeArray DamageCauser) "None"))
  (for (_array_element _array_index) _outhits
    (if (or (Actor|ActorHasTag (.HitActor (Collision|BreakHitResult _array_element)) "EnemyAI") (Actor|ActorHasTag (.HitActor (Collision|BreakHitResult _array_element)) "Player"))
      (if (> (Utilities|Array|Length _outhits) 1)
        (LocalVariables|SetArrayCurrentActor (.HitActor (Collision|BreakHitResult _array_element)))
        (bind _returnvalue_2 (Effects|SpawnEmitteratLocation 0 0 "0, 0, 0" "0, 0, 0" "0.100000,0.100000,0.100000"))
        (Utilities|Array|Add (LocalVariables|GetSpawnedLightningLocal) _returnvalue_2)
        (Effects|Components|ParticleSystem|SetActorParameter _returnvalue_2 "Source" (select (== _array_index 0) Actor (.HitActor (Collision|BreakHitResult (Utilities|Array|Get(acopy) _outhits (- _array_index 1))))))
        (Effects|Components|ParticleSystem|SetActorParameter _returnvalue_2 "Target" (LocalVariables|GetArrayCurrentActor))
        (if (!= (LocalVariables|GetArrayCurrentActor) HitActor)
          _))))
  (return (LocalVariables|GetSpawnedLightningLocal)))

(fn RandomMinMaxValue
  (params (Damage :type Float%20%28double-precision%29))
  (return (Math|Random|RandomFloatinRange (* Damage 0.75) Damage)))

(fn ButtonHover
  (return 0))

(fn ButtonPress
  (return 0))

(fn PassAttackAnimation
  (params (Weapon%20Type :type Byte :default 0) (Anim%20Type :type Byte :default 0)))

(fn PassAnimation
  (params (Animation%20 :type Byte :default 0)))