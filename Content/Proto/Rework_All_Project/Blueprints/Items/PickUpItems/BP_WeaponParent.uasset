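; Parent Blueprint for pickup weapons that provides helpers for attaching special Niagara VFX to the weapon mesh.
; PassWeapon returns the static mesh if valid, otherwise the skeletal mesh.
; SpawnNiagara attaches the system from ItemInfo's WeaponVFX data at that mesh's VFXSocket, then feeds the mesh and tuning values into its user parameters.
; Event graph and construction script are empty, so nothing in this Blueprint calls SpawnNiagara.
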(event EventBeginPlay)

(event Collision|EventActorBeginOverlap
  (params (OtherActor :type Actor%20Object%20Reference)))

(event EventTick
  (params (DeltaSeconds :type Float%20%28single-precision%29)))

(fn ConstructionScript)

(fn PassWeapon
  (bind _itemstatic (Variables|Default|GetItemStatic))
  (return (select (Utilities|IsValid _itemstatic) _itemstatic (Variables|Default|GetItemSkeletal))))

(fn SpawnNiagara
  (bind _weapon (CallFunction|PassWeapon))
  (bind _iteminfo (Variables|Default|GetItemInfo))
  (bind _iteminfo_2 (Variables|Default|GetItemInfo))
  (bind _itemstructure (Utilities|Struct|BreakS_SlotInfo _iteminfo_2))
  (bind _itemstructure_2 (Utilities|Struct|BreakS_SlotInfo _iteminfo))
  (bind _weaponvfx (Utilities|Struct|BreakS_ItemData _itemstructure))
  (bind _weaponvfx_2 (Utilities|Struct|BreakS_ItemData _itemstructure_2))
  (bind _weaponvfx_3 (Utilities|Struct|BreakS_WeaponVFXInfo _weaponvfx))
  (bind (_height _radius _size _spawnrate) (Utilities|Struct|BreakS_WeaponVFXInfo _weaponvfx_2))
  ;[1 1 1] Spawns Niagara For Special VFX Weapons
  (Utilities|IsValid _weaponvfx_3
    (:Is%20Valid
      (Niagara|SpawnSystemAttached 0 _weapon "VFXSocket" "0, 0, 0" "0, 0, 0" "SnapToTarget" false)
      (bind _returnvalue (Niagara|SpawnSystemAttached _weaponvfx_3 _weapon "VFXSocket" "0, 0, 0" "0, 0, 0" "SnapToTarget" false))
      ;[1 1 1] Updates Niagara Variables
      (Class|NiagaraComponent|SetVariableObject _returnvalue "User.YourStaticMesh" (CallFunction|PassWeapon))
      (Niagara|SetNiagaraVariable(Float) _returnvalue "User.Height" _height)
      (Niagara|SetNiagaraVariable(Float) _returnvalue "User.Radius" _radius)
      (Niagara|SetNiagaraVariable(Float) _returnvalue "User.SpawnRate" _spawnrate)
      (Niagara|SetNiagaraVariable(Float) _returnvalue "User.Size" _size))))