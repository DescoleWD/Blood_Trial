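; Actor that spawns a wave of five assassination training dummies when activated.
; ActivateActor spawns a BP_AssassinateDummy with the mixed combat behaviour tree at each of five spawn points, yawed 90 degrees from the spawner, and tracks them in an array.
; Later activations destroy and respawn the set only once every tracked dummy is dead; otherwise they do nothing.
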(event EventActivateActor
  (bind _returnvalue (Transformation|GetActorRotation))
  (bind _ai (Variables|Default|GetAI))
  (if (== (Utilities|Array|Length (Variables|Default|GetAI)) 0)
    (for _array_element (Utilities|Array|MakeArray (Variables|Default|GetSpawn_1) (Variables|Default|GetSpawn_2) (Variables|Default|GetSpawn_0) (Variables|Default|GetSpawn_3) (Variables|Default|GetSpawn_4)) :!label _label
      (bind _returnvalue_2 (Game|SpawnActorfromClass :Class "/Game/FlexibleCombatSystem/DemoFolder/Blueprint/BP_AssassinateDummy.BP_AssassinateDummy_C" :SpawnTransform (Math|Transform|MakeTransform (Transformation|GetWorldLocation _array_element) (Math|Rotator|MakeRotator (.roll _returnvalue) (.pitch _returnvalue) (+ (.yaw _returnvalue) 9e+01)) "1,1,1") :CollisionHandlingOverride "Undefined" :BehaviourTree "/Game/FlexibleCombatSystem/Blueprints/AI/BehaviourTrees/BT_MixedCombat.BT_MixedCombat" :ActivateActorOnDeath 0 :Quest%20ID "None" :Instigator 0))
      (Utilities|Array|Add (Variables|Default|GetAI) _returnvalue_2))
    (else
      (Variables|Default|SetAllDead true)
      (bind _array_element_2 (Utilities|Array|ForEachLoopwithBreak (Variables|Default|GetAI) :!label _label_2)
        (:LoopBody
          (if (not (Variables|/Game/FlexibleCombatSystem/DemoFolder/Blueprint/BP_AssassinateDummy.BP_AssassinateDummy_C|GetDead _array_element_2))
            (Variables|Default|SetAllDead false)
            (goto _label_2 Break)))
        (:Completed
          (if (Variables|Default|GetAllDead)
            (for _array_element_3 _ai
              (Actor|DestroyActor _array_element_3))
            (Utilities|Array|Clear _ai)
            (goto _label)))))))

(fn ConstructionScript)