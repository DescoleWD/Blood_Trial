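; Base AI minion that picks a BP_MainBase target, chases it and can be damaged and killed.
; On possession it retries target search every half second, balancing minions by choosing the lowest NumberAIAttacker and incrementing it, except with a lone candidate.
; AIMoveTo is reissued after a delay on success or failure while alive.
; Lethal damage triggers death, which decrements the target's count and destroys the minion only if that target is valid.
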(event Custom|Move_To_Player
  (if (Variables|Default|GetIs_Alive)
    (AI|AIMoveTo self "0, 0, 0" (Variables|Default|GetTarget_Player) 1e+02 false
      (:OnSuccess
        _)
      (:OnFail
        _))
    (Utilities|FlowControl|Delay 2.0)
    (CallFunction|MovetoPlayer)))

(event Custom|On_AI_Spawned
  (bind (_is_valid_player_found _new_enemy) (CallFunction|FindEnemy :!label _label))
  (if _is_valid_player_found
    (Variables|Default|SetTarget_Player _new_enemy)
    (CallFunction|MovetoPlayer)
    (else
      (Utilities|FlowControl|Delay 0.5)
      (goto _label))))

(event Custom|Die_Event
  (bind _target_player (Variables|Default|GetTarget_Player))
  (Utilities|IsValid _target_player
    (:Is%20Valid
      (Math|Integer|DecrementInt (Variables|/Game/Proto/Main/Blueprint/BP_MainBase.BP_MainBase_C|GetNumber_AI_Attacker _target_player)
        (:%20%20
          (Components|Movement|StopMovementImmediately (Variables|Character|GetCharacterMovement))
          (Actor|DestroyActor))))))

(event EventBeginPlay)

(event Collision|EventActorBeginOverlap
  (params (OtherActor :type Actor%20Object%20Reference)))

(event EventTick
  (params (DeltaSeconds :type Float%20%28single-precision%29)))

(event EventPossessed
  (params (NewController :type Controller%20Object%20Reference))
  (bind _asbp_ai_controller_base_last (Utilities|Casting|CastToBP_AI_Controller_Base_Last NewController))
  (Variables|Default|SetAs%20BP%20AI%20Controller%20Base%20Last _asbp_ai_controller_base_last)
  (CallFunction|OnAISpawned))

(fn ConstructionScript)

(fn FindEnemy
  (bind _outactors (Actor|GetAllActorsOfClass "/Game/Proto/Main/Blueprint/BP_MainBase.BP_MainBase_C"))
  (bind _output_get (LocalVariables|SetLocal_All_Player _outactors))
  (if (Utilities|Array|IsNotEmpty _output_get)
    (if (== (Utilities|Array|Length (LocalVariables|GetLocal_All_Player)) 1)
      (LocalVariables|SetLocal_Is_Valid_Player_Found true)
      (LocalVariables|SetLocal_New_Enemy (Utilities|Array|Get(acopy) (LocalVariables|GetLocal_All_Player)))
      (else
        (for _array_element (LocalVariables|GetLocal_All_Player)
          (Utilities|Array|Add (LocalVariables|GetLocal_All_Attackers_Number) (Variables|/Game/Proto/Main/Blueprint/BP_MainBase.BP_MainBase_C|GetNumber_AI_Attacker _array_element)))
        (LocalVariables|SetLocal_LowestIndex (.IndexOfMinValue (Math|Integer|MinOfIntArray (LocalVariables|GetLocal_All_Attackers_Number))))
        (if (== (LocalVariables|GetLocal_LowestIndex) -1)
          (LocalVariables|SetLocal_Is_Valid_Player_Found false)
          (else
            (Math|Integer|IncrementInt (Variables|/Game/Proto/Main/Blueprint/BP_MainBase.BP_MainBase_C|GetNumber_AI_Attacker (Utilities|Array|Get(acopy) (LocalVariables|GetLocal_All_Player) (LocalVariables|GetLocal_LowestIndex)))
              (:%20%20
                (LocalVariables|SetLocal_New_Enemy (Utilities|Array|Get(acopy) (LocalVariables|GetLocal_All_Player) (LocalVariables|GetLocal_LowestIndex)))
                (LocalVariables|SetLocal_Is_Valid_Player_Found true)))))))
    (else
      (LocalVariables|SetLocal_Is_Valid_Player_Found false)))
  (return (LocalVariables|GetLocal_Is_Valid_Player_Found) (LocalVariables|GetLocal_New_Enemy)))

(fn TakeDamage
  (params (Attacker :type Actor%20Object%20Reference) (Ammout_Damage :type Float%20%28double-precision%29))
  (if (Variables|Default|GetIs_Alive)
    (bind _output_get (Variables|Default|SetHealth (- (Variables|Default|GetHealth) Ammout_Damage)))
    (if (<= _output_get 0.0)
      (Variables|Default|SetIs_Alive false)
      (CallFunction|DieEvent)))
  (return (not (Variables|Default|GetIs_Alive)) 0))