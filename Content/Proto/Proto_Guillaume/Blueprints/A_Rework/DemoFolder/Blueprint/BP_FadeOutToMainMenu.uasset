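; Trigger actor that starts a distance-driven screen fade as the player approaches a stairway reference, presumably leading out to the main menu.
; The first player overlap with its box creates a WB_StairwayFade widget, using the trigger's distance to StairwayReach as RangeMin.
; A fast looping timer then feeds the player's distance to StairwayReach into the widget, adding it to the viewport on the first tick.
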(event OnComponentBeginOverlap(Box)
  (params (OverlappedComponent :type Primitive%20Component%20Object%20Reference) (OtherActor :type Actor%20Object%20Reference) (OtherComp :type Primitive%20Component%20Object%20Reference) (OtherBodyIndex :type Integer) (bFromSweep :type Boolean) (SweepResult :type Hit%20Result%20Structure%20%28by%20ref%29))
  (bind _stairwayreach (Variables|Default|GetStairwayReach))
  (bind _asbp_player_character (Utilities|Casting|CastToBP_PlayerCharacter OtherActor))
  (Utilities|FlowControl|DoOnce false
    (:Completed
      (Variables|Default|SetBP%20Player%20Character _asbp_player_character)
      (bind _returnvalue (UserInterface|CreateWidget "/Game/FlexibleCombatSystem/DemoFolder/Widgets/WB_StairwayFade.WB_StairwayFade_C"))
      (bind _output_get (Variables|Default|SetStairWayFade _returnvalue))
      (Utilities|IsValid _stairwayreach
        (:Is%20Valid
          (Variables|/Game/FlexibleCombatSystem/DemoFolder/Widgets/WB_StairwayFade.WB_StairwayFade_C|SetRange%20Min _output_get (Transformation|GetDistanceTo _stairwayreach self)))
        (:Is%20Not%20Valid
          _))
      (Utilities|Time|SetTimerbyEvent (delegate Custom|UpdateDistance) 0.01 true))))

(event Custom|UpdateDistance
  (Variables|/Game/FlexibleCombatSystem/DemoFolder/Widgets/WB_StairwayFade.WB_StairwayFade_C|SetCurrentDistance (Variables|Default|GetStairWayFade) (Transformation|GetDistanceTo (Variables|Default|GetBP%20Player%20Character) (Variables|Default|GetStairwayReach)))
  (Utilities|FlowControl|DoOnce false
    (:Completed
      (UserInterface|Viewport|AddtoViewport (Variables|Default|GetStairWayFade) 0))))

(event EventBeginPlay)

(event Collision|EventActorBeginOverlap
  (params (OtherActor :type Actor%20Object%20Reference)))

(fn ConstructionScript)