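; BP_DamageNumberActor is a short-lived actor that shows a floating damage number through a WI_FloatingDamage widget.
; On BeginPlay it passes the UIAmountAttack value read from GetInst to the widget and launches its static mesh with a random upward-biased velocity impulse, so the number is tossed physically.
; It binds to the widget's lifetime-over event and destroys itself when that fires.
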(event Custom|WidgetDead
  (Actor|DestroyActor))

(event EventBeginPlay
  (bind _aswi_floating_damage (Utilities|Casting|CastToWI_FloatingDamage (UserInterface|GetUserWidgetObject (Variables|Default|GetWidget))))
  (EventDispatchers|BindEventtoWidgetLifeTimeOver _aswi_floating_damage (delegate Custom|WidgetDead))
  (Class|SetDamageValue|SetDamageValue(Message) _aswi_floating_damage (Variables|/Game/Proto/Main/Blueprint/Save_BFL_GameInstance/BloodTrial_GameInstance.BloodTrial_GameInstance_C|GetUI_Amount_Attack (CallFunction|GetInst)))
  (Physics|AddImpulse (Variables|Default|GetStaticMesh) (Math|Vector|MakeVector (Math|Random|RandomFloatinRange 0.0 4e+02) (Math|Random|RandomFloatinRange 0.0 4e+02) (Math|Random|RandomFloatinRange 4e+02 8e+02)) "None" true))

(fn ConstructionScript)