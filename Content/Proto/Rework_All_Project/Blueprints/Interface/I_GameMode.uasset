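; Blueprint interface I_GameMode, which by its name exposes the game mode's save, checkpoint and level-restart functions to other objects.
; It declares signatures only, covering saving, loading, checkpoint reached, spawning at level start and restarting the level.
; Further calls report world changes for persistence: dead AI, picked items, chest loot changes and their removal, quest and dialogue state, activated actors by unique ID, and placed runes.
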(fn SaveGame)

(fn CheckpointReached
  (params (CheckpointActor :type Actor%20Object%20Reference)))

(fn SpawnatLevelStart)

(fn LoadSave)

(fn RestartLevel)

(fn AddDeadAI
  (params (AI%20Save%20Info :type S%20AI%20Save%20Info%20Structure))
  (return))

(fn StorePickedItem
  (params (ActorToStore :type String))
  (return))

(fn SaveLootChanges
  (params (ChestActor :type Actor%20Object%20Reference) (LootType :type E_ObjectLootType%20Enum :default "NewEnumerator0"))
  (return))

(fn RemoveLootChangesSave
  (params (ChestActor :type Actor%20Object%20Reference))
  (return))

(fn QuestComponentSaving
  (params (QuestGiver :type Actor%20Object%20Reference))
  (return))

(fn ActorActivated
  (params (Unique%20ID :type String)))

(fn DialogueComponentSaving
  (params (DialogueActor :type Actor%20Object%20Reference))
  (return 0))

(fn RunePlaced
  (params (Add :type Boolean) (RuneSave :type S%20Rune%20Save%20Info%20Structure)))