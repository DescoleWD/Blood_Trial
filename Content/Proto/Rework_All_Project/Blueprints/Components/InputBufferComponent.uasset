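; Combat input buffer component that gates character actions and queues inputs arriving while the character is busy or stunned.
; Montages open and close the buffer window, with Block kept in a separate low-priority slot that other actions can override.
; Closing calls ConsumeBuffer, which clears for AI, otherwise dispatches to melee or movement components.
; Both dispatch branches switch on the low-priority slot, even when the main slot is filled.
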(event Custom|OnActionBegin
  (params (Action :type E_CharacterAction%20Enum :default "NewEnumerator4"))
  ;[1 1 1] OnActionBegin Called When Action Fired
  (bind _output_get (Variables|Default|SetConsumeInputBuffer Action))
  (CallFunction|RemoveLowPriorityStatus _output_get))

(event Custom|ClearBuffer
  (params (ClearLowPriority :type Boolean))
  ;[1 1 1] Clear Low Priority Input
  (Variables|Default|SetConsumeInputBuffer "NewEnumerator4")
  (Variables|Default|SetInputBuffer "NewEnumerator4")
  (if ClearLowPriority
    (Variables|Default|SetInputBufferLowerPrio "NewEnumerator4")))

(event Custom|OpenBuffer
  ;[1 1 1] Buffer Open/Close & Consume - Called In Each Animation Montage
  (Variables|Default|SetBufferOpen? true))

(event Custom|CloseBuffer
  ;[1 1 1] Buffer Open/Close & Consume - Called In Each Animation Montage
  (Variables|Default|SetBufferOpen? false)
  (CallFunction|ConsumeBuffer))

(event Custom|StoreBuffer
  (params (Input :type E_CharacterAction%20Enum :default "NewEnumerator4"))
  ;[1 1 1] Store Input Buffer - Called When Action Fire But Buffer Full
  (CallFunction|StoreBufferFunction Input))

(event Custom|ConsumeBuffer
  ;[1 1 1] Consume Input Buffer
  (if (Variables|Default|GetEnemyAI)
    (Variables|Default|SetConsumeInputBuffer "NewEnumerator4")
    (Variables|Default|SetInputBuffer "NewEnumerator4")
    (else
      (Variables|Default|SetConsumeInputBuffer "NewEnumerator4")
      (if (CallFunction|MainInputBufferEmpty)
        ;;[1 1 1] Consume Lower Input (Inputs Which Require Holding Down Keys)
        (switch Utilities|FlowControl|Switch|SwitchonE_CharacterAction (Variables|Default|GetInputBufferLowerPrio)
          (:NewEnumerator4
            (Variables|Default|SetConsumeInputBuffer "NewEnumerator4"))
          (:NewEnumerator2
            (Default|SendBlock (Variables|Default|GetMeleeComponent))
            (Variables|Default|SetInputBufferLowerPrio "NewEnumerator4")))
        (else
          ;;[1 1 1] Consume Main Buffer
          (switch Utilities|FlowControl|Switch|SwitchonE_CharacterAction (Variables|Default|GetInputBufferLowerPrio)
            (:NewEnumerator0
              (Default|EventLightAttack (Variables|Default|GetMeleeComponent)))
            (:NewEnumerator9
              (Default|EventHeavyAttack (Variables|Default|GetMeleeComponent)))
            (:NewEnumerator5
              (Default|EventRoll (Variables|Default|GetMovementComponent))))
          ;;[1 1 1] Remove Consume - Can Load Next Attack
          (Variables|Default|SetInputBuffer "NewEnumerator4"))))))

(event Custom|ClearLowPriority
  ;[1 1 1] Clear Low Priority Input
  (Variables|Default|SetInputBufferLowerPrio "NewEnumerator4"))

(event EventBeginPlay
  ;[1 1 1] Store References
  (CallFunction|StoreComponents))

(fn MainInputBufferEmpty
  (return (Utilities|Enum|Equal(Enum) (Variables|Default|GetInputBuffer) "NewEnumerator4")))

(fn RemoveLowPriorityStatus
  (params (Input :type E_CharacterAction%20Enum :default "NewEnumerator4"))
  (bind _meleecomponent (Variables|Default|GetMeleeComponent))
  ;[1 1 1] Remove Low Priority (Usually Right Click Charge Action) And Store It
  (if (and (Utilities|Enum|NotEqual(Enum) Input "NewEnumerator4") (Variables|/Game/Proto/Rework_All_Project/Blueprints/Components/MeleeComponent.MeleeComponent_C|GetBlockUp _meleecomponent))
    (Default|ReleaseBlock _meleecomponent)
    (Variables|Default|SetInputBufferLowerPrio "NewEnumerator4")))

(fn StoreBufferFunction
  (params (IncomingInputBuffer :type E_CharacterAction%20Enum :default "NewEnumerator4"))
  ;[1 1 1] If Buffer Currently Open - Set Input as Input Buffer OR Low Priority Input Buffer
  (if (Utilities|Enum|Equal(Enum) IncomingInputBuffer "NewEnumerator2")
    (Variables|Default|SetInputBufferLowerPrio (Utilities|Enum|ByteToEnumE_CharacterAction IncomingInputBuffer))
    (elif (Variables|Default|GetBufferOpen?)
      (Variables|Default|SetInputBuffer (Utilities|Enum|ByteToEnumE_CharacterAction IncomingInputBuffer))
      (elif (Variables|Default|GetEnemyAI)
        (Variables|Default|SetInputBuffer (Utilities|Enum|ByteToEnumE_CharacterAction IncomingInputBuffer))))))

(fn CanAnimationPlay
  (params (IncomingMontage :type E_CharacterAction%20Enum :default "NewEnumerator4"))
  ;[1 1 1] Overwrites Lower Priority Animation, Stores as Buffer If High Priority
  (if (Variables|/Game/Proto/Rework_All_Project/Blueprints/Components/MeleeComponent.MeleeComponent_C|GetStunned (Variables|Default|GetMeleeComponent))
    (CallFunction|StoreBuffer IncomingMontage)
    (return false)
    (elif (Utilities|Enum|Equal(Enum) (Variables|Default|GetConsumeInputBuffer) "NewEnumerator4")
      (return true)
      (elif (Utilities|Enum|Equal(Enum) (Variables|Default|GetConsumeInputBuffer) "NewEnumerator2")
        (return true)
        (else
          (CallFunction|StoreBuffer IncomingMontage)
          (return false))))))

(fn StoreComponents
  (bind _returnvalue (Components|GetOwner))
  (Variables|Default|SetMovementComponent (Actor|GetComponentbyClass _returnvalue "/Game/Proto/Rework_All_Project/Blueprints/Components/MovementStatusComponent.MovementStatusComponent_C"))
  (Variables|Default|SetMeleeComponent (Actor|GetComponentbyClass _returnvalue "/Game/Proto/Rework_All_Project/Blueprints/Components/MeleeComponent.MeleeComponent_C"))
  (Variables|Default|SetCombatStatusComponent (Actor|GetComponentbyClass _returnvalue "/Game/Proto/Rework_All_Project/Blueprints/Components/CombatStatusComponent.CombatStatusComponent_C")))