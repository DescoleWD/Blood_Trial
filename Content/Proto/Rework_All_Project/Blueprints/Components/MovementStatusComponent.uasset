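; Character component that manages movement state: walk speed, sprint, roll, crouch, encumbrance and movement noise.
; Speed changes select a target by enum, apply encumbrance or percentage slows, then ease MaxWalkSpeed on a looping timer.
; Sprint and roll check stamina, state and the action buffer, then drain stamina through the resource component.
; Rolls ignore two collision channels for the montage length and use a cooldown flag against double rolls.
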(event Custom|EventRoll
  (bind _anim (CallFunction|PassAnimation "NewEnumerator0"))
  ;[1 1 1] Roll
  (bind _canroll (CallFunction|RollingConditions))
  (if _canroll
    (if (not (Variables|Default|GetRollSpam))
      (Utilities|FlowControl|Sequence
        (:then_0
          (Variables|Default|SetRollSpam true)
          (CallFunction|PlayRollMontage _anim)
          (CallFunction|OnActionBegin (.StateBufferComponent (Variables|Default|GetStateBufferComponent)) 0)
          (CallFunction|ResetMeleeAttack (.MeleeComponent (Variables|Default|GetMeleeComponent)))
          (CallFunction|DamageResource (.ResourceComp (Variables|Default|GetResourceComp)) (Variables|Default|GetRollStaminaCost) false)
          (Utilities|FlowControl|Delay 0.2)
          (Audio|PlaySound2D 0 0.3 1.0 0.0 0 0)
          ;;[1 1 1] Input Buffer Usually Controls Spamming of Actions, however Inpout buffer can sometimes get reset mid roll by Attack, this is a safety check to prevent double rolling
          (Utilities|FlowControl|Delay 0.5)
          (Variables|Default|SetRollSpam false))
        (:then_1
          (CallFunction|AdjustRollCollision true)
          (Utilities|FlowControl|Delay (Animation|GetPlayLength _anim))
          (CallFunction|AdjustRollCollision false))))))

(event Custom|StartCrouch
  ;[1 1 1] Crouch
  (if (not (Variables|Default|GetPlayerCrouched?))
    (Variables|Default|SetPlayerCrouched? true)
    (CallFunction|ChangeMovementSpeed 0)
    (Character|Crouch (Variables|Components|GetCharacter))))

(event Custom|EventNotEncumered
  ;[1 1 1] Speed Control
  ;;[1 1 1] Encumbered
  (Variables|Default|SetEncumbered false)
  (CallFunction|ResumeMovement))

(event Custom|StopCrouch
  ;[1 1 1] Crouch
  (if (Variables|Default|GetPlayerCrouched?)
    (Variables|Default|SetPlayerCrouched? false)
    (CallFunction|ChangeMovementSpeed)
    (Character|UnCrouch (Variables|Components|GetCharacter))))

(event Custom|EventCrouch
  (params (Character :type Character%20Object%20Reference))
  ;[1 1 1] Crouch
  (Variables|Components|SetCharacter Character)
  (if (not (Variables|Default|GetEncumbered))
    (if (Variables|Default|GetPlayerCrouched?)
      (Variables|Default|SetPlayerCrouched? false)
      (CallFunction|ChangeMovementSpeed)
      (Character|UnCrouch (Variables|Components|GetCharacter))
      (else
        (Variables|Default|SetPlayerCrouched? true)
        (CallFunction|ChangeMovementSpeed 0)
        (Character|Crouch (Variables|Components|GetCharacter))))))

(event Custom|EventReleaseSprint
  ;[1 1 1] Sprint
  ;;[1 1 1] Deactivate
  (if (Variables|Default|GetSprint)
    (Variables|Default|SetSprint false)
    (CallFunction|ClearDrainStamina (.ResourceComp (Variables|Default|GetResourceComp)))
    (CallFunction|ChangeMovementSpeed)
    (CallFunction|ConsumeBuffer (.StateBufferComponent (Variables|Default|GetStateBufferComponent)))
    (else
      (CallFunction|ClearLowPriority (.StateBufferComponent (Variables|Default|GetStateBufferComponent))))))

(event Custom|Distraction
  (bind _returnvalue (Components|GetOwner))
  ;[1 1 1] Distraction?
  (Class|Actor|MakeNoise _returnvalue 1.0 0 (Transformation|GetActorLocation _returnvalue) 1e+03 "None"))

(event Custom|EventSprint
  (bind _statebuffercomponent (Variables|Default|GetStateBufferComponent))
  ;[1 1 1] Sprint
  ;;[1 1 1] Activate
  (bind _cansprint (CallFunction|SprintConditions))
  (if _cansprint
    (bind _runanimation (CallFunction|CanAnimationPlay _statebuffercomponent 0))
    (if _runanimation
      (CallFunction|OnActionBegin _statebuffercomponent 0)
      (Variables|Default|SetSprint true)
      (CallFunction|DamageResource (.ResourceComp (Variables|Default|GetResourceComp)) 0.0 true)
      (CallFunction|ChangeMovementSpeed 0))))

(event Custom|FootstepNoise
  (bind _returnvalue (Components|GetOwner))
  ;[1 1 1] Sending Footstep Noise
  (if (not (AI|Components|NavMovement|IsCrouching (Variables|Default|GetCharacterMovement)))
    (bind _moving (Class|Object|IsMoving?(Message) _returnvalue))
    (if _moving
      (if (not (CallFunction|IsPlayingMontage (Variables|Default|GetMesh) (CallFunction|PassAnimation "NewEnumerator0")))
        (Class|Actor|MakeNoise _returnvalue 1.0 0 (Transformation|GetActorLocation _returnvalue) 1e+03 "None")))))

(event Custom|LockedMovement
  (params (SlowSpeedPercent :type Float%20%28double-precision%29) (Lock :type Boolean))
  ;[1 1 1] Speed Control
  ;;[1 1 1] Change Movement Over Time Depending On Enum
  (bind _output_get (Variables|Default|SetLockedSpeed Lock))
  (if _output_get
    (CallFunction|SetSlowSpeed SlowSpeedPercent)
    (Variables|MovementSpeed|SetMovementSpeedRef (Variables|/Script/Engine.CharacterMovementComponent|GetMaxWalkSpeed (Variables|Default|GetCharacterMovement)))
    (bind _returnvalue (Utilities|Time|SetTimerbyEvent (delegate Custom|LerpMovement) 0.01 true))
    (else
      (CallFunction|ChangeMovementSpeed (Variables|MovementSpeed|GetMovementSpeed)))))

(event Custom|LerpMovement
  ;[1 1 1] Speed Control
  ;;[1 1 1] Change Movement Over Time Depending On Enum
  (Variables|/Script/Engine.CharacterMovementComponent|SetMaxWalkSpeed (Variables|Default|GetCharacterMovement) (Math|Interpolation|FInterpTo (Variables|/Script/Engine.CharacterMovementComponent|GetMaxWalkSpeed (Variables|Default|GetCharacterMovement)) (Variables|MovementSpeed|GetWalkSpeedTarget) (Utilities|Time|GetWorldDeltaSeconds) 1e+01))
  (if (Math|Float|NearlyEqual(Float) (Variables|/Script/Engine.CharacterMovementComponent|GetMaxWalkSpeed (Variables|Default|GetCharacterMovement)) (Variables|MovementSpeed|GetWalkSpeedTarget) 1.0)
    (Utilities|Time|ClearandInvalidateTimerbyHandle (stale Custom|LockedMovement _returnvalue))))

(event Custom|ResumeMovement
  ;[1 1 1] Speed Control
  ;;[1 1 1] Change Movement Over Time Depending On Enum
  (Variables|MovementSpeed|SetMovementSpeed (stale Custom|ChangeMovementSpeed Movement))
  (if (or (Variables|Default|GetEncumbered) (Variables|Default|GetLockedSpeed))
    (CallFunction|UpdateSlowSpeed)
    (else
      (Variables|MovementSpeed|SetWalkSpeedTarget (Utilities|Select :Index (Variables|MovementSpeed|GetMovementSpeed) :Option%200 0.0 :Option%201 0.0 :Option%202 0.0 :Option%203 0.0 :Option%204 0.0 :Option%205 0.0))))
  (Variables|MovementSpeed|SetMovementSpeedRef (Variables|/Script/Engine.CharacterMovementComponent|GetMaxWalkSpeed (Variables|Default|GetCharacterMovement)))
  (bind _returnvalue (Utilities|Time|SetTimerbyEvent (delegate Custom|LerpMovement) 0.01 true)))

(event Custom|ChangeMovementSpeed
  (params (Movement :type Byte :default 0))
  ;[1 1 1] Speed Control
  ;;[1 1 1] Change Movement Over Time Depending On Enum
  (Variables|MovementSpeed|SetMovementSpeed Movement)
  (if (or (Variables|Default|GetEncumbered) (Variables|Default|GetLockedSpeed))
    (CallFunction|UpdateSlowSpeed)
    (else
      (Variables|MovementSpeed|SetWalkSpeedTarget (Utilities|Select :Index (Variables|MovementSpeed|GetMovementSpeed) :Option%200 0.0 :Option%201 0.0 :Option%202 0.0 :Option%203 0.0 :Option%204 0.0 :Option%205 0.0))))
  (Variables|MovementSpeed|SetMovementSpeedRef (Variables|/Script/Engine.CharacterMovementComponent|GetMaxWalkSpeed (Variables|Default|GetCharacterMovement)))
  (bind _returnvalue (Utilities|Time|SetTimerbyEvent (delegate Custom|LerpMovement) 0.01 true)))

(event Custom|EventEncumbered
  (bind _charactermovement (Variables|Default|GetCharacterMovement))
  ;[1 1 1] Speed Control
  ;;[1 1 1] Encumbered
  (Utilities|IsValid _charactermovement :!label _label
    (:Is%20Valid
      (Variables|Default|SetEncumbered true)
      (Variables|/Script/Engine.CharacterMovementComponent|SetMaxWalkSpeed _charactermovement 1.5e+02))
    (:Is%20Not%20Valid
      (Utilities|FlowControl|Delay 0.1)
      (goto _label))))

(event EventBeginPlay
  ;[1 1 1] Speed Control
  ;;[1 1 1] Setup
  (CallFunction|Initialize))

(fn RollingConditions
  ;[1 1 1] Is Encumered?
  (if (Variables|Default|GetEncumbered)
    _
    (else
      ;[1 1 1] Is Stamina Greater Than 5
      (if (>= (Variables|Default|GetStamina (.EquipmentComponent (Variables|Default|GetEquipmentComponent))) (Variables|Default|GetRollStaminaCost))
        ;[1 1 1] Is Falling?
        (if (AI|Components|NavMovement|IsFalling (Variables|Default|GetCharacterMovement))
          _
          (else
            (bind _runanimation (CallFunction|CanAnimationPlay (.StateBufferComponent (Variables|Default|GetStateBufferComponent)) 0))
            (if _runanimation
              (return true)
              (else
                (return false)))))
        (else
          (CallFunction|NotEnoughResource (.ResourceComp (Variables|Default|GetResourceComp)))))))
  (return false))

(fn PlayRollMontage
  (params (Montage :type Anim%20Montage%20Object%20Reference))
  (Variables|/Script/Engine.Pawn|SetbUseControllerRotationYaw (Variables|Components|GetCharacter) false)
  (Pawn|Components|CharacterMovement|SetMovementMode (Variables|Default|GetCharacterMovement) "MOVE_Walking" 0)
  (Animation|PlayAnimMontage (Class|CharacterMovementComponent|GetCharacterOwner (Variables|Default|GetCharacterMovement)) Montage 1.0 "None")
  (return))

(fn IsLungeAttacking
  (return (Animation|Montage|MontageIsPlaying (Components|SkeletalMesh|GetAnimInstance (Variables|Default|GetMesh)) 0)))

(fn IsPlayingMontage
  (return (Animation|Montage|MontageIsPlaying (Components|SkeletalMesh|GetAnimInstance (Variables|Default|GetMesh)) 0)))

(fn SetSlowSpeed
  (params (SlowPercent :type Float%20%28double-precision%29))
  (bind _returnvalue (Math|Float|MakeLiteralFloat 1e+02))
  (bind _returnvalue_2 (- _returnvalue SlowPercent))
  (Variables|Default|SetCurrentSlowPercent _returnvalue_2)
  ;[1 1 1] Divide Walk Speed By 100, Multiply By Slow % To Give Slow
  (Variables|MovementSpeed|SetWalkSpeedTarget (* (/ (Utilities|Select :Index (Variables|MovementSpeed|GetMovementSpeed) :Option%200 0.0 :Option%201 0.0 :Option%202 0.0 :Option%203 0.0 :Option%204 0.0 :Option%205 0.0) 1e+02) _returnvalue_2)))

(fn SprintConditions
  (bind _charactermovement (Variables|Default|GetCharacterMovement))
  (if (AI|Components|NavMovement|IsCrouching _charactermovement)
    _
    (elif (AI|Components|NavMovement|IsFalling _charactermovement)
      _
      (elif (Variables|Default|GetEncumbered)
        _
        (elif (> (Variables|Default|GetStamina (.EquipmentComponent (Variables|Default|GetEquipmentComponent))) 0.0)
          (return true)
          (else
            _)))))
  (return false))

(fn Initialize
  (bind _returnvalue (Components|GetOwner))
  (Variables|Default|SetResourceComp 0 (Actor|GetComponentbyClass _returnvalue 0))
  (Variables|Default|SetMeleeComponent 0 (Actor|GetComponentbyClass _returnvalue 0))
  (Variables|Default|SetEquipmentComponent 0 (Actor|GetComponentbyClass _returnvalue 0))
  (Variables|Default|SetStateBufferComponent 0 (Actor|GetComponentbyClass _returnvalue 0))
  (bind _ascharacter (Utilities|Casting|CastToCharacter _returnvalue))
  (Variables|Default|SetMesh (Variables|/Script/Engine.Character|GetMesh _ascharacter))
  (Variables|Default|SetCharacterMovement (Variables|/Script/Engine.Character|GetCharacterMovement _ascharacter))
  (Variables|Components|SetCharacter _ascharacter)
  (Variables|Default|SetDefaultMaxWalkSpeed (Variables|/Script/Engine.CharacterMovementComponent|GetMaxWalkSpeed (Variables|/Script/Engine.Character|GetCharacterMovement _ascharacter))))

(fn UpdateSlowSpeed
  (if (Variables|Default|GetEncumbered)
    (Variables|MovementSpeed|SetWalkSpeedTarget 1.5e+02)
    (else
      (Variables|MovementSpeed|SetWalkSpeedTarget (* (/ (Utilities|Select :Index (Variables|MovementSpeed|GetMovementSpeed) :Option%200 0.0 :Option%201 0.0 :Option%202 0.0 :Option%203 0.0 :Option%204 0.0 :Option%205 0.0) 1e+02) (Variables|Default|GetCurrentSlowPercent))))))

(fn AdjustRollCollision
  (params (RollStart :type Boolean))
  (bind _mesh (Variables|Default|GetMesh))
  (Collision|SetCollisionResponsetoChannel _mesh "ECC_GameTraceChannel1" (select RollStart "ECR_Ignore" "ECR_Block"))
  (Collision|SetCollisionResponsetoChannel _mesh "ECC_GameTraceChannel3" (select RollStart "ECR_Ignore" "ECR_Block")))