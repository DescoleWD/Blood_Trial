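; Parent Blueprint for interactable loot containers that open an inventory component in the player's external inventory UI.
; Interact checks conditions on the player controller, toggles the chest UI with or without sort options, then flips the open state and triggers an animation hook left for children.
; Leaving the sphere while open reruns that toggle to close it.
; Retrieve functions supply inventory setup and outline data; loot info is empty.
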(event OnComponentEndOverlap(Sphere)
  (params (OverlappedComponent :type Primitive%20Component%20Object%20Reference) (OtherActor :type Actor%20Object%20Reference) (OtherComp :type Primitive%20Component%20Object%20Reference) (OtherBodyIndex :type Integer))
  ;[1 1 1] Interact - Open Loot
  (if (Variables|Default|GetOpen)
    (switch Utilities|FlowControl|Switch|SwitchonE_ChestType (Variables|SetupinGame|GetContainerType)
      (:NewEnumerator0
        ;;[1 1 1] Chest No Sort Options
        (Class|IPlayerController|ToggleExternalContainerInv(Message) (Game|GetPlayerController 0) (Variables|Default|GetInventoryComponent) self))
      (:NewEnumerator1
        ;;[1 1 1] Chest With Sort Options
        (Class|IPlayerController|ToggleExternalInventory(Message) (Game|GetPlayerController 0) (Variables|Default|GetInventoryComponent) 0 false)))
    (Variables|Default|SetOpen (not (Variables|Default|GetOpen)))
    (Class|ILootInterface|ToggleAnimation(Message) self)))

(event EventInteract
  (params (Character :type Character%20Object%20Reference))
  ;[1 1 1] Interact - Open Loot
  (bind _interact (Class|IPlayerController|ExternalInventoryConditions(Message) (Game|GetPlayerController 0)))
  (if _interact
    (switch Utilities|FlowControl|Switch|SwitchonE_ChestType (Variables|SetupinGame|GetContainerType)
      (:NewEnumerator0
        ;;[1 1 1] Chest No Sort Options
        (Class|IPlayerController|ToggleExternalContainerInv(Message) (Game|GetPlayerController 0) (Variables|Default|GetInventoryComponent) self))
      (:NewEnumerator1
        ;;[1 1 1] Chest With Sort Options
        (Class|IPlayerController|ToggleExternalInventory(Message) (Game|GetPlayerController 0) (Variables|Default|GetInventoryComponent) 0 false)))
    (Variables|Default|SetOpen (not (Variables|Default|GetOpen)))
    (Class|ILootInterface|ToggleAnimation(Message) self)))

(event EventToggleAnimation
  ;[1 1 1] Interact - Open Loot
  ;;[1 1 1] Left Open For Child
)

(fn ConstructionScript)

(fn RetrieveInventoryInfo
  (return (Utilities|Select :Index (Variables|SetupinGame|GetContainerType) :NewEnumerator0 "NewEnumerator1" :NewEnumerator1 "NewEnumerator4") (Variables|SetupinGame|GetContainerName) (Variables|SetupinGame|GetContainerImage) (Variables|SetupinGame|GetContainerInventory) (Variables|SetupinGame|GetUseDataTable?) (Variables|SetupInGame|GetContainerDataTable) (Variables|SetupInGame|GetContainerSize)))

(fn RetrieveLootInfo
  (return ""))

(fn RetrieveOutlineInfo
  (return (Variables|SetupinGame|GetContainerName) (Variables|SetupinGame|GetContainerRarity) "NewEnumerator1" 0 (Variables|Default|GetItem) (Variables|Default|GetItem2) 0))