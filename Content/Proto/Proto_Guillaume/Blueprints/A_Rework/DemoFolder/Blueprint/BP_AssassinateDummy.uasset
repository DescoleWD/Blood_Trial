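; Enemy AI dummy character that always reports itself assassinable and passes its assassination camera and rotator through interface functions.
; BeginPlay flags components as AI and spawns combat-style weapons from data tables, while stat, armor and arrow setup end in stubs.
; Death notifies quests, drops weapons and ragdolls the mesh, with SendDeath also releasing target lock and granting XP.
; Most other status queries return fixed or empty values.
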(event EventBeginPlay
  ;[0.6825 1 0.783] Setup AI
  (CallFunction|SetupStats)
  (CallFunction|SetupArmor)
  (CallFunction|SetupWeapon)
  (CallFunction|SetupCustomArrows)
  (CallFunction|SetupComponents))

(fn ConstructionScript)

(fn SetupStats)

(fn StoreStats
  (params (Custom%20Values :type S%20Custom%20AI%20Values%20Structure))
  (bind (_usecustomstats _basehealth _basestamina _basemana _basecritchance _basearmor _baseshieldblock _baseintellectspelldamage _basemainhanddamage _baseoffhanddamage _baserangeddamage _basexp_given) (Utilities|Struct|BreakS_Custom_AI_Values Custom%20Values))
  (bind _equipmentcomponent (Variables|Default|GetEquipmentComponent))
  (Utilities|FlowControl|Sequence
    (:then_0
      (bind _output_get (Variables|/Game/FlexibleCombatSystem/Blueprints/Components/EquipmentComponent.EquipmentComponent_C|SetHealth _equipmentcomponent (* (Variables|SetupInGame|GetEnemyLevel) _basehealth)))
      (Variables|/Game/FlexibleCombatSystem/Blueprints/Components/EquipmentComponent.EquipmentComponent_C|SetMaxHealth _equipmentcomponent _output_get))
    (:then_1
      (bind _output_get_2 (Variables|/Game/FlexibleCombatSystem/Blueprints/Components/EquipmentComponent.EquipmentComponent_C|SetStamina _equipmentcomponent (* (Variables|SetupInGame|GetEnemyLevel) _basestamina)))
      (Variables|/Game/FlexibleCombatSystem/Blueprints/Components/EquipmentComponent.EquipmentComponent_C|SetMaxStamina _equipmentcomponent _output_get_2))
    (:then_2
      (bind _output_get_3 (Variables|/Game/FlexibleCombatSystem/Blueprints/Components/EquipmentComponent.EquipmentComponent_C|SetMana _equipmentcomponent (* (Variables|SetupInGame|GetEnemyLevel) _basemana)))
      (Variables|/Game/FlexibleCombatSystem/Blueprints/Components/EquipmentComponent.EquipmentComponent_C|SetMaxMana _equipmentcomponent _output_get_3))
    (:then_3
      (Variables|/Game/FlexibleCombatSystem/Blueprints/Components/EquipmentComponent.EquipmentComponent_C|SetCritValue _equipmentcomponent (* (Variables|SetupInGame|GetEnemyLevel) _basecritchance)))
    (:then_4
      (Variables|/Game/FlexibleCombatSystem/Blueprints/Components/EquipmentComponent.EquipmentComponent_C|SetArmor _equipmentcomponent (* (Variables|SetupInGame|GetEnemyLevel) _basearmor)))
    (:then_5
      (Variables|/Game/FlexibleCombatSystem/Blueprints/Components/EquipmentComponent.EquipmentComponent_C|SetShieldBlock _equipmentcomponent (* (Variables|SetupInGame|GetEnemyLevel) _baseshieldblock)))
    (:then_6
      (Variables|/Game/FlexibleCombatSystem/Blueprints/Components/EquipmentComponent.EquipmentComponent_C|SetIntellect _equipmentcomponent (* (Variables|SetupInGame|GetEnemyLevel) _baseintellectspelldamage)))
    (:then_7
      (Variables|/Game/FlexibleCombatSystem/Blueprints/Components/EquipmentComponent.EquipmentComponent_C|SetMainHandWepDamage _equipmentcomponent (* (Variables|SetupInGame|GetEnemyLevel) _basemainhanddamage)))
    (:then_8
      (Variables|/Game/FlexibleCombatSystem/Blueprints/Components/EquipmentComponent.EquipmentComponent_C|SetOffHandWepDamage _equipmentcomponent (* (Variables|SetupInGame|GetEnemyLevel) _baseoffhanddamage)))
    (:then_9
      (Variables|/Game/FlexibleCombatSystem/Blueprints/Components/EquipmentComponent.EquipmentComponent_C|SetRangedWepDamage _equipmentcomponent (* (Variables|SetupInGame|GetEnemyLevel) _baserangeddamage)))
    (:then_11
      (Default|UpdateDamageValues _equipmentcomponent))))

(fn SetupDefaultStats
  (params (AICombatStyle :type E_AICombatStyle%20Enum :default "NewEnumerator7"))
  (return (Utilities|Select :Index AICombatStyle :NewEnumerator7 (Utilities|Struct|MakeS_Custom_AI_Values false 1e+02 1e+02 0.0 1.0 0 0 0.0 5 0 0 20) :NewEnumerator0 (Utilities|Struct|MakeS_Custom_AI_Values false 1.5e+02 7e+01 0.0 1.0 15 10 0.0 10 0 0 20) :NewEnumerator1 (Utilities|Struct|MakeS_Custom_AI_Values false 1e+02 7e+01 0.0 2.0 10 0 0.0 20 0 0 20) :NewEnumerator2 (Utilities|Struct|MakeS_Custom_AI_Values false 1e+02 1.5e+02 0.0 5.0 5 0 0.0 7 7 0 20) :NewEnumerator3 (Utilities|Struct|MakeS_Custom_AI_Values false 1e+02 1.5e+02 0.0 5.0 5 0 0.0 7 0 0 20) :NewEnumerator4 (Utilities|Struct|MakeS_Custom_AI_Values false 1e+02 1.5e+02 0.0 5.0 5 0 0.0 5 0 20 20) :NewEnumerator5 (Utilities|Struct|MakeS_Custom_AI_Values false 1e+02 7e+01 2e+02 1.0 2 0 5.0 5 0 0 20))))

(fn SetupArmor
  ;[1 1 1] Sets Either Default OR Custom Armor
  (if (Utilities|Struct|BreakS_Custom_AI_Equipment (Variables|SetupInGame|GetCustomEquipment))
    (CallFunction|StoreArmor (Variables|SetupInGame|GetCustomEquipment))
    (else
      (bind _customequipment (CallFunction|SetupDefaultArmor (Variables|SetupinGame|GetAI%20Combat%20Style)))
      (CallFunction|StoreArmor _customequipment))))

(fn StoreArmor
  (params (S_Custom_AI_Equipment :type S%20Custom%20AI%20Equipment%20Structure%20%28by%20ref%29)))

(fn SetupDefaultArmor
  (params (AICombatStyle :type E_AICombatStyle%20Enum :default "NewEnumerator7"))
  (return (Utilities|Select :Index AICombatStyle :NewEnumerator7 (Utilities|Struct|MakeS_Custom_AI_Equipment false) :NewEnumerator0 (Utilities|Struct|MakeS_Custom_AI_Equipment false) :NewEnumerator1 (Utilities|Struct|MakeS_Custom_AI_Equipment false) :NewEnumerator2 (Utilities|Struct|MakeS_Custom_AI_Equipment false) :NewEnumerator3 (Utilities|Struct|MakeS_Custom_AI_Equipment false) :NewEnumerator4 (Utilities|Struct|MakeS_Custom_AI_Equipment false) :NewEnumerator5 (Utilities|Struct|MakeS_Custom_AI_Equipment false))))

(fn SetupWeapon
  ;[1 1 1] Sets Up The Attack Styles And Weapon Outputs For AI Controller, Combat Component & Mele Component
  (Class|IAIController|UpdateAttackStyle(Message) (AI|GetAIController self) (Utilities|Select :Index (Variables|SetupinGame|GetAI%20Combat%20Style) :NewEnumerator7 "NewEnumerator0" :NewEnumerator0 "NewEnumerator0" :NewEnumerator1 "NewEnumerator0" :NewEnumerator2 "NewEnumerator0" :NewEnumerator3 "NewEnumerator0" :NewEnumerator4 "NewEnumerator1" :NewEnumerator5 "NewEnumerator2") (Utilities|Select :Index (Variables|SetupinGame|GetAI%20Combat%20Style) :NewEnumerator7 "NewEnumerator2" :NewEnumerator0 "NewEnumerator6" :NewEnumerator1 "NewEnumerator1" :NewEnumerator2 "NewEnumerator3" :NewEnumerator3 "NewEnumerator0" :NewEnumerator4 "NewEnumerator5" :NewEnumerator5 "NewEnumerator9"))
  ;[1 1 1] Set Range Based On Combat Style
  (Variables|Default|SetMelee%20Weapon%20Range (Utilities|Select :Index (Variables|SetupinGame|GetAI%20Combat%20Style) :NewEnumerator7 1.5e+02 :NewEnumerator0 4e+02 :NewEnumerator1 4e+02 :NewEnumerator2 4e+02 :NewEnumerator3 4e+02 :NewEnumerator4 4e+02 :NewEnumerator5 4e+02))
  (if (not (.UseCustomEquipment (Utilities|Struct|BreakS_Custom_AI_Weapon (Variables|SetupInGame|GetCustomWeapon))))
    ;[1 1 1] Create Weapons
    (switch Utilities|FlowControl|Switch|SwitchonE_AICombatStyle (Variables|SetupinGame|GetAI%20Combat%20Style)
      (:NewEnumerator7
        (CallFunction|SpawnAIWeapon true "NewEnumerator9"))
      (:NewEnumerator0
        (CallFunction|SpawnAIWeapon false "NewEnumerator9" (LocalVariables|GetMainHandSword))
        (CallFunction|SpawnAIWeapon false "NewEnumerator20" (LocalVariables|GetShieldInfo))
        (if (Variables|SetupInGame|GetCanSwitchAttackStyle) :!label _label
          (CallFunction|SpawnAIWeapon false "NewEnumerator13" (LocalVariables|GetBowInfo))))
      (:NewEnumerator1
        (CallFunction|SpawnAIWeapon false "NewEnumerator9" (LocalVariables|GetTwoHandedInfo))
        (goto _label))
      (:NewEnumerator2
        (CallFunction|SpawnAIWeapon false "NewEnumerator9" (LocalVariables|GetDaggerInfo))
        (CallFunction|SpawnAIWeapon false "NewEnumerator10" (LocalVariables|GetDaggerInfo))
        (goto _label))
      (:NewEnumerator3
        (CallFunction|SpawnAIWeapon false "NewEnumerator9" (LocalVariables|GetMainHandSword))
        (goto _label))
      (:NewEnumerator4
        (CallFunction|SpawnAIWeapon false "NewEnumerator13" (LocalVariables|GetBowInfo))
        (CallFunction|SpawnAIWeapon false "NewEnumerator17" (LocalVariables|GetQuiverInfo))
        (if (Variables|SetupInGame|GetCanSwitchAttackStyle)
          (CallFunction|SpawnAIWeapon false "NewEnumerator9" (LocalVariables|GetDaggerInfo)))))))

(fn Death
  (params (SavedDeath :type Boolean))
  (bind _combatstatuscomponent (Variables|Default|GetCombatStatusComponent))
  (bind _mesh (Variables|Character|GetMesh))
  (Utilities|FlowControl|DoOnce false
    (:Completed
      (Class|IItemInterface|ActivateActor(Message) (Variables|SetupInGame|GetActivateActorOnDeath))
      (CallFunction|IsQuestActor (Game|GetPlayerController 0) 1 (Variables|SetupInGame|GetQuest%20ID))
      ;[1 1 1] Detach Weapon
      (Class|IWeaponInterface|PlayerDied(Message) (Variables|/Game/FlexibleCombatSystem/Blueprints/Components/CombatStatusComponent.CombatStatusComponent_C|GetEquippedOffHand _combatstatuscomponent))
      (Class|IWeaponInterface|PlayerDied(Message) (Variables|/Game/FlexibleCombatSystem/Blueprints/Components/CombatStatusComponent.CombatStatusComponent_C|GetEquippedMainHand _combatstatuscomponent))
      (Class|IWeaponInterface|PlayerDied(Message) (Variables|/Game/FlexibleCombatSystem/Blueprints/Components/CombatStatusComponent.CombatStatusComponent_C|GetEquippedRangedWeapon _combatstatuscomponent))
      (Variables|Character|SetDead true)
      (Variables|AttackVariables|SetBlockUp false)
      (Variables|/Game/FlexibleCombatSystem/Blueprints/Components/RangedComponent.RangedComponent_C|SetOwnerDead (Variables|Default|GetRangedComponent) true)
      ;[1 1 1] Remove Capsule Collision
      (Components|DestroyComponent (Variables|Collision|GetCapsuleComponent))
      (Collision|SetCollisionResponsetoChannel _mesh "ECC_WorldStatic" "ECR_Block")
      (Collision|SetCollisionResponsetoChannel _mesh "ECC_WorldDynamic" "ECR_Block")
      (Collision|SetCollisionResponsetoChannel _mesh "ECC_Pawn" "ECR_Overlap")
      ;[1 1 1] Go Ragdoll
      (Physics|SetSimulatePhysics (Variables|Character|GetMesh) true)
      ;[1 1 1] Stops Running Anim BP
      (Components|Animation|SetAnimationMode (Variables|Character|GetMesh) "AnimationCustomMode")
      (if SavedDeath
        ;[1 1 1] Remove Player Lock On Target and Give Player XP
        (Default|CheckforNextLock (Actor|GetComponentbyClass (Game|GetPlayerCharacter 0) "/Game/FlexibleCombatSystem/Blueprints/Components/TargetingComponent.TargetingComponent_C"))
        (Default|IncreaseXP (Actor|GetComponentbyClass (Game|GetPlayerCharacter 0) "/Game/FlexibleCombatSystem/Blueprints/Components/EquipmentComponent.EquipmentComponent_C") (Variables|SetupInGame|GetXP_GivenWhenKilled))))))

(fn SlowMotionRunning
  (params (Running? :type Boolean))
  (if Running?
    (Variables|AttackVariables|SetSlowMotionOccuring true)
    (Input|DisableInput (Game|GetPlayerController 0))
    (else
      (Input|EnableInput (Game|GetPlayerController 0))
      (Variables|AttackVariables|SetSlowMotionOccuring false))))

(fn SlowMotionConditions
  (params (IncomingDamage :type Integer))
  (if (Variables|Character|GetDead)
    (LocalVariables|SetCanTriggerKIllCam false :!label _label)
    (else
      ;[1 1 1] Close Enough To Player To Trigger
      (if (Variables|AttackVariables|GetInPlayerRange)
        ;[1 1 1] If Incoming Damage is more then current Health
        (if (>= IncomingDamage 0)
          (if (Variables|AttackVariables|GetBlockUp)
            (goto _label)
            (else
              (LocalVariables|SetCanTriggerKIllCam true)))
          (else
            (goto _label)))
        (else
          (goto _label)))))
  (return (LocalVariables|GetCanTriggerKIllCam)))

(fn ReportNoise
  (params (NoiseLocation :type Vector) (Instigator :type Actor%20Object%20Reference))
  (Class|AISenseHearing|ReportNoiseEvent NoiseLocation 1.0 Instigator 2e+02 "None")
  (Class|AISenseDamage|ReportDamageEvent self Instigator 1e+01 NoiseLocation "0, 0, 0" "None"))

(fn UpdateWidgetValues
  (bind _equipmentcomponent (Variables|Default|GetEquipmentComponent))
  (bind _equipmentcomponent_2 (Variables|Default|GetEquipmentComponent))
  (bind _equipmentcomponent_3 (Variables|Default|GetEquipmentComponent))
  (bind _maxhealth (Variables|/Game/FlexibleCombatSystem/Blueprints/Components/EquipmentComponent.EquipmentComponent_C|GetMaxHealth _equipmentcomponent_2))
  (bind _maxmana (Variables|/Game/FlexibleCombatSystem/Blueprints/Components/EquipmentComponent.EquipmentComponent_C|GetMaxMana _equipmentcomponent_3))
  (bind _maxstamina (Variables|/Game/FlexibleCombatSystem/Blueprints/Components/EquipmentComponent.EquipmentComponent_C|GetMaxStamina _equipmentcomponent))
  (Default|CallUpdateHealth _equipmentcomponent_2 _maxhealth _maxhealth)
  (Default|CallUpdateStamina (Variables|Default|GetResourceComponent) _maxstamina _maxstamina)
  (Default|CallUpdateMana (Variables|Default|GetResourceComponent) _maxmana _maxmana))

(fn BeginPlayDeathCheck)

(fn InitializeComponents)

(fn SetupComponents
  (Default|InitializeCombatStatus (Variables|Default|GetCombatStatusComponent) true)
  (Variables|/Game/FlexibleCombatSystem/Blueprints/Components/InputBufferComponent.InputBufferComponent_C|SetEnemyAI (Variables|Default|GetInputBufferComponent) true)
  (Variables|/Game/FlexibleCombatSystem/Blueprints/Components/TakingDamage.TakingDamage_C|SetEnemyAI (Variables|Default|GetTakingDamage) true)
  (Variables|/Game/FlexibleCombatSystem/Blueprints/Components/RangedComponent.RangedComponent_C|SetEnemyAI (Variables|Default|GetRangedComponent) true)
  (Variables|/Game/FlexibleCombatSystem/Blueprints/Components/ResourceComponent.ResourceComponent_C|SetEnemyAI (Variables|Default|GetResourceComponent) true))

(fn FindAvailableCamera
  (Components|Activation|Deactivate (Variables|Default|GetAssasinationCamera))
  (bind _array_element (Utilities|Array|ForEachLoopwithBreak (Utilities|Array|MakeArray (Variables|Default|GetAssasinationCamera) 0 0 0 0 0 0) :!label _label)
    (:LoopBody
      (LocalVariables|SetCurrentCamera _array_element)
      (bind _returnvalue (Collision|SphereTraceForObjects (Transformation|GetWorldLocation _array_element) (Transformation|GetActorLocation) 2e+01 (Utilities|Array|MakeArray "ObjectTypeQuery1") false 0 "None"))
      (if (not _returnvalue)
        (LocalVariables|SetSuccess true)
        (goto _label Break)))
    (:Completed
      (if (LocalVariables|GetSuccess)
        (return (LocalVariables|GetCurrentCamera))
        (else
          (return (Variables|Default|GetCharacterCamera)))))))

(fn SetupCustomArrows
  ;[1 1 1] Provide Custom Arrows and Rank
)

(fn SpawnAIWeapon
  (params (Fists :type Boolean) (Item%20Type :type E_ItemType%20Enum :default "NewEnumerator18") (Weapon%20Info :type S%20Item%20Setup%20Data%20Structure))
  (bind _datatableinfo (Utilities|Struct|BreakS_ItemSetupData Weapon%20Info))
  (bind (_datatable _rowname) (Utilities|Struct|BreakDataTableRowHandle _datatableinfo))
  (if Fists
    ;[1 1 1] Fist Combat
    (bind _returnvalue (Game|SpawnActorfromClass "/Game/FlexibleCombatSystem/Blueprints/Items/PickUpItems/BP_Fists.BP_Fists_C" (Math|Transform|MakeTransform "0, 0,10000.000000" "0, 0, 0" "1,1,1") "Undefined" 0 0))
    (Default|AttachtoPlayer _returnvalue self)
    (Variables|/Game/FlexibleCombatSystem/Blueprints/Components/MeleeComponent.MeleeComponent_C|SetFistsRef (Variables|Default|GetMeleeComponent) _returnvalue)
    (else
      ;[1 1 1] Spawn Set Weapon
      (switch Utilities|FlowControl|Switch|SwitchonE_ItemType Item%20Type
        (:NewEnumerator9
          (bind _returnvalue_2 (Game|SpawnActorfromClass :Class "/Game/FlexibleCombatSystem/Blueprints/Items/PickUpItems/BP_WeaponParent.BP_WeaponParent_C" :SpawnTransform (Math|Transform|MakeTransform (Transformation|GetActorLocation self) "0, 0, 0" "1,1,1") :CollisionHandlingOverride "Undefined" :Instigator 0 :!label _label))
          (LocalVariables|SetWeaponRef _returnvalue_2))
        (:NewEnumerator12
          (goto _label))
        (:NewEnumerator11
          (goto _label))
        (:NewEnumerator10
          (goto _label))
        (:NewEnumerator20
          (goto _label))
        (:NewEnumerator13
          (bind _returnvalue_3 (Game|SpawnActorfromClass :Class "/Game/FlexibleCombatSystem/Blueprints/Items/PickUpItems/BP_BowParent.BP_BowParent_C" :SpawnTransform (Math|Transform|MakeTransform (Transformation|GetActorLocation self) "0, 0, 0" "1,1,1") :CollisionHandlingOverride "Undefined" :Instigator 0))
          (LocalVariables|SetWeaponRef _returnvalue_3))
        (:NewEnumerator17
          (bind _returnvalue_4 (Game|SpawnActorfromClass :Class "/Game/FlexibleCombatSystem/Blueprints/Items/PickUpItems/BP_ArrowQuiverAI.BP_ArrowQuiverAI_C" :SpawnTransform (Math|Transform|MakeTransform (Transformation|GetActorLocation self) "0, 0, 0" "1,1,1") :CollisionHandlingOverride "Undefined" :Instigator 0))
          (LocalVariables|SetWeaponRef _returnvalue_4)))
      ;[1 1 1] Retreive Item Data
      (bind _returnvalue_5 (Utilities|GetDataTableRow _datatable _rowname)
        (:then
          (bind _structout (Utilities|Struct|SetmembersinS_ItemData (Utilities|Struct|BreakS_SlotInfo (Utilities|Struct|MakeS_SlotInfo _returnvalue_5 _datatableinfo)) Item%20Type))
          (bind _structout_2 (Utilities|Struct|SetmembersinS_SlotInfo (Utilities|Struct|MakeS_SlotInfo _returnvalue_5 _datatableinfo) _structout))
          (Class|IItemInterface|Spawn&Use(Message) (LocalVariables|GetWeaponRef) self _structout_2)
          (Class|IWeaponInterface|AttachWeapontoBack(Message) (LocalVariables|GetWeaponRef))
          ;[1 1 1] Set Appropriate Variables
          (switch Utilities|FlowControl|Switch|SwitchonE_ItemType Item%20Type
            (:NewEnumerator9
              (Variables|/Game/FlexibleCombatSystem/Blueprints/Components/CombatStatusComponent.CombatStatusComponent_C|SetEquippedMainHand (Variables|Default|GetCombatStatusComponent) (LocalVariables|GetWeaponRef) :!label _label_2)
              (Variables|/Game/FlexibleCombatSystem/Blueprints/Components/MeleeComponent.MeleeComponent_C|SetEquippedMainHand (Variables|Default|GetMeleeComponent) (LocalVariables|GetWeaponRef)))
            (:NewEnumerator12
              (goto _label_2))
            (:NewEnumerator10
              (Variables|/Game/FlexibleCombatSystem/Blueprints/Components/CombatStatusComponent.CombatStatusComponent_C|SetEquippedOffHand (Variables|Default|GetCombatStatusComponent) (LocalVariables|GetWeaponRef) :!label _label_3)
              (Variables|/Game/FlexibleCombatSystem/Blueprints/Components/MeleeComponent.MeleeComponent_C|SetEquippedOffHand (Variables|Default|GetMeleeComponent) (LocalVariables|GetWeaponRef)))
            (:NewEnumerator20
              (goto _label_3))
            (:NewEnumerator13
              (Default|SetupBow (Variables|Default|GetRangedComponent) (LocalVariables|GetWeaponRef))
              (Variables|/Game/FlexibleCombatSystem/Blueprints/Components/CombatStatusComponent.CombatStatusComponent_C|SetEquippedRangedWeapon (Variables|Default|GetCombatStatusComponent) (LocalVariables|GetWeaponRef)))
            (:NewEnumerator17
              (Default|SetupQuiver (Variables|Default|GetRangedComponent) (LocalVariables|GetWeaponRef)))))))))

(fn DestroyWeaponIFValid)

(fn CanbeAssassinated
  (return true))

(fn FindAvailableAssassinationCam
  (return 0))

(fn GetWeaponRange
  (return (Variables|Default|GetMelee%20Weapon%20Range)))

(fn IsDead
  (return (Variables|Character|GetDead)))

(fn IsFacingEnemy?
  (return false))

(fn IsMoving?
  (return false))

(fn IsPlayer?
  (return false))

(fn IsWeaponDrawn?
  (return false))

(fn PassArmorMeshes
  (return 0 0 0 0 0 0 0 0 0 0 0))

(fn PassAssassinationComps
  (return (Variables|Default|GetAssasinationCamera) (Variables|Default|GetAssassinationRotator)))

(fn PassAttackStyle
  (return (Variables|SetupinGame|GetAI%20Combat%20Style)))

(fn PassBehaviourTree
  (return (Variables|SetupInGame|GetBehaviourTree)))

(fn PassBody
  (return 0 0 0 0 0 0 0 0))

(fn PassCamera
  (return (Variables|Default|GetAssasinationCamera) 0))

(fn PassHealthHUD
  (return 0))

(fn PassMovementMode
  (return (Variables|/Script/Engine.CharacterMovementComponent|GetMovementMode (Variables|Character|GetCharacterMovement))))

(fn PassSpline
  (return (Variables|SetupInGame|GetPathwaySplineRef)))

(fn PassSwitchAttackStyle
  (return false))

(fn PassWarningMesh
  (return 0))

(fn PassWeaponRange
  (return (Variables|Default|GetMelee%20Weapon%20Range)))

(fn RemoveEnemyHUD)

(fn RetrieveInventoryInfo
  (return "NewEnumerator0" "" 0 0 false 0 0))

(fn RetrieveLootInfo
  (return ""))

(fn RetrieveOutlineInfo
  (bind _enemylootinfo (Variables|SetupInGame|GetEnemyLootInfo))
  (bind (_lootname _rarityoflootcolour) (Utilities|Struct|BreakS_LootSetupInfo _enemylootinfo))
  (return _lootname _rarityoflootcolour "NewEnumerator1" 0 0 0 (Variables|Character|GetMesh)))

(fn RetrievePlayerStatus
  (return false "NewEnumerator2" "NewEnumerator0"))

(fn SendDeath
  (CallFunction|Death true)
  (return))

(fn SetDisableControls
  (params (DisableMovement :type Boolean) (DisableCamera :type Boolean))
  (return))

(fn UpdateMovementMode
  (params (MovementMode :type EMovementMode%20Enum :default "MOVE_None"))
  (Pawn|Components|CharacterMovement|SetMovementMode (Variables|Character|GetCharacterMovement) MovementMode 0)
  (return true))