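; Player character with fixed diagonal world-axis movement, melee attacks, a bolas throw, dashing and health.
; Basic attack calls ACMeleePlayer and triggers nearby rope levers; bolas re-arms on BolasReturn.
; Game Instance sacrifice flags unlock blood waves and the dash, which has limited charges and briefly ignores Pawn and WorldDynamic collision.
; Damage knocks back, lowers Game Instance health and the HUD bar, then plays a hit reaction or destroys the actor.
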(event Custom|NearTheLever
  (params (nearLever :type Actor%20Object%20Reference))
  ;[1 1 1] Attaque Basique
  ;;[0 1 0.01273] Rope Code
  (Variables|Default|SetNearRope nearLever))

(event Custom|BolasReturn
  ;[1 0.8279 0] Bolas
  (Utilities|FlowControl|DoOnce false) ; enters at Reset
)

(event Game|Damage|EventAnyDamage
  (params (Damage :type Float%20%28single-precision%29) (DamageType :type Damage%20Type%20Object%20Reference) (InstigatedBy :type Controller%20Object%20Reference) (DamageCauser :type Actor%20Object%20Reference))
  ;[1 1 1] HP Player
  (CallFunction|KnockBack)
  (bind _output_get (Variables|/Game/Proto/Main/Blueprint/BloodTrial_GameInstance.BloodTrial_GameInstance_C|SetChoose_Life (CallFunction|GetInst) (- (Variables|/Game/Proto/Main/Blueprint/BloodTrial_GameInstance.BloodTrial_GameInstance_C|GetChoose_Life (CallFunction|GetInst)) Damage)))
  (Progress|SetPercent (Variables|/Game/Proto/Proto_Guillaume/Blueprints/Player/HP_Bar_Player.HP_Bar_Player_C|GetProgressBar_40 (stale EventBeginPlay _output_get)) (Math|Float|SafeDivide _output_get 3e+02))
  (Math|Float|CompareFloat (Math|Float|SafeDivide _output_get 3e+02) 0.0
    (:>
      (if (Variables|Actor|GetbCanBeDamaged)
        (Variables|Actor|SetbCanBeDamaged false)
        (Animation|Montage|PlayMontage (Variables|Character|GetMesh) "/Game/Proto/Proto_Guillaume/Blueprints/Anim_Mixamo/30FPS/MediumHitToHead_UE_Montage.MediumHitToHead_UE_Montage" 0.5
          (:then
            _)
          (:OnNotifyBegin
            _))
        (Variables|Actor|SetbCanBeDamaged true)
        (Game|Feedback|ClientPlayForceFeedback (Game|GetPlayerController 0) "/Game/Proto/Proto_Guillaume/Blueprints/Player/Damage.Damage" "None" false false false)))
    (:==
      (Actor|DestroyActor :!label _label))
    (:<
      (goto _label))))

(event EventBeginPlay
  ;[1 1 1] HP Player
  (bind _returnvalue (UserInterface|CreateWidget "/Game/Proto/Proto_Guillaume/Blueprints/Player/HP_Bar_Player.HP_Bar_Player_C"))
  (UserInterface|Viewport|AddtoViewport _returnvalue 0)
  (bind _output_get (Variables|Default|SetAs_HP_Bar_Player _returnvalue)))

(event Input|ActionEvents|InputActionDash
  (params (Key :type Key%20Structure :default "None"))
  (bind _asblood_trial_game_instance (CallFunction|GetInst))
  (bind _charactermovement (Variables|Character|GetCharacterMovement))
  (bind _returnvalue (Pawn|Components|PawnMovement|GetLastInputVector _charactermovement))
  (bind _returnvalue_2 (* _returnvalue 2e+01))
  ;[0 0.05597 1] Dash + besoin anim / SFX/VFX
  (:Pressed
    (if (Variables|/Game/Proto/Main/Blueprint/BloodTrial_GameInstance.BloodTrial_GameInstance_C|GetSacrify_1 _asblood_trial_game_instance)
      (if (< (Variables|/Game/Proto/Main/Blueprint/BloodTrial_GameInstance.BloodTrial_GameInstance_C|GetNB_Dash _asblood_trial_game_instance) (Variables|/Game/Proto/Main/Blueprint/BloodTrial_GameInstance.BloodTrial_GameInstance_C|GetMaxDash _asblood_trial_game_instance))
        (Collision|SetCollisionResponsetoChannel (Variables|Collision|GetCapsuleComponent) "ECC_Pawn" "ECR_Ignore")
        (Collision|SetCollisionResponsetoChannel (Variables|Collision|GetCapsuleComponent) "ECC_WorldDynamic" "ECR_Ignore")
        (Variables|/Game/Proto/Main/Blueprint/BloodTrial_GameInstance.BloodTrial_GameInstance_C|SetNB_Dash _asblood_trial_game_instance (+ (Variables|/Game/Proto/Main/Blueprint/BloodTrial_GameInstance.BloodTrial_GameInstance_C|GetNB_Dash _asblood_trial_game_instance) 1))
        (Character|LaunchCharacter (Math|Vector|MakeVector (.x _returnvalue_2) (.y _returnvalue_2) 0.0) false false)
        (Utilities|FlowControl|Delay 0.5)
        (Collision|SetCollisionResponsetoChannel (Variables|Collision|GetCapsuleComponent) "ECC_WorldDynamic" "ECR_Block")
        (Collision|SetCollisionResponsetoChannel (Variables|Collision|GetCapsuleComponent) "ECC_Pawn" "ECR_Block")
        (Utilities|FlowControl|Delay 0.5)
        (Variables|/Game/Proto/Main/Blueprint/BloodTrial_GameInstance.BloodTrial_GameInstance_C|SetNB_Dash (CallFunction|GetInst) 0)
        (Class|NavMovementComponent|StopMovementKeepPathing (Variables|Character|GetCharacterMovement))
        (else
          (Utilities|FlowControl|Delay 0.5)
          (Variables|/Game/Proto/Main/Blueprint/BloodTrial_GameInstance.BloodTrial_GameInstance_C|SetNB_Dash _asblood_trial_game_instance 0))))))

(event Input|ActionEvents|InputActionSpecialAttack
  (params (Key :type Key%20Structure :default "None"))
  ;[1 0.8279 0] Bolas
  (:Pressed
    (Utilities|FlowControl|DoOnce false
      (:Completed
        (Game|SpawnActorfromClass "/Game/Proto/Proto_Florian/Blueprints/BP_Bolas.BP_Bolas_C" (Math|Transform|MakeTransform (Transformation|GetWorldLocation (Variables|Default|GetSpawnBolas)) (Class|CharacterMovementComponent|GetLastUpdateRotation (Variables|Character|GetCharacterMovement))) "Undefined" 0 0)))))

(event Input|ActionEvents|InputActionBasicAttack
  (params (Key :type Key%20Structure :default "None"))
  (bind _charactermovement (Variables|Character|GetCharacterMovement))
  (bind _returnvalue (Class|CharacterMovementComponent|GetLastUpdateRotation _charactermovement))
  ;[1 1 1] Attaque Basique
  (:Pressed
    (Default|Attaque (Variables|Default|GetAC_Melee_Player))
    (Utilities|FlowControl|Sequence
      (:then_0
        ;;[1 0.8279 0] Blood Wave À mettre en lien avec les anims
        (if (Variables|/Game/Proto/Main/Blueprint/BloodTrial_GameInstance.BloodTrial_GameInstance_C|GetSacrify_6 (CallFunction|GetInst))
          (Game|SpawnActorfromClass "/Game/Proto/Proto_Florian/Blueprints/BP_Blood_Waves.BP_Blood_Waves_C" (Math|Transform|MakeTransform (+ (Transformation|GetWorldLocation (Variables|Default|GetSpawnBloodWave)) (* (Math|Vector|GetForwardVector _returnvalue) 5e+01)) _returnvalue (Transformation|GetWorldScale (Variables|Default|GetChildActor))) "Undefined" 0 0)))
      (:then_1
        ;;[0 1 0.01273] Rope Code
        (if (!= (Variables|Default|GetNearRope) 0)
          (Default|LeverActive (.AsBP%20Rope (Utilities|Casting|CastToBP_Rope (Variables|Default|GetNearRope)))))))))

(event Input|AxisEvents|InputAxisMoveForward/Backward
  (params (AxisValue :type Float%20%28single-precision%29))
  ;[0 1 0.01267] Déplacement
  (if (>= (Math|Float|Absolute(Float) (* AxisValue 1e+01)) 1.0)
    (Pawn|Input|AddMovementInput (Class|PawnMovementComponent|GetPawnOwner (Variables|Character|GetCharacterMovement)) "100.000000,-100.000000,0.000000" AxisValue false)))

(event Input|AxisEvents|InputAxisMoveLeft/Right
  (params (AxisValue :type Float%20%28single-precision%29))
  ;[0 1 0.01267] Déplacement
  (if (>= (Math|Float|Absolute(Float) (* AxisValue 1e+01)) 1.0)
    (Pawn|Input|AddMovementInput (Class|PawnMovementComponent|GetPawnOwner (Variables|Character|GetCharacterMovement)) "-100.000000,-100.000000, 0" AxisValue false)))

(fn ConstructionScript)

(fn KnockBack
  (bind _returnvalue (Transformation|GetActorRotation))
  (bind _returnvalue_2 (Math|Vector|GetForwardVector _returnvalue))
  (bind _returnvalue_3 (* _returnvalue_2 -1e+02))
  (bind (_x _y _z) (Math|Vector|BreakVector _returnvalue_3))
  (Character|LaunchCharacter (Math|Vector|MakeVector _x _y (+ _z 5e+01)) false false))