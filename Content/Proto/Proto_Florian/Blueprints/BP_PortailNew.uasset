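; Prototype gate (portail) actor that drops when a rope has been cut.
; BeginPlay stores the static mesh's starting relative location.
; Tick polls the RopeCut flag from GetInst and, while it is set, calls an eased MoveComponentTo every frame toward a fixed point below that origin, with a sub-second duration.
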(event EventBeginPlay
  (Variables|Default|SetPortail_Origin_Position (Variables|/Script/Engine.SceneComponent|GetRelativeLocation (Variables|Default|GetStaticMesh))))

(event EventTick
  (params (DeltaSeconds :type Float%20%28single-precision%29))
  (if (Variables|/Game/Proto/Main/Blueprint/BloodTrial_GameInstance.BloodTrial_GameInstance_C|GetRopeCut? (CallFunction|GetInst))
    (Components|MoveComponentTo (Variables|Default|GetStaticMesh) (+ (Variables|Default|GetPortail_Origin_Position) "0,0,-500.000000") "0, 0, 0" true true 0.42 false)))

(fn ConstructionScript)