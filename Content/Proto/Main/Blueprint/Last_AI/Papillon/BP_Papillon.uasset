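; Papillon enemy AI character that closes on the player, randomly attacks or strafes, and can fire an impulse-launched projectile.
; Movement loops through AIMoveTo and Tick-driven strafing, with a sighting routine that alerts every Papillon.
; Damage drains a floating health bar, triggering hit stop, knockback and invincibility frames, or death with score and optional player vampirism.
; Bolas events play a strangle montage, pause the AI, then explode and fly the bolas back.
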(event OnSeePawn(PawnSensing)
  (params (Pawn :type Pawn%20Object%20Reference)))

(event Custom|PlayerIsSeen
  ;[1 1 1] General Behavior Logic
  (Animation|Montage|PlayMontage (Variables|Character|GetMesh) "/Game/Proto/Animation/Papillon/Animation/papillon_TakeBigdamage_Montage.papillon_TakeBigdamage_Montage"
    (:OnCompleted
      (bind _outactors (Actor|GetAllActorsOfClass "BP_Papillon_C"))
      (CallFunction|Weknowurlocation _outactors))))

(event Custom|Boule2Feu
  ;[1 1 1] General Behavior Logic
  (CallFunction|SpawnSpell))

(event Custom|Weknowurlocation
  (bind _returnvalue (Game|GetPlayerCharacter 0))
  (bind _returnvalue_2 (Game|GetPlayerCharacter 0))
  ;[1 1 1] General Behavior Logic
  (Variables|/Script/AIModule.PawnSensingComponent|SetSightRadius (Variables|Default|GetPawnSensing) 0.0)
  (if true
    (if (Variables|Default|GetisHit)
      (Utilities|FlowControl|Delay 0.7)
      (Variables|Default|SetisHit false)
      (else
        (AI|AIMoveTo self (Transformation|GetWorldLocation (Variables|/Script/Engine.Character|GetCapsuleComponent _returnvalue)) _returnvalue 1e+03 true
          (:OnSuccess
            (if (Variables|Default|GetMustAttack)
              (AI|AIMoveTo self (Transformation|GetWorldLocation (Variables|/Script/Engine.Character|GetCapsuleComponent _returnvalue_2)) _returnvalue_2 6e+02 true :!label _label
                (:OnSuccess
                  (CallFunction|ServerNPCMeleeAttack)
                  (Utilities|FlowControl|Delay 1.0)
                  (Variables|Default|SetMustAttack false)
                  (CallFunction|Weknowurlocation)))
              (else
                (switch int (Math|Random|RandomInteger 3)
                  (:0
                    (goto _label))
                  (:1
                    (Variables|Default|SetStrafingDirection "NewEnumerator0")
                    (Variables|Default|SetStrafing? true))
                  (:2
                    (Variables|Default|SetStrafingDirection "NewEnumerator1")
                    (Variables|Default|SetStrafing? true))
                  (:3
                    (Variables|Default|SetStrafingDirection "NewEnumerator2")
                    (Variables|Default|SetStrafing? true)))
                (Utilities|FlowControl|Delay (Math|Random|RandomFloatinRange 0.5 1.3))
                (Variables|Default|SetStrafing? false)
                (Variables|Default|SetMustAttack true)
                (CallFunction|Weknowurlocation)))))))))

(event Custom|Mort_IA
  (bind _returnvalue (Transformation|GetActorLocation))
  ;[0.08256 1 0] Mort IA
  (Utilities|FlowControl|Sequence
    (:then_0
      (if (Variables|/Game/Proto/Main/Blueprint/Save_BFL_GameInstance/BloodTrial_GameInstance.BloodTrial_GameInstance_C|GetSacrifice_5 (CallFunction|GetInst))
        (bind _asbp_main_base (Utilities|Casting|CastToBP_MainBase (Game|GetPlayerCharacter 0)))
        (Default|VampirismeonDeath _asbp_main_base)))
    (:then_1
      (Utilities|FlowControl|DoOnce false
        (:Completed
          (CallFunction|IncrScore (Variables|/Game/Proto/Main/Blueprint/Save_BFL_GameInstance/BloodTrial_GameInstance.BloodTrial_GameInstance_C|GetScore_Enemy1 (CallFunction|GetInst))))))
    (:then_2
      (Collision|SetCollisionResponsetoChannel (Variables|Default|GetCapsuleComponent) "ECC_GameTraceChannel2" "ECR_Ignore")
      (Audio|PlaySoundatLocation "/Game/Proto/Main/Blueprint/SFX_Player/Death_Tzitzimine/249813__spookymodem__goblin-death.249813__spookymodem__goblin-death" _returnvalue "0, 0, 0" 0.2 1.0 0.0 0 0 0 0)
      (Effects|SpawnEmitteratLocation "/Game/Proto/Proto_Guillaume/Blueprints/DynamicHealthbars/_Demo/FX/EnemyDeath/P_EnemyDeath.P_EnemyDeath" _returnvalue)
      (CallFunction|PlayHighPriorityMontage "/Game/Proto/Animation/Papillon/Animation/papillon_death_Montage.papillon_death_Montage" "None" 1.0))))

(event Custom|Collision_Explosion
  ;[1 0 0.7108] Explosion
  ;;[1 0.9631 0] Step 1 : Spawn sphere collision pour explosion et identifier les actors touchés
  (Game|SpawnActorfromClass "/Game/Proto/Proto_Guillaume/Blueprints/Player/Explosion.Explosion_C" (Math|Conversions|ToTransform(Vector) (Transformation|GetWorldLocation (Variables|Default|GetBolasAttached))) "Undefined" 0 0)
  (CallFunction|BolasReturnPlayer))

(event Custom|Event_Death
  ;[0.08256 1 0] Mort IA
  (Actor|DestroyActor))

(event Custom|Trigger_Again)

(event Custom|SpawnBolas_T
  ;[1 0 0.7542] Step 1 : Bolas s'attache sur l'ennemi
  (Animation|Montage|MontageStop (Components|SkeletalMesh|GetAnimInstance (Variables|Character|GetMesh)) 0.0 0))

(event Custom|Explosion_M
  ;[1 0 0.7108] Explosion
  ;;[0.1952 1 0] Step 1 : Déclencher l'explosion + Throw bolas pas valide
  (Variables|/Game/Proto/Main/Blueprint/Save_BFL_GameInstance/BloodTrial_GameInstance.BloodTrial_GameInstance_C|SetCanThrowBolas? (CallFunction|GetInst) false)
  ;;[0.1836 1 0] Step 1.5 : Stop anim being strangled
  (Animation|StopAnimMontage "/Game/Proto/Proto_Guillaume/Blueprints/Anim_Mixamo/30FPS/BeingStrangled_UE_Montage.BeingStrangled_UE_Montage")
  ;;[0.1621 1 0] Step 3 : Call debug de l'explosion + valide variable explosion
  (CallFunction|CollisionExplosion)
  (Variables|Default|SetExplosion true))

(event Custom|BolasReturn_Player
  (bind _asblood_trial_game_instance (CallFunction|GetInst))
  (bind _mesh (Variables|Character|GetMesh))
  (bind _returnvalue (Transformation|GetWorldLocation _mesh))
  ;[0.8705 1 0] Bolas en cours
  (bind _returnvalue_2 (Game|SpawnActorfromClass "/Game/Proto/Proto_Florian/Blueprints/BP_Apparence_Bolas.BP_Apparence_Bolas_C" (Math|Transform|MakeTransform (Math|Vector|MakeVector (.x _returnvalue) (.y _returnvalue) (+ (.z _returnvalue) 2e+02)) (Transformation|GetWorldRotation _mesh) "0.300000,0.300000,0.300000") "AlwaysSpawn" 0 0))
  (bind _returnvalue_3 (Actor|GetActorOfClass "/Game/Proto/Main/Blueprint/BP_MainBase.BP_MainBase_C"))
  (Components|MoveComponentTo (Variables|/Game/Proto/Proto_Florian/Blueprints/BP_Apparence_Bolas.BP_Apparence_Bolas_C|GetStaticMesh _returnvalue_2) (Math|Vector|MakeVector (.x (Transformation|GetWorldLocation (Variables|/Script/Engine.Character|GetMesh _returnvalue_3))) (.y (Transformation|GetWorldLocation (Variables|/Script/Engine.Character|GetMesh _returnvalue_3))) (.z (Transformation|GetWorldLocation (Variables|/Script/Engine.Character|GetMesh _returnvalue_3)))) "0, 0, 0" true true 0.3 true)
  (Variables|/Game/Proto/Main/Blueprint/Save_BFL_GameInstance/BloodTrial_GameInstance.BloodTrial_GameInstance_C|SetIsBolas_Attached? _asblood_trial_game_instance false)
  (Variables|/Game/Proto/Main/Blueprint/Save_BFL_GameInstance/BloodTrial_GameInstance.BloodTrial_GameInstance_C|SetCanThrowBolas? _asblood_trial_game_instance true)
  (Actor|DestroyActor _returnvalue_2))

(event Custom|AI_IS_Bolassed
  (Variables|Default|SetbCanBeDamaged true))

(event Custom|Finito
  ;[1 0 0.7542] Step 1 : Bolas s'attache sur l'ennemi
  (Utilities|FlowControl|DoOnce false ; enters at Reset
    (:Completed
      ;;[0.2174 1 0] Step 1 : Faire spawn 1 fois le bolas attaché + Validation bolas attached.
      ;; Bolas attached condition ==> Lead to explosion if 2nd input
      (Variables|/Game/Proto/Main/Blueprint/Save_BFL_GameInstance/BloodTrial_GameInstance.BloodTrial_GameInstance_C|SetIsBolas_Attached? (CallFunction|GetInst) true)
      ;;[0.9325 1 0] Step 3  :Jouer l'animation d'étranglement - Besoin anim étranglement Tzitzimine
      (bind _notifyname (Animation|Montage|PlayMontage (Variables|Character|GetMesh) "/Game/Proto/Animation/Papillon/Animation/papillon_TakeBigdamage_Montage.papillon_TakeBigdamage_Montage" 3.0)
        (:OnCompleted
          ;;[0.2224 1 0] Step 5 : Si animation étranglement completed / interrupted alors bolas return player + Cast contre attaque
          (CallFunction|ExplosionM))
        (:OnNotifyBegin
          (switch name _notifyname :!label _label
            (:GetBolassed_1
              ;;[1 0.6248 0] Step 6 : Notify begin then stop mvt AI + Cast AI state bolassed
              (Pawn|Components|CharacterMovement|SetMovementMode (Variables|Character|GetCharacterMovement) "MOVE_None" 0)
              (bind _asai_controler_melee (Utilities|Casting|CastToAI_Controler_Melee (AI|GetAIController 0)))
              (Default|GetBolassed _asai_controler_melee))
            (:GetBolassed_2
              ;;[1 0.6248 0] Step 7 : Notify end then stop mvt AI + Cast AI state bolassed
              (Pawn|Components|CharacterMovement|SetMovementMode (Variables|Character|GetCharacterMovement) "MOVE_Walking" 0)
              (bind _asai_controler_melee_2 (Utilities|Casting|CastToAI_Controler_Melee (AI|GetAIController 0)))
              (Default|EndGetBolassed _asai_controler_melee_2))))
        (:OnNotifyEnd
          (goto _label))))))

(event Game|Damage|EventAnyDamage
  (params (Damage :type Float%20%28single-precision%29) (DamageType :type Damage%20Type%20Object%20Reference) (InstigatedBy :type Controller%20Object%20Reference) (DamageCauser :type Actor%20Object%20Reference))
  (bind _newparam (CallFunction|GetHealthBarWidget0))
  (bind _capsulecomponent (Variables|Default|GetCapsuleComponent))
  (bind _value (Default|GetCurrentValue _newparam "NewEnumerator0"))
  (Variables|Default|SetDamage_0 Damage)
  (Variables|Default|SetDamage%20Causer DamageCauser)
  (Variables|Default|SetImpact%20Normal (Math|Vector|GetForwardVector (Variables|/Script/Engine.Character|GetCapsuleComponent (Game|GetPlayerCharacter 0))))
  (if (Variables|Default|GetAIDead)
    (CallFunction|EventDeath)
    (elif (>= _value 1.0)
      (Default|SubtractValue _newparam "NewEnumerator0" (Variables|Default|GetDamage_0))
      (Variables|Default|SetValue _value)
      (if (>= (Variables|Default|GetValue) 1.0)
        (Camera|PlayWorldCameraShake "/Game/Proto/Main/Blueprint/BP_CameraShake.BP_CameraShake_C" (Transformation|GetActorLocation (Game|GetPlayerCharacter 0)) 0.0 4e+03)
        (Utilities|HitStop 0.05)
        (CallFunction|KnockBack (Variables|Default|GetDamage%20Causer))
        (Audio|PlaySoundatLocation "/Game/Proto/Main/SFX/SFXHADES/Player/Player_Hurt/EmoteHurt_5.EmoteHurt_5" (Transformation|GetActorLocation) "0, 0, 0" 0.2 1.0 0.0 0 0 0 0)
        (Utilities|FlowControl|Delay 0.2)
        (Variables|/Script/Engine.CharacterMovementComponent|SetGroundFriction (Variables|Character|GetCharacterMovement) 3.0)
        (Variables|Default|SetFirstLook true)
        (Variables|Default|SetisHit false)
        ;[1 1 1] Delay Invincible Frame
        (Utilities|FlowControl|Delay 0.02)
        (Collision|SetCollisionResponsetoChannel _capsulecomponent "ECC_GameTraceChannel4" "ECR_Block")
        (Collision|SetCollisionResponsetoChannel _capsulecomponent "ECC_GameTraceChannel5" "ECR_Block")
        (Variables|Default|SetbCanBeDamaged true)
        (Variables|Default|SetFirstLook true)
        (else
          (CallFunction|MortIA)
          (Variables|Default|SetAIDead false)
          (CallFunction|KnockBack (Variables|Default|GetDamage%20Causer))))
      (else
        (Variables|Default|SetAIDead true)
        (CallFunction|MortIA)))))

(event EventTick
  (params (DeltaSeconds :type Float%20%28single-precision%29))
  (bind _returnvalue (Game|GetPlayerCharacter 0))
  (bind _closestplayer (Variables|Default|GetClosestPlayer))
  (bind _capsulecomponent (Variables|/Script/Engine.Character|GetCapsuleComponent _returnvalue))
  ;[1 1 1] Look At Target Player and add movement input for strafing
  (if (Variables|Default|GetAIDead)
    (Actor|DestroyActor)
    (elif (Variables|Default|GetFirstLook)
      (if (Variables|Default|GetStrafing?) :!label _label
        (Utilities|IsValid _capsulecomponent
          (:Is%20Valid
            (Transformation|SetActorRotation (Math|Rotator|FindLookatRotation (Transformation|GetActorLocation) (Transformation|GetWorldLocation _capsulecomponent)))
            (Pawn|Input|AddMovementInput (CallFunction|WorldStrafingDirection) 1.0 false)
            (Utilities|FlowControl|Delay 0.02)
            (goto _label))))
      (else
        (if (Variables|Default|GetStrafing?) :!label _label_2
          (Utilities|IsValid _closestplayer
            (:Is%20Valid
              (Transformation|SetActorRotation (Math|Rotator|FindLookatRotation (Transformation|GetActorLocation) (Transformation|GetActorLocation _closestplayer)))
              (Pawn|Input|AddMovementInput (CallFunction|WorldStrafingDirection) 1.0 false)
              (Utilities|FlowControl|Delay 0.02)
              (goto _label_2))))))))

(event EventMovement
  (params (On%20/%20Off :type Boolean))
  (Variables|Default|SetMovementOn On%20/%20Off))

(event EventBeginPlay
  (Variables|Default|SetMaxWalkSpeed 6e+02)
  (Default|Initialise (CallFunction|GetHealthBarWidget0) self 1.0 (Variables|Default|GetPapillonMaxHP) -1 false false 0 "(R=0.500000,G=0.004823,B=0.000000,A=1.000000)" 0.0 1 false false true true -1.0 3e+03 "")
  ;[1 1 1] General Behavior Logic
  (Variables|/Script/AIModule.PawnSensingComponent|SetSightRadius (Variables|Default|GetPawnSensing) 6e+01)
  (if (Variables|Default|GetFirstLook)
    (CallFunction|PlayerIsSeen)
    (elif (not (Variables|Default|GetHasTarget))
      (CallFunction|ServerFindClosestPLayer)
      (Variables|Default|SetHasTarget true)
      (Variables|Default|SetFirstLook true)
      (if (Variables|Default|GetisHit)
        (Utilities|FlowControl|Delay 0.7)
        (Variables|Default|SetisHit false)
        (else
          (AI|AIMoveTo self (Transformation|GetWorldLocation (Variables|/Script/Engine.Character|GetMesh (Variables|Default|GetClosestPlayer))) (Variables|Default|GetClosestPlayer) 1e+03 true
            (:OnSuccess
              (if (Variables|Default|GetMustAttack)
                (AI|AIMoveTo self (Transformation|GetWorldLocation (Variables|/Script/Engine.Character|GetMesh (Variables|Default|GetClosestPlayer))) (Variables|Default|GetClosestPlayer) 6e+02 true :!label _label
                  (:OnSuccess
                    (CallFunction|ServerNPCMeleeAttack)
                    (Utilities|FlowControl|Delay 1.0)
                    (Variables|Default|SetMustAttack false)))
                (else
                  (switch int (Math|Random|RandomInteger 3)
                    (:0
                      (goto _label))
                    (:1
                      (Variables|Default|SetStrafingDirection "NewEnumerator0")
                      (Variables|Default|SetStrafing? true))
                    (:2
                      (Variables|Default|SetStrafingDirection "NewEnumerator1")
                      (Variables|Default|SetStrafing? true))
                    (:3
                      (Variables|Default|SetStrafingDirection "NewEnumerator2")
                      (Variables|Default|SetStrafing? true)))
                  (Utilities|FlowControl|Delay (Math|Random|RandomFloatinRange 0.5 1.5))
                  (Variables|Default|SetStrafing? false)
                  (Variables|Default|SetMustAttack true)))
              (Variables|Default|SetHasTarget false))))))))

(fn ConstructionScript
  (|CallParentFunction))

(fn WorldStrafingDirection
  (return "0, 0, 0"))

(fn GetHealthBarWidget0
  (bind _aswidget_floating_healthbar (Utilities|Casting|CastToWidget_FloatingHealthbar (UserInterface|GetUserWidgetObject (Variables|Default|GetWidget))))
  (return _aswidget_floating_healthbar))

(fn SpawnSpell
  (bind _spelldirection (Variables|Default|GetSpellDirection))
  (bind _returnvalue (Transformation|GetWorldTransform _spelldirection))
  (bind _returnvalue_2 (Game|SpawnActorfromClass "/Game/Proto/Proto_Florian/Blueprints/ProjPapillon.ProjPapillon_C" (Math|Transform|MakeTransform (.location _returnvalue) (.rotation _returnvalue) "0.300000,0.300000,0.300000") "AlwaysSpawn" self 0))
  (Physics|AddImpulse (Variables|/Game/Proto/Proto_Florian/Blueprints/ProjPapillon.ProjPapillon_C|GetBoule _returnvalue_2) (* (Math|Vector|GetForwardVector _spelldirection) 1e+03) "None" false))

(fn PlayHighPriorityMontage
  (params (Montage :type Anim%20Montage%20Object%20Reference) (StartSectionName :type Name) (InPlayRate :type Float%20%28double-precision%29))
  (if (not (Animation|Montage|MontageIsPlaying (Components|SkeletalMesh|GetAnimInstance (Variables|Character|GetMesh)) Montage))
    (bind _output_get (Variables|Default|SetHighPriorityMontage Montage))
    (bind _returnvalue (Animation|PlayAnimMontage _output_get InPlayRate StartSectionName))
    (return _returnvalue)))

(fn KnockBack
  (params (HitActor :type Actor%20Object%20Reference))
  (Variables|Default|SetNewVar_0 (Transformation|GetActorForwardVector HitActor))
  (CallFunction|InvincibleFrame)
  (Character|LaunchCharacter (Math|Vector|MakeVector (* (.x (Variables|Default|GetNewVar_0)) 1.5e+03) (* (.y (Variables|Default|GetNewVar_0)) 1.5e+03) 0.0) false false))

(fn InvincibleFrame
  (bind _capsulecomponent (Variables|Default|GetCapsuleComponent))
  (bind _charactermovement (Variables|Character|GetCharacterMovement))
  (Collision|SetCollisionResponsetoChannel _capsulecomponent "ECC_GameTraceChannel4" "ECR_Ignore")
  (Collision|SetCollisionResponsetoChannel _capsulecomponent "ECC_GameTraceChannel5" "ECR_Ignore")
  (Variables|Default|SetbCanBeDamaged false)
  (Variables|/Script/Engine.CharacterMovementComponent|SetGroundFriction _charactermovement 0.0)
  (Variables|/Script/Engine.MovementComponent|SetVelocity _charactermovement "0, 0, 0"))