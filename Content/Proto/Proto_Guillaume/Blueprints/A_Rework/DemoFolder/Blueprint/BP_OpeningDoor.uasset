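; BP_OpeningDoor is a training-area door that slides its cube upward when activated.
; ActivateActor runs once: it reports the door's name and location to the game mode, destroys a referenced actor, then plays a timeline that lerps the cube's relative position.
; The construction script picks the cube's material from a systems-room flag or a combat-type selection, with no material assigned for Magic.
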(event EventActivateActor
  (Utilities|FlowControl|DoOnce false
    (:Completed
      (Class|IGameMode|ActorActivated(Message) (Game|GetGameMode) (Utilities|String|Append (Utilities|GetObjectName self) (Utilities|String|ToString(Vector) (Transformation|GetActorLocation))))
      (Actor|DestroyActor (Variables|Default|GetActor))
      (bind _newtrack_0 (Timeline|Move PlayFromStart)
        (:Update
          (Transformation|SetRelativeLocation (Variables|Default|GetCube1) (Math|Vector|Lerp(Vector) "0, 0, 0" "0.000000, 0,600.000000" _newtrack_0) false false))))))

(fn ConstructionScript
  (if (Variables|Default|GetSystemsRoom)
    (Rendering|Material|SetMaterial (Variables|Default|GetCube1) 0 "/Game/FlexibleCombatSystem/DemoFolder/Materials/MI_SystemsTraining.MI_SystemsTraining")
    (else
      (Rendering|Material|SetMaterial (Variables|Default|GetCube1) 0 (Utilities|Select :Index (Variables|Default|GetColour) :NewEnumerator0 "/Game/FlexibleCombatSystem/DemoFolder/Materials/MI_MeleeTraining.MI_MeleeTraining" :NewEnumerator1 "/Game/FlexibleCombatSystem/DemoFolder/Materials/MI_RangedTraining.MI_RangedTraining" :NewEnumerator2 0)))))