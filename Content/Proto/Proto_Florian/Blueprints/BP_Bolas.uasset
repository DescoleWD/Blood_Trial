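; Work-in-progress prototype bolas projectile that damages enemies and notifies the main character when it returns.
; On mesh hit, a debug-drawn pawn sphere trace finds enemies to attach and damage using BloodWaveDamage; misses or non-damageable hits attach and stop movement.
; Both outcomes schedule Return after a delay, calling BolasReturn and destroying the actor, but a BeginPlay timeout of equal length also destroys it.
; Overlap and special-attack explosion logic is disconnected.
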(event OnComponentHit(StaticMesh)
  (params (HitComponent :type Primitive%20Component%20Object%20Reference) (OtherActor :type Actor%20Object%20Reference) (OtherComp :type Primitive%20Component%20Object%20Reference) (NormalImpulse :type Vector :default "0, 0, 0") (Hit :type Hit%20Result%20Structure%20%28by%20ref%29))
  (bind _returnvalue (Transformation|GetWorldLocation HitComponent))
  (bind _defaultsceneroot (Variables|Default|GetDefaultSceneRoot))
  ;[1 0 0.005617] Work In progress
  (bind _outactors (Actor|GetAllActorswithTag "Player"))
  (bind (_outhit _returnvalue_2) (Collision|SphereTraceForObjects _returnvalue _returnvalue 5.0 (Utilities|Array|MakeArray "ObjectTypeQuery3") false _outactors "ForDuration"))
  (Development|PrintText (Utilities|Text|FormatText "BlockingHit={in1} 
returnValue={in2}  
InitialOverlap={in3} 
ImpactPoint={6} 
HitActor={10}" (.bBlockingHit (Collision|BreakHitResult _outhit)) _returnvalue_2 (.bInitialOverlap (Collision|BreakHitResult _outhit)) 0 (.HitActor (Collision|BreakHitResult _outhit))))
  ;;[1 0 0.113] Zone de merde
  (if _returnvalue_2
    (if (Variables|/Script/Engine.Actor|GetbCanBeDamaged (.HitActor (Collision|BreakHitResult _outhit)))
      (if (Actor|ActorHasTag (.HitActor (Collision|BreakHitResult _outhit)) "Ennemy")
        (Transformation|AttachComponentToComponent (.HitActor (Collision|BreakHitResult _outhit)) _defaultsceneroot "None" "KeepWorld" "KeepWorld" "KeepWorld" true)
        (Game|Damage|ApplyDamage (.HitActor (Collision|BreakHitResult _outhit)) (Variables|/Game/Proto/Main/Blueprint/BloodTrial_GameInstance.BloodTrial_GameInstance_C|GetBloodWave_Damage (CallFunction|GetInst)) 0 0)
        (Utilities|FlowControl|Delay 5.0)
        (CallFunction|Return))
      (else
        (Transformation|AttachComponentToComponent OtherComp _defaultsceneroot "None" "KeepWorld" "KeepWorld" "KeepWorld" true :!label _label)
        (Components|Movement|StopMovementImmediately (Variables|Default|GetProjectileMovement))
        (Utilities|FlowControl|Delay 5.0)
        (CallFunction|Return)))
    (else
      (goto _label))))

(event OnComponentBeginOverlap(Sphere)
  (params (OverlappedComponent :type Primitive%20Component%20Object%20Reference) (OtherActor :type Actor%20Object%20Reference) (OtherComp :type Primitive%20Component%20Object%20Reference) (OtherBodyIndex :type Integer) (bFromSweep :type Boolean) (SweepResult :type Hit%20Result%20Structure%20%28by%20ref%29))
  ;[1 0 0.005617] Work In progress
)

(event Custom|Explosion
  ;[1 0 0.005617] Work In progress
  (Audio|PlaySound2D "/Game/StarterContent/Audio/Collapse01.Collapse01" 1.0 1.0 0.0 0 0))

(event Custom|Return
  ;[1 0 0.005617] Work In progress
  (bind _asbp_main_character (Utilities|Casting|CastToBP_MainCharacter (Game|GetPlayerCharacter 0)))
  (Components|MoveComponentTo (Variables|/Game/Proto/Main/Blueprint/BP_MainCharacter.BP_MainCharacter_C|GetSpawnBolas _asbp_main_character) (.location (Transformation|GetWorldTransform (Variables|/Game/Proto/Main/Blueprint/BP_MainCharacter.BP_MainCharacter_C|GetSpawnBolas _asbp_main_character))) (.rotation (Transformation|GetWorldTransform (Variables|/Game/Proto/Main/Blueprint/BP_MainCharacter.BP_MainCharacter_C|GetSpawnBolas _asbp_main_character))) false false 1.0 false)
  (bind _asbp_main_character_2 (Utilities|Casting|CastToBP_MainCharacter (Game|GetPlayerCharacter 0)))
  (Default|BolasReturn _asbp_main_character_2)
  (Actor|DestroyActor))

(event EventBeginPlay
  ;[1 0 0.005617] Work In progress
  (Utilities|FlowControl|Delay 5.0)
  (Actor|DestroyActor))

(fn ConstructionScript)