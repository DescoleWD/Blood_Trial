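; TestPoint is a prototype collectible that awards points to the player character.
; On BeginPlay, two chained MoveComponentTo calls loop endlessly, swinging the static mesh through a half turn and back.
; When BP_MainCharacter overlaps the sphere, the pickup destroys itself, adds StarPoint to that character's Score and plays the Secret sound.
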(event OnComponentBeginOverlap(Sphere)
  (params (OverlappedComponent :type Primitive%20Component%20Object%20Reference) (OtherActor :type Actor%20Object%20Reference) (OtherComp :type Primitive%20Component%20Object%20Reference) (OtherBodyIndex :type Integer) (bFromSweep :type Boolean) (SweepResult :type Hit%20Result%20Structure%20%28by%20ref%29))
  (bind _asbp_florian_character (Utilities|Casting|CastToBP_MainCharacter OtherActor))
  (Actor|DestroyActor)
  (Variables|/Game/Proto/Main/Blueprint/BP_MainCharacter.BP_MainCharacter_C|SetScore _asbp_florian_character (+ (Variables|Default|GetStarPoint) (Variables|/Game/Proto/Main/Blueprint/BP_MainCharacter.BP_MainCharacter_C|GetScore _asbp_florian_character)))
  (Audio|PlaySound2D "/Game/Proto/Proto_Florian/SFX/Secret.Secret" 1.0 1.0 0.0 0 0))

(event EventBeginPlay
  (Components|MoveComponentTo (Variables|Default|GetStaticMesh) "0, 0, 0" "0,180.000000, 0" false false 5.0 false :!label _label)
  (Components|MoveComponentTo (Variables|Default|GetStaticMesh) "0, 0, 0" "0, 0, 0" false false 5.0 false)
  (goto _label))

(fn ConstructionScript)