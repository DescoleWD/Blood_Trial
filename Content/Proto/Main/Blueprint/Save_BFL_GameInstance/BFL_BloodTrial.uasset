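; Blueprint function library for Blood Trial that reads and writes shared run state on BloodTrial_GameInstance through a GetInst cast helper.
; It covers score, calendar pieces, combos, difficulty-based max life, hazard damage, sacrifice-based player life and level-flag resets.
; Mid-level upgrade functions adjust combat stats and abilities, with some left unfinished.
; Warrior and Divine Rage temporarily change attack, dash cooldown and walk speed, each undone by a paired reset.
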(fn GetScore
  (return (Variables|/Game/Proto/Main/Blueprint/Save_BFL_GameInstance/BloodTrial_GameInstance.BloodTrial_GameInstance_C|GetScore (Inst|GetInst))))

(fn SetScore
  (bind _asblood_trial_game_instance (Inst|GetInst))
  (Variables|/Game/Proto/Main/Blueprint/Save_BFL_GameInstance/BloodTrial_GameInstance.BloodTrial_GameInstance_C|SetScore _asblood_trial_game_instance (Score|GetScore _asblood_trial_game_instance)))

(fn IncrScore
  (params (incValue :type Integer))
  (bind _asblood_trial_game_instance (Inst|GetInst))
  (bind _output_get (Variables|/Game/Proto/Main/Blueprint/Save_BFL_GameInstance/BloodTrial_GameInstance.BloodTrial_GameInstance_C|SetScore _asblood_trial_game_instance (+ (Score|GetScore _asblood_trial_game_instance) incValue)))
  (return _output_get))

(fn BacktoZero
  (bind _asblood_trial_game_instance (Inst|GetInst))
  (bind _score (Score|GetScore _asblood_trial_game_instance))
  (Score|IncrScore (- _score (* _score 2)) _asblood_trial_game_instance)
  (Variables|/Game/Proto/Main/Blueprint/Save_BFL_GameInstance/BloodTrial_GameInstance.BloodTrial_GameInstance_C|SetCalendar_Pieces _asblood_trial_game_instance 0)
  (Variables|/Game/Proto/Main/Blueprint/Save_BFL_GameInstance/BloodTrial_GameInstance.BloodTrial_GameInstance_C|SetGlobalTime _asblood_trial_game_instance 0.0)
  (Variables|/Game/Proto/Main/Blueprint/Save_BFL_GameInstance/BloodTrial_GameInstance.BloodTrial_GameInstance_C|SetTotalTime _asblood_trial_game_instance 0.0))

(fn ChooseLife
  (params (Difficulty_Button :type Float%20%28double-precision%29))
  (bind _asblood_trial_game_instance (Inst|GetInst))
  (bind _output_get (Variables|/Game/Proto/Main/Blueprint/Save_BFL_GameInstance/BloodTrial_GameInstance.BloodTrial_GameInstance_C|SetChoose_Life _asblood_trial_game_instance Difficulty_Button))
  (bind _maxhp_s (PlayerLife|SetMaxHP Difficulty_Button _asblood_trial_game_instance))
  (return _output_get _maxhp_s))

(fn SetMaxHP
  (params (MaxHP_E :type Float%20%28double-precision%29))
  (bind _output_get (Variables|/Game/Proto/Main/Blueprint/Save_BFL_GameInstance/BloodTrial_GameInstance.BloodTrial_GameInstance_C|SetMaxLife (Inst|GetInst) MaxHP_E))
  (return _output_get))

(fn GetNBCombo
  (return (Variables|/Game/Proto/Main/Blueprint/Save_BFL_GameInstance/BloodTrial_GameInstance.BloodTrial_GameInstance_C|GetNB_Combos (Inst|GetInst))))

(fn SetNBCombo
  (params (NB_Combos :type Integer))
  (Variables|/Game/Proto/Main/Blueprint/Save_BFL_GameInstance/BloodTrial_GameInstance.BloodTrial_GameInstance_C|SetNB_Combos (Inst|GetInst) NB_Combos))

(fn GetCalendarPieces
  (return (Variables|/Game/Proto/Main/Blueprint/Save_BFL_GameInstance/BloodTrial_GameInstance.BloodTrial_GameInstance_C|GetCalendar_Pieces (Inst|GetInst))))

(fn SetCalendarPieces
  (bind _asblood_trial_game_instance (Inst|GetInst))
  (Variables|/Game/Proto/Main/Blueprint/Save_BFL_GameInstance/BloodTrial_GameInstance.BloodTrial_GameInstance_C|SetCalendar_Pieces _asblood_trial_game_instance (Calendar|GetCalendarPieces _asblood_trial_game_instance)))

(fn IncrCalendarPieces
  (params (IncrValue :type Integer))
  (bind _asblood_trial_game_instance (Inst|GetInst))
  (bind _output_get (Variables|/Game/Proto/Main/Blueprint/Save_BFL_GameInstance/BloodTrial_GameInstance.BloodTrial_GameInstance_C|SetCalendar_Pieces _asblood_trial_game_instance (+ (Calendar|GetCalendarPieces _asblood_trial_game_instance) 1)))
  (return _output_get))

(fn SetEnviroDamage
  (params (Spike_Damage :type Float%20%28double-precision%29))
  (Variables|/Game/Proto/Main/Blueprint/Save_BFL_GameInstance/BloodTrial_GameInstance.BloodTrial_GameInstance_C|SetEnviroDamage (Inst|GetInst) (* Spike_Damage 0.15)))

(fn SetLavaDamage
  (params (Lava_Damage :type Float%20%28double-precision%29))
  (Variables|/Game/Proto/Main/Blueprint/Save_BFL_GameInstance/BloodTrial_GameInstance.BloodTrial_GameInstance_C|SetLavaDamage (Inst|GetInst) 1e+01))

(fn GetPLayerLife
  (params (Basic_HP :type Float%20%28double-precision%29))
  (bind _asblood_trial_game_instance (Inst|GetInst))
  (bind _asblood_trial_game_instance_2 (Inst|GetInst))
  (bind _asblood_trial_game_instance_3 (Inst|GetInst))
  (bind _asblood_trial_game_instance_4 (Inst|GetInst))
  (bind _asblood_trial_game_instance_5 (Inst|GetInst))
  (Variables|/Game/Proto/Main/Blueprint/Save_BFL_GameInstance/BloodTrial_GameInstance.BloodTrial_GameInstance_C|SetPlayer_Life (Inst|GetInst) Basic_HP)
  (if (Variables|/Game/Proto/Main/Blueprint/Save_BFL_GameInstance/BloodTrial_GameInstance.BloodTrial_GameInstance_C|GetSacrifice_0_Neutre (Inst|GetInst))
    (return 3e+02 (Variables|/Game/Proto/Main/Blueprint/Save_BFL_GameInstance/BloodTrial_GameInstance.BloodTrial_GameInstance_C|GetPL_S0 _asblood_trial_game_instance_3))
    (elif (and (Variables|/Game/Proto/Main/Blueprint/Save_BFL_GameInstance/BloodTrial_GameInstance.BloodTrial_GameInstance_C|GetSacrifice_0_Neutre _asblood_trial_game_instance_4) (Variables|/Game/Proto/Main/Blueprint/Save_BFL_GameInstance/BloodTrial_GameInstance.BloodTrial_GameInstance_C|GetSacrifice_1_BolasExplosion _asblood_trial_game_instance_4))
      (return 2.5e+02 (Variables|/Game/Proto/Main/Blueprint/Save_BFL_GameInstance/BloodTrial_GameInstance.BloodTrial_GameInstance_C|GetPL_S1 _asblood_trial_game_instance_3))
      (elif (Math|Boolean|ANDBoolean (Variables|/Game/Proto/Main/Blueprint/Save_BFL_GameInstance/BloodTrial_GameInstance.BloodTrial_GameInstance_C|GetSacrifice_0_Neutre _asblood_trial_game_instance_5) (Variables|/Game/Proto/Main/Blueprint/Save_BFL_GameInstance/BloodTrial_GameInstance.BloodTrial_GameInstance_C|GetSacrifice_1_BolasExplosion _asblood_trial_game_instance_5) (Variables|/Game/Proto/Main/Blueprint/Save_BFL_GameInstance/BloodTrial_GameInstance.BloodTrial_GameInstance_C|GetSacrifice_2_BloodWave _asblood_trial_game_instance_5))
        (return 2e+02 (Variables|/Game/Proto/Main/Blueprint/Save_BFL_GameInstance/BloodTrial_GameInstance.BloodTrial_GameInstance_C|GetPL_S2 _asblood_trial_game_instance_3))
        (elif (Math|Boolean|ANDBoolean (Variables|/Game/Proto/Main/Blueprint/Save_BFL_GameInstance/BloodTrial_GameInstance.BloodTrial_GameInstance_C|GetSacrifice_0_Neutre _asblood_trial_game_instance_2) (Variables|/Game/Proto/Main/Blueprint/Save_BFL_GameInstance/BloodTrial_GameInstance.BloodTrial_GameInstance_C|GetSacrifice_1_BolasExplosion _asblood_trial_game_instance_2) (Variables|/Game/Proto/Main/Blueprint/Save_BFL_GameInstance/BloodTrial_GameInstance.BloodTrial_GameInstance_C|GetSacrifice_2_BloodWave _asblood_trial_game_instance_2) (Variables|/Game/Proto/Main/Blueprint/Save_BFL_GameInstance/BloodTrial_GameInstance.BloodTrial_GameInstance_C|GetSacrifice_3_Hurricane _asblood_trial_game_instance_2))
          (return 1.5e+02 (Variables|/Game/Proto/Main/Blueprint/Save_BFL_GameInstance/BloodTrial_GameInstance.BloodTrial_GameInstance_C|GetPL_S3 _asblood_trial_game_instance_3))
          (elif (Math|Boolean|ANDBoolean (Variables|/Game/Proto/Main/Blueprint/Save_BFL_GameInstance/BloodTrial_GameInstance.BloodTrial_GameInstance_C|GetSacrifice_0_Neutre _asblood_trial_game_instance) (Variables|/Game/Proto/Main/Blueprint/Save_BFL_GameInstance/BloodTrial_GameInstance.BloodTrial_GameInstance_C|GetSacrifice_1_BolasExplosion _asblood_trial_game_instance) (Variables|/Game/Proto/Main/Blueprint/Save_BFL_GameInstance/BloodTrial_GameInstance.BloodTrial_GameInstance_C|GetSacrifice_2_BloodWave _asblood_trial_game_instance) (Variables|/Game/Proto/Main/Blueprint/Save_BFL_GameInstance/BloodTrial_GameInstance.BloodTrial_GameInstance_C|GetSacrifice_3_Hurricane _asblood_trial_game_instance) (Variables|/Game/Proto/Main/Blueprint/Save_BFL_GameInstance/BloodTrial_GameInstance.BloodTrial_GameInstance_C|GetSacrifice_4_Vampirisme _asblood_trial_game_instance))
            (return 5e+01 (Variables|/Game/Proto/Main/Blueprint/Save_BFL_GameInstance/BloodTrial_GameInstance.BloodTrial_GameInstance_C|GetPL_S4 _asblood_trial_game_instance_3))))))))

(fn GetInst
  (return (.AsBlood%20Trial%20Game%20Instance (Utilities|Casting|CastToBloodTrial_GameInstance (Game|GetGameInstance)))))

(fn ResetBoolean
  (bind _asblood_trial_game_instance (Inst|GetInst))
  (Variables|/Game/Proto/Main/Blueprint/Save_BFL_GameInstance/BloodTrial_GameInstance.BloodTrial_GameInstance_C|SetInOut1 _asblood_trial_game_instance false)
  (Variables|/Game/Proto/Main/Blueprint/Save_BFL_GameInstance/BloodTrial_GameInstance.BloodTrial_GameInstance_C|SetInOut2 _asblood_trial_game_instance false)
  (Variables|/Game/Proto/Main/Blueprint/Save_BFL_GameInstance/BloodTrial_GameInstance.BloodTrial_GameInstance_C|SetInOut3 _asblood_trial_game_instance false)
  (Variables|/Game/Proto/Main/Blueprint/Save_BFL_GameInstance/BloodTrial_GameInstance.BloodTrial_GameInstance_C|SetRopeCut? _asblood_trial_game_instance false)
  (Variables|/Game/Proto/Main/Blueprint/Save_BFL_GameInstance/BloodTrial_GameInstance.BloodTrial_GameInstance_C|SetHaveKey? _asblood_trial_game_instance false)
  (Variables|/Game/Proto/Main/Blueprint/Save_BFL_GameInstance/BloodTrial_GameInstance.BloodTrial_GameInstance_C|SetCalendarObtain1 _asblood_trial_game_instance false)
  (Variables|/Game/Proto/Main/Blueprint/Save_BFL_GameInstance/BloodTrial_GameInstance.BloodTrial_GameInstance_C|SetCalendarObtain2 _asblood_trial_game_instance false)
  (Variables|/Game/Proto/Main/Blueprint/Save_BFL_GameInstance/BloodTrial_GameInstance.BloodTrial_GameInstance_C|SetCalendarObtain3 _asblood_trial_game_instance false)
  (Variables|/Game/Proto/Main/Blueprint/Save_BFL_GameInstance/BloodTrial_GameInstance.BloodTrial_GameInstance_C|SetCalendarObtain4 _asblood_trial_game_instance false)
  (Variables|/Game/Proto/Main/Blueprint/Save_BFL_GameInstance/BloodTrial_GameInstance.BloodTrial_GameInstance_C|SetCalendarObtain5 _asblood_trial_game_instance false)
  (Variables|/Game/Proto/Main/Blueprint/Save_BFL_GameInstance/BloodTrial_GameInstance.BloodTrial_GameInstance_C|SetCalendarObtain6 _asblood_trial_game_instance false)
  (Variables|/Game/Proto/Main/Blueprint/Save_BFL_GameInstance/BloodTrial_GameInstance.BloodTrial_GameInstance_C|SetEnemyZone1Done _asblood_trial_game_instance false)
  (Variables|/Game/Proto/Main/Blueprint/Save_BFL_GameInstance/BloodTrial_GameInstance.BloodTrial_GameInstance_C|SetEnemyZone2Done _asblood_trial_game_instance false)
  (Variables|/Game/Proto/Main/Blueprint/Save_BFL_GameInstance/BloodTrial_GameInstance.BloodTrial_GameInstance_C|SetEnemyZone3Done _asblood_trial_game_instance false)
  (Variables|/Game/Proto/Main/Blueprint/Save_BFL_GameInstance/BloodTrial_GameInstance.BloodTrial_GameInstance_C|SetEnemyZone4Done _asblood_trial_game_instance false)
  (Variables|/Game/Proto/Main/Blueprint/Save_BFL_GameInstance/BloodTrial_GameInstance.BloodTrial_GameInstance_C|SetEnemyZone5Done _asblood_trial_game_instance false)
  (Variables|/Game/Proto/Main/Blueprint/Save_BFL_GameInstance/BloodTrial_GameInstance.BloodTrial_GameInstance_C|SetEnemyZone6Done _asblood_trial_game_instance false)
  (Variables|/Game/Proto/Main/Blueprint/Save_BFL_GameInstance/BloodTrial_GameInstance.BloodTrial_GameInstance_C|SetEnemyZone7Done _asblood_trial_game_instance false)
  (Variables|/Game/Proto/Main/Blueprint/Save_BFL_GameInstance/BloodTrial_GameInstance.BloodTrial_GameInstance_C|SetEnemyZone8Done _asblood_trial_game_instance false)
  (Variables|/Game/Proto/Main/Blueprint/Save_BFL_GameInstance/BloodTrial_GameInstance.BloodTrial_GameInstance_C|SetEnemyZone9Done _asblood_trial_game_instance false)
  (Variables|/Game/Proto/Main/Blueprint/Save_BFL_GameInstance/BloodTrial_GameInstance.BloodTrial_GameInstance_C|SetWallDestroy? _asblood_trial_game_instance false)
  (return))

(fn GetPlayerLife0
  (bind _asblood_trial_game_instance (Inst|GetInst))
  (return (Variables|/Game/Proto/Main/Blueprint/Save_BFL_GameInstance/BloodTrial_GameInstance.BloodTrial_GameInstance_C|GetPL_S0 _asblood_trial_game_instance) (Variables|/Game/Proto/Main/Blueprint/Save_BFL_GameInstance/BloodTrial_GameInstance.BloodTrial_GameInstance_C|GetPL_S1 _asblood_trial_game_instance) (Variables|/Game/Proto/Main/Blueprint/Save_BFL_GameInstance/BloodTrial_GameInstance.BloodTrial_GameInstance_C|GetPL_S2 _asblood_trial_game_instance) (Variables|/Game/Proto/Main/Blueprint/Save_BFL_GameInstance/BloodTrial_GameInstance.BloodTrial_GameInstance_C|GetPL_S3 _asblood_trial_game_instance) (Variables|/Game/Proto/Main/Blueprint/Save_BFL_GameInstance/BloodTrial_GameInstance.BloodTrial_GameInstance_C|GetPL_S4 _asblood_trial_game_instance)))

(fn UpgradeMidLevel11
  (Variables|/Game/Proto/Main/Blueprint/Save_BFL_GameInstance/BloodTrial_GameInstance.BloodTrial_GameInstance_C|SetMaxDash (Inst|GetInst) 2))

(fn UpgradeMidLevel21
  (bind _asblood_trial_game_instance (Inst|GetInst))
  (Variables|/Game/Proto/Main/Blueprint/Save_BFL_GameInstance/BloodTrial_GameInstance.BloodTrial_GameInstance_C|SetBolasExplosion_Damage _asblood_trial_game_instance (* (Variables|/Game/Proto/Main/Blueprint/Save_BFL_GameInstance/BloodTrial_GameInstance.BloodTrial_GameInstance_C|GetBolasExplosion_Damage _asblood_trial_game_instance) 1.5)))

(fn UpgradeMidLevel31
  (bind _asblood_trial_game_instance (Inst|GetInst))
  (Variables|/Game/Proto/Main/Blueprint/Save_BFL_GameInstance/BloodTrial_GameInstance.BloodTrial_GameInstance_C|SetVampirisme_Value _asblood_trial_game_instance (+ (Variables|/Game/Proto/Main/Blueprint/Save_BFL_GameInstance/BloodTrial_GameInstance.BloodTrial_GameInstance_C|GetVampirisme_Value _asblood_trial_game_instance) 5.0)))

(fn UpgradeMidLevel12
  (Variables|/Game/Proto/Main/Blueprint/Save_BFL_GameInstance/BloodTrial_GameInstance.BloodTrial_GameInstance_C|SetNBCoup_Parable (Inst|GetInst) 4))

(fn UpgradeMidLevel13
  (bind _returnvalue (Actor|GetActorOfClass 0 "/Game/Proto/Proto_Guillaume/Blueprints/Player/Explosion.Explosion_C"))
  (Variables|/Game/Proto/Proto_Guillaume/Blueprints/Player/Explosion.Explosion_C|SetSphere%20Radius _returnvalue (+ (Variables|/Game/Proto/Proto_Guillaume/Blueprints/Player/Explosion.Explosion_C|GetSphere%20Radius _returnvalue) 1e+02)))

(fn UpgradeMidLevel14
  (bind _asblood_trial_game_instance (Inst|GetInst))
  (Variables|/Game/Proto/Main/Blueprint/Save_BFL_GameInstance/BloodTrial_GameInstance.BloodTrial_GameInstance_C|SetPlayerAttack _asblood_trial_game_instance (* (Variables|/Game/Proto/Main/Blueprint/Save_BFL_GameInstance/BloodTrial_GameInstance.BloodTrial_GameInstance_C|GetPlayerAttack _asblood_trial_game_instance) 1.5)))

(fn UpgradeMidLevel22
  (bind _asblood_trial_game_instance (Inst|GetInst))
  ;[1 1 1] Need patch
  (Variables|/Game/Proto/Main/Blueprint/Save_BFL_GameInstance/BloodTrial_GameInstance.BloodTrial_GameInstance_C|SetBolasExplosion_Damage _asblood_trial_game_instance (- (Variables|/Game/Proto/Main/Blueprint/Save_BFL_GameInstance/BloodTrial_GameInstance.BloodTrial_GameInstance_C|GetCD_Bolas _asblood_trial_game_instance) 0.0))
  (Development|PrintString 0 "Capacité pas encore finie !" true true "(R=1.000000,G=0.013690,B=0.000000,A=1.000000)" 22.0))

(fn UpgradeMidLevel23
  (bind _asblood_trial_game_instance (Inst|GetInst))
  (Variables|/Game/Proto/Main/Blueprint/Save_BFL_GameInstance/BloodTrial_GameInstance.BloodTrial_GameInstance_C|SetBloodWave_Damage _asblood_trial_game_instance (* (Variables|/Game/Proto/Main/Blueprint/Save_BFL_GameInstance/BloodTrial_GameInstance.BloodTrial_GameInstance_C|GetBloodWave_Damage _asblood_trial_game_instance) 1.5)))

(fn UpgradeMidLevel24
  (bind _asblood_trial_game_instance (Inst|GetInst))
  (Variables|/Game/Proto/Main/Blueprint/Save_BFL_GameInstance/BloodTrial_GameInstance.BloodTrial_GameInstance_C|SetPlayerAttack _asblood_trial_game_instance (* (Variables|/Game/Proto/Main/Blueprint/Save_BFL_GameInstance/BloodTrial_GameInstance.BloodTrial_GameInstance_C|GetPlayerAttack _asblood_trial_game_instance) 1.5)))

(fn UpgradeMidLevel32
  (Variables|/Game/Proto/Main/Blueprint/Save_BFL_GameInstance/BloodTrial_GameInstance.BloodTrial_GameInstance_C|SetUpdate_3_2 (Inst|GetInst) true))

(fn UpgradeMidLevel33
  (bind _asblood_trial_game_instance (Inst|GetInst))
  (Variables|/Game/Proto/Main/Blueprint/Save_BFL_GameInstance/BloodTrial_GameInstance.BloodTrial_GameInstance_C|SetHurricane_Damage _asblood_trial_game_instance (Variables|/Game/Proto/Main/Blueprint/Save_BFL_GameInstance/BloodTrial_GameInstance.BloodTrial_GameInstance_C|GetHurricane_Damage _asblood_trial_game_instance)))

(fn UpgradeMidLevel34
  (bind _asblood_trial_game_instance (Inst|GetInst))
  (Variables|/Game/Proto/Main/Blueprint/Save_BFL_GameInstance/BloodTrial_GameInstance.BloodTrial_GameInstance_C|SetPlayerAttack _asblood_trial_game_instance (* (Variables|/Game/Proto/Main/Blueprint/Save_BFL_GameInstance/BloodTrial_GameInstance.BloodTrial_GameInstance_C|GetPlayerAttack _asblood_trial_game_instance) 1.5)))

(fn RageGuerriere
  (bind _asblood_trial_game_instance (Inst|GetInst))
  (Variables|/Game/Proto/Main/Blueprint/Save_BFL_GameInstance/BloodTrial_GameInstance.BloodTrial_GameInstance_C|SetPlayerAttack _asblood_trial_game_instance (* (Variables|/Game/Proto/Main/Blueprint/Save_BFL_GameInstance/BloodTrial_GameInstance.BloodTrial_GameInstance_C|GetPlayerAttack _asblood_trial_game_instance) 1.5))
  (Variables|/Game/Proto/Main/Blueprint/Save_BFL_GameInstance/BloodTrial_GameInstance.BloodTrial_GameInstance_C|SetCD_Dash _asblood_trial_game_instance 0.5)
  (Variables|/Script/Engine.CharacterMovementComponent|SetMaxWalkSpeed (Variables|/Script/Engine.Character|GetCharacterMovement (Game|GetPlayerCharacter 0)) 1e+03)
  (Variables|/Game/Proto/Main/Blueprint/Save_BFL_GameInstance/BloodTrial_GameInstance.BloodTrial_GameInstance_C|SetRage_Guerriere _asblood_trial_game_instance true))

(fn RageGuerriereReset
  (bind _asblood_trial_game_instance (Inst|GetInst))
  (Variables|/Game/Proto/Main/Blueprint/Save_BFL_GameInstance/BloodTrial_GameInstance.BloodTrial_GameInstance_C|SetPlayerAttack _asblood_trial_game_instance (/ (Variables|/Game/Proto/Main/Blueprint/Save_BFL_GameInstance/BloodTrial_GameInstance.BloodTrial_GameInstance_C|GetPlayerAttack _asblood_trial_game_instance) 1.5))
  (Variables|/Game/Proto/Main/Blueprint/Save_BFL_GameInstance/BloodTrial_GameInstance.BloodTrial_GameInstance_C|SetCD_Dash _asblood_trial_game_instance 1.0)
  (Variables|/Script/Engine.CharacterMovementComponent|SetMaxWalkSpeed (Variables|/Script/Engine.Character|GetCharacterMovement (Game|GetPlayerCharacter 0)) 8e+02)
  (Variables|/Game/Proto/Main/Blueprint/Save_BFL_GameInstance/BloodTrial_GameInstance.BloodTrial_GameInstance_C|SetRage_Guerriere _asblood_trial_game_instance false))

(fn RageDivine
  (bind _asblood_trial_game_instance (Inst|GetInst))
  (Variables|/Game/Proto/Main/Blueprint/Save_BFL_GameInstance/BloodTrial_GameInstance.BloodTrial_GameInstance_C|SetPlayerAttack _asblood_trial_game_instance (* (Variables|/Game/Proto/Main/Blueprint/Save_BFL_GameInstance/BloodTrial_GameInstance.BloodTrial_GameInstance_C|GetPlayerAttack _asblood_trial_game_instance) 4.0))
  (Variables|/Game/Proto/Main/Blueprint/Save_BFL_GameInstance/BloodTrial_GameInstance.BloodTrial_GameInstance_C|SetCD_Dash _asblood_trial_game_instance 0.5)
  (Variables|/Script/Engine.CharacterMovementComponent|SetMaxWalkSpeed (Variables|/Script/Engine.Character|GetCharacterMovement (Game|GetPlayerCharacter 0)) 1.1e+03)
  (Variables|/Game/Proto/Main/Blueprint/Save_BFL_GameInstance/BloodTrial_GameInstance.BloodTrial_GameInstance_C|SetRage_DIvine _asblood_trial_game_instance true))

(fn RageDivineReset
  (bind _asblood_trial_game_instance (Inst|GetInst))
  (Variables|/Game/Proto/Main/Blueprint/Save_BFL_GameInstance/BloodTrial_GameInstance.BloodTrial_GameInstance_C|SetPlayerAttack _asblood_trial_game_instance (/ (Variables|/Game/Proto/Main/Blueprint/Save_BFL_GameInstance/BloodTrial_GameInstance.BloodTrial_GameInstance_C|GetPlayerAttack _asblood_trial_game_instance) 4.0))
  (Variables|/Game/Proto/Main/Blueprint/Save_BFL_GameInstance/BloodTrial_GameInstance.BloodTrial_GameInstance_C|SetCD_Dash _asblood_trial_game_instance 1.0)
  (Variables|/Script/Engine.CharacterMovementComponent|SetMaxWalkSpeed (Variables|/Script/Engine.Character|GetCharacterMovement (Game|GetPlayerCharacter 0)) 8e+02)
  (Variables|/Game/Proto/Main/Blueprint/Save_BFL_GameInstance/BloodTrial_GameInstance.BloodTrial_GameInstance_C|SetRage_DIvine _asblood_trial_game_instance false))