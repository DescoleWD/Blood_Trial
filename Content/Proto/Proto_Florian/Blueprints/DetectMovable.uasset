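; Prototype platform actor that moves its StaticMesh while the player stands inside its Box trigger.
; On overlap by a Player-tagged BP_MainCharacter, it eases the mesh to PlatLocation2 with MoveComponentTo.
; When that character leaves, it waits briefly, then eases the mesh back to PlatLocation1.
; The Move event is an empty stub, and its only call is unreachable.
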(event OnComponentBeginOverlap(Box)
  (params (OverlappedComponent :type Primitive%20Component%20Object%20Reference) (OtherActor :type Actor%20Object%20Reference) (OtherComp :type Primitive%20Component%20Object%20Reference) (OtherBodyIndex :type Integer) (bFromSweep :type Boolean) (SweepResult :type Hit%20Result%20Structure%20%28by%20ref%29))
  (bind _asbp_florian_character (Utilities|Casting|CastToBP_MainCharacter OtherActor))
  (if (Actor|ActorHasTag _asbp_florian_character "Player")
    (Components|MoveComponentTo (Variables|Default|GetStaticMesh) (Variables|Default|GetPlatLocation2) "0, 0, 0" true true 2.0 false)))

(event OnComponentEndOverlap(Box)
  (params (OverlappedComponent :type Primitive%20Component%20Object%20Reference) (OtherActor :type Actor%20Object%20Reference) (OtherComp :type Primitive%20Component%20Object%20Reference) (OtherBodyIndex :type Integer))
  (bind _asbp_florian_character (Utilities|Casting|CastToBP_MainCharacter OtherActor))
  (if (Actor|ActorHasTag _asbp_florian_character "Player")
    (Utilities|FlowControl|Delay 0.5)
    (Components|MoveComponentTo (Variables|Default|GetStaticMesh) (Variables|Default|GetPlatLocation1) "0, 0, 0" true true 2.0 false)))

(event Custom|Move)

(fn ConstructionScript)