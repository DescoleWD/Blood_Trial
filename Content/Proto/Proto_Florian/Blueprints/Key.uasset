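; Key pickup Blueprint in a prototype, collected when the main character overlaps its sphere.
; On overlap it sets HaveKey on the DetectMovableKey actor found by class lookup, destroys itself, plays a 2D sound and adds KeyPoints to the character's Score.
; The class lookup flags only the first DetectMovableKey found in the level.
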(event OnComponentBeginOverlap(Sphere)
  (params (OverlappedComponent :type Primitive%20Component%20Object%20Reference) (OtherActor :type Actor%20Object%20Reference) (OtherComp :type Primitive%20Component%20Object%20Reference) (OtherBodyIndex :type Integer) (bFromSweep :type Boolean) (SweepResult :type Hit%20Result%20Structure%20%28by%20ref%29))
  (bind _asbp_florian_character (Utilities|Casting|CastToBP_MainCharacter OtherActor))
  (CallFunction|Touch)
  (Actor|DestroyActor)
  (Audio|PlaySound2D "/Game/Proto/Proto_Florian/SFX/Key.Key" 1.0 1.0 0.0 0 0)
  (Variables|/Game/Proto/Main/Blueprint/BP_MainCharacter.BP_MainCharacter_C|SetScore _asbp_florian_character (+ (Variables|/Game/Proto/Main/Blueprint/BP_MainCharacter.BP_MainCharacter_C|GetScore _asbp_florian_character) (Variables|Default|GetKeyPoints))))

(event Custom|Touch
  (bind _returnvalue (Actor|GetActorOfClass "/Game/Proto/Proto_Florian/Blueprints/DetectMovableKey.DetectMovableKey_C"))
  (Variables|/Game/Proto/Proto_Florian/Blueprints/DetectMovableKey.DetectMovableKey_C|SetHaveKey? _returnvalue true))

(fn ConstructionScript)