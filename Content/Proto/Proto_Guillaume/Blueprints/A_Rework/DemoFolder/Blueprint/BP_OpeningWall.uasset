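; BP_OpeningWall is a wall of two cubes that slide apart along local X when the actor is activated.
; ActivateActor runs through a DoOnce, reports the actor's name and location to the game mode, then plays the Move timeline to lerp both cubes outward.
; The construction script colors both cubes with a Systems training material or, failing that, a Melee, Ranged or Magic training material chosen by Colour.
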(event EventActivateActor
  (Utilities|FlowControl|DoOnce false
    (:Completed
      (Class|IGameMode|ActorActivated(Message) (Game|GetGameMode) (Utilities|String|Append (Utilities|GetObjectName self) (Utilities|String|ToString(Vector) (Transformation|GetActorLocation))))
      (bind _newtrack_0 (Timeline|Move PlayFromStart)
        (:Update
          (Transformation|SetRelativeLocation (Variables|Default|GetCube) (Math|Vector|Lerp(Vector) "510.000000, 0, 0" "700.000000, 0, 0" _newtrack_0) false false)
          (Transformation|SetRelativeLocation (Variables|Default|GetCube1) (Math|Vector|Lerp(Vector) "-510.000000, 0, 0" "-700.000000, 0, 0" _newtrack_0) false false))))))

(fn ConstructionScript
  (if (Variables|Default|GetSystemsTraining)
    (Rendering|Material|SetMaterial (Variables|Default|GetCube) 0 "/Game/FlexibleCombatSystem/DemoFolder/Materials/MI_SystemsTraining.MI_SystemsTraining")
    (else
      (Rendering|Material|SetMaterial (Variables|Default|GetCube) 0 (Utilities|Select :Index (Variables|Default|GetColour) :NewEnumerator0 "/Game/FlexibleCombatSystem/DemoFolder/Materials/MI_MeleeTraining.MI_MeleeTraining" :NewEnumerator1 "/Game/FlexibleCombatSystem/DemoFolder/Materials/MI_RangedTraining.MI_RangedTraining" :NewEnumerator2 "/Game/FlexibleCombatSystem/DemoFolder/Materials/MI_MagicTraining.MI_MagicTraining")))))