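; Arena gate actor that raises to let the player through and lowers to block passage, doubling as a one-time checkpoint.
; Activation opens the gate, resets the linked ArenaSpawner and, once, reports the actor's name and location to the game mode.
; The first opening also triggers a delayed checkpoint message and on-screen widget.
; Opening and closing toggle Blocker collision and play a timeline forward or in reverse to slide the gate vertically.
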(event Custom|OpenGates
  ;[1 1 1] Open/Close Gates
  (Utilities|FlowControl|Sequence
    (:then_0
      ;[1 1 1] Save Game Before First Arena
      (Utilities|FlowControl|DoOnce false
        (:Completed
          (Utilities|FlowControl|Delay 0.5)
          (Class|IGameMode|CheckpointReached(Message) (Game|GetGameMode) self)
          (bind _returnvalue (UserInterface|CreateWidget "/Game/FlexibleCombatSystem/Widgets/General/WB_CheckpointReached.WB_CheckpointReached_C"))
          (UserInterface|Viewport|AddtoViewport _returnvalue 0))))
    (:then_1
      (Collision|SetCollisionEnabled (Variables|Default|GetBlocker) "NoCollision")
      (bind _newtrack_0 (Timeline|OpenLeGate PlayFromStart)
        (:Update
          (Transformation|SetRelativeLocation (Variables|Default|GetScene) (Math|Vector|Lerp(Vector) "0, 0, 0" "0, 0,250.000000" _newtrack_0) false false))))))

(event Custom|CloseGates
  ;[1 1 1] Open/Close Gates
  (Collision|SetCollisionEnabled (Variables|Default|GetBlocker) "QueryAndPhysics")
  (bind _newtrack_0 (Timeline|OpenLeGate ReverseFromEnd)
    (:Update
      (Transformation|SetRelativeLocation (Variables|Default|GetScene) (Math|Vector|Lerp(Vector) "0, 0, 0" "0, 0,250.000000" _newtrack_0) false false))))

(event EventActivateActor
  ;[1 1 1] Open Gates & Save
  (CallFunction|OpenGates)
  (Default|ResetArena (Variables|Default|GetArenaSpawner))
  (Utilities|FlowControl|DoOnce false
    (:Completed
      (Class|IGameMode|ActorActivated(Message) (Game|GetGameMode) (Utilities|String|Append (Utilities|GetObjectName self) (Utilities|String|ToString(Vector) (Transformation|GetActorLocation)))))))

(fn ConstructionScript)