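; BP_ActivateActorParent is a prototype parent Blueprint for actors that restore their activated state from a save game.
; On BeginPlay it loads BP_SaveGame from slot "save1" and searches its ActivatedActors list for its own key.
; That key is the object name concatenated with the actor location, and a match calls ActivateActorMessage once.
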(event EventBeginPlay
  ;[1 1 1] Activates Actor If In Save
  (bind _returnvalue (SaveGame|LoadGamefromSlot "save1"))
  (bind _asbp_save_game (Utilities|Casting|CastToBP_SaveGame _returnvalue))
  (bind _array_element (Utilities|Array|ForEachLoopwithBreak (Variables|/Game/FlexibleCombatSystem/Blueprints/BP_SaveGame.BP_SaveGame_C|GetActivatedActors _asbp_save_game) :!label _label)
    (:LoopBody
      (if (Utilities|Enum|Equal(Enum) _array_element (Utilities|String|Append (Utilities|GetObjectName self) (Utilities|String|ToString(Vector) (Transformation|GetActorLocation))))
        (Class|IItemInterface|ActivateActor(Message) self)
        (goto _label Break)))))

(fn ConstructionScript)