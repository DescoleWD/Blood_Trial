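; Quest component for NPCs that act as quest giver, receiver or both, running quests from offer to hand-in or abandon.
; It loads each numbered quest from DT_QuestInfo, restores state from the save game and opens WB_Quest.
; A quest log dispatcher advances objectives by ID, while collect quests also check and clear inventory items.
; Giver and receiver components message each other, and marker meshes reflect progress and level or prerequisite conditions.
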(event Custom|Open%20Quest
  (params (ActorToActivate :type Actor%20Object%20Reference))
  ;[1 1 1] Offer Quest - Triggered From NPC when Dialogue Component Runs Quest
  (CallFunction|LoadQuest (Variables|Default|GetAllQuestsInfo) false)
  (CallFunction|CreateQuest (Variables|QuestStatus|GetQuestFinished) ActorToActivate))

(event Custom|AcceptQuest
  ;[1 1 1] Accept & Decline Quest
  ;;[1 1 1] Called From "WB_Quest" Tells Quest Giver Quest Accepted
  (CallFunction|QuestAdjustments) ; Checks If Quest Complete (Quest Item Already Owned)
  (Class|INPC|EndConversation(Message) (Variables|Default|GetNPC_Ref))
  (Variables|QuestStatus|SetQuestAccepted true)
  (CallFunction|UpdateQuestMesh)
  ;;[1 1 1] Quest Comp Will Be Saved
  (Class|IGameMode|QuestComponentSaving(Message) (Game|GetGameMode) (Components|GetOwner)))

(event Custom|QuestReceived
  (params (QuestInfo :type S%20Quest%20Info%20Structure) (Quest%20Giver :type Quest%20Component%20Object%20Reference))
  ;[1 1 1] Accept & Decline Quest
  ;;[1 1 1] Called From "WB_Quest" - Tells The Quest Receiver (hand in) that Quests Accepted
  (CallFunction|StoreQuest QuestInfo Quest%20Giver)
  (CallFunction|QuestAdjustments) ; Checks If Quest Complete (Quest Item Already Owned)
  (Variables|QuestStatus|SetQuestAccepted true)
  (CallFunction|UpdateQuestMesh)
  ;;[1 1 1] Quest Comp Will Be Saved
  (Class|IGameMode|QuestComponentSaving(Message) (Game|GetGameMode) (Components|GetOwner)))

(event Custom|QuestHandedInExternal
  ;[1 1 1] Hand In Quest
  ;;[1 1 1] Triggered From "EventQuestComplete" (above) - Tells The Quest Giver The Quests Been Handed In
  (Math|Integer|IncrementInt (Variables|QuestStatus|GetQuestNumber)
    (:%20%20
      (CallFunction|ResetValues)
      (CallFunction|LoadQuest (Variables|Default|GetAllQuestsInfo) false)
      (CallFunction|UpdateQuestMesh))))

(event Custom|DeclineQuest
  ;[1 1 1] Accept & Decline Quest
  ;;[1 1 1] Called From WB_Quest Decline Button
  (Class|INPC|EndConversation(Message) (Variables|Default|GetNPC_Ref)))

(event Custom|EventUpdateQuest
  (params (Quantity :type Integer))
  ;[1 1 1 1 29] Update & Complete Quest - Triggered From "CanQuestUpdateFunction" - When Quest Objective has been handled
  (if (not (== (Variables|QuestStatus|GetQuestStatus) (Variables|QuestStatus|GetQuestTotalStatus)))
    (Variables|QuestStatus|SetQuestStatus (+ Quantity (Variables|QuestStatus|GetQuestStatus)))
    (switch Utilities|FlowControl|Switch|SwitchonE_QuestType (Variables|QuestInfo|GetQuestType)
      (:NewEnumerator3
        (Variables|QuestStatus|SetQuestFinished true :!label _label)
        (Variables|QuestStatus|SetQuestCompleted true)
        (CallFunction|UpdateQuestMesh))
      (:NewEnumerator0
        (if (CallFunction|QuestStatusReached) :!label _label_2
          (goto _label)))
      (:NewEnumerator1
        (goto _label_2))
      (:NewEnumerator2
        (goto _label)))))

(event Custom|CloseConversation
  ;[1 1 1] Accept & Decline Quest
  ;;[1 1 1] Called From WB_Quest Decline Button
  (Class|INPC|EndConversation(Message) (Variables|Default|GetNPC_Ref)))

(event Custom|EventQuestComplete
  (params (QuestStorageInfo :type S%20Quest%20Storage%20Info%20Structure))
  (bind _questgiverref (Variables|QuestGiverType|GetQuestGiverRef))
  ;[1 1 1] Hand In Quest
  ;;[1 1 1] Triggered From WB_Quest When "Complete" Button Is Pressed
  (Variables|QuestStatus|SetQuestStatus 0)
  (Math|Integer|IncrementInt (Variables|QuestStatus|GetQuestNumber)
    (:%20%20
      (CallFunction|QuestComplete QuestStorageInfo)
      (Utilities|IsValid _questgiverref
        (:Is%20Valid
          (CallFunction|QuestHandedinExternal _questgiverref))
        (:Is%20Not%20Valid
          _))
      (Class|INPC|EndConversation(Message) (Variables|Default|GetNPC_Ref))
      (CallFunction|RemoveItemfromInventory)
      (CallFunction|LoadQuest (Variables|Default|GetAllQuestsInfo) false)
      (CallFunction|UpdateQuestMesh))))

(event Custom|AbandonQuest
  (bind _questreceivercomp (Variables|QuestGiverType|GetQuestReceiverComp))
  ;[1 1 1 1 29] Abandon Quest - Called from WB_Quest Abandon Button
  ;;[1 1 1] Handles Dialogue Line
  (Variables|QuestStatus|SetQuestAccepted false)
  (Variables|QuestStatus|SetQuestCompleted false)
  ;;[1 1 1] Handles Quest Widget Accept/Hand In
  (Variables|QuestStatus|SetQuestFinished false)
  (CallFunction|UpdateQuestMesh)
  ;;[1 1 1] Tells The Receiver Quest Abandoned
  (Utilities|IsValid _questreceivercomp
    (:Is%20Valid
      (CallFunction|AbandonQuest _questreceivercomp))))

(event Custom|SetupQuest
  (params (NPC_Ref :type BP%20NPC%20Parent%20Object%20Reference) (QuestInfo :type Array%20of%20S%20Quest%20Setup%20Structures))
  ;[1 1 1] Load Save Data
  (Variables|Default|SetNPC_Ref NPC_Ref)
  (CallFunction|Initialize)
  (CallFunction|LoadQuest QuestInfo true)
  (CallFunction|UpdateQuestMesh))

(fn CreateQuest
  (params (QuestFinished :type Boolean) (ActorToActivate :type Actor%20Object%20Reference))
  (bind _self self)
  (if QuestFinished
    _
    (else
      ;[1 1 1] If New Quest Retreive New ID (Used For Remove Q for QLog)
      (Variables|Default|SetQuestID (Variables|/Game/FlexibleCombatSystem/Widgets/NPC/WB_QuestLog.WB_QuestLog_C|GetQuestCounter (Variables|Default|GetWB%20Quest%20Log)))))
  (bind _returnvalue (UserInterface|CreateWidget "/Game/FlexibleCombatSystem/Widgets/NPC/WB_Quest.WB_Quest_C" 0 (Utilities|Select :Index (Variables|QuestGiverType|GetQuestGiverType) :NewEnumerator0 _self :NewEnumerator1 (Variables|QuestGiverType|GetQuestReceiverComp) :NewEnumerator2 _self) self QuestFinished ActorToActivate))
  (Default|UpdateQuest _returnvalue (Utilities|Struct|MakeS_QuestStorageInfo (Variables|QuestInfo|GetQuestInfo) self (Variables|Default|GetQuestID) false))
  (UserInterface|Viewport|AddtoViewport _returnvalue 0))

(fn QuestStatusReached
  (return (>= (Variables|QuestStatus|GetQuestStatus) (Variables|QuestStatus|GetQuestTotalStatus))))

(fn CanQuestUpdateFunction
  (params (Quest%20Objective%20ID :type Text) (Quest%20ID :type Integer) (Quantity :type Integer))
  ;[1 1 1] Run From Event Dispatcher - When "Quest Objective" Complete, Quest Log Sends Message To All Quest Components Checking if their Quest is Updated
  (if (Utilities|Enum|Equal(Enum) Quest%20Objective%20ID (.QuestID (Utilities|Struct|BreakS_QuestInfo (Variables|QuestInfo|GetQuestInfo))))
    (CallFunction|EventUpdateQuest Quantity)
    (Default|UpdateQuestStatus (Variables|Default|GetWB%20Quest%20Log) Quest%20ID)))

(fn QuestAdjustments
  (bind _questinfo (Variables|QuestInfo|GetQuestInfo))
  (bind _questtype (Utilities|Struct|BreakS_QuestInfo _questinfo))
  ;[1 1 1] Checks If Quest Already Complete
  (switch Utilities|FlowControl|Switch|SwitchonE_QuestGiverType (Variables|QuestGiverType|GetQuestGiverType)
    (:NewEnumerator0
      _)
    (:NewEnumerator2
      _))
  ;;[1 1 1] Does Player Already Have Quest Item
  (if (Utilities|Enum|Equal(Enum) _questtype "NewEnumerator0")
    (bind _inventorycomponent (Class|IPlayerController|PassInventoryComp(Message) (Game|GetPlayerController 0)))
    (bind _array_element (Utilities|Array|ForEachLoopwithBreak (Variables|/Game/FlexibleCombatSystem/Blueprints/Components/InventoryComponent.InventoryComponent_C|GetInventorySlots _inventorycomponent) :!label _label)
      (:LoopBody
        (if (Utilities|Enum|Equal(Enum) (CallFunction|GetQuestID (.ItemStructure (Utilities|Struct|BreakS_SlotInfo (Variables|/Game/FlexibleCombatSystem/Widgets/InventorySystem/WB_InventorySlot.WB_InventorySlot_C|GetSlotContents _array_element)))) (.QuestID (Utilities|Struct|BreakS_QuestInfo (Variables|QuestInfo|GetQuestInfo))))
          (Default|CheckQuestUpdate (Variables|Default|GetWB%20Quest%20Log) (Variables|Default|GetQuest%20ID) (.Quantity (Utilities|Struct|BreakS_SlotInfo (Variables|/Game/FlexibleCombatSystem/Widgets/InventorySystem/WB_InventorySlot.WB_InventorySlot_C|GetSlotContents _array_element))))
          (goto _label Break))))
    (else
      ;;[1 1 1] If Talk - Quest Finished
      (if (Utilities|Enum|Equal(Enum) _questtype "NewEnumerator4")
        (Variables|QuestStatus|SetQuestFinished true)
        (Variables|QuestStatus|SetQuestCompleted true)))))

(fn RemoveItemfromInventory
  (if (Utilities|Enum|Equal(Enum) (Variables|QuestInfo|GetQuestType) "NewEnumerator0")
    (bind _inventorycomponent (Class|IPlayerController|PassInventoryComp(Message) (Game|GetPlayerController 0)))
    (bind _array_element (Utilities|Array|ForEachLoopwithBreak (Variables|/Game/FlexibleCombatSystem/Blueprints/Components/InventoryComponent.InventoryComponent_C|GetInventorySlots _inventorycomponent))
      (:LoopBody
        (if (Utilities|Enum|Equal(Enum) (CallFunction|GetQuestID (.ItemStructure (Utilities|Struct|BreakS_SlotInfo (Variables|/Game/FlexibleCombatSystem/Widgets/InventorySystem/WB_InventorySlot.WB_InventorySlot_C|GetSlotContents _array_element)))) (.QuestID (Utilities|Struct|BreakS_QuestInfo (Variables|QuestInfo|GetQuestInfo))))
          (Default|ClearSlotDataGeneral _inventorycomponent (Variables|/Game/FlexibleCombatSystem/Widgets/InventorySystem/WB_InventorySlot.WB_InventorySlot_C|GetSlotContents _array_element))
          (Default|ClearSlot _array_element))))))

(fn Initialize
  (bind _hudref (Class|IPlayerController|PassHUDWB(Message) (Game|GetPlayerController 0)))
  (Variables|Default|SetWB%20Quest%20Log (Variables|/Game/FlexibleCombatSystem/Widgets/HUD/WB_HUD.WB_HUD_C|GetWB_QuestLog _hudref))
  (bind _equipmentcomp (Class|IPlayerController|PassEquipmentComp(Message) (Game|GetPlayerController 0)))
  (Variables|Default|SetEquipment%20Comp _equipmentcomp)
  (EventDispatchers|BindEventtoCanQuestUpdate (EventDispatchers|CreateEvent :!event CanQuestUpdateFunction))
  (bind _returnvalue (SaveGame|LoadGamefromSlot "save1"))
  (bind _asbp_save_game (Utilities|Casting|CastToBP_SaveGame _returnvalue))
  (for _array_element (Variables|/Game/FlexibleCombatSystem/Blueprints/BP_SaveGame.BP_SaveGame_C|GetQuestGiverStatus _asbp_save_game)
    (if (Utilities|Enum|Equal(Enum) (Utilities|GetObjectName (Components|GetOwner)) (.QuestGiverName (Utilities|Struct|BreakS_QuestSaveData _array_element)))
      (Variables|QuestStatus|SetQuestAccepted (.QuestAccepted (Utilities|Struct|BreakS_QuestSaveData _array_element)))
      (Variables|QuestStatus|SetQuestFinished (.QuestFinished (Utilities|Struct|BreakS_QuestSaveData _array_element)))
      (Variables|QuestStatus|SetQuestCompleted (.QuestCompleteDialogueVariable (Utilities|Struct|BreakS_QuestSaveData _array_element)))
      (Variables|QuestStatus|SetQuestNumber (.QuestNumber (Utilities|Struct|BreakS_QuestSaveData _array_element)))
      (Variables|QuestStatus|SetQuestStatus (.QuestStatus (Utilities|Struct|BreakS_QuestSaveData _array_element)))
      (Variables|Default|SetQuestID (.QuestID (Utilities|Struct|BreakS_QuestSaveData _array_element)))
      (Variables|QuestGiverType|SetQuestReceiverComp (.QuestReceiver (Utilities|Struct|BreakS_QuestSaveData _array_element)))
      (Variables|QuestGiverType|SetQuestGiverRef (.QuestGiver (Utilities|Struct|BreakS_QuestSaveData _array_element)))
      (Class|IGameMode|QuestComponentSaving(Message) (Game|GetGameMode) (Components|GetOwner))))
  (return))

(fn UpdateQuestMesh
  (bind _npc_ref (Variables|Default|GetNPC_Ref))
  (bind _npc_ref_2 (Variables|Default|GetNPC_Ref))
  (bind _npc_ref_3 (Variables|Default|GetNPC_Ref))
  (bind _npc_ref_4 (Variables|Default|GetNPC_Ref))
  (bind _npc_ref_5 (Variables|Default|GetNPC_Ref))
  (bind _questionmark (Variables|/Game/FlexibleCombatSystem/Blueprints/AI/BP_NPC_Parent.BP_NPC_Parent_C|GetQuestionmark _npc_ref))
  (bind _questionmark_2 (Variables|/Game/FlexibleCombatSystem/Blueprints/AI/BP_NPC_Parent.BP_NPC_Parent_C|GetQuestionmark _npc_ref_2))
  (bind _questionmark_3 (Variables|/Game/FlexibleCombatSystem/Blueprints/AI/BP_NPC_Parent.BP_NPC_Parent_C|GetQuestionmark _npc_ref_3))
  (bind _questionmark_4 (Variables|/Game/FlexibleCombatSystem/Blueprints/AI/BP_NPC_Parent.BP_NPC_Parent_C|GetQuestionmark _npc_ref_4))
  (bind _questionmark_5 (Variables|/Game/FlexibleCombatSystem/Blueprints/AI/BP_NPC_Parent.BP_NPC_Parent_C|GetQuestionmark _npc_ref_5))
  ;[1 1 1] Update Quest Mesh Based Upon Current Quest Status
  (CallFunction|CheckQuestCondition)
  (switch Utilities|FlowControl|Switch|SwitchonE_QuestGiverType (Variables|QuestGiverType|GetQuestGiverType)
    (:NewEnumerator0
      ;;[1 1 1] All Quests Complete
      (if (> (Variables|QuestStatus|GetQuestNumber) (Variables|QuestInfo|GetNumberOfQuests))
        (Development|SetHiddeninGame (Variables|/Game/FlexibleCombatSystem/Blueprints/AI/BP_NPC_Parent.BP_NPC_Parent_C|GetExclamationmark (Variables|Default|GetNPC_Ref)) true false)
        (Development|SetHiddeninGame (Variables|/Game/FlexibleCombatSystem/Blueprints/AI/BP_NPC_Parent.BP_NPC_Parent_C|GetQuestionmark (Variables|Default|GetNPC_Ref)) true false)
        (else
          ;;[1 1 1] Quest Ready For Hand In
          (if (Variables|QuestStatus|GetQuestFinished)
            (Development|SetHiddeninGame (Variables|/Game/FlexibleCombatSystem/Blueprints/AI/BP_NPC_Parent.BP_NPC_Parent_C|GetExclamationmark (Variables|Default|GetNPC_Ref)) true false)
            (Development|SetHiddeninGame _questionmark_4 false false)
            (Rendering|Material|SetMaterial _questionmark_4 0 "/Game/FlexibleCombatSystem/Meshes/Materials/M_QuestComplete.M_QuestComplete")
            (else
              ;;[1 1 1] Quest Accepted
              (if (Variables|QuestStatus|GetQuestAccepted)
                (Development|SetHiddeninGame (Variables|/Game/FlexibleCombatSystem/Blueprints/AI/BP_NPC_Parent.BP_NPC_Parent_C|GetExclamationmark (Variables|Default|GetNPC_Ref)) true false)
                (Development|SetHiddeninGame _questionmark_5 false false)
                (Rendering|Material|SetMaterial _questionmark_5 0 "/Game/FlexibleCombatSystem/Meshes/Materials/M_QuestIncomplete.M_QuestIncomplete")
                (else
                  ;;[1 1 1] IF Quest Available
                  (if (>= (Variables|QuestInfo|GetNumberOfQuests) (Variables|QuestStatus|GetQuestNumber))
                    (Development|SetHiddeninGame (Variables|/Game/FlexibleCombatSystem/Blueprints/AI/BP_NPC_Parent.BP_NPC_Parent_C|GetExclamationmark (Variables|Default|GetNPC_Ref)) false false)
                    (Development|SetHiddeninGame (Variables|/Game/FlexibleCombatSystem/Blueprints/AI/BP_NPC_Parent.BP_NPC_Parent_C|GetQuestionmark (Variables|Default|GetNPC_Ref)) true false)
                    (Rendering|Material|SetMaterial (Variables|/Game/FlexibleCombatSystem/Blueprints/AI/BP_NPC_Parent.BP_NPC_Parent_C|GetExclamationmark (Variables|Default|GetNPC_Ref)) 0 (select (Variables|Default|GetQuestConditionsMet) "/Game/FlexibleCombatSystem/Meshes/Materials/M_QuestComplete.M_QuestComplete" "/Game/FlexibleCombatSystem/Meshes/Materials/M_QuestIncomplete.M_QuestIncomplete"))
                    (else
                      (Development|SetHiddeninGame (Variables|/Game/FlexibleCombatSystem/Blueprints/AI/BP_NPC_Parent.BP_NPC_Parent_C|GetExclamationmark (Variables|Default|GetNPC_Ref)) true false))))))))))
    (:NewEnumerator1
      ;;[1 1 1] Quest Giver - Turn Off Mesh When Accepted
      (if (Variables|QuestStatus|GetQuestAccepted)
        (Development|SetHiddeninGame (Variables|/Game/FlexibleCombatSystem/Blueprints/AI/BP_NPC_Parent.BP_NPC_Parent_C|GetExclamationmark (Variables|Default|GetNPC_Ref)) true false)
        (Development|SetHiddeninGame _questionmark_2 true false)
        (Rendering|Material|SetMaterial _questionmark_2 0 "/Game/FlexibleCombatSystem/Meshes/Materials/M_QuestIncomplete.M_QuestIncomplete")
        (else
          (Development|SetHiddeninGame (Variables|/Game/FlexibleCombatSystem/Blueprints/AI/BP_NPC_Parent.BP_NPC_Parent_C|GetExclamationmark (Variables|Default|GetNPC_Ref)) false false)
          (Development|SetHiddeninGame (Variables|/Game/FlexibleCombatSystem/Blueprints/AI/BP_NPC_Parent.BP_NPC_Parent_C|GetQuestionmark (Variables|Default|GetNPC_Ref)) true false)
          (Rendering|Material|SetMaterial (Variables|/Game/FlexibleCombatSystem/Blueprints/AI/BP_NPC_Parent.BP_NPC_Parent_C|GetExclamationmark (Variables|Default|GetNPC_Ref)) 0 (select (Variables|Default|GetQuestConditionsMet) "/Game/FlexibleCombatSystem/Meshes/Materials/M_QuestComplete.M_QuestComplete" "/Game/FlexibleCombatSystem/Meshes/Materials/M_QuestIncomplete.M_QuestIncomplete")))))
    (:NewEnumerator2
      (if (Variables|QuestStatus|GetQuestFinished)
        (Development|SetHiddeninGame (Variables|/Game/FlexibleCombatSystem/Blueprints/AI/BP_NPC_Parent.BP_NPC_Parent_C|GetExclamationmark (Variables|Default|GetNPC_Ref)) true false)
        (Development|SetHiddeninGame _questionmark_3 false false)
        (Rendering|Material|SetMaterial _questionmark_3 0 "/Game/FlexibleCombatSystem/Meshes/Materials/M_QuestComplete.M_QuestComplete")
        (else
          ;;[1 1 1] Quest Giver - Turn Off Mesh When Accepted
          (if (Variables|QuestStatus|GetQuestAccepted)
            (Development|SetHiddeninGame (Variables|/Game/FlexibleCombatSystem/Blueprints/AI/BP_NPC_Parent.BP_NPC_Parent_C|GetExclamationmark (Variables|Default|GetNPC_Ref)) true false)
            (Development|SetHiddeninGame (Variables|/Game/FlexibleCombatSystem/Blueprints/AI/BP_NPC_Parent.BP_NPC_Parent_C|GetQuestionmark (Variables|Default|GetNPC_Ref)) false false)
            (else
              (Development|SetHiddeninGame (Variables|/Game/FlexibleCombatSystem/Blueprints/AI/BP_NPC_Parent.BP_NPC_Parent_C|GetExclamationmark (Variables|Default|GetNPC_Ref)) true false)
              (Development|SetHiddeninGame _questionmark true false)
              (Rendering|Material|SetMaterial _questionmark 0 "/Game/FlexibleCombatSystem/Meshes/Materials/M_QuestIncomplete.M_QuestIncomplete"))))))))

(fn StoreQuest
  (params (QuestInfo :type S%20Quest%20Info%20Structure) (QuestGiver :type Quest%20Component%20Object%20Reference))
  ;[1 1 1] Comment
  (Variables|QuestGiverType|SetQuestGiverRef QuestGiver)
  (bind _output_get (Variables|QuestInfo|SetQuestInfo QuestInfo))
  (Variables|QuestInfo|SetQuestType (.QuestType (Utilities|Struct|BreakS_QuestInfo _output_get)))
  (Variables|QuestStatus|SetQuestTotalStatus (.QuestCollectionNumber (Utilities|Struct|BreakS_QuestInfo _output_get))))

(fn AddQuestComplete
  (params (QuestStorageInfo :type S%20Quest%20Storage%20Info%20Structure))
  (bind _quest_id (Variables|Default|GetQuest%20ID))
  (bind _hudref (Class|IPlayerController|PassHUDWB(Message) (Game|GetPlayerController 0)))
  (if (not (Utilities|Array|ContainsItem (Variables|/Game/FlexibleCombatSystem/Widgets/NPC/WB_QuestLog.WB_QuestLog_C|GetCompleteQuests (Variables|/Game/FlexibleCombatSystem/Widgets/HUD/WB_HUD.WB_HUD_C|GetWB_QuestLog _hudref)) _quest_id))
    (Utilities|Array|Add (Variables|/Game/FlexibleCombatSystem/Widgets/NPC/WB_QuestLog.WB_QuestLog_C|GetCompleteQuests (Variables|/Game/FlexibleCombatSystem/Widgets/HUD/WB_HUD.WB_HUD_C|GetWB_QuestLog _hudref)) _quest_id)
    (Default|QuestComplete (Variables|/Game/FlexibleCombatSystem/Widgets/HUD/WB_HUD.WB_HUD_C|GetWB_QuestLog _hudref) QuestStorageInfo)))

(fn LoadQuest
  (params (AllQuestsInfo :type Array%20of%20S%20Quest%20Setup%20Structures) (SetupQuests :type Boolean))
  ;[1 1 1] Sets up The Quest Variables Based Upon The Quest DT Info
  (if SetupQuests
    (Variables|Default|SetAllQuestsInfo AllQuestsInfo))
  (Variables|QuestInfo|SetNumberOfQuests (Utilities|Array|Length (Variables|Default|GetAllQuestsInfo)))
  (Variables|QuestGiverType|SetQuestGiverType (.questtype (Utilities|Array|Get(acopy) (Variables|Default|GetAllQuestsInfo) (- (Variables|QuestStatus|GetQuestNumber) 1))))
  (Utilities|IsValid (.questreceiverref (Utilities|Array|Get(acopy) (Variables|Default|GetAllQuestsInfo) (- (Variables|QuestStatus|GetQuestNumber) 1)))
    (:Is%20Valid
      (Variables|QuestGiverType|SetQuestReceiverComp (Actor|GetComponentbyClass (.questreceiverref (Utilities|Array|Get(acopy) (Variables|Default|GetAllQuestsInfo) (- (Variables|QuestStatus|GetQuestNumber) 1))) "QuestComponent_C")))
    (:Is%20Not%20Valid
      _))
  (bind _returnvalue (Utilities|GetDataTableRow "/Game/FlexibleCombatSystem/DataTables/DT_QuestInfo.DT_QuestInfo" (.questrowname (Utilities|Array|Get(acopy) (Variables|Default|GetAllQuestsInfo) (- (Variables|QuestStatus|GetQuestNumber) 1))))
    (:then
      (bind _output_get (Variables|QuestInfo|SetQuestInfo _returnvalue))
      (Variables|Default|SetQuest%20ID (.QuestID (Utilities|Struct|BreakS_QuestInfo _output_get)))
      (Variables|QuestInfo|SetQuestType (.QuestType (Utilities|Struct|BreakS_QuestInfo _output_get)))
      (Variables|QuestStatus|SetQuestTotalStatus (.QuestCollectionNumber (Utilities|Struct|BreakS_QuestInfo _output_get)))
      (Variables|Default|SetQuestConditions (.QuestConditions (Utilities|Struct|BreakS_QuestInfo _output_get))))))

(fn QuestComplete
  (params (QuestStorageInfo :type S%20Quest%20Storage%20Info%20Structure))
  (CallFunction|AddQuestComplete QuestStorageInfo)
  (Variables|QuestStatus|SetQuestAccepted false)
  (Variables|QuestStatus|SetQuestFinished false)
  ;[1 1 1] Used By Dialogue
  (Variables|QuestStatus|SetQuestCompleted true))

(fn CheckQuestCondition
  (bind _questconditions (Variables|Default|GetQuestConditions))
  ;[1 1 1] Update Quest Conditions
  (switch Utilities|FlowControl|Switch|SwitchonE_QuestConditions (Utilities|Struct|BreakS_QuestCondition (Variables|Default|GetQuestConditions))
    (:NewEnumerator0
      (Variables|Default|SetQuestConditionsMet true))
    (:NewEnumerator1
      (Variables|Default|SetQuestConditionsMet (>= (Variables|/Game/FlexibleCombatSystem/Blueprints/Components/EquipmentComponent.EquipmentComponent_C|GetCharacterLevel (Variables|Default|GetEquipment%20Comp)) (Utilities|Struct|BreakS_QuestCondition (Variables|Default|GetQuestConditions)))))
    (:NewEnumerator2
      (Variables|Default|SetQuestConditionsMet true)
      (bind _array_element (Utilities|Array|ForEachLoopwithBreak (Variables|/Game/FlexibleCombatSystem/Widgets/NPC/WB_QuestLog.WB_QuestLog_C|GetCompleteQuests (Variables|Default|GetWB%20Quest%20Log)) :!label _label)
        (:LoopBody
          (if (Utilities|Enum|Equal(Enum) _array_element (Utilities|Struct|BreakS_QuestCondition (Variables|Default|GetQuestConditions)))
            (Variables|Default|SetQuestConditionsMet true)
            (goto _label Break)))))
    (:NewEnumerator4
      (Variables|Default|SetQuestConditionsMet (and (Utilities|Array|ContainsItem (Variables|/Game/FlexibleCombatSystem/Widgets/NPC/WB_QuestLog.WB_QuestLog_C|GetCompleteQuests (Variables|Default|GetWB%20Quest%20Log)) (.QuestNameIFSet (Utilities|Struct|BreakS_QuestCondition _questconditions))) (>= (Variables|/Game/FlexibleCombatSystem/Blueprints/Components/EquipmentComponent.EquipmentComponent_C|GetCharacterLevel (Variables|Default|GetEquipment%20Comp)) (Utilities|Struct|BreakS_QuestCondition _questconditions)))))))

(fn GetQuestID
  (params (S_ItemData :type S%20Item%20Data%20Structure%20%28by%20ref%29))
  (bind _questinfo (Utilities|Struct|BreakS_ItemData S_ItemData))
  (bind _questitem (Utilities|Struct|BreakS_QuestData _questinfo))
  (bind (_datatable _rowname) (Utilities|Struct|BreakDataTableRowHandle _questitem))
  (Utilities|IsValid _datatable
    (:Is%20Valid
      (bind _returnvalue (Utilities|GetDataTableRow _datatable _rowname)
        (:then
          (return (.QuestID (Utilities|Struct|BreakS_QuestInfo _returnvalue))))))))

(fn ResetValues
  (Variables|QuestStatus|SetQuestAccepted false)
  (Variables|QuestStatus|SetQuestFinished false)
  ;[1 1 1] Used By Dialogue
  (Variables|QuestStatus|SetQuestCompleted true))