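; Player character Blueprint for a melee action game, with montage combos, dash, bolas, hurricane, life steal and checkpoint respawn.
; GameInstance holds health, timer, checkpoint and ability state, with Sacrifice flags gating dash, bolas detonation and hurricane.
; BeginPlay creates HUD widgets, starts the timer and a Delay-looped custom tick for the hurricane.
; Tick sphere-traces from camera to mesh, fading tagged walls via dynamic materials and an animated parameter-collection radius.
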(event Game|Damage|EventAnyDamage
  (params (Damage :type Float%20%28single-precision%29) (DamageType :type Damage%20Type%20Object%20Reference) (InstigatedBy :type Controller%20Object%20Reference) (DamageCauser :type Actor%20Object%20Reference))
  ;[0.2362 1 0] Code Globale
  ;;[0.5417 0 0.2769] Rework et diff origine damage
)

(event EventTick
  (params (DeltaSeconds :type Float%20%28single-precision%29))
  (bind _value (Variables|Default|GetValue))
  ;[0.01042 0.000728 0] ShaderCullingWall
  (bind _output_get (Variables|Default|SetPlayerPos (Transformation|GetWorldLocation (Variables|Character|GetMesh))))
  (bind _output_get_2 (Variables|Default|SetCamPos (Transformation|GetWorldLocation (Variables|Default|GetCamera))))
  (bind (_outhit _returnvalue) (Collision|SphereTraceByChannel _output_get_2 _output_get 2.5e+02 "TraceTypeQuery1" false 0 "None"))
  (if (and _returnvalue (Actor|ActorHasTag (.hitactor _outhit) "shaderEnable"))
    (bind _outhits (Collision|MultiSphereTraceByChannel (Variables|Default|GetCamPos) (Variables|Default|GetPlayerPos) (Math|Float|Clamp(Float) (Variables|Default|Getradius) 2.5e+02 (Variables|Default|Getradius)) "TraceTypeQuery3" false 0 "None" true "(R=1.000000,G=0.000000,B=0.000000,A=1.000000)" "(R=0.000000,G=1.000000,B=0.000000,A=1.000000)" 0.2))
    (for _array_element _outhits
      (if (Actor|ActorHasTag (.HitActor (Collision|BreakHitResult _array_element)) "shaderEnable")
        (if (== (Rendering|Material|GetNumMaterials (.HitComponent (Collision|BreakHitResult _array_element))) 1)
          (bind _returnvalue_2 (Rendering|Material|CreateDynamicMaterialInstance (.HitComponent (Collision|BreakHitResult _array_element)) 0 (Rendering|Material|GetMaterial (.HitComponent (Collision|BreakHitResult _array_element)) 0) "None" :!class /Script/Engine.PrimitiveComponent))
          (Rendering|Material|SetScalarParameterValue _returnvalue_2 "value" _value :!class /Script/Engine.MaterialInstanceDynamic)
          (bind _radiuscurv (Timeline|Timeline_3 Play)
            (:Update
              (bind _output_get_3 (Variables|Default|Setradius (* _radiuscurv 8e+02)))
              (Rendering|Material|SetScalarParameterValue "/Game/TA/Assets/Shader/MatrialFuction/ShaderCulling.ShaderCulling" "radius" _output_get_3 :!class /Script/Engine.KismetMaterialLibrary)))
          (else
            (for _index (range 0 1)
              (bind _returnvalue_3 (Rendering|Material|CreateDynamicMaterialInstance (.HitComponent (Collision|BreakHitResult _array_element)) _index (Rendering|Material|GetMaterial (.HitComponent (Collision|BreakHitResult _array_element)) _index) "None" :!class /Script/Engine.PrimitiveComponent))
              (Rendering|Material|SetScalarParameterValue _returnvalue_3 "value" _value :!class /Script/Engine.MaterialInstanceDynamic)
              (Timeline|Timeline_3 Play))))))
    (else
      (Timeline|Timeline_3 Reverse))))

(event Collision|EventActorBeginOverlap
  (params (OtherActor :type Actor%20Object%20Reference))
  ;[0.2362 1 0] Code Globale
  ;;[1 1 1] Create widget abilities + Timer + score
)

(event EventStartCustomTick
  ;[0.2362 1 0] Code Globale
  ;;[0.0107 1 0] Hurricane
  ;;;[1 0 0.07711] 5
  (CallFunction|EventTickCustom :!label _label)
  (Utilities|FlowControl|Delay 0.01)
  (goto _label))

(event EventEventTickCustom
  ;[0.2362 1 0] Code Globale
  ;;[0.0107 1 0] Hurricane
  (Utilities|IsValid (stale Input|ActionEvents|InputActionHurricane _returnvalue)
    (:Is%20Valid
      (Transformation|SetActorRelativeLocation (stale Input|ActionEvents|InputActionHurricane _returnvalue) (Math|Interpolation|VInterpTo (Transformation|GetActorLocation) (Transformation|GetActorLocation (Game|GetPlayerCharacter 0)) (Utilities|Time|GetWorldDeltaSeconds) 3e+02))
      (Utilities|FlowControl|Delay 2.0)
      (Actor|DestroyActor (stale Input|ActionEvents|InputActionHurricane _returnvalue))
      (Utilities|FlowControl|Delay 0.1)
      (Utilities|FlowControl|DoOnce false) ; enters at Reset
    )))

(event EventRespawn
  (bind _asblood_trial_game_instance (CallFunction|GetInst))
  (bind _check_rotation (Variables|/Game/Proto/Main/Blueprint/BloodTrial_GameInstance.BloodTrial_GameInstance_C|GetCheck_Rotation _asblood_trial_game_instance))
  ;[0.2362 1 0] Code Globale
  ;;[0 1 0.007329] Respawn
  (Input|DisableInput (Game|GetPlayerController 0))
  (Utilities|FlowControl|Delay 0.2)
  (Utilities|FlowControl|Delay 0.4)
  (Transformation|SetActorTransform (Math|Transform|MakeTransform (Variables|/Game/Proto/Main/Blueprint/BloodTrial_GameInstance.BloodTrial_GameInstance_C|GetCheck_Location _asblood_trial_game_instance) _check_rotation "1.000000,1.000000,1.000000"))
  (Pawn|SetControlRotation (Game|GetPlayerController 0) _check_rotation)
  (Pawn|Components|CharacterMovement|DisableMovement (Variables|Character|GetCharacterMovement))
  (Utilities|FlowControl|Delay 1.0)
  (Pawn|Components|CharacterMovement|SetMovementMode (Variables|Character|GetCharacterMovement) "MOVE_Walking" 0)
  (Input|EnableInput (Game|GetPlayerController 0)))

(event EventVampirisme
  (bind _asblood_trial_game_instance (CallFunction|GetInst))
  (bind _asblood_trial_game_instance_2 (CallFunction|GetInst))
  ;[0.2362 1 0] Code Globale
  ;;[0.08068 1 0] Vampirisme
  (if (<= (Variables|/Game/Proto/Main/Blueprint/BloodTrial_GameInstance.BloodTrial_GameInstance_C|GetChoose_Life _asblood_trial_game_instance) (Variables|/Game/Proto/Main/Blueprint/BloodTrial_GameInstance.BloodTrial_GameInstance_C|GetMaxLife _asblood_trial_game_instance))
    (Variables|/Game/Proto/Main/Blueprint/BloodTrial_GameInstance.BloodTrial_GameInstance_C|SetChoose_Life _asblood_trial_game_instance_2 (+ (Variables|/Game/Proto/Main/Blueprint/BloodTrial_GameInstance.BloodTrial_GameInstance_C|GetChoose_Life _asblood_trial_game_instance_2) 2.0))))

(event EventLockon
  (params (LockOn :type Boolean) (LockOnto :type Actor%20Object%20Reference))
  (bind _charactermovement (Variables|Character|GetCharacterMovement))
  ;[1 0 0.01425] Rework
  (if LockOn
    (Utilities|IsValid LockOnto
      (:Is%20Valid
        (Variables|Default|SetLock%20Onto LockOnto)
        (Variables|Default|SetLocked%20On false)
        (Variables|/Script/Engine.CharacterMovementComponent|SetbOrientRotationToMovement _charactermovement false)))
    (else
      (Variables|Default|SetLocked%20On true)
      (Variables|/Script/Engine.CharacterMovementComponent|SetbOrientRotationToMovement _charactermovement true))))

(event EventVampirismeonDeath
  (bind _asblood_trial_game_instance (CallFunction|GetInst))
  (bind _asblood_trial_game_instance_2 (CallFunction|GetInst))
  ;[0.2362 1 0] Code Globale
  ;;[0.08068 1 0] Vampirisme
  (if (<= (Variables|/Game/Proto/Main/Blueprint/BloodTrial_GameInstance.BloodTrial_GameInstance_C|GetChoose_Life _asblood_trial_game_instance) (Variables|/Game/Proto/Main/Blueprint/BloodTrial_GameInstance.BloodTrial_GameInstance_C|GetMaxLife _asblood_trial_game_instance))
    (Variables|/Game/Proto/Main/Blueprint/BloodTrial_GameInstance.BloodTrial_GameInstance_C|SetChoose_Life _asblood_trial_game_instance_2 (+ (Variables|/Game/Proto/Main/Blueprint/BloodTrial_GameInstance.BloodTrial_GameInstance_C|GetChoose_Life _asblood_trial_game_instance_2) 1e+02))))

(event EventDebugCamp
  ;[0.2362 1 0] Code Globale
)

(event EventTimelineTimer
  (bind _asblood_trial_game_instance (CallFunction|GetInst))
  ;[0.2362 1 0] Code Globale
  ;;[1 1 1] Create widget abilities + Timer + score
  ;;;[1 0.0313 0] 4
  (Variables|/Game/Proto/Main/Blueprint/BloodTrial_GameInstance.BloodTrial_GameInstance_C|SetTotalTime _asblood_trial_game_instance (+ (Variables|/Game/Proto/Main/Blueprint/BloodTrial_GameInstance.BloodTrial_GameInstance_C|GetGlobalTime _asblood_trial_game_instance) (Variables|/Game/Proto/Main/Blueprint/BloodTrial_GameInstance.BloodTrial_GameInstance_C|GetTotalTime _asblood_trial_game_instance)))
  (bind _newtrack_0 (Timeline|Timeline_2 Play)
    (:Update
      (Variables|/Game/Proto/Main/Blueprint/BloodTrial_GameInstance.BloodTrial_GameInstance_C|SetGlobalTime (CallFunction|GetInst) _newtrack_0))))

(event EventCreateScoreWidget
  ;[0.2362 1 0] Code Globale
  ;;[1 1 1] Create widget abilities + Timer + score
  ;;;[1 0.7891 0] 3
  (bind _returnvalue (UserInterface|CreateWidget "/Game/Proto/Main/HUD/Score.Score_C"))
  (UserInterface|Viewport|AddtoViewport _returnvalue 1)
  (bind _output_get (Variables|Default|SetAs_Score _returnvalue)))

(event EventCalendarReceived
  ;[0.2362 1 0] Code Globale
  ;;[1 1 1] Create widget abilities + Timer + score
  ;;;[1 0.7891 0] 3
  (Default|Collection (stale EventCreateScoreWidget _output_get)))

(event EventCreateAbilitiesWidget
  ;[0.2362 1 0] Code Globale
  ;;[1 1 1] Create widget abilities + Timer + score
  ;;;[0.173 1 0] 1
  (bind _returnvalue (UserInterface|CreateWidget "/Game/Proto/Main/HUD/Abilities.Abilities_C"))
  (UserInterface|Viewport|AddtoViewport _returnvalue 0))

(event EventCreateHPBarPlayerWidget
  ;[0.2362 1 0] Code Globale
  ;;[0.5417 0 0.2769] Rework et diff origine damage
  (bind _returnvalue (UserInterface|CreateWidget "/Game/Proto/Proto_Guillaume/Blueprints/Player/HP_Bar_Player.HP_Bar_Player_C" (Game|GetPlayerController 0)))
  (UserInterface|Viewport|AddtoViewport _returnvalue 0)
  (bind _output_get (Variables|Default|SetNewVar_0 _returnvalue)))

(event EventBeginPlay
  ;[0.2362 1 0] Code Globale
  ;;[1 1 1] Create widget abilities + Timer + score
  (Utilities|FlowControl|Sequence
    (:then_0
      ;;;[0 1 0.08258] 1
      (CallFunction|CreateAbilitiesWidget)
      ;;;[0.4924 1 0] 2
      (CallFunction|CreateHPBarPlayerWidget)
      ;;;[1 0.8181 0] 3
      (CallFunction|CreateScoreWidget))
    (:then_1
      ;;;[1 0 0.01027] 4
      (CallFunction|TimelineTimer))
    (:then_2
      ;;;;[1 0 0.1127] 5
      (CallFunction|StartCustomTick))
    (:then_3
      (CallFunction|DebugCamp))))

(event Input|ActionEvents|InputActionDash
  (params (Key :type Key%20Structure))
  (bind _asblood_trial_game_instance (CallFunction|GetInst))
  (bind _charactermovement (Variables|Character|GetCharacterMovement))
  (bind _returnvalue (Pawn|Components|PawnMovement|GetLastInputVector _charactermovement))
  (bind _returnvalue_2 (* _returnvalue 2.0))
  ;[1 0 0.7685] Dash + besoin anim / SFX/VFX
  (:Pressed
    (if (Variables|/Game/Proto/Main/Blueprint/BloodTrial_GameInstance.BloodTrial_GameInstance_C|GetSacrifice_1 _asblood_trial_game_instance)
      (if (< (Variables|/Game/Proto/Main/Blueprint/BloodTrial_GameInstance.BloodTrial_GameInstance_C|GetNB_Dash _asblood_trial_game_instance) (Variables|/Game/Proto/Main/Blueprint/BloodTrial_GameInstance.BloodTrial_GameInstance_C|GetMaxDash _asblood_trial_game_instance))
        (Collision|SetCollisionResponsetoChannel (Variables|Default|GetCapsuleComponent) "ECC_Pawn" "ECR_Ignore")
        (Variables|/Game/Proto/Main/Blueprint/BloodTrial_GameInstance.BloodTrial_GameInstance_C|SetNB_Dash _asblood_trial_game_instance (+ (Variables|/Game/Proto/Main/Blueprint/BloodTrial_GameInstance.BloodTrial_GameInstance_C|GetNB_Dash _asblood_trial_game_instance) 1))
        (Character|LaunchCharacter (Math|Vector|MakeVector (.x _returnvalue_2) (.y _returnvalue_2) 0.0) false false)
        (CallFunction|CheckUpHurricane)
        (Utilities|FlowControl|Delay 0.5)
        (Collision|SetCollisionResponsetoChannel (Variables|Default|GetCapsuleComponent) "ECC_WorldDynamic" "ECR_Block")
        (Collision|SetCollisionResponsetoChannel (Variables|Default|GetCapsuleComponent) "ECC_Pawn" "ECR_Block")
        (Utilities|FlowControl|Delay 1.0)
        (Variables|/Game/Proto/Main/Blueprint/BloodTrial_GameInstance.BloodTrial_GameInstance_C|SetNB_Dash (CallFunction|GetInst) 0)
        (Class|NavMovementComponent|StopMovementKeepPathing (Variables|Character|GetCharacterMovement))
        (else
          (Utilities|FlowControl|Delay 1.0)
          (Variables|/Game/Proto/Main/Blueprint/BloodTrial_GameInstance.BloodTrial_GameInstance_C|SetNB_Dash _asblood_trial_game_instance 0))))))

(event Input|ActionEvents|InputActionSpecialAttack
  (params (Key :type Key%20Structure))
  (bind _asblood_trial_game_instance (CallFunction|GetInst))
  (bind _sacrifice_2 (Variables|/Game/Proto/Main/Blueprint/BloodTrial_GameInstance.BloodTrial_GameInstance_C|GetSacrifice_2 _asblood_trial_game_instance))
  ;[1 0 0.01425] Rework
  ;;[1 0 0.5512] Bolas V2
  ;;;[0.1691 1 0] Step 1 : Action input Bolas
  (:Pressed
    ;;;[0.1949 1 0] Step 2 : Vérifier que le Bolas n'est pas déjà lancé
    (if (Variables|/Game/Proto/Main/Blueprint/BloodTrial_GameInstance.BloodTrial_GameInstance_C|GetThrowBolas _asblood_trial_game_instance)
      ;;;[0.1303 1 0] Step 3 : Si pas lancé ==> lancer le Bolas
      (Variables|/Game/Proto/Main/Blueprint/BloodTrial_GameInstance.BloodTrial_GameInstance_C|SetThrowBolas (CallFunction|GetInst) false)
      (CallFunction|ThrowBolas)
      (else
        ;;;[0.1856 1 0] Step 4 : Le bolas est il attaché ?
        (if (Variables|/Game/Proto/Main/Blueprint/BloodTrial_GameInstance.BloodTrial_GameInstance_C|GetBolas_Attache _asblood_trial_game_instance)
          ;;;[0.1565 1 0] Step 6 : Si attaché sur un ennemi, alors déclenché l'explosion
          (if _sacrifice_2
            (Utilities|FlowControl|Sequence
              (:then_0
                (bind _returnvalue (Actor|GetActorOfClass "/Game/Proto/Proto_Guillaume/Blueprints/Enemy/IA_V2/Distance/Distance.Distance_C"))
                (Default|ExplosionD _returnvalue))
              (:then_1
                (bind _returnvalue_2 (Actor|GetActorOfClass "/Game/Proto/Proto_Guillaume/Blueprints/Enemy/IA_V2/Melee/Melee.Melee_C"))
                (Default|ExplosionM _returnvalue_2))))
          (else
            ;;;[0.2834 1 0] Step 5 : Si pas attaché pas 2ème input alors le bolas explose
            (if _sacrifice_2
              (bind _returnvalue_3 (Actor|GetActorOfClass "/Game/Proto/Proto_Florian/Blueprints/BP_Bolas.BP_Bolas_C"))
              (Default|ExplosionSubtile _returnvalue_3))))))))

(event Input|ActionEvents|InputActionHurricane
  (params (Key :type Key%20Structure))
  ;[0.2362 1 0] Code Globale
  ;;[0.0107 1 0] Hurricane
  (:Pressed
    (if (Variables|/Game/Proto/Main/Blueprint/BloodTrial_GameInstance.BloodTrial_GameInstance_C|GetSacrifice_4 (CallFunction|GetInst))
      (Utilities|IsValid (stale _returnvalue)
        (:Is%20Not%20Valid
          (Utilities|FlowControl|DoOnce false :!label _label
            (:Completed
              (bind _returnvalue (Game|SpawnActorfromClass "/Game/Proto/Proto_Florian/Blueprints/BP_Hurricane.BP_Hurricane_C" (Math|Transform|MakeTransform (Transformation|GetWorldLocation (Variables|Default|GetSpawnHurricane)) (Class|CharacterMovementComponent|GetLastUpdateRotation (Variables|Character|GetCharacterMovement))) "Undefined" 0 0))
              (Transformation|SetActorRelativeLocation _returnvalue (Math|Interpolation|VInterpTo (Transformation|GetActorLocation) (Transformation|GetActorLocation (Game|GetPlayerCharacter 0)) (Utilities|Time|GetWorldDeltaSeconds) 3e+02))
              (Utilities|FlowControl|Delay 2.0)
              (Actor|DestroyActor _returnvalue)
              (Utilities|FlowControl|Delay 0.1)
              (goto _label Reset))))))))

(event Input|ActionEvents|InputActionParry
  (params (Key :type Key%20Structure))
  ;[1 0 0.01425] Rework
  ;;[1 0 0.75 0.396] Parade : PRBM il faut mettre l'animation sur le uper Body
)

(event Input|ActionEvents|InputActionBasicAttack
  (params (Key :type Key%20Structure))
  ;[1 0 0.01425] Rework
  ;;[1 0 0.828] Rajouter des anims pour les coup 2, 3 et 4 ?
  (:Pressed
    (CallFunction|CutwithAttack1)
    (CallFunction|CutwithAttack2)
    (Utilities|Attack)))

(event EventMovement
  (params (On%20/%20Off :type Boolean))
  (Variables|Default|SetMovementOn On%20/%20Off))

(event Input|AxisEvents|InputAxisMoveForward
  (params (AxisValue :type Float%20%28single-precision%29))
  ;[0.707 1 0] Character movement
  (if (>= (Math|Float|Absolute(Float) (* AxisValue 1e+01)) 1.0)
    (if (Variables|Default|GetMovementOn)
      (Pawn|Input|AddMovementInput (Class|PawnMovementComponent|GetPawnOwner (Variables|Character|GetCharacterMovement)) "1000.000000,-1000.000000, 0" AxisValue false))))

(event Input|AxisEvents|InputAxisMoveBackward
  (params (AxisValue :type Float%20%28single-precision%29))
  ;[0.707 1 0] Character movement
  (if (>= (Math|Float|Absolute(Float) (* AxisValue 1e+01)) 1.0)
    (if (Variables|Default|GetMovementOn)
      (Pawn|Input|AddMovementInput (Class|PawnMovementComponent|GetPawnOwner (Variables|Character|GetCharacterMovement)) "1000.000000,-1000.000000, 0" AxisValue false))))

(event Input|AxisEvents|InputAxisMoveLeft
  (params (AxisValue :type Float%20%28single-precision%29))
  ;[0.707 1 0] Character movement
  (if (>= (Math|Float|Absolute(Float) (* AxisValue 1e+01)) 1.0)
    (if (Variables|Default|GetMovementOn)
      (Pawn|Input|AddMovementInput (Class|PawnMovementComponent|GetPawnOwner (Variables|Character|GetCharacterMovement)) "1000.000000,1000.000000, 0" AxisValue false))))

(event Input|AxisEvents|InputAxisMoveRight
  (params (AxisValue :type Float%20%28single-precision%29))
  ;[0.707 1 0] Character movement
  (if (>= (Math|Float|Absolute(Float) (* AxisValue 1e+01)) 1.0)
    (if (Variables|Default|GetMovementOn)
      (Pawn|Input|AddMovementInput (Class|PawnMovementComponent|GetPawnOwner (Variables|Character|GetCharacterMovement)) "1000.000000,1000.000000, 0" AxisValue false))))

(fn ConstructionScript
  (|CallParentFunction))

(event EventCheckHit
  (bind _nearestenemy (Variables|Default|GetNearestEnemy))
  (Utilities|IsValid _nearestenemy
    (:Is%20Valid
      _)
    (:Is%20Not%20Valid
      (CallFunction|GetNearestEnemy)))
  (Utilities|IsValid _nearestenemy
    (:Is%20Valid
      (if (< (Math|Vector|VectorLength (- (Transformation|GetSocketLocation (Variables|Default|GetSword_Mesh) "CheckHitSocket") (Transformation|GetActorLocation _nearestenemy))) (Variables|Default|GetHitRange))
        (Audio|PlaySoundatLocation "/Engine/VREditor/Sounds/VR_ungrab.VR_ungrab" "0, 0, 0" "0, 0, 0" 1.0 1.0 0.0 0 0 0 0)
        (Class|BPInterfaceCharacterActions|OnHit(Message) (Variables|Default|GetNearestEnemy) self)))))

(event EventOnHit
  (params (ActorHited :type Actor%20Object%20Reference))
  (Animation|PlayAnimMontage "/Game/Proto/Proto_Guillaume/Blueprints/Anim_Mixamo/30FPS/MediumHitToHead_UE_Montage.MediumHitToHead_UE_Montage" 1.0 "None")
  (Utilities|ChangeHealth (Variables|/Game/Proto/Main/Blueprint/BloodTrial_GameInstance.BloodTrial_GameInstance_C|GetEnemyDamage_Melee (CallFunction|GetInst))
    (:True
      (Physics|AddImpulse (Variables|Character|GetCharacterMovement) (* (Transformation|GetActorForwardVector self) -8e+02) true)
      (Utilities|FlowControl|Delay 0.5)
      (Utilities|TurntoActor ActorHited))))

(event EventAttackSway
  (params (Strenght :type Float%20%28double-precision%29))
  (Physics|AddImpulse (Variables|Character|GetCharacterMovement) (* Strenght (Math|Vector|GetForwardVector (Variables|Default|GetCapsuleComponent))) true))