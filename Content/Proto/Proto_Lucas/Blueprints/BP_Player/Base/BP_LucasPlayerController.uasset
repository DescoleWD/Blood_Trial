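; Prototype player controller that opens the pause menu on the PauseMenu input action.
; It creates WBP_PauseMenu, stores the reference, adds it to the viewport and switches to UI-only input focused on it.
; Gamepad presses also pause the game, while other keys only show the mouse cursor without pausing.
; No unpause logic runs here, and several leftover nodes are disconnected.
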(event EventBeginPlay)

(event EventTick
  (params (DeltaSeconds :type Float%20%28single-precision%29)))

(event Input|ActionEvents|InputActionPauseMenu
  (params (Key :type Key%20Structure :default "None"))
  ;[1 1 1] Pause/Unpause Game
  (:Pressed
    (if (Class|KismetInputLibrary|KeyIsGamepadKey Key)
      ;;[1 1 1] Gamepad
      (bind _returnvalue (UserInterface|CreateWidget "/Game/Proto/Proto_Lucas/Blueprints/Menus/Widgets/WBP_PauseMenu.WBP_PauseMenu_C"))
      (bind _output_get (Variables|Default|SetPauseMenuRef _returnvalue))
      (UserInterface|Viewport|AddtoViewport _output_get 0)
      (Input|SetInputModeUIOnly self (Variables|Default|GetPauseMenuRef) "DoNotLock")
      (Game|SetGamePaused true)
      (else
        ;;[1 1 1] Keyboard
        (bind _returnvalue_2 (UserInterface|CreateWidget "/Game/Proto/Proto_Lucas/Blueprints/Menus/Widgets/WBP_PauseMenu.WBP_PauseMenu_C"))
        (bind _output_get_2 (Variables|Default|SetPauseMenuRef _returnvalue_2))
        (UserInterface|Viewport|AddtoViewport _output_get_2 0)
        (Input|SetInputModeUIOnly self (Variables|Default|GetPauseMenuRef) "DoNotLock")
        (Variables|Default|SetbShowMouseCursor true)))))

(fn ConstructionScript)