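; Prototype child character Blueprint that adds a dash and test sword-and-shield attack animations.
; Dash launches the character along its facing with a gravity-based vertical velocity, gated by a DoOnce that resets after a short delay.
; Basic and special attack inputs play animations directly on the mesh, without montages or hit logic.
; BeginPlay prints registered input device details for debugging, and a few unconnected experimental nodes remain.
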(event EventBeginPlay
  (for _array_element (Class|RawInputFunctionLibrary|GetRegisteredDevices)
    (Development|PrintString (Utilities|String|Append (Utilities|String|Append (Utilities|String|Append (Utilities|String|ToString(Integer) (.Handle (Utilities|Struct|BreakRegisteredDeviceInfo _array_element))) "-") (Utilities|String|Append (Utilities|String|ToString(Integer) (.VendorID (Utilities|Struct|BreakRegisteredDeviceInfo _array_element))) "-")) (Utilities|String|Append (Utilities|String|Append (Utilities|String|ToString(Integer) (.ProductID (Utilities|Struct|BreakRegisteredDeviceInfo _array_element))) "-") (Utilities|String|Append (.DeviceName (Utilities|Struct|BreakRegisteredDeviceInfo _array_element)) "."))))))

(event Collision|EventActorBeginOverlap
  (params (OtherActor :type Actor%20Object%20Reference)))

(event EventTick
  (params (DeltaSeconds :type Float%20%28single-precision%29)))

(event Input|ActionEvents|InputActionDash
  (params (Key :type Key%20Structure :default "None"))
  (bind _returnvalue (Transformation|GetActorRotation))
  (bind _returnvalue_2 (Math|Vector|GetForwardVector _returnvalue))
  (bind _returnvalue_3 (* _returnvalue_2 "3000.000000,3000.000000,0"))
  ;[1 0.8096 0] Dash
  (:Pressed
    ;;[1 1 1] Faire un syst increment (1 puis 2)
    (Utilities|FlowControl|DoOnce false :!label _label
      (:Completed
        (Character|LaunchCharacter (Math|Vector|MakeVector (.x _returnvalue_3) (.y _returnvalue_3) (+ (Components|Movement|GetGravityZ (Variables|Character|GetCharacterMovement)) 2e+02)) false false)
        (Utilities|FlowControl|Delay 1.0)
        (goto _label Reset)))))

(event Input|ActionEvents|InputActionBasicAttack
  (params (Key :type Key%20Structure :default "None"))
  ;[1 1 1] Test anim
  (:Pressed
    (Components|Animation|PlayAnimation (Variables|Character|GetMesh) "/Game/Proto/Proto_Guillaume/Blueprints/Anim_Mixamo/30FPS/SwordAndShieldAttack_1__UE.SwordAndShieldAttack_1__UE" false)))

(event Input|ActionEvents|InputActionSpecialAttack
  (params (Key :type Key%20Structure :default "None"))
  ;[1 1 1] Test anim
  (:Pressed
    (Components|Animation|PlayAnimation (Variables|Character|GetMesh) "/Game/Proto/Proto_Guillaume/Blueprints/Anim_Mixamo/30FPS/SwordAndShieldSlash_2__UE.SwordAndShieldSlash_2__UE" false)))

(event Input|KeyboardEvents|AnyKey
  (params (Key :type Key%20Structure :default "None")))

(fn ConstructionScript
  (|CallParentFunction))