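; BP_WaveWalls is a prototype arena actor that closes three walls around a wave fight and starts the wave countdown.
; The first BP_MainBase overlap of its box immediately calls StartCountdown on the BP_WaveManager actors, and after a short delay teleports the walls to their translucent placeholder positions.
; A FightOver event moves the walls back to their reset positions, while the DoOnce gates are never reset here.
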(event OnComponentBeginOverlap(Box)
  (params (OverlappedComponent :type Primitive%20Component%20Object%20Reference) (OtherActor :type Actor%20Object%20Reference) (OtherComp :type Primitive%20Component%20Object%20Reference) (OtherBodyIndex :type Integer) (bFromSweep :type Boolean) (SweepResult :type Hit%20Result%20Structure%20%28by%20ref%29))
  ;[1 1 1] Start Fight
  (Utilities|Casting|CastToBP_MainBase OtherActor)
  (Utilities|FlowControl|DoOnce false
    (:Completed
      (Utilities|FlowControl|Sequence
        (:then_0
          (Utilities|FlowControl|Delay 1.0)
          (Utilities|FlowControl|DoOnce false
            (:Completed
              (Transformation|SetWorldLocation (Variables|Default|GetWall1) (Transformation|GetWorldLocation (Variables|Default|GetWall1_Transluscent)) false false)
              (Transformation|SetWorldLocation (Variables|Default|GetWall2) (Transformation|GetWorldLocation (Variables|Default|GetWall2_Transluscent)) false false)
              (Transformation|SetWorldLocation (Variables|Default|GetWall3) (Transformation|GetWorldLocation (Variables|Default|GetWall3_Transluscent)) false false))))
        (:then_1
          (bind _outactors (Actor|GetAllActorsOfClass "/Game/Proto/Proto_Lucas/Blueprints/SpawnSystem/BaseSpawnSystem/BP_WaveManager.BP_WaveManager_C"))
          (for _array_element _outactors
            (bind _asbp_wave_manager (Utilities|Casting|CastToBP_WaveManager _array_element))
            (Default|StartCountdown _asbp_wave_manager)))))))

(event Custom|FightOver
  ;[1 1 1] FightOver
  (Transformation|SetWorldLocation (Variables|Default|GetWall1) (Transformation|GetWorldLocation (Variables|Default|GetWall1_ResetPosition)) false false)
  (Transformation|SetWorldLocation (Variables|Default|GetWall2) (Transformation|GetWorldLocation (Variables|Default|GetWall2_ResetPosition)) false false)
  (Transformation|SetWorldLocation (Variables|Default|GetWall3) (Transformation|GetWorldLocation (Variables|Default|GetWall3_ResetPosition)) false false))

(event EventBeginPlay)

(event Collision|EventActorBeginOverlap
  (params (OtherActor :type Actor%20Object%20Reference)))

(event EventTick
  (params (DeltaSeconds :type Float%20%28single-precision%29)))

(fn ConstructionScript)