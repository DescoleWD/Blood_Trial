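; Prototype player character child class handling fixed-axis movement, combat abilities, health and checkpoint respawn.
; Inputs drive melee with delayed blood wave and rope lever activation, bolas, an attached hurricane and a Sacrify1-gated, charge-limited dash that ignores pawn and dynamic collision.
; BeginPlay creates HP and score widgets and attaches a sword to the hand.
; Damage updates shared instance health, triggering knockback and hit feedback, or destroying the actor at zero.
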(event Custom|CustomEvent
  (params (nearLever :type Actor%20Object%20Reference))
  ;[1 0 0] Need Urgent Rwork
  ;;[0.4072 0.3372 0] Attaque Basique
  ;;;[0 1 0.01273] Rope Code
  (Variables|Default|SetNearRope nearLever))

(event Custom|CustomEvent_1
  ;[1 0 0] Need Urgent Rwork
  ;;[1 0.8279 0] Bolas
  (Utilities|FlowControl|DoOnce false ; enters at Reset
    (:Completed
      (CallFunction|ThrowBolas))))

(event Custom|CustomEvent_4
  (bind _checkpointrotation (Variables|Default|GetCheckpointRotation))
  ;[1 0.6893 0] Respawn
  (Input|DisableInput (Game|GetPlayerController 0))
  (Utilities|FlowControl|Delay 0.2)
  (Utilities|FlowControl|Sequence
    (:then_0
      (Utilities|FlowControl|Delay 0.4)
      (Transformation|Teleport (Variables|Default|GetCheckpointLocation) _checkpointrotation)
      (Pawn|SetControlRotation (Game|GetPlayerController 0) _checkpointrotation)
      (Pawn|Components|CharacterMovement|DisableMovement (Variables|Character|GetCharacterMovement))
      (Utilities|FlowControl|Delay 1.0)
      (Pawn|Components|CharacterMovement|SetMovementMode (Variables|Character|GetCharacterMovement) "MOVE_Walking" 0)
      (Input|EnableInput (Game|GetPlayerController 0)))))

(event Custom|CustomEvent_2
  ;[1 0 0] Need Urgent Rwork
  ;;[0.4072 0.3372 0] Attaque Basique
  (Utilities|FlowControl|Delay 0.4)
  (CallFunction|SpawnBloodWaveBPPlayer))

(event Custom|CustomEvent_3
  ;[1 1 1] HP Player
  (Default|Collection (stale EventBeginPlay _output_get_2)))

(event Game|Damage|EventAnyDamage
  (params (Damage :type Float%20%28single-precision%29) (DamageType :type Damage%20Type%20Object%20Reference) (InstigatedBy :type Controller%20Object%20Reference) (DamageCauser :type Actor%20Object%20Reference))
  ;[1 1 1] HP Player
  (CallFunction|KnockBack)
  (bind _output_get (Variables|/Game/Proto/Main/Blueprint/BloodTrial_GameInstance.BloodTrial_GameInstance_C|SetChoose_Life (CallFunction|GetInst) (- (Variables|/Game/Proto/Main/Blueprint/BloodTrial_GameInstance.BloodTrial_GameInstance_C|GetChoose_Life (CallFunction|GetInst)) Damage)))
  (Progress|SetPercent (Variables|/Game/Proto/Proto_Guillaume/Blueprints/Player/HP_Bar_Player.HP_Bar_Player_C|GetProgressBar_40 (stale EventBeginPlay _output_get)) (Math|Float|SafeDivide _output_get 3e+02))
  (Math|Float|CompareFloat (Math|Float|SafeDivide _output_get 3e+02) 0.0
    (:>
      (if (Variables|Default|GetbCanBeDamaged)
        (Variables|Default|SetbCanBeDamaged false)
        (Animation|Montage|PlayMontage (Variables|Character|GetMesh) "/Game/Proto/Proto_Guillaume/Blueprints/Anim_Mixamo/30FPS/MediumHitToHead_UE_Montage.MediumHitToHead_UE_Montage" 0.5
          (:then
            _)
          (:OnNotifyBegin
            _))
        (Variables|Default|SetbCanBeDamaged true)
        (Game|Feedback|ClientPlayForceFeedback (Game|GetPlayerController 0) "/Game/Proto/Proto_Guillaume/Blueprints/Player/Damage.Damage" "None" false false false)
        (Camera|PlayWorldCameraShake "/Game/Proto/Proto_Guillaume/Blueprints/Plaisir_Coupable/CameraShakes.CameraShakes_C" (Transformation|GetActorLocation) 0.0 5e+02)))
    (:==
      (Actor|DestroyActor :!label _label))
    (:<
      (goto _label))))

(event EventBeginPlay
  ;[1 1 1] HP Player
  (Utilities|FlowControl|Sequence
    (:then_0
      (bind _returnvalue (UserInterface|CreateWidget "/Game/Proto/Proto_Guillaume/Blueprints/Player/HP_Bar_Player.HP_Bar_Player_C"))
      (UserInterface|Viewport|AddtoViewport _returnvalue 1)
      (bind _output_get (Variables|Default|SetAs_HP_Bar_Player _returnvalue)))
    (:then_1
      (bind _returnvalue_2 (UserInterface|CreateWidget "/Game/Proto/Main/HUD/Score.Score_C"))
      (UserInterface|Viewport|AddtoViewport _returnvalue_2 0)
      (bind _output_get_2 (Variables|Default|SetAs_Score _returnvalue_2)))
    (:then_2
      (bind _returnvalue_3 (Game|SpawnActorfromClass "/Game/Proto/Proto_Guillaume/Blueprints/Plaisir_Coupable/source/Sword.Sword_C" (Transformation|GetActorTransform) "AlwaysSpawn" 0 0))
      (bind _output_get_3 (Variables|Default|SetSet_Sword _returnvalue_3))
      (Transformation|AttachComponentToComponent _output_get_3 (Variables|Character|GetMesh) "hand_r" "SnapToTarget" "SnapToTarget" "KeepRelative" true))))

(event Input|ActionEvents|InputActionDash
  (params (Key :type Key%20Structure))
  (bind _asblood_trial_game_instance (CallFunction|GetInst))
  (bind _charactermovement (Variables|Character|GetCharacterMovement))
  (bind _returnvalue (Pawn|Components|PawnMovement|GetLastInputVector _charactermovement))
  (bind _returnvalue_2 (* _returnvalue 13.0))
  ;[0 0.05597 1] Dash + besoin anim / SFX/VFX
  (:Pressed
    (if (Variables|/Game/Proto/Main/Blueprint/BloodTrial_GameInstance.BloodTrial_GameInstance_C|GetSacrify_1 _asblood_trial_game_instance)
      (if (< (Variables|/Game/Proto/Main/Blueprint/BloodTrial_GameInstance.BloodTrial_GameInstance_C|GetNB_Dash _asblood_trial_game_instance) (Variables|/Game/Proto/Main/Blueprint/BloodTrial_GameInstance.BloodTrial_GameInstance_C|GetMaxDash _asblood_trial_game_instance))
        (Collision|SetCollisionResponsetoChannel (Variables|Default|GetCapsuleComponent) "ECC_Pawn" "ECR_Ignore")
        (Collision|SetCollisionResponsetoChannel (Variables|Default|GetCapsuleComponent) "ECC_WorldDynamic" "ECR_Ignore")
        (Variables|/Game/Proto/Main/Blueprint/BloodTrial_GameInstance.BloodTrial_GameInstance_C|SetNB_Dash _asblood_trial_game_instance (+ (Variables|/Game/Proto/Main/Blueprint/BloodTrial_GameInstance.BloodTrial_GameInstance_C|GetNB_Dash _asblood_trial_game_instance) 1))
        (Character|LaunchCharacter (Math|Vector|MakeVector (.x _returnvalue_2) (.y _returnvalue_2) 1e+01) false false)
        (Utilities|FlowControl|Delay 0.5)
        (Collision|SetCollisionResponsetoChannel (Variables|Default|GetCapsuleComponent) "ECC_WorldDynamic" "ECR_Block")
        (Collision|SetCollisionResponsetoChannel (Variables|Default|GetCapsuleComponent) "ECC_Pawn" "ECR_Block")
        (Utilities|FlowControl|Delay 1.0)
        (Variables|/Game/Proto/Main/Blueprint/BloodTrial_GameInstance.BloodTrial_GameInstance_C|SetNB_Dash (CallFunction|GetInst) 0)
        (Class|NavMovementComponent|StopMovementKeepPathing (Variables|Character|GetCharacterMovement))
        (else
          (Utilities|FlowControl|Delay 1.0)
          (Variables|/Game/Proto/Main/Blueprint/BloodTrial_GameInstance.BloodTrial_GameInstance_C|SetNB_Dash _asblood_trial_game_instance 0))))))

(event Input|ActionEvents|InputActionSpecialAttack
  (params (Key :type Key%20Structure))
  ;[1 0 0] Need Urgent Rwork
  ;;[1 0.8279 0] Bolas
  (:Pressed
    (CallFunction|CheckUpThrowBolas)
    (CallFunction|ThrowBolas)))

(event Input|ActionEvents|InputActionHurricane
  (params (Key :type Key%20Structure))
  (:Pressed
    (bind _returnvalue (Game|SpawnActorfromClass "/Game/Proto/Proto_Florian/Blueprints/BP_Hurricane.BP_Hurricane_C" (Math|Transform|MakeTransform (.location (Math|Conversions|ToTransform(Vector) (Transformation|GetWorldLocation (Variables|Default|GetSpawnHurricane_0)))) "0, 0, 0" "1.000000,1.000000,1.000000") "AlwaysSpawn" 0 0))
    (Transformation|AttachComponentToComponent _returnvalue (Variables|Default|GetSpawnHurricane_0) "" "KeepWorld" "KeepWorld" "KeepRelative" true)))

(event Input|ActionEvents|InputActionBasicAttack
  (params (Key :type Key%20Structure))
  ;[1 0 0] Need Urgent Rwork
  ;;[0.4072 0.3372 0] Attaque Basique
  (:Pressed
    (Default|Attaque (Variables|Default|GetAC_Melee_Player))
    (Utilities|FlowControl|Sequence
      (:then_0
        ;;;[1 0.8279 0] Blood Wave : ajuster avec anim pour cast + délais anim
        (CallFunction|DelayBW))
      (:then_1
        ;;;[0 1 0.01273] Rope Code
        (if (!= (Variables|Default|GetNearRope) 0)
          (Default|LeverActive (.AsBP%20Rope (Utilities|Casting|CastToBP_Rope (Variables|Default|GetNearRope)))))))))

(event Input|AxisEvents|InputAxisMoveForward/Backward
  (params (AxisValue :type Float%20%28single-precision%29))
  ;[1 0 0] Need Urgent Rwork
  ;;[0 1 0.01267] Déplacement
  (if (>= (Math|Float|Absolute(Float) (* AxisValue 1e+01)) 1.0)
    (Pawn|Input|AddMovementInput (Class|PawnMovementComponent|GetPawnOwner (Variables|Character|GetCharacterMovement)) "100.000000,-100.000000,0.000000" AxisValue false)))

(event Input|AxisEvents|InputAxisMoveLeft/Right
  (params (AxisValue :type Float%20%28single-precision%29))
  ;[1 0 0] Need Urgent Rwork
  ;;[0 1 0.01267] Déplacement
  (if (>= (Math|Float|Absolute(Float) (* AxisValue 1e+01)) 1.0)
    (Pawn|Input|AddMovementInput (Class|PawnMovementComponent|GetPawnOwner (Variables|Character|GetCharacterMovement)) "-100.000000,-100.000000, 0" AxisValue false)))

(event Input|KeyboardEvents|H
  (params (Key :type Key%20Structure))
  ;[1 0.6893 0] Respawn
  (:Pressed
    (Development|PrintString (Utilities|String|ToString(Vector) (Variables|Default|GetCheckpointLocation)))))

(fn ConstructionScript
  (|CallParentFunction))