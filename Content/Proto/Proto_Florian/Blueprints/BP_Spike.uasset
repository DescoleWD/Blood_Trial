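; BP_Spike is a prototype spike trap whose pike rises and retracts while its trigger box is active.
; Entering Box starts a delayed MoveComponentTo cycle between StaticMesh's starting position and a lowered offset, repeating until an end overlap clears the flag.
; A separate BoxCollision detects BP_MainCharacter hits, printing a debug cry with a DoOnce cooldown; no damage is applied.
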(event OnComponentBeginOverlap(Box)
  (params (OverlappedComponent :type Primitive%20Component%20Object%20Reference) (OtherActor :type Actor%20Object%20Reference) (OtherComp :type Primitive%20Component%20Object%20Reference) (OtherBodyIndex :type Integer) (bFromSweep :type Boolean) (SweepResult :type Hit%20Result%20Structure%20%28by%20ref%29))
  (Development|PrintString "In")
  (Variables|Default|SetIsInSpike? true)
  (Utilities|FlowControl|Delay 0.5 :!label _label)
  (Components|MoveComponentTo (Variables|Default|GetPike) (+ (Variables|Default|GetSpike_Origin_Position) "") "0, 0, 0" true true 0.1 false)
  (Utilities|FlowControl|Delay 1.5)
  (Components|MoveComponentTo (Variables|Default|GetPike) (+ (Variables|Default|GetSpike_Origin_Position) "0,0,-288.000000") "0, 0, 0" true true 0.5 false)
  (if (Variables|Default|GetIsInSpike?)
    (goto _label)))

(event OnComponentEndOverlap(Box)
  (params (OverlappedComponent :type Primitive%20Component%20Object%20Reference) (OtherActor :type Actor%20Object%20Reference) (OtherComp :type Primitive%20Component%20Object%20Reference) (OtherBodyIndex :type Integer))
  (Variables|Default|SetIsInSpike? false)
  (Development|PrintString "Out"))

(event OnComponentBeginOverlap(BoxCollision)
  (params (OverlappedComponent :type Primitive%20Component%20Object%20Reference) (OtherActor :type Actor%20Object%20Reference) (OtherComp :type Primitive%20Component%20Object%20Reference) (OtherBodyIndex :type Integer) (bFromSweep :type Boolean) (SweepResult :type Hit%20Result%20Structure%20%28by%20ref%29))
  (Utilities|Casting|CastToBP_MainCharacter OtherActor)
  (Utilities|FlowControl|DoOnce false :!label _label
    (:Completed
      (Development|PrintString "AIE" true true "(R=1.000000,G=0.019552,B=0.000000,A=1.000000)")
      (Utilities|FlowControl|Delay 1.5)
      (goto _label Reset))))

(event EventBeginPlay
  (Variables|Default|SetSpike_Origin_Position (Variables|/Script/Engine.SceneComponent|GetRelativeLocation (Variables|Default|GetStaticMesh))))

(fn ConstructionScript)