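; Parent Blueprint for arrow quiver pickups, showing ammo as arrow actors attached to the quiver mesh.
; On load it builds a slot array from fixed arrow components and fills it with the item's arrow type, capped by capacity.
; It passes out arrows, refills free slots, and frees a fired arrow's slot only when equipped ammo doesn't exceed capacity.
; Player death destroys the spawned arrows; self-destruction also removes the quiver.
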(event EventDestroySelf&Attachments
  ;[1 1 1] Destroying Quiver & Spawned Arrows
  ;;[1 1 1] Called When Ready To Destroy
  (for _array_element (Variables|Default|GetArrowSlots)
    (Utilities|IsValid (.arrowref _array_element)
      (:Is%20Valid
        (Actor|DestroyActor (.arrowref _array_element)))))
  (Actor|DestroyActor))

(event EventBeginPlay
  ;[1 1 1] Load Arrows - IF Data Exists Load Arrows, IF Placed in Level Begin Play
  (CallFunction|InitializeItem)
  (CallFunction|SetMesh)
  (CallFunction|PickedUpCheck)
  (Utilities|FlowControl|Delay 0.1)
  (Utilities|FlowControl|DoOnce false
    (:Completed
      (Variables|Default|SetAvailableArrowSlots (Variables|Default|GetTotalArrowSlots))
      (CallFunction|LoadSlots)
      (CallFunction|SpawnArrowsIntoQuiver))))

(event EventPlayerDied
  ;[1 1 1] Destroying Quiver & Spawned Arrows
  ;;[1 1 1] Removing Functionality From Parent
  (for _array_element (Variables|Default|GetArrowSlots)
    (Utilities|IsValid (.arrowref _array_element)
      (:Is%20Valid
        (Actor|DestroyActor (.arrowref _array_element))))))

(event EventLowerArrowQuantity
  ;[1 1 1] Remove Arrow Data - Called When Arrow Fired
  (CallFunction|RemoveArrowData))

(event EventLoadArrows
  ;[1 1 1] Load Arrows - IF Data Exists Load Arrows, IF Placed in Level Begin Play
  (Utilities|FlowControl|DoOnce false
    (:Completed
      (Variables|Default|SetAvailableArrowSlots (Variables|Default|GetTotalArrowSlots))
      (CallFunction|LoadSlots)
      (CallFunction|SpawnArrowsIntoQuiver))))

(event EventIncreaseArrowNumber
  (params (Quantity :type Integer))
  ;[1 1 1] Update Arrow Number
  (CallFunction|IncreaseArrowQuantity Quantity))

(fn ConstructionScript
  (|CallParentFunction))

(fn SpawnArrowsIntoQuiver
  (bind _iteminfo (Variables|Default|GetItemInfo))
  (bind _itemstructure (Utilities|Struct|BreakS_SlotInfo _iteminfo))
  (bind _equipmentinfo (Utilities|Struct|BreakS_ItemData _itemstructure))
  (bind (_damagetype _specialdamageinfo) (Utilities|Struct|BreakS_EquipmentInfo _equipmentinfo))
  ;[1 1 1] Spawn Arrows
  (LocalVariables|SetArrowLoopCountLocal (- (Math|Integer|Clamp(Integer) (Utilities|Struct|BreakS_SlotInfo (Variables|Default|GetItemInfo)) 0 (Variables|Default|GetAvailableArrowSlots)) 1))
  (for _index (range 0 (LocalVariables|GetArrowLoopCountLocal))
    (if (not (.slottaken (Utilities|Array|Get(acopy) (Variables|Default|GetArrowSlots) _index)))
      (bind _returnvalue (Game|SpawnActorfromClass (CallFunction|GetArrowType) (Math|Transform|MakeTransform (.location (Transformation|GetWorldTransform (.arrowslot (Utilities|Array|Get(acopy) (Variables|Default|GetArrowSlots) _index)))) (.rotation (Transformation|GetWorldTransform (.arrowslot (Utilities|Array|Get(acopy) (Variables|Default|GetArrowSlots) _index)))) "1,1,1") "AlwaysSpawn" 0 0))
      (Default|InitializeArrow _returnvalue _damagetype _specialdamageinfo)
      (Utilities|IsValid _returnvalue
        (:Is%20Valid
          (Transformation|AttachComponentToComponent _returnvalue (Variables|Default|GetItemStatic) "" "KeepWorld" "KeepWorld" "KeepWorld" true)
          (Math|Integer|DecrementInt (Variables|Default|GetAvailableArrowSlots)
            (:%20%20
              (CallFunction|SetSlot _index true _returnvalue))))))))

(fn PassArrow
  (bind _arrowslots (Variables|Default|GetArrowSlots))
  ;[1 1 1] Look For An Arrow In Quiver
  (LocalVariables|SetDecrementCounter 0)
  (while (not (Utilities|IsValid (.arrowref (Utilities|Array|Get(acopy) _arrowslots (- (Utilities|Array|Length _arrowslots) (LocalVariables|GetDecrementCounter))))))
    (Math|Integer|IncrementInt (LocalVariables|GetDecrementCounter)))
  (Variables|Default|SetArrowToPass (.arrowref (Utilities|Array|Get(acopy) _arrowslots (- (Utilities|Array|Length _arrowslots) (LocalVariables|GetDecrementCounter)))))
  (Variables|Default|SetArrowIndexToPass (- (Utilities|Array|Length _arrowslots) (LocalVariables|GetDecrementCounter)))
  (return (Variables|Default|GetArrowToPass)))

(fn ResetSingleArrow
  (params (Target :type Actor%20Object%20Reference))
  (bind _arrowindextopass (Variables|Default|GetArrowIndexToPass))
  (bind _arrowslots (Variables|Default|GetArrowSlots))
  (bind _output (Utilities|Array|Get(acopy) _arrowslots _arrowindextopass))
  ;[1 1 1] Reset Arrow
  (Utilities|IsValid (.arrowslot _output)
    (:Is%20Valid
      (Transformation|AttachComponentToComponent Target (.arrowslot _output) "None" "SnapToTarget" "SnapToTarget" "KeepWorld" true))))

(fn RemoveArrowData
  (if (not (> (Utilities|Struct|BreakS_SlotInfo (Variables|/Game/FlexibleCombatSystem/Blueprints/Components/EquipmentComponent.EquipmentComponent_C|GetAmmoQuiverInfo (Variables|Default|GetEquipmentComponent))) (Variables|Default|GetTotalArrowSlots)))
    (CallFunction|SetSlot (Variables|Default|GetArrowIndexToPass) false)
    (Math|Integer|IncrementInt (Variables|Default|GetAvailableArrowSlots))))

(fn IncreaseArrowQuantity
  (params (New%20Arrows :type Integer))
  (bind _availablearrowslots (Variables|Default|GetAvailableArrowSlots))
  ;[1 1 1] Adding New Arrows
  (LocalVariables|SetNewArrowsLocal New%20Arrows)
  (if (>= (Variables|Default|GetAvailableArrowSlots) 0)
    (Utilities|FlowControl|ForLoopwithBreak 1 (LocalVariables|GetNewArrowsLocal) :!label _label
      (:LoopBody
        (bind (_array_element _array_index) (Utilities|Array|ForEachLoopwithBreak (Variables|Default|GetArrowSlots) :!label _label_2)
          (:LoopBody
            (if (not (.slottaken _array_element))
              (bind _returnvalue (Game|SpawnActorfromClass (CallFunction|GetArrowType) (Math|Transform|MakeTransform (.location (Transformation|GetWorldTransform (.arrowslot _array_element))) (.rotation (Transformation|GetWorldTransform (.arrowslot _array_element))) "1,1,1") "Undefined" 0 0))
              (Transformation|AttachComponentToComponent _returnvalue (Variables|Default|GetItemStatic) "None" "KeepWorld" "KeepWorld" "KeepWorld" true)
              (CallFunction|SetSlot _array_index true _returnvalue)
              (Math|Integer|DecrementInt _availablearrowslots
                (:%20%20
                  (if (== _availablearrowslots 0)
                    (Utilities|FlowControl|Sequence
                      (:then_0
                        (goto _label_2 Break))
                      (:then_1
                        (goto _label Break)))
                    (else
                      (goto _label_2 Break))))))))))))

(fn LoadSlots
  (for _array_element (Utilities|Array|MakeArray (Variables|Default|GetArrow0) (Variables|Default|GetArrow1) (Variables|Default|GetArrow2) (Variables|Default|GetArrow3) (Variables|Default|GetArrow4) (Variables|Default|GetArrow5Central) (Variables|Default|GetArrow6) (Variables|Default|GetArrow7) (Variables|Default|GetArrow8) (Variables|Default|GetArrow9) (Variables|Default|GetArrow10) (Variables|Default|GetArrow11) (Variables|Default|GetArrow12) (Variables|Default|GetArrow13) (Variables|Default|GetArrow14))
    (Utilities|Array|Add (Variables|Default|GetArrowSlots) (Utilities|Struct|MakeS_QuiverStatus _array_element false))))

(fn SetSlot
  (params (Index :type Integer) (SlotTaken :type Boolean) (ArrowRef :type BP%20Arrow%20Parent%20Object%20Reference))
  ;[1 1 1] Sets The Slot
  (Utilities|Array|SetArrayElem (Variables|Default|GetArrowSlots) Index (Utilities|Struct|MakeS_QuiverStatus (.arrowslot (Utilities|Array|Get(acopy) (Variables|Default|GetArrowSlots) Index)) SlotTaken ArrowRef)))

(fn ContainsArrow
  (return (> (- (Variables|Default|GetTotalArrowSlots) (Variables|Default|GetAvailableArrowSlots)) 0)))

(fn GetArrowType
  (return (.ArrowsForQuiver (Utilities|Struct|BreakS_EquipmentInfo (.EquipmentInfo (Utilities|Struct|BreakS_ItemData (.ItemStructure (Utilities|Struct|BreakS_SlotInfo (Variables|Default|GetItemInfo)))))))))

(fn ArrowsinQuiver
  (return (- (Variables|Default|GetTotalArrowSlots) (Variables|Default|GetAvailableArrowSlots))))

(fn GetArrowName&Quantity
  (return (.Name (Utilities|Struct|BreakS_ItemData (.ItemStructure (Utilities|Struct|BreakS_SlotInfo (Variables|Default|GetItemInfo))))) (.quantity (Variables|/Game/FlexibleCombatSystem/Blueprints/Components/EquipmentComponent.EquipmentComponent_C|GetAmmoQuiverInfo (Variables|Default|GetEquipmentComponent)))))

(fn GetBowAttachments
  (return 0 0 0 0 0))

(fn GetQuiverRef
  (return self))

(fn PassArrowRef
  (return 0))