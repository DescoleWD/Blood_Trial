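; Character equipment component that tracks gear-driven stats, weapon damage and mesh materials.
; InitializeEquipment caches owner references, waits briefly for inventory, loads equipment and some stats from a save slot, then refreshes derived values.
; Item stats raise attributes, with Vitality setting max health and Strength plus armor bonus feeding melee damage.
; Much logic is disconnected, including weapon assignment, restocking, armor mesh storage and part of save loading.
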(event Custom|InitializeEquipment
  ;[1 0.3585 0.9007] Initialize Equipment
  (CallFunction|StoreComponents)
  (bind _handsmesh (Class|ICharacter|PassArmorMeshes(Message) (Variables|Components|GetCharacterRef)))
  (CallFunction|StoreArmor _handsmesh)
  (Utilities|FlowControl|Delay 0.1) ; Give time for Inventory to Equip items
  (CallFunction|LoadSaveData)
  (CallFunction|UpdateDamageValues)
  (CallFunction|UpdateMaxValues)
  (Default|CallStatsUpdated)
  (CallFunction|UpdateMaterials))

(fn IncreaseCharacterStats
  (params (S_ItemInfo :type S%20Slot%20Info%20Structure%20%28by%20ref%29))
  (bind _itemstructure (Utilities|Struct|BreakS_SlotInfo S_ItemInfo))
  (bind _equipmentinfo (Utilities|Struct|BreakS_ItemData _itemstructure))
  (bind _itemstats (Utilities|Struct|BreakS_EquipmentInfo _equipmentinfo))
  (bind (_vitality _dexterity _wisdom _strength _agility _intellect _critchance _bonusdamage _armor _block) (Utilities|Struct|BreakS_ItemStats _itemstats))
  (Utilities|FlowControl|Sequence
    (:then_0
      ;[1 1 1] Create A Ref To Stat B4 Increase
      (LocalVariables|SetMaxHealthRef (Variables|CharacterValues|GetMaxHealth))
      ;[1 1 1] Set Health Based Upon Vitality
      (Variables|CharacterStats|SetVitality (Math|Conversions|ToFloat(Integer) (+ (Math|Float|Round (Variables|CharacterStats|GetVitality)) _vitality)))
      (bind _output_get (Variables|CharacterValues|SetMaxHealth (+ (* (Variables|CharacterStats|GetVitality) 1e+01) (Variables|CharacterValues|GetBaseHealth))))
      ;[1 1 1] Increase Health By Amount Gained
      (Variables|CharacterValues|SetHealth (+ (- _output_get (LocalVariables|GetMaxHealthRef)) (Variables|CharacterValues|GetHealth))))
    (:then_1
      ;[1 1 1] Strength
      (Variables|CharacterStats|SetStrength (+ (Variables|CharacterStats|GetStrength) (Math|Conversions|ToFloat(Integer) _strength))))
    (:then_2
      ;[1 1 1] Crit Chance (0.1 Crit Per Agility + Flat Crit)
      (Variables|CharacterStats|SetCritValue (+ (Variables|CharacterStats|GetCritValue) (Math|Conversions|ToFloat(Integer) _critchance))))
    (:then_3
      ;[1 1 1] Armor Damage
      (Variables|CharacterStats|SetArmorBonusDamage (+ (Variables|CharacterStats|GetArmorBonusDamage) _bonusdamage)))
    (:then_4
      ;[1 1 1] Armor
      (Variables|CharacterStats|SetArmor (+ (Variables|CharacterStats|GetArmor) _armor)))
    (:then_5
      ;[1 1 1] Block - Reduces the amount of stamina drained from a block
      (Variables|CharacterStats|SetShieldBlock _block))
    (:then_6
      (CallFunction|UpdateMaxValues))))

(fn ReplaceWeaponActor
  (params (ItemType :type E_ItemType%20Enum :default "NewEnumerator18"))
  (bind _mainhandactor (Variables|References|GetMainHandActor))
  (bind _offhandactor (Variables|References|GetOffhandActor))
  (switch Utilities|FlowControl|Switch|SwitchonE_ItemType ItemType
    (:NewEnumerator9
      _)
    (:NewEnumerator12
      _)
    (:NewEnumerator11
      _)
    (:NewEnumerator10
      _)
    (:NewEnumerator20
      _))
  ;[1 1 1] Equipping Melee Weapon
  (bind _returnvalue (Game|SpawnActorfromClass "/Game/Proto/Rework_All_Project/Blueprints/Items/PickUpItems/BP_WeaponParent.BP_WeaponParent_C" (Math|Transform|MakeTransform (Transformation|GetActorLocation (Variables|Components|GetCharacterRef)) "0, 0,0.000000" "1.000000,1.000000,1.000000") "Undefined" 0 0))
  (Class|IItemInterface|Spawn&Use(Message) (Variables|Components|GetCharacterRef) (Variables|Default|GetItemInfo))
  (switch Utilities|FlowControl|Switch|SwitchonE_ItemType (Utilities|Enum|ByteToEnumE_ItemType ItemType)
    (:NewEnumerator9
      (Utilities|IsValid _mainhandactor :!label _label
        (:Is%20Valid
          (Actor|DestroyActor _mainhandactor))))
    (:NewEnumerator12
      (goto _label))
    (:NewEnumerator10
      (Utilities|IsValid _offhandactor :!label _label_2
        (:Is%20Valid
          (Actor|DestroyActor _offhandactor))))
    (:NewEnumerator20
      (goto _label_2))))

(fn IncreaseStats
  ;[1 1 1] Increase Character Level
  (Math|Integer|IncrementInt 0
    (:%20%20
      ;[1 1 1] Increment Stats Set Number of Times
      (Utilities|FlowControl|DoN (LocalVariables|GetStatsGainedPerLevelUp)
        (:Exit
          (Math|Float|IncrementFloat (Variables|CharacterStats|GetVitality)
            (:%20%20
              (Math|Float|IncrementFloat (Variables|CharacterStats|GetDexterity)
                (:%20%20
                  (Math|Float|IncrementFloat 0.0
                    (:%20%20
                      (Math|Float|IncrementFloat (Variables|CharacterStats|GetStrength)
                        (:%20%20
                          (Math|Float|IncrementFloat 0.0
                            (:%20%20
                              (Math|Float|IncrementFloat 0.0))))))))))))))))

(fn UpdateMaxValues
  ;[1 1 1] Update Values (Called After Stats Been Updated)
  (Variables|CharacterValues|SetMaxHealth (+ (* (Variables|CharacterStats|GetVitality) 1e+01) (Variables|CharacterValues|GetBaseHealth))))

(fn UpdateDamageValues
  (Utilities|FlowControl|Sequence
    (:then_0
      ;[1 1 1] MainHand Weapon Damage
      (if (== (Variables|CharacterStats|GetMainHandWepDamage) 0)
        (Variables|DamageValues|SetMaxMainHandDmg 0.0)
        (else
          (Variables|DamageValues|SetMaxMainHandDmg (+ (Variables|CharacterStats|GetStrength) (Math|Conversions|ToFloat(Integer) (Variables|CharacterStats|GetMainHandWepDamage)) (Math|Conversions|ToFloat(Integer) (Variables|CharacterStats|GetArmorBonusDamage)))))))
    (:then_1
      ;[1 1 1] OffHand Weapon Damage
      (if (== (Variables|CharacterStats|GetOffHandWepDamage) 0)
        (Variables|DamageValues|SetMaxOffHandDmg 0.0)
        (else
          (Variables|DamageValues|SetMaxOffHandDmg (+ (Variables|CharacterStats|GetStrength) (Math|Conversions|ToFloat(Integer) (Variables|CharacterStats|GetOffHandWepDamage)) (Math|Conversions|ToFloat(Integer) (Variables|CharacterStats|GetArmorBonusDamage)))))))))

(fn RestockEquipmentFunction
  (for (_ _array_index) 0
    _))

(fn SetWeaponDamage
  (params (S_ItemInfo :type S%20Slot%20Info%20Structure%20%28by%20ref%29) (DamageType :type E_DamageCategory%20Enum :default "NewEnumerator0"))
  (bind _itemstructure (Utilities|Struct|BreakS_SlotInfo S_ItemInfo))
  (bind _equipmentinfo (Utilities|Struct|BreakS_ItemData _itemstructure))
  (bind _weapondamage (Utilities|Struct|BreakS_EquipmentInfo _equipmentinfo))
  (bind _returnvalue (Math|Float|Round _weapondamage))
  ;[1 1 1] Set Damage Values For Tooltip
  (switch Utilities|FlowControl|Switch|SwitchonE_DamageCategory DamageType
    (:NewEnumerator0
      (Variables|CharacterStats|SetMainHandWepDamage _returnvalue))
    (:NewEnumerator1
      (Variables|CharacterStats|SetOffHandWepDamage _returnvalue))
    (:NewEnumerator2
      (Variables|CharacterStats|SetRangedWepDamage _returnvalue))))

(fn StoreComponents
  (bind _returnvalue (Components|GetOwner))
  (bind _ascharacter (Utilities|Casting|CastToCharacter _returnvalue))
  (Variables|Components|SetCharacterRef _ascharacter)
  (Variables|Default|SetMeleeComponent (Actor|GetComponentbyClass _returnvalue "/Game/Proto/Rework_All_Project/Blueprints/Components/MeleeComponent.MeleeComponent_C")))

(fn UpdateHealthDispatch
  (Default|CallUpdateHealth (Variables|CharacterValues|GetHealth) (Variables|CharacterValues|GetMaxHealth)))

(fn RetrieveMesh
  (params (S_SlotInfo :type S%20Slot%20Info%20Structure%20%28by%20ref%29))
  (return (Utilities|Struct|BreakS_EquipmentInfo (Utilities|Struct|BreakS_ItemData (Utilities|Struct|BreakS_SlotInfo S_SlotInfo)))))

(fn SetMaterials
  (params (Mesh :type Skeletal%20Mesh%20Component%20Object%20Reference) (Materials :type Array%20of%20Skeletal%20Material%20Structures))
  ;[1 1 1] Sets The Material To the Default Mesh Material
  (Utilities|IsValid Mesh
    (:Is%20Valid
      (for (_array_element _array_index) Materials
        (Rendering|Material|SetMaterial Mesh _array_index (Utilities|Struct|BreakSkeletalMaterial _array_element))))))

(fn UpdateMaterials
  ;[1 1 1] Update Mesh Materials, Used For Taking Damage - Changing The Mesh Materials
  (Variables|Default|SetMaterialsSet true)
  (Utilities|Array|Clear (Variables|Default|GetMeshMaterials))
  (bind (_meshconstant _hands) (Class|ICharacter|PassBody(Message) (Components|GetOwner)))
  (bind _output_get (Variables|Default|SetCharacterMeshes (Utilities|Array|MakeArray _meshconstant _hands)))
  (for _array_element _output_get
    (Utilities|IsValid _array_element
      (:Is%20Valid
        (for _array_element_2 (Rendering|Material|GetMaterials _array_element)
          (Utilities|Array|Add (Variables|Default|GetMeshMaterials) _array_element_2))))))

(fn StoreArmor
  (params (HandsMesh :type Skeletal%20Mesh%20Component%20Object%20Reference)))

(fn LoadSaveData
  (bind _returnvalue (SaveGame|LoadGamefromSlot "save1"))
  ;[1 1 1] Load Equipment
  (bind _asbp_save_game (Utilities|Casting|CastTo _returnvalue))
  (Variables|Default|SetEquipmentRef (Variables|Default|GetEquippedItems_SaveGame _asbp_save_game))
  ;[1 1 1] Load Stats
  (Variables|CharacterStats|SetVitality (.CharacterVitality (Utilities|Struct|Break (Variables|Default|GetCharacterStatistics_SaveGame _asbp_save_game))))
  (Variables|CharacterStats|SetDexterity (.CharacterDexterity (Utilities|Struct|Break (Variables|Default|GetCharacterStatistics_SaveGame _asbp_save_game)))))