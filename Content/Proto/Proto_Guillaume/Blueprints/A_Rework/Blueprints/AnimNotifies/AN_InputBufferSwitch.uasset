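; Anim notify state that defines the window in an animation during which player inputs can be buffered.
; On begin it finds the InputBufferComponent on the mesh owner and opens the buffer so inputs are stored.
; On end it closes the buffer on that component, so inputs stop being stored.
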(fn ReceivedNotifyBegin
  (params (MeshComp :type Skeletal%20Mesh%20Component%20Object%20Reference) (Animation :type Anim%20Sequence%20Base%20Object%20Reference) (TotalDuration :type Float%20%28single-precision%29))
  (bind _returnvalue (Components|GetOwner MeshComp))
  (bind _returnvalue_2 (Actor|GetComponentbyClass _returnvalue "/Game/FlexibleCombatSystem/Blueprints/Components/InputBufferComponent.InputBufferComponent_C"))
  ;[1 1 1] Open Buffer Allowing Inputs To Be Stored
  (Utilities|IsValid _returnvalue_2
    (:Is%20Valid
      (Default|OpenBuffer _returnvalue_2)
      (return true))))

(fn ReceivedNotifyEnd
  (params (MeshComp :type Skeletal%20Mesh%20Component%20Object%20Reference) (Animation :type Anim%20Sequence%20Base%20Object%20Reference))
  (bind _returnvalue (Components|GetOwner MeshComp))
  (bind _returnvalue_2 (Actor|GetComponentbyClass _returnvalue "/Game/FlexibleCombatSystem/Blueprints/Components/InputBufferComponent.InputBufferComponent_C"))
  ;[1 1 1] Close Buffer Preventing Inputs being Stored
  (Utilities|IsValid _returnvalue_2
    (:Is%20Valid
      (Default|CloseBuffer _returnvalue_2)
      (return true))))