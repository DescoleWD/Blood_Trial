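; Blueprint function library for Blood Trial that gives shared access to game state stored in BloodTrial_GameInstance.
; Wrappers built on GetInst read or write score, numbered player life values, max HP, combos, calendar pieces and hazard damage.
; Sacrify functions apply percentage attack or speed boosts with debug prints, and Damage wraps ApplyDamage.
; Several functions are empty stubs, and the Score, CalendarPieces and PlayerLife 5–8 setters only reassign current values.
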(fn GetInst
  (return (.AsBlood%20Trial%20Game%20Instance (Utilities|Casting|CastToBloodTrial_GameInstance (Game|GetGameInstance)))))

(fn GetScore
  (return (Variables|/Game/Proto/Main/Blueprint/BloodTrial_GameInstance.BloodTrial_GameInstance_C|GetScore (Main_Syst|GetInst))))

(fn SetScore
  (bind _asblood_trial_game_instance (Main_Syst|GetInst))
  (Variables|/Game/Proto/Main/Blueprint/BloodTrial_GameInstance.BloodTrial_GameInstance_C|SetScore _asblood_trial_game_instance (Score|GetScore _asblood_trial_game_instance)))

(fn IncrScore
  (params (incValue :type Integer))
  (bind _asblood_trial_game_instance (Main_Syst|GetInst))
  (bind _output_get (Variables|/Game/Proto/Main/Blueprint/BloodTrial_GameInstance.BloodTrial_GameInstance_C|SetScore _asblood_trial_game_instance (+ (Score|GetScore _asblood_trial_game_instance) incValue)))
  (return _output_get))

(fn GetPlayerLife0
  (return (Variables|/Game/Proto/Main/Blueprint/BloodTrial_GameInstance.BloodTrial_GameInstance_C|GetPlayerLife_0 (Main_Syst|GetInst))))

(fn SetPlayerLife0
  (params (GetPlayerLife :type Float%20%28double-precision%29))
  (bind _output_get (Variables|/Game/Proto/Main/Blueprint/BloodTrial_GameInstance.BloodTrial_GameInstance_C|SetPlayerLife_0 (Main_Syst|GetInst) GetPlayerLife))
  (return _output_get))

(fn IncrPlayerLife)

(fn DecrPlayerLife)

(fn GetPlayerLife1
  (return (Variables|/Game/Proto/Main/Blueprint/BloodTrial_GameInstance.BloodTrial_GameInstance_C|GetPlayerLife_1 (Main_Syst|GetInst))))

(fn GetPlayerLife2
  (return (Variables|/Game/Proto/Main/Blueprint/BloodTrial_GameInstance.BloodTrial_GameInstance_C|GetPlayerLife_2 (Main_Syst|GetInst))))

(fn GetPlayerLife3
  (return (Variables|/Game/Proto/Main/Blueprint/BloodTrial_GameInstance.BloodTrial_GameInstance_C|GetPlayerLife_3 (Main_Syst|GetInst))))

(fn GetPlayerLife4
  (return (Variables|/Game/Proto/Main/Blueprint/BloodTrial_GameInstance.BloodTrial_GameInstance_C|GetPlayerLife_4 (Main_Syst|GetInst))))

(fn GetPlayerLife5
  (return (Variables|/Game/Proto/Main/Blueprint/BloodTrial_GameInstance.BloodTrial_GameInstance_C|GetPlayerLife_5 (Main_Syst|GetInst))))

(fn GetPlayerLife6
  (return (Variables|/Game/Proto/Main/Blueprint/BloodTrial_GameInstance.BloodTrial_GameInstance_C|GetPlayerLife_6 (Main_Syst|GetInst))))

(fn GetPlayerLife7
  (return (Variables|/Game/Proto/Main/Blueprint/BloodTrial_GameInstance.BloodTrial_GameInstance_C|GetPlayerLife_7 (Main_Syst|GetInst))))

(fn GetPlayerLife8
  (return (Variables|/Game/Proto/Main/Blueprint/BloodTrial_GameInstance.BloodTrial_GameInstance_C|GetPlayerLife_8 (Main_Syst|GetInst))))

(fn SetPlayerLife1
  (params (GetPlayerLife :type Float%20%28double-precision%29))
  (bind _output_get (Variables|/Game/Proto/Main/Blueprint/BloodTrial_GameInstance.BloodTrial_GameInstance_C|SetPlayerLife_1 (Main_Syst|GetInst) GetPlayerLife))
  (return _output_get))

(fn SetPlayerLife2
  (params (GetPlayerLife :type Float%20%28double-precision%29))
  (bind _output_get (Variables|/Game/Proto/Main/Blueprint/BloodTrial_GameInstance.BloodTrial_GameInstance_C|SetPlayerLife_2 (Main_Syst|GetInst) GetPlayerLife))
  (return _output_get))

(fn SetPlayerLife3
  (params (GetPlayerLife :type Float%20%28double-precision%29))
  (bind _output_get (Variables|/Game/Proto/Main/Blueprint/BloodTrial_GameInstance.BloodTrial_GameInstance_C|SetPlayerLife_3 (Main_Syst|GetInst) GetPlayerLife))
  (return _output_get))

(fn SetPlayerLife4
  (params (GetPlayerLife :type Float%20%28double-precision%29))
  (bind _output_get (Variables|/Game/Proto/Main/Blueprint/BloodTrial_GameInstance.BloodTrial_GameInstance_C|SetPlayerLife_4 (Main_Syst|GetInst) GetPlayerLife))
  (return _output_get))

(fn SetPlayerLife5
  (params (GetPlayerLife :type Float%20%28double-precision%29))
  (bind _asblood_trial_game_instance (Main_Syst|GetInst))
  (bind _output_get (Variables|/Game/Proto/Main/Blueprint/BloodTrial_GameInstance.BloodTrial_GameInstance_C|SetPlayerLife_5 _asblood_trial_game_instance (GetPlayerLife|GetPlayerLife5 _asblood_trial_game_instance)))
  (return _output_get))

(fn SetPlayerLife6
  (params (GetPlayerLife :type Float%20%28double-precision%29))
  (bind _asblood_trial_game_instance (Main_Syst|GetInst))
  (bind _output_get (Variables|/Game/Proto/Main/Blueprint/BloodTrial_GameInstance.BloodTrial_GameInstance_C|SetPlayerLife_6 _asblood_trial_game_instance (GetPlayerLife|GetPlayerLife6 _asblood_trial_game_instance)))
  (return _output_get))

(fn SetPlayerLife7
  (params (GetPlayerLife :type Float%20%28double-precision%29))
  (bind _asblood_trial_game_instance (Main_Syst|GetInst))
  (bind _output_get (Variables|/Game/Proto/Main/Blueprint/BloodTrial_GameInstance.BloodTrial_GameInstance_C|SetPlayerLife_7 _asblood_trial_game_instance (GetPlayerLife|GetPlayerLife7 _asblood_trial_game_instance)))
  (return _output_get))

(fn SetPlayerLife8
  (params (GetPlayerLife :type Float%20%28double-precision%29))
  (bind _asblood_trial_game_instance (Main_Syst|GetInst))
  (bind _output_get (Variables|/Game/Proto/Main/Blueprint/BloodTrial_GameInstance.BloodTrial_GameInstance_C|SetPlayerLife_8 _asblood_trial_game_instance (GetPlayerLife|GetPlayerLife8 _asblood_trial_game_instance)))
  (return _output_get))

(fn ChooseLife
  (params (Difficulty_Button :type Float%20%28double-precision%29))
  (bind _asblood_trial_game_instance (Main_Syst|GetInst))
  (bind _output_get (Variables|/Game/Proto/Main/Blueprint/BloodTrial_GameInstance.BloodTrial_GameInstance_C|SetChoose_Life _asblood_trial_game_instance Difficulty_Button))
  (Utilities|FlowControl|Sequence
    (:then_0
      (bind _maxhp_s (CallFunction|SetMaxHP _output_get _asblood_trial_game_instance)))
    (:then_1
      (return _output_get _maxhp_s))))

(fn SetChooseLife)

(fn SetMaxHP
  (params (MaxHP_E :type Float%20%28double-precision%29))
  (bind _output_get (Variables|/Game/Proto/Main/Blueprint/BloodTrial_GameInstance.BloodTrial_GameInstance_C|SetMaxLife (Main_Syst|GetInst) MaxHP_E))
  (return _output_get))

(fn GetNBCombo
  (return (Variables|/Game/Proto/Main/Blueprint/BloodTrial_GameInstance.BloodTrial_GameInstance_C|GetNB_Combos (Main_Syst|GetInst))))

(fn SetNBCombo
  (params (NB_Combos :type Integer))
  (Variables|/Game/Proto/Main/Blueprint/BloodTrial_GameInstance.BloodTrial_GameInstance_C|SetNB_Combos (Main_Syst|GetInst) NB_Combos))

(fn Sacrify2
  (bind _asblood_trial_game_instance (Main_Syst|GetInst))
  (bind _output_get (Variables|/Game/Proto/Main/Blueprint/BloodTrial_GameInstance.BloodTrial_GameInstance_C|SetPlayerAttack _asblood_trial_game_instance (+ (Variables|/Game/Proto/Main/Blueprint/BloodTrial_GameInstance.BloodTrial_GameInstance_C|GetPlayerAttack _asblood_trial_game_instance) (* (Variables|/Game/Proto/Main/Blueprint/BloodTrial_GameInstance.BloodTrial_GameInstance_C|GetPlayerAttack _asblood_trial_game_instance) 0.15))))
  (Development|PrintString 0 (Utilities|String|ToString(Float) _output_get)))

(fn Sacrify3)

(fn Sacrify4
  (bind _asblood_trial_game_instance (Main_Syst|GetInst))
  (bind _output_get (Variables|/Game/Proto/Main/Blueprint/BloodTrial_GameInstance.BloodTrial_GameInstance_C|SetPlayerSpeed _asblood_trial_game_instance (+ (Variables|/Game/Proto/Main/Blueprint/BloodTrial_GameInstance.BloodTrial_GameInstance_C|GetPlayerSpeed _asblood_trial_game_instance) (* (Variables|/Game/Proto/Main/Blueprint/BloodTrial_GameInstance.BloodTrial_GameInstance_C|GetPlayerSpeed _asblood_trial_game_instance) 0.5))))
  (Development|PrintString 0 (Utilities|String|ToString(Float) _output_get)))

(fn Sacrify5
  (bind _asblood_trial_game_instance (Main_Syst|GetInst))
  (bind _output_get (Variables|/Game/Proto/Main/Blueprint/BloodTrial_GameInstance.BloodTrial_GameInstance_C|SetPlayerAttack _asblood_trial_game_instance (+ (+ (Variables|/Game/Proto/Main/Blueprint/BloodTrial_GameInstance.BloodTrial_GameInstance_C|GetPlayerAttack _asblood_trial_game_instance) (* (Variables|/Game/Proto/Main/Blueprint/BloodTrial_GameInstance.BloodTrial_GameInstance_C|GetPlayerAttack _asblood_trial_game_instance) 0.15)) (* (Variables|/Game/Proto/Main/Blueprint/BloodTrial_GameInstance.BloodTrial_GameInstance_C|GetPlayerAttack _asblood_trial_game_instance) 0.15))))
  (Development|PrintString 0 (Utilities|String|ToString(Float) _output_get)))

(fn Sacrify6)

(fn Sacrify7)

(fn Sacrify8)

(fn GetCalendarPieces
  (return (Variables|/Game/Proto/Main/Blueprint/BloodTrial_GameInstance.BloodTrial_GameInstance_C|GetCalendar_Pieces (Main_Syst|GetInst))))

(fn SetCalendarPieces
  (bind _asblood_trial_game_instance (Main_Syst|GetInst))
  (Variables|/Game/Proto/Main/Blueprint/BloodTrial_GameInstance.BloodTrial_GameInstance_C|SetCalendar_Pieces _asblood_trial_game_instance (Calendar|GetCalendarPieces _asblood_trial_game_instance)))

(fn IncrCalendarPieces
  (params (IncrValue :type Integer))
  (bind _asblood_trial_game_instance (Main_Syst|GetInst))
  (bind _output_get (Variables|/Game/Proto/Main/Blueprint/BloodTrial_GameInstance.BloodTrial_GameInstance_C|SetCalendar_Pieces _asblood_trial_game_instance (+ (Calendar|GetCalendarPieces _asblood_trial_game_instance) 1)))
  (return _output_get))

(fn SetEnviroDamage
  (params (Spike_Damage :type Float%20%28double-precision%29))
  (Variables|/Game/Proto/Main/Blueprint/BloodTrial_GameInstance.BloodTrial_GameInstance_C|SetEnviroDamage (Main_Syst|GetInst) (* Spike_Damage 0.15)))

(fn SetLavaDamage
  (params (Lava_Damage :type Float%20%28double-precision%29) (__WorldContext :type Object%20Object%20Reference))
  (Variables|/Game/Proto/Main/Blueprint/BloodTrial_GameInstance.BloodTrial_GameInstance_C|SetLavaDamage (Main_Syst|GetInst) (* Lava_Damage 0.05)))

(fn Damage
  (params (Who :type Actor%20Object%20Reference) (Damage :type Float%20%28double-precision%29) (To_Who :type Actor%20Object%20Reference))
  (Game|Damage|ApplyDamage Who Damage 0 To_Who))