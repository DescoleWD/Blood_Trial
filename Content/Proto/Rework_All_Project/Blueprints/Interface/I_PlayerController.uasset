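; Blueprint interface for the player controller, letting other objects drive the HUD and menus without casting to the concrete controller class.
; It declares toggles for inventory, loot, container, external or vendor inventory, pause, spell book, spell trainer and quest log screens.
; Query functions report which menus are open, while others set up character and HUD references and pass equipment, outline and options-menu data.
; It holds only signatures, with no logic.
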(fn ShowHUD)

(fn HideHUD)

(fn ToggleInventory)

(fn ToggleContainerMenu
  (params (LootComponent :type %20Object%20Reference) (ToggleTag :type Boolean)))

(fn TogglePauseMenu)

(fn ToggleSpellBook)

(fn SetupReferences
  (params (CharacterRef :type Character%20Object%20Reference) (HUDRef :type %20Object%20Reference)))

(fn SetCanUpdateWidget
  (params (CanUpdateWidget :type Boolean))
  (return))

(fn LootMenuStatus
  (return false))

(fn InventoryStatus
  (return false))

(fn PassEquipmentComp
  (return 0))

(fn ContainerStatus
  (return false))

(fn ToggleLootMenu
  (params (Loot%20Component :type %20Object%20Reference)))

(fn ToggleExternalInventory
  (params (ExternalInventoryComponent :type %20Object%20Reference) (ActorRef :type Actor%20Object%20Reference) (Vendor :type Boolean))
  (return))

(fn ToggleExternalContainerInv
  (params (Inventory%20Component :type %20Object%20Reference) (Actor%20Ref :type Actor%20Object%20Reference)))

(fn PassInventoryState
  (return 0))

(fn RecieveOptionsMenu
  (params (Options%20Menu :type %20Object%20Reference))
  (return))

(fn ToggleQuestLog)

(fn ToggleSpellTrainer)

(fn WidgetMenuOpen
  (return false))

(fn ExternalInventoryOpen
  (return false))

(fn PassOutlineComponent
  (params (OutlineComponent :type %20Object%20Reference))
  (return))

(fn ExternalInventoryConditions
  (return false))