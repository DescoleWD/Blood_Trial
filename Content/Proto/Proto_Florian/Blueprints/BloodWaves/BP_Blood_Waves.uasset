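; Prototype blood wave actor that damages the first enemy it touches.
; When its Box overlaps a Master_Enemy, it applies BloodWaveDamage read through GetInst, then destroys itself.
; The static mesh hit event is empty, and an alternative box-trace damage path that ignores Player-tagged BP_MainBase actors is left disconnected.
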(event OnComponentHit(StaticMesh)
  (params (HitComponent :type Primitive%20Component%20Object%20Reference) (OtherActor :type Actor%20Object%20Reference) (OtherComp :type Primitive%20Component%20Object%20Reference) (NormalImpulse :type Vector :default "0, 0, 0") (Hit :type Hit%20Result%20Structure%20%28by%20ref%29)))

(event OnComponentBeginOverlap(Box)
  (params (OverlappedComponent :type Primitive%20Component%20Object%20Reference) (OtherActor :type Actor%20Object%20Reference) (OtherComp :type Primitive%20Component%20Object%20Reference) (OtherBodyIndex :type Integer) (bFromSweep :type Boolean) (SweepResult :type Hit%20Result%20Structure%20%28by%20ref%29))
  (bind _asmaster_enemy (Utilities|Casting|CastToMaster_Enemy OtherActor))
  (Game|Damage|ApplyDamage _asmaster_enemy (Variables|/Game/Proto/Main/Blueprint/Save_BFL_GameInstance/BloodTrial_GameInstance.BloodTrial_GameInstance_C|GetBloodWave_Damage (CallFunction|GetInst)) 0 0)
  (Actor|DestroyActor))

(event EventBeginPlay)

(fn ConstructionScript)