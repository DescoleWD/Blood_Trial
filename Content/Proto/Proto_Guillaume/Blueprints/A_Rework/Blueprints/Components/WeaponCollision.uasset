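; Weapon collision component that detects melee hits during attack windows and applies damage.
; StartAttack starts a fast looping timer that sphere-traces each weapon socket from its last position to its current one, until StopAttack clears it.
; Each newly hit actor with a TakingDamage component receives damage info and point damage, once until the hit list resets.
; Player attacks also request a camera shake; the friendly-fire check is defined but unused here.
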(event Custom|SendTraces
  ;[1 1 1] Triggered From Anim Notify - Generate LineTrace For Hit
  (bind (_arrayindex _arrayelement) (Utilities|Array|ReverseforEachLoop (Variables|Default|GetWeaponSockets))
    (:LoopBody
      (bind _outhits (Collision|MultiSphereTraceForObjects (Transformation|GetSocketLocation (Variables|Default|GetWeaponMesh) _arrayelement) (Utilities|Array|Get(acopy) (Variables|Default|GetTraceStartLocation) _arrayindex) 1e+01 (Variables|Default|GetObjectTypes) false (Utilities|Array|MakeArray (Components|GetOwner) (Variables|Default|GetCharacter)) "None"))
      (for _array_element _outhits
        (if (not (Utilities|Array|ContainsItem (Variables|Default|GetAlreadyDamagedEnemy) (.HitActor (Collision|BreakHitResult _array_element))))
          (Utilities|Array|Add (Variables|Default|GetAlreadyDamagedEnemy) (.HitActor (Collision|BreakHitResult _array_element)))
          (Utilities|IsValid (Actor|GetComponentbyClass (.HitActor (Collision|BreakHitResult _array_element)) "/Game/Proto/Proto_Guillaume/Blueprints/A_Rework/Blueprints/Components/TakingDamage.TakingDamage_C")
            (:Is%20Valid
              (CallFunction|PassDamageInfo (Actor|GetComponentbyClass (.HitActor (Collision|BreakHitResult _array_element)) "/Game/Proto/Proto_Guillaume/Blueprints/A_Rework/Blueprints/Components/TakingDamage.TakingDamage_C") (Variables|Default|GetWeaponPS) (Variables|Default|GetAttackType) (Variables|Default|GetDamage%20Type) (Variables|AttackInfo|GetCriticalHit))
              (Game|Damage|ApplyPointDamage (.HitActor (Collision|BreakHitResult _array_element)) (Variables|AttackInfo|GetWeaponOutputDamage) (.ImpactPoint (Collision|BreakHitResult _array_element)) _array_element 0 (Variables|Default|GetCharacter))))))
      (Utilities|Array|SetArrayElem (Variables|Default|GetTraceStartLocation) _arrayindex (Transformation|GetSocketLocation (Variables|Default|GetWeaponMesh) _arrayelement)))))

(event Custom|PassWeaponInfo
  (params (Mesh :type Primitive%20Component%20Object%20Reference) (Sockets :type Array%20of%20Names) (Character :type Character%20Object%20Reference) (Damage%20Type :type Byte :default 0) (Special%20Damage%20Info :type %20Structure))
  ;[1 1 1] Pass Over Weapon Ref & Sockets
  (Variables|Default|SetWeaponMesh Mesh)
  (Variables|Default|SetWeaponSockets Sockets)
  (Variables|Default|SetCharacter Character)
  (Variables|Default|SetDamage%20Type Damage%20Type))

(event EventStopAttack
  ;[1 1 1] Triggered From Anim Notify - Generate LineTrace For Hit
  (Utilities|Time|ClearandInvalidateTimerbyHandle (stale EventStartAttack _returnvalue))
  (CallFunction|SetupTraceLocations)
  ;;[1 1 1] For Fists
  (Class|Object|StopAttack(Message) (Components|GetOwner)))

(event EventStartAttack
  ;[1 1 1] Triggered From Anim Notify - Generate LineTrace For Hit
  (CallFunction|PlayShakeIFPlayer)
  (CallFunction|SetupTraceLocations)
  (Utilities|Array|Clear (Variables|Default|GetAlreadyDamagedEnemy))
  (bind _returnvalue (Utilities|Time|SetTimerbyEvent (delegate Custom|SendTraces) 0.01 true)))

(event EventResetAttackTargets
  ;[1 1 1] Triggered From Anim Notify - Generate LineTrace For Hit
  (Utilities|Array|Clear (Variables|Default|GetAlreadyDamagedEnemy)))

(fn SetupTraceLocations
  (Utilities|Array|Clear (Variables|Default|GetTraceStartLocation))
  (for (_array_element _array_index) (Variables|Default|GetWeaponSockets)
    (Utilities|Array|SetArrayElem (Variables|Default|GetTraceStartLocation) _array_index (Transformation|GetSocketLocation (Variables|Default|GetWeaponMesh) _array_element) true)))

(fn PreventFriendlyFire
  (params (HitActor :type Actor%20Object%20Reference))
  (return (and (Actor|ActorHasTag HitActor "EnemyAI") (Actor|ActorHasTag (Variables|Default|GetCharacter) "EnemyAI"))))

(fn PlayShakeIFPlayer
  (bind _character (Variables|Default|GetCharacter))
  (if (Actor|ActorHasTag _character "Player")
    (Camera|PlayWorldCameraShake 0 (Transformation|GetActorLocation _character) 0.0 1e+03 0.0)))