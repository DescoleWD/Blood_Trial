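; CombatStatusComponent is an actor component whose only logic is an Interact function for picking up items overlapping the character's capsule.
; It skips equipped weapons and quiver, then messages interface-implementing actors that are tag-visible or were last interacted with, remembering the latest.
; A fallback search for the next item has no action, and the pickup-success step is disconnected.
; A constant condition currently prevents the whole Interact body from running.
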(event EventBeginPlay)

(event EventTick
  (params (DeltaSeconds :type Float%20%28single-precision%29)))

(fn Interact
  (bind _equipmentcomponent (Variables|Default|GetEquipmentComponent))
  ;[1 1 1] Interact With Overlapping Actors, IF Current One Outlined Pick up
  (if (not true)
    (bind _array_element (Utilities|Array|ForEachLoopwithBreak (Collision|GetOverlappingActors (Variables|/Script/Engine.Character|GetCapsuleComponent (Variables|Default|GetCharacterRef)) "/Script/Engine.Actor" :!class /Script/Engine.PrimitiveComponent))
      (:LoopBody
        (if (Math|Boolean|ANDBoolean (!= _array_element (Variables|Default|GetMainHandActor _equipmentcomponent)) (!= _array_element (Variables|Default|GetOffhandActor _equipmentcomponent)) (!= _array_element (Variables|Default|GetRangedActor _equipmentcomponent)) (!= _array_element (Variables|Default|GetAmmoQuiver _equipmentcomponent)))
          (Utilities|IsValid (Actor|GetComponentbyClass _array_element 0)
            (:Is%20Valid
              (if (and (Utilities|DoesObjectImplementInterface _array_element 0) (or (Variables|Default|GetActorTagVisible (Actor|GetComponentbyClass _array_element 0)) (== _array_element (Variables|Default|GetLastInteractedActor))))
                (CallFunction|Interact _array_element (Variables|Default|GetCharacterRef))
                (Variables|Default|SetLastInteractedActor _array_element))))))
      (:Completed
        ;[1 1 1] IF Last Interacted Actor IS Valid (Not Picked Up) Do Nothing. IF Item Gone, Find next item
        (Utilities|IsValid (Variables|Default|GetLastInteractedActor)
          (:Is%20Not%20Valid
            (bind _array_element_2 (Utilities|Array|ForEachLoopwithBreak (Collision|GetOverlappingActors (Variables|/Script/Engine.Character|GetCapsuleComponent (Variables|Default|GetCharacterRef)) "/Script/Engine.Actor" :!class /Script/Engine.PrimitiveComponent))
              (:LoopBody
                (Utilities|IsValid (Actor|GetComponentbyClass _array_element_2 0)
                  (:Is%20Valid
                    (if (Utilities|DoesObjectImplementInterface _array_element_2 0)
                      _)))))))))))