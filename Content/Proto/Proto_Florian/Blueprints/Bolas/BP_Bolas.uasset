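; BP_Bolas is a prototype thrown bolas projectile that plays a pitch-varied sound on spawn.
; If pawns are near a hit, it records the hit actor on BP_MainBase and triggers SpawnBolasT on Papillon or Tzitzimine targets before destroying itself.
; Player hits or a timeout move the mesh to the player, re-enable throwing and destroy it.
; AfterExplosion also re-enables throwing; a helper applies bolas damage.
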(event OnComponentHit(StaticMesh)
  (params (HitComponent :type Primitive%20Component%20Object%20Reference) (OtherActor :type Actor%20Object%20Reference) (OtherComp :type Primitive%20Component%20Object%20Reference) (NormalImpulse :type Vector :default "0, 0, 0") (Hit :type Hit%20Result%20Structure%20%28by%20ref%29))
  (Variables|Default|SetHit%20Actor (.hitactor Hit))
  (bind (_outactors _returnvalue) (Collision|SphereOverlapActors (Transformation|GetWorldLocation (Variables|/Script/Engine.Actor|GetRootComponent (.hitactor Hit))) (Variables|Default|GetSphere%20Radius) (Utilities|Array|MakeArray "ObjectTypeQuery3") 0))
  (if _returnvalue
    (for _array_element _outactors
      (Utilities|FlowControl|Sequence
        (:then_0
          (bind _asbp_main_base (Utilities|Casting|CastToBP_MainBase (Game|GetPlayerCharacter 0)))
          (bind _output_get (Variables|/Game/Proto/Main/Blueprint/BP_MainBase.BP_MainBase_C|SetIdentifiedTarget_BolasExplosion _asbp_main_base (Variables|Default|GetHit%20Actor)))
          (Development|PrintString (Utilities|GetDisplayName _output_get)))
        (:then_1
          ;[1 0.1078 0] Need identification pour bp main base
          (Utilities|IsValid (Variables|Default|GetHit%20Actor)
            (:Is%20Valid
              (bind _asbp_papillon (Utilities|Casting|CastToBP_Papillon (Variables|Default|GetHit%20Actor)))
              (Default|SpawnBolasT _asbp_papillon)
              (Actor|DestroyActor :!label _label))))
        (:then_2
          (Utilities|IsValid (Variables|Default|GetHit%20Actor)
            (:Is%20Valid
              (bind _astzitzimine (Utilities|Casting|CastToTzitzimine (Variables|Default|GetHit%20Actor)))
              (Default|SpawnBolasT _astzitzimine)
              (goto _label))))
        (:then_3
          (Utilities|IsValid (Variables|Default|GetHit%20Actor)
            (:Is%20Valid
              (Utilities|Casting|CastToBP_MainBase (Variables|Default|GetHit%20Actor))
              (CallFunction|HitCollisionFalse))))))))

(event Custom|AfterExplosion
  ;[1 1 1] Step 1 Bis : Does not hit + return to player
  (Variables|/Game/Proto/Main/Blueprint/Save_BFL_GameInstance/BloodTrial_GameInstance.BloodTrial_GameInstance_C|SetCanThrowBolas? (CallFunction|GetInst) true)
  (Actor|DestroyActor))

(event Custom|HitCollisionFalse
  (bind _returnvalue (Game|GetPlayerCharacter 0))
  (bind _capsulecomponent (Variables|/Script/Engine.Character|GetCapsuleComponent _returnvalue))
  (bind _returnvalue_2 (Transformation|GetWorldLocation _capsulecomponent))
  ;[1 1 1] Step 1 Bis : Does not hit + return to player
  (Collision|SetCollisionEnabled (Variables|Default|GetStaticMesh) "QueryAndPhysics")
  (Components|MoveComponentTo (Variables|Default|GetStaticMesh) (Math|Vector|MakeVector (.x _returnvalue_2) (.y _returnvalue_2) (+ (.z _returnvalue_2) 1e+02)) "0, 0, 0" true true 0.0 true)
  (Variables|/Game/Proto/Main/Blueprint/Save_BFL_GameInstance/BloodTrial_GameInstance.BloodTrial_GameInstance_C|SetCanThrowBolas? (CallFunction|GetInst) true)
  (Actor|DestroyActor))

(event EventBeginPlay
  (Audio|PlaySound2D "/Game/Proto/Rework_All_Project/SoundFX/Sfx/Sword.Sword" 1.0 (Math|Random|RandomFloatinRange 0.7 1.0) 0.0 0 0)
  (Utilities|FlowControl|Delay 3.0)
  (CallFunction|HitCollisionFalse))

(fn ConstructionScript)

(fn ApplyDamage
  (params (DamagedActor :type Actor%20Object%20Reference))
  (Game|Damage|ApplyDamage DamagedActor (Variables|/Game/Proto/Main/Blueprint/Save_BFL_GameInstance/BloodTrial_GameInstance.BloodTrial_GameInstance_C|GetDamageBolas (CallFunction|GetInst)) 0 0))