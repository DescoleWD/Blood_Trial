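; BP_WaveManager is a prototype manager for enemy waves, with much of its logic left disconnected.
; A looping timer counts down to BeginWave, and a half-second polling loop checks CurrentEnemies for valid actors, incrementing WaveNumber and restarting the countdown when none remain.
; BeginPlay, BeginWave and SpawnEnemies are empty entry points.
; Their apparent logic (spawn-point sorting by type, data-table wave lookup, AI spawning, starting the check) sits in unreachable nodes.
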(event Custom|StartCountdown
  ;[1 1 1] Countdown
  (bind _returnvalue (Utilities|Time|SetTimerbyEvent (delegate Custom|Count) 1.0 true))
  (Variables|Default|SetTime 3))

(event Custom|Count
  ;[1 1 1] Countdown
  (Development|PrintString (Utilities|String|ToString(Integer) (Variables|Default|GetTime)) true true "(R=0.023731,G=0.000000,B=0.473958,A=1.000000)")
  (if (== (Variables|Default|GetTime) 0)
    (Utilities|Time|ClearandInvalidateTimerbyHandle (stale Custom|StartCountdown _returnvalue))
    (CallFunction|BeginWave)
    (else
      (Math|Integer|DecrementInt (Variables|Default|GetTime)))))

(event Custom|BeginWave
  ;[1 1 1] Spawn Enemies for wave
)

(event Custom|StartCheckingIfEnemiesAreDead
  ;[1 1 1] Check if enemies are dead and start new wave
  (bind _aredead_1 (CallFunction|CheckifAllEnemiesAreDead :!label _label))
  (if _aredead_1
    (Audio|SpawnSound2D "/Game/StarterContent/Audio/Fire01.Fire01" 1.0 1.0 0.0 0)
    (Math|Integer|IncrementInt (Variables|Default|GetWaveNumber)
      (:%20%20
        (CallFunction|StartCountdown)))
    (else
      (Utilities|FlowControl|Delay 0.5)
      (goto _label))))

(event EventBeginPlay)

(fn ConstructionScript)

(fn SpawnEnemies
  (params (Struct_EnemyInfo :type %20Structure%20%28by%20ref%29)))

(fn CheckifAllEnemiesAreDead
  (LocalVariables|SetAreDead? true)
  (for _array_element (Variables|Default|GetCurrentEnemies)
    (Utilities|IsValid _array_element
      (:Is%20Valid
        (LocalVariables|SetAreDead? false))))
  (return (LocalVariables|GetAreDead?)))