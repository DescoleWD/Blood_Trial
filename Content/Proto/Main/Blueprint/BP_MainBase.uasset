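; Main player character Blueprint handling movement, combat, health, checkpoint respawn, HUD, game timer and lever/wall interactions.
; Combo montages and damage use server-to-multicast events, with weapon sphere traces and box traces for hits.
; Game Instance stores health and counters, and its Sacrifice flags gate dash, hurricane, bolas detonation, blood wave and vampirism.
; Camera-to-player sphere traces drive timeline-animated material parameters to cull tagged occluding walls.
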(event Custom|TestPlayerGuillaume
  (bind _charactermovement (Variables|Character|GetCharacterMovement))
  ;[1 1 1] Setting up starting Weapon
  (Components|StaticMesh|SetStaticMesh (Variables|Default|GetPrimaryWeaponMesh) (.WeaponMesh1 (Utilities|Struct|BreakS_WeaponsDetails (Variables|Default|GetPrimaryWeapon))))
  (Transformation|AttachComponentToComponent (Variables|Default|GetPrimaryWeaponMesh) (Variables|Character|GetMesh) "hand_r" "SnapToTarget" "SnapToTarget" "SnapToTarget" true)
  ;[1 1 1] Orient rotation
  (Variables|/Script/Engine.CharacterMovementComponent|SetbUseControllerDesiredRotation _charactermovement true)
  (Variables|/Script/Engine.CharacterMovementComponent|SetbOrientRotationToMovement _charactermovement true))

(event Custom|Create_Abilities_Widget
  ;[0.2362 1 0] Code Globale
  ;;[1 1 1] Create widget abilities + Timer + score
  ;;;[0.173 1 0] 1
  (bind _returnvalue (UserInterface|CreateWidget "/Game/Proto/Main/HUD/Abilities.Abilities_C"))
  (UserInterface|Viewport|AddtoViewport _returnvalue 0))

(event Custom|CalendarReceived
  ;[0.2362 1 0] Code Globale
  ;;[1 1 1] Create widget abilities + Timer + score
  ;;;[1 0.7891 0] 3
  (Default|Collection (stale Custom|Create_Score_Widget _output_get)))

(event Custom|Timeline_Timer
  (bind _asblood_trial_game_instance (CallFunction|GetInst))
  ;[0.2362 1 0] Code Globale
  ;;[1 1 1] Create widget abilities + Timer + score
  ;;;[1 0.0313 0] 4
  (Variables|/Game/Proto/Main/Blueprint/Save_BFL_GameInstance/BloodTrial_GameInstance.BloodTrial_GameInstance_C|SetTotalTime _asblood_trial_game_instance (+ (Variables|/Game/Proto/Main/Blueprint/Save_BFL_GameInstance/BloodTrial_GameInstance.BloodTrial_GameInstance_C|GetGlobalTime _asblood_trial_game_instance) (Variables|/Game/Proto/Main/Blueprint/Save_BFL_GameInstance/BloodTrial_GameInstance.BloodTrial_GameInstance_C|GetTotalTime _asblood_trial_game_instance)))
  (bind _newtrack_0 (Timeline|Timeline_0 Play)
    (:Update
      (Variables|/Game/Proto/Main/Blueprint/Save_BFL_GameInstance/BloodTrial_GameInstance.BloodTrial_GameInstance_C|SetGlobalTime (CallFunction|GetInst) _newtrack_0))))

(event Custom|Start_Custom_Tick
  ;[0.2362 1 0] Code Globale
  ;;[1 0 0.07711] 5
  (CallFunction|EventTickCustom :!label _label)
  (Utilities|FlowControl|Delay 0.01)
  (goto _label))

(event Custom|NearTheLever
  (params (nearLever :type Actor%20Object%20Reference))
  ;[1 0 0.01425] Rework
  ;;[1 0 0.03767] Rope Code : a mieux faire
  (Variables|Code|SetActor_Ref nearLever))

(event Custom|Cut_with_Attack_1
  ;[1 0 0.01425] Rework
  ;;[1 0 0.03767] Rope Code : a mieux faire
  (if (!= (Variables|Code|GetActor_Ref) 0)
    (Default|LeverActive (.AsBP%20Rope%20Able (Utilities|Casting|CastToBP_RopeAble (Variables|Code|GetActor_Ref))))))

(event Custom|Create_Score_Widget
  ;[0.2362 1 0] Code Globale
  ;;[1 1 1] Create widget abilities + Timer + score
  ;;;[1 0.7891 0] 3
  (bind _returnvalue (UserInterface|CreateWidget "/Game/Proto/Main/HUD/Score.Score_C"))
  (UserInterface|Viewport|AddtoViewport _returnvalue 1)
  (bind _output_get (Variables|Score|SetAs_Score _returnvalue)))

(event Custom|MultiCast_EquipWeapon
  (params (NewMesh :type Static%20Mesh%20Object%20Reference))
  (Components|StaticMesh|SetStaticMesh (Variables|Default|GetPrimaryWeaponMesh) NewMesh)
  (Transformation|AttachComponentToComponent (Variables|Default|GetPrimaryWeaponMesh) (Variables|Character|GetMesh) "hand_r" "SnapToTarget" "SnapToTarget" "SnapToTarget" true))

(event Custom|Cut_With_Attack_2
  ;[1 0 0.01425] Rework
  ;;[1 0 0.03767] Rope Code : a mieux faire
  (if (!= (Variables|Code|GetNear%20Wall) 0)
    (Default|WallDestroy (.AsBP%20Wall%20Destroy (Utilities|Casting|CastToBP_WallDestroy (Variables|Code|GetNear%20Wall))))))

(event Custom|NearTheWall
  (params (NearWall :type Actor%20Object%20Reference))
  ;[1 0 0.01425] Rework
  ;;[1 0 0.03767] Rope Code : a mieux faire
  (Variables|Code|SetNear%20Wall NearWall))

(event Custom|Server_EquipWeapon
  (params (NewMesh :type Static%20Mesh%20Object%20Reference))
  (CallFunction|MultiCastEquipWeapon NewMesh))

(event EventBeginPlay
  ;[0.2362 1 0] Code Globale
  ;;[1 1 1] Create widget abilities + Timer + score
  (Utilities|FlowControl|Sequence
    (:then_0
      (CallFunction|TestPlayerGuillaume))
    (:then_1
      ;;;[0 1 0.08258] 1
      (CallFunction|CreateAbilitiesWidget)
      ;;;[0.4924 1 0] 2
      (CallFunction|CreateHPBarPlayerWidget)
      (CallFunction|SetProgressBar)
      (CallFunction|SetProgressBarPercent 1.0)
      ;;;[1 0.8181 0] 3
      (CallFunction|CreateScoreWidget))
    (:then_2
      ;;;[1 0 0.01027] 4
      (CallFunction|TimelineTimer))
    (:then_3
      ;;;;[1 0 0.1127] 5
      (CallFunction|StartCustomTick))))

(event EventMovement
  (params (On%20/%20Off :type Boolean))
  (Variables|Character|SetMovementOn On%20/%20Off))

(event Input|AxisEvents|InputAxisMoveForward
  (params (AxisValue :type Float%20%28single-precision%29))
  ;[0.707 1 0] Character movement
  (if (>= (Math|Float|Absolute(Float) (* AxisValue 1e+01)) 1.0)
    (if (Variables|Character|GetMovementOn)
      (Pawn|Input|AddMovementInput (Class|PawnMovementComponent|GetPawnOwner (Variables|Character|GetCharacterMovement)) "1000.000000,-1000.000000, 0" AxisValue false))))

(event Input|AxisEvents|InputAxisMoveBackward
  (params (AxisValue :type Float%20%28single-precision%29))
  ;[0.707 1 0] Character movement
  (if (>= (Math|Float|Absolute(Float) (* AxisValue 1e+01)) 1.0)
    (if (Variables|Character|GetMovementOn)
      (Pawn|Input|AddMovementInput (Class|PawnMovementComponent|GetPawnOwner (Variables|Character|GetCharacterMovement)) "1000.000000,-1000.000000, 0" AxisValue false))))

(event Input|AxisEvents|InputAxisMoveLeft
  (params (AxisValue :type Float%20%28single-precision%29))
  ;[0.707 1 0] Character movement
  (if (>= (Math|Float|Absolute(Float) (* AxisValue 1e+01)) 1.0)
    (if (Variables|Character|GetMovementOn)
      (Pawn|Input|AddMovementInput (Class|PawnMovementComponent|GetPawnOwner (Variables|Character|GetCharacterMovement)) "1000.000000,1000.000000, 0" AxisValue false))))

(event Input|AxisEvents|InputAxisMoveRight
  (params (AxisValue :type Float%20%28single-precision%29))
  ;[0.707 1 0] Character movement
  (if (>= (Math|Float|Absolute(Float) (* AxisValue 1e+01)) 1.0)
    (if (Variables|Character|GetMovementOn)
      (Pawn|Input|AddMovementInput (Class|PawnMovementComponent|GetPawnOwner (Variables|Character|GetCharacterMovement)) "1000.000000,1000.000000, 0" AxisValue false))))

(event Custom|ServerAttack
  (params (Attack1 :type Anim%20Montage%20Object%20Reference) (Attack2 :type Anim%20Montage%20Object%20Reference) (Attack3 :type Anim%20Montage%20Object%20Reference) (Attack4 :type Anim%20Montage%20Object%20Reference) (MaxCombo :type Integer))
  ;[1 1 1] Attack
  (CallFunction|MultiCastAttack Attack1 Attack2 Attack3 Attack4 MaxCombo))

(event Custom|MultiCast_Attack
  (params (Attack1 :type Anim%20Montage%20Object%20Reference) (Attack2 :type Anim%20Montage%20Object%20Reference) (Attack3 :type Anim%20Montage%20Object%20Reference) (Attack4 :type Anim%20Montage%20Object%20Reference) (MaxComboAmount :type Integer))
  ;[1 1 1] Attack
  (Animation|PlayAnimMontage (Utilities|Select :Index (Math|Integer|%(Integer) (Variables|Default|GetComboCount) MaxComboAmount) :Option%200 Attack1 :Option%201 Attack2 :Option%202 Attack3 :Option%203 Attack4) 1.0 "None")
  (Math|Integer|IncrementInt (Variables|Default|GetComboCount)))

(event Custom|Server_TakeDamageAnim
  ;[1 1 1] Damage
  (CallFunction|MCTakesDamageAnim))

(event Custom|MC_TakesDamageAnim
  ;[1 1 1] Damage
  (bind _returnvalue (Animation|PlayAnimMontage "/Game/Proto/Animation/MainChara/attacks/Bolas/MainCharacter_BolasCast_Montage.MainCharacter_BolasCast_Montage" 1.0 "None"))
  (Development|PrintString (Utilities|String|ToString(Float) _returnvalue)))

(event Custom|WeaponTrace
  (bind _primaryweaponmesh (Variables|Default|GetPrimaryWeaponMesh))
  ;[1 1 1] Weapon Trace for hit
  (if (Variables|Default|GetWeaponTraceOn?) :!label _label
    (bind _outhit (Collision|SphereTraceByChannel (Transformation|GetSocketLocation _primaryweaponmesh "TopSocket") (Transformation|GetSocketLocation _primaryweaponmesh "BottomSpcket") 15.0 "TraceTypeQuery1" false 0 "ForDuration"))
    (bind _asmaster_enemy (Utilities|Casting|CastToMaster_Enemy (.HitActor (Collision|BreakHitResult _outhit)))
      (:then
        (if (not (Utilities|Array|ContainsItem (Variables|Default|GetAlreadyDamagedEnemies) _asmaster_enemy))
          (CallFunction|ServerApplyDamagetoAI _asmaster_enemy (.Damage (Utilities|Struct|BreakS_WeaponsDetails (Variables|Default|GetPrimaryWeapon))) (Game|GetPlayerController 0) self)
          (Utilities|Array|Add (Variables|Default|GetAlreadyDamagedEnemies) _asmaster_enemy)
          (Utilities|FlowControl|Delay 0.01 :!label _label_2)
          (goto _label)))
      (:CastFailed
        (goto _label_2)))))

(event Custom|MC_ApplyDamageToAI
  (params (DamagedActor :type Actor%20Object%20Reference) (BaseDamage :type Float%20%28single-precision%29) (EventInstigator :type Controller%20Object%20Reference) (DamageCauser :type Actor%20Object%20Reference))
  ;[1 1 1] Apply Damage
  (Game|Damage|ApplyDamage DamagedActor BaseDamage EventInstigator DamageCauser))

(event Custom|Server_ApplyDamageToAI
  (params (DamagedActor :type Actor%20Object%20Reference) (BaseDamage :type Float%20%28single-precision%29) (EventInstigator :type Controller%20Object%20Reference) (DamageCauser :type Actor%20Object%20Reference))
  ;[1 1 1] Apply Damage
  (CallFunction|MCApplyDamagetoAI DamagedActor BaseDamage EventInstigator DamageCauser))

(event Input|ActionEvents|InputActionBasicAttack
  (params (Key :type Key%20Structure :default "None"))
  (bind _primaryweapon (Variables|Default|GetPrimaryWeapon))
  (bind (_weaponmesh1 _attack1 _attack2 _attack3 _attack4 _handsocket _maxcomboamount) (Utilities|Struct|BreakS_WeaponsDetails _primaryweapon))
  ;[1 1 1] Attack
  (:Pressed
    (if (not (Variables|Character|GetIsAttacking))
      (CallFunction|ServerAttack _attack1 _attack2 _attack3 _attack4 _maxcomboamount))))

(event Input|KeyboardEvents|Add
  (params (Key :type Key%20Structure :default "None"))
  ;[1 1 1] Damage
  (:Pressed
    (bind _returnvalue (Animation|PlayAnimMontage "/Game/Proto/Animation/MainChara/attacks/Bolas/MainCharacter_BolasCast_Montage.MainCharacter_BolasCast_Montage" 1.0 "None"))
    (Development|PrintString (Utilities|String|ToString(Float) _returnvalue))))

(event EventTick
  (params (DeltaSeconds :type Float%20%28single-precision%29))
  (bind _value (Variables|shader|GetValue))
  ;[0.01042 0.000728 0] ShaderCullingWall
  (bind _output_get (Variables|shader|SetPlayerPos (Transformation|GetWorldLocation (Variables|Character|GetMesh))))
  (bind _output_get_2 (Variables|shader|SetCamPos (Transformation|GetWorldLocation (Variables|Camera|GetCamera))))
  (bind (_outhit _returnvalue) (Collision|SphereTraceByChannel _output_get_2 _output_get 2.5e+02 "TraceTypeQuery1" false 0 "None"))
  (Utilities|IsValid 0
    (:Is%20Valid
      (if (and _returnvalue (Actor|ActorHasTag (.hitactor _outhit) "shaderEnable"))
        (bind _outhits (Collision|MultiSphereTraceByChannel (Variables|shader|GetCamPos) (Variables|shader|GetPlayerPos) (Math|Float|Clamp(Float) (Variables|shader|Getradius) 2.5e+02 (Variables|shader|Getradius)) "TraceTypeQuery3" false 0 "None" true "(R=1.000000,G=0.000000,B=0.000000,A=1.000000)" "(R=0.000000,G=1.000000,B=0.000000,A=1.000000)" 0.2))
        (for _array_element _outhits
          (if (Actor|ActorHasTag (.HitActor (Collision|BreakHitResult _array_element)) "shaderEnable")
            (if (== (Rendering|Material|GetNumMaterials (.HitComponent (Collision|BreakHitResult _array_element))) 1)
              (bind _returnvalue_2 (Rendering|Material|CreateDynamicMaterialInstance (.HitComponent (Collision|BreakHitResult _array_element)) 0 (Rendering|Material|GetMaterial (.HitComponent (Collision|BreakHitResult _array_element)) 0) "None" :!class /Script/Engine.PrimitiveComponent))
              (Rendering|Material|SetScalarParameterValue _returnvalue_2 "value" _value :!class /Script/Engine.MaterialInstanceDynamic)
              (bind _radiuscurv (Timeline|Timeline_1 Play)
                (:Update
                  (bind _output_get_3 (Variables|shader|Setradius (* _radiuscurv 8e+02)))
                  (Rendering|Material|SetScalarParameterValue "/Game/TA/Assets/Shader/MatrialFuction/ShaderCulling.ShaderCulling" "radius" _output_get_3 :!class /Script/Engine.KismetMaterialLibrary)))
              (else
                (for _index (range 0 1)
                  (bind _returnvalue_3 (Rendering|Material|CreateDynamicMaterialInstance (.HitComponent (Collision|BreakHitResult _array_element)) _index (Rendering|Material|GetMaterial (.HitComponent (Collision|BreakHitResult _array_element)) _index) "None" :!class /Script/Engine.PrimitiveComponent))
                  (Rendering|Material|SetScalarParameterValue _returnvalue_3 "value" _value :!class /Script/Engine.MaterialInstanceDynamic)
                  (Timeline|Timeline_1 Play))))))
        (else
          (Timeline|Timeline_1 Reverse))))))

(event Input|ActionEvents|InputActionSpecialAttack
  (params (Key :type Key%20Structure))
  (bind _asblood_trial_game_instance (CallFunction|GetInst))
  (bind _sacrifice_2 (Variables|/Game/Proto/Main/Blueprint/Save_BFL_GameInstance/BloodTrial_GameInstance.BloodTrial_GameInstance_C|GetSacrifice_2 _asblood_trial_game_instance))
  ;[1 0 0.5512] Bolas V2
  ;;[0.1691 1 0] Step 1 : Action input Bolas
  (:Pressed
    ;;[0.1949 1 0] Step 2 : Vérifier que le Bolas n'est pas déjà lancé
    (if (Variables|/Game/Proto/Main/Blueprint/Save_BFL_GameInstance/BloodTrial_GameInstance.BloodTrial_GameInstance_C|GetThrowBolas _asblood_trial_game_instance)
      ;;[0.1303 1 0] Step 3 : Si pas lancé ==> lancer le Bolas
      (Variables|/Game/Proto/Main/Blueprint/Save_BFL_GameInstance/BloodTrial_GameInstance.BloodTrial_GameInstance_C|SetThrowBolas (CallFunction|GetInst) false)
      (Bolas|ThrowBolas)
      (else
        ;;[0.1856 1 0] Step 4 : Le bolas est il attaché ?
        (if (Variables|/Game/Proto/Main/Blueprint/Save_BFL_GameInstance/BloodTrial_GameInstance.BloodTrial_GameInstance_C|GetBolas_Attache _asblood_trial_game_instance)
          ;;[0.1565 1 0] Step 6 : Si attaché sur un ennemi, alors déclenché l'explosion
          (if _sacrifice_2
            (Utilities|FlowControl|Sequence
              (:then_0
                (bind _returnvalue (Actor|GetActorOfClass "/Game/Proto/Proto_Guillaume/Blueprints/Enemy/IA_V2/Distance/Distance.Distance_C"))
                (Default|ExplosionD _returnvalue))
              (:then_1
                (bind _returnvalue_2 (Actor|GetActorOfClass "/Game/Proto/Proto_Guillaume/Blueprints/Enemy/IA_V2/Melee/Melee.Melee_C"))
                (Default|ExplosionM _returnvalue_2))))
          (else
            ;;[0.2834 1 0] Step 5 : Si pas attaché pas 2ème input alors le bolas explose
            (if _sacrifice_2
              (bind _returnvalue_3 (Actor|GetActorOfClass "/Game/Proto/Proto_Florian/Blueprints/BP_Bolas.BP_Bolas_C"))
              (Default|ExplosionSubtile _returnvalue_3))))))))

(event Input|ActionEvents|InputActionDash
  (params (Key :type Key%20Structure))
  (bind _asblood_trial_game_instance (CallFunction|GetInst))
  (bind _charactermovement (Variables|Character|GetCharacterMovement))
  (bind _returnvalue (Pawn|Components|PawnMovement|GetLastInputVector _charactermovement))
  (bind _returnvalue_2 (* _returnvalue 2.0))
  ;[1 0 0.7685] Dash + besoin anim / SFX/VFX
  (:Pressed
    (if (Variables|/Game/Proto/Main/Blueprint/Save_BFL_GameInstance/BloodTrial_GameInstance.BloodTrial_GameInstance_C|GetSacrifice_1 _asblood_trial_game_instance)
      (if (< (Variables|/Game/Proto/Main/Blueprint/Save_BFL_GameInstance/BloodTrial_GameInstance.BloodTrial_GameInstance_C|GetNB_Dash _asblood_trial_game_instance) (Variables|/Game/Proto/Main/Blueprint/Save_BFL_GameInstance/BloodTrial_GameInstance.BloodTrial_GameInstance_C|GetMaxDash _asblood_trial_game_instance))
        (Collision|SetCollisionResponsetoChannel (Variables|Collision|GetCapsuleComponent) "ECC_Pawn" "ECR_Ignore")
        (Variables|/Game/Proto/Main/Blueprint/Save_BFL_GameInstance/BloodTrial_GameInstance.BloodTrial_GameInstance_C|SetNB_Dash _asblood_trial_game_instance (+ (Variables|/Game/Proto/Main/Blueprint/Save_BFL_GameInstance/BloodTrial_GameInstance.BloodTrial_GameInstance_C|GetNB_Dash _asblood_trial_game_instance) 1))
        (Character|LaunchCharacter (Math|Vector|MakeVector (.x _returnvalue_2) (.y _returnvalue_2) 0.0) false false)
        (Hurricane|CheckUpHurricane)
        (Utilities|FlowControl|Delay 0.5)
        (Collision|SetCollisionResponsetoChannel (Variables|Collision|GetCapsuleComponent) "ECC_WorldDynamic" "ECR_Block")
        (Collision|SetCollisionResponsetoChannel (Variables|Collision|GetCapsuleComponent) "ECC_Pawn" "ECR_Block")
        (Utilities|FlowControl|Delay 1.0)
        (Variables|/Game/Proto/Main/Blueprint/Save_BFL_GameInstance/BloodTrial_GameInstance.BloodTrial_GameInstance_C|SetNB_Dash (CallFunction|GetInst) 0)
        (Class|NavMovementComponent|StopMovementKeepPathing (Variables|Character|GetCharacterMovement))
        (else
          (Utilities|FlowControl|Delay 1.0)
          (Variables|/Game/Proto/Main/Blueprint/Save_BFL_GameInstance/BloodTrial_GameInstance.BloodTrial_GameInstance_C|SetNB_Dash _asblood_trial_game_instance 0))))))

(event Custom|Event%20Tick%20Custom
  (Utilities|IsValid (stale Input|ActionEvents|InputActionHurricane _returnvalue)
    (:Is%20Valid
      (Transformation|SetActorRelativeLocation (stale Input|ActionEvents|InputActionHurricane _returnvalue) (Math|Interpolation|VInterpTo (Transformation|GetActorLocation) (Transformation|GetActorLocation (Game|GetPlayerCharacter 0)) (Utilities|Time|GetWorldDeltaSeconds) 3e+02))
      (Utilities|FlowControl|Delay 2.0)
      (Actor|DestroyActor (stale Input|ActionEvents|InputActionHurricane _returnvalue))
      (Utilities|FlowControl|Delay 0.1)
      (Utilities|FlowControl|DoOnce false) ; enters at Reset
    )))

(event Input|ActionEvents|InputActionHurricane
  (params (Key :type Key%20Structure))
  (:Pressed
    (if (Variables|/Game/Proto/Main/Blueprint/Save_BFL_GameInstance/BloodTrial_GameInstance.BloodTrial_GameInstance_C|GetSacrifice_4 (CallFunction|GetInst))
      (Utilities|IsValid (stale _returnvalue)
        (:Is%20Not%20Valid
          (Utilities|FlowControl|DoOnce false :!label _label
            (:Completed
              (bind _returnvalue (Game|SpawnActorfromClass "/Game/Proto/Proto_Florian/Blueprints/BP_Hurricane.BP_Hurricane_C" (Math|Transform|MakeTransform (Transformation|GetWorldLocation (Variables|Default|GetSpawnHurricane)) (Class|CharacterMovementComponent|GetLastUpdateRotation (Variables|Character|GetCharacterMovement))) "Undefined" 0 0))
              (Transformation|SetActorRelativeLocation _returnvalue (Math|Interpolation|VInterpTo (Transformation|GetActorLocation) (Transformation|GetActorLocation (Game|GetPlayerCharacter 0)) (Utilities|Time|GetWorldDeltaSeconds) 3e+02))
              (Utilities|FlowControl|Delay 2.0)
              (Actor|DestroyActor _returnvalue)
              (Utilities|FlowControl|Delay 0.1)
              (goto _label Reset))))))))

(event Custom|Respawn
  (bind _asblood_trial_game_instance (CallFunction|GetInst))
  (bind _check_rotation (Variables|/Game/Proto/Main/Blueprint/Save_BFL_GameInstance/BloodTrial_GameInstance.BloodTrial_GameInstance_C|GetCheck_Rotation _asblood_trial_game_instance))
  ;[0 1 0.007329] Respawn
  (Input|DisableInput (Game|GetPlayerController 0))
  (Utilities|FlowControl|Delay 0.2)
  (Utilities|FlowControl|Delay 0.4)
  (Transformation|SetActorTransform (Math|Transform|MakeTransform (Variables|/Game/Proto/Main/Blueprint/Save_BFL_GameInstance/BloodTrial_GameInstance.BloodTrial_GameInstance_C|GetCheck_Location _asblood_trial_game_instance) _check_rotation "1.000000,1.000000,1.000000"))
  (Pawn|SetControlRotation (Game|GetPlayerController 0) _check_rotation)
  (Pawn|Components|CharacterMovement|DisableMovement (Variables|Character|GetCharacterMovement))
  (Utilities|FlowControl|Delay 1.0)
  (Pawn|Components|CharacterMovement|SetMovementMode (Variables|Character|GetCharacterMovement) "MOVE_Walking" 0)
  (Input|EnableInput (Game|GetPlayerController 0)))

(event Custom|Vampirisme_On_Death
  (bind _asblood_trial_game_instance (CallFunction|GetInst))
  (bind _asblood_trial_game_instance_2 (CallFunction|GetInst))
  ;[0.08068 1 0] Vampirisme
  (if (<= (Variables|/Game/Proto/Main/Blueprint/Save_BFL_GameInstance/BloodTrial_GameInstance.BloodTrial_GameInstance_C|GetChoose_Life _asblood_trial_game_instance) (Variables|/Game/Proto/Main/Blueprint/Save_BFL_GameInstance/BloodTrial_GameInstance.BloodTrial_GameInstance_C|GetMaxLife _asblood_trial_game_instance))
    (Variables|/Game/Proto/Main/Blueprint/Save_BFL_GameInstance/BloodTrial_GameInstance.BloodTrial_GameInstance_C|SetChoose_Life _asblood_trial_game_instance_2 (+ (Variables|/Game/Proto/Main/Blueprint/Save_BFL_GameInstance/BloodTrial_GameInstance.BloodTrial_GameInstance_C|GetChoose_Life _asblood_trial_game_instance_2) 1e+02))))

(event Custom|Vampirisme
  (bind _asblood_trial_game_instance (CallFunction|GetInst))
  (bind _asblood_trial_game_instance_2 (CallFunction|GetInst))
  ;[0.08068 1 0] Vampirisme
  (if (<= (Variables|/Game/Proto/Main/Blueprint/Save_BFL_GameInstance/BloodTrial_GameInstance.BloodTrial_GameInstance_C|GetChoose_Life _asblood_trial_game_instance) (Variables|/Game/Proto/Main/Blueprint/Save_BFL_GameInstance/BloodTrial_GameInstance.BloodTrial_GameInstance_C|GetMaxLife _asblood_trial_game_instance))
    (Variables|/Game/Proto/Main/Blueprint/Save_BFL_GameInstance/BloodTrial_GameInstance.BloodTrial_GameInstance_C|SetChoose_Life _asblood_trial_game_instance_2 (+ (Variables|/Game/Proto/Main/Blueprint/Save_BFL_GameInstance/BloodTrial_GameInstance.BloodTrial_GameInstance_C|GetChoose_Life _asblood_trial_game_instance_2) 2.0))))

(event Custom|setProgressBarPercent
  (params (InPercent :type Float%20%28double-precision%29))
  ;[1 1 1] Set le percent des HP
  (Default|SetPercentage (Variables|Default|GetProgressBarRef) InPercent))

(event Custom|CreateHPBarPlayerWidget
  ;[1 1 1] Initialise hp bar
  (bind _returnvalue (UserInterface|CreateWidget "/Game/Proto/Proto_Guillaume/Blueprints/Player/HP_Bar_Player.HP_Bar_Player_C" (Game|GetPlayerController 0)))
  (bind _output_get (Variables|Default|SetProgressBarRef _returnvalue))
  (Utilities|IsValid _output_get
    (:Is%20Valid
      (UserInterface|Viewport|AddtoViewport _returnvalue 0))))

(event Game|Damage|EventAnyDamage
  (params (Damage :type Float%20%28single-precision%29) (DamageType :type Damage%20Type%20Object%20Reference) (InstigatedBy :type Controller%20Object%20Reference) (DamageCauser :type Actor%20Object%20Reference))
  ;[1 1 1] Je bloque ?
  (if (not (Variables|Code|GetBlocking))
    ;[1 1 1] Prend ses damages
    (bind _output_get (CallFunction|PlayerTakesDamage Damage))
    (CallFunction|SetProgressBarPercent (Math|Float|SafeDivide _output_get (Variables|/Game/Proto/Main/Blueprint/Save_BFL_GameInstance/BloodTrial_GameInstance.BloodTrial_GameInstance_C|GetMaxLife (CallFunction|GetInst))))
    (Math|Float|CompareFloat (Math|Float|SafeDivide _output_get (Variables|/Game/Proto/Main/Blueprint/Save_BFL_GameInstance/BloodTrial_GameInstance.BloodTrial_GameInstance_C|GetMaxLife (CallFunction|GetInst))) 0.0
      (:==
        _)
      (:<
        _))
    (Actor|DestroyActor)))

(fn ConstructionScript)

(fn SpawnBloodWaveBPPlayer
  (bind _charactermovement (Variables|Character|GetCharacterMovement))
  (bind _returnvalue (Class|CharacterMovementComponent|GetLastUpdateRotation _charactermovement))
  (if (Variables|/Game/Proto/Main/Blueprint/Save_BFL_GameInstance/BloodTrial_GameInstance.BloodTrial_GameInstance_C|GetSacrifice_2 (CallFunction|GetInst))
    (Game|SpawnActorfromClass "/Game/Proto/Proto_Florian/Blueprints/BP_Blood_Waves.BP_Blood_Waves_C" (Math|Transform|MakeTransform (+ (Transformation|GetWorldLocation (Variables|/Script/Engine.MovementComponent|GetUpdatedPrimitive _charactermovement)) (* (Math|Vector|GetForwardVector _returnvalue) 5e+01)) _returnvalue "0.500000,2.000000,1.000000") "AdjustIfPossibleButAlwaysSpawn" 0 0)))

(fn ThrowBolas
  (bind _spawnbolas (Variables|Default|GetSpawnBolas))
  (bind _charactermovement (Variables|Character|GetCharacterMovement))
  (bind _returnvalue (Transformation|GetWorldLocation _spawnbolas))
  (bind _returnvalue_2 (Class|CharacterMovementComponent|GetLastUpdateRotation _charactermovement))
  (bind _returnvalue_3 (Math|Transform|MakeTransform _returnvalue _returnvalue_2 "0.400000,0.400000,0.400000"))
  (bind _returnvalue_4 (Game|SpawnActorfromClass "/Game/Proto/Proto_Florian/Blueprints/BP_Bolas_Child.BP_Bolas_Child_C" (Math|Transform|MakeTransform (Math|Vector|MakeVector (.x (.location _returnvalue_3)) (.y (.location _returnvalue_3)) (.z (.location _returnvalue_3))) (.rotation _returnvalue_3) (.scale _returnvalue_3)) "AdjustIfPossibleButAlwaysSpawn" self 0))
  (Physics|AddImpulse (Variables|/Game/Proto/Proto_Florian/Blueprints/BP_Bolas.BP_Bolas_C|GetStaticMesh _returnvalue_4) (* (Math|Vector|GetForwardVector _spawnbolas) 3e+03) "None" true)
  (return _returnvalue_4))

(fn CheckUpThrowBolas
  (bind _asblood_trial_game_instance (CallFunction|GetInst))
  (if (< (Variables|/Game/Proto/Main/Blueprint/Save_BFL_GameInstance/BloodTrial_GameInstance.BloodTrial_GameInstance_C|GetCounterBolas _asblood_trial_game_instance) (Variables|/Game/Proto/Main/Blueprint/Save_BFL_GameInstance/BloodTrial_GameInstance.BloodTrial_GameInstance_C|GetMaxBolas _asblood_trial_game_instance))
    (bind _output_get (Variables|/Game/Proto/Main/Blueprint/Save_BFL_GameInstance/BloodTrial_GameInstance.BloodTrial_GameInstance_C|SetCounterBolas (CallFunction|GetInst) (+ (Variables|/Game/Proto/Main/Blueprint/Save_BFL_GameInstance/BloodTrial_GameInstance.BloodTrial_GameInstance_C|GetCounterBolas _asblood_trial_game_instance) 1)))
    (return _output_get)))

(fn CheckUpHurricane
  ;[1 1 1] Prbm a régler (is valid doit pas être nécessaire)
  (bind _returnvalue (Actor|GetActorOfClass "/Game/Proto/Proto_Florian/Blueprints/BP_Hurricane.BP_Hurricane_C"))
  (Utilities|IsValid _returnvalue
    (:Is%20Valid
      (Default|DashActive _returnvalue))))

(fn NotifyBegin)

(fn TriggerComplexeHit
  (bind _returnvalue (Transformation|GetActorLocation))
  (bind _returnvalue_2 (Transformation|GetActorForwardVector))
  (Utilities|FlowControl|DoOnce false :!label _label
    (:Completed
      (bind (_outhit _returnvalue_3) (Class|KismetSystemLibrary|BoxTraceSingleforObjects _returnvalue (+ _returnvalue (* _returnvalue_2 1.2e+02)) "100.000000,100.000000,50.000000" (Math|Conversions|RotationFromXVector _returnvalue_2) (Utilities|Array|MakeArray "ObjectTypeQuery3") true 0 "ForDuration" true "(R=1.000000,G=0.000000,B=0.000000,A=1.000000)" "(R=0.000000,G=1.000000,B=0.000000,A=1.000000)" 1.0))
      (if _returnvalue_3
        (if (Variables|/Script/Engine.Actor|GetbCanBeDamaged (.HitActor (Collision|BreakHitResult _outhit)))
          (Utilities|FlowControl|Sequence
            (:then_0
              (if (Variables|/Game/Proto/Main/Blueprint/Save_BFL_GameInstance/BloodTrial_GameInstance.BloodTrial_GameInstance_C|GetSacrifice_5 (CallFunction|GetInst))
                (CallFunction|Vampirisme)))
            (:then_1
              (Game|Damage|ApplyDamage (.HitActor (Collision|BreakHitResult _outhit)) (Variables|/Game/Proto/Main/Blueprint/Save_BFL_GameInstance/BloodTrial_GameInstance.BloodTrial_GameInstance_C|GetPlayerAttack (CallFunction|GetInst)) 0 (Variables|Character|GetPlayer))
              (goto _label Reset))))))))

(fn TriggerSimpleHit
  (bind _returnvalue (Transformation|GetActorLocation))
  (bind _returnvalue_2 (Transformation|GetActorForwardVector))
  (Class|KismetSystemLibrary|BoxTraceSingleforObjects _returnvalue (+ _returnvalue (* _returnvalue_2 1.2e+02)) "20.000000,100.000000,50.000000" (Math|Conversions|RotationFromXVector _returnvalue_2) (Utilities|Array|MakeArray "ObjectTypeQuery3") false 0 "None" true))

(fn PlayerTakesDamage
  (params (DamageTaken :type Float%20%28double-precision%29))
  (bind _asblood_trial_game_instance (CallFunction|GetInst))
  (bind _output_get (Variables|/Game/Proto/Main/Blueprint/Save_BFL_GameInstance/BloodTrial_GameInstance.BloodTrial_GameInstance_C|SetChoose_Life _asblood_trial_game_instance (- (Variables|/Game/Proto/Main/Blueprint/Save_BFL_GameInstance/BloodTrial_GameInstance.BloodTrial_GameInstance_C|GetChoose_Life _asblood_trial_game_instance) DamageTaken)))
  (CallFunction|ServerTakeDamageAnim)
  (Variables|Default|SetWeaponTraceOn? false)
  (Variables|Character|SetIsAttacking false)
  (return _output_get))

(fn SetProgressBar
  (bind _ashp_bar_player (Utilities|Casting|CastToHP_Bar_Player (UserInterface|GetUserWidgetObject (Variables|Default|GetWidget)))
    (:then
      (Variables|Default|SetProgressBarRef _ashp_bar_player))
    (:CastFailed
      _))
  (return))

(event EventAttackSway
  (params (Strenght :type Float%20%28double-precision%29))
  (Physics|AddImpulse (Variables|Character|GetCharacterMovement) (* (Math|Vector|GetForwardVector (Variables|Collision|GetCapsuleComponent)) Strenght) true))