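; BP_WallDestroy is a prototype destructible wall that breaks when WallDestroy is called while a BP_MainBase character is in range.
; Overlap on LeverCollider sets the collision flag, caches the character and registers the wall through NearTheWall.
; WallDestroy clears the character's NearWall, plays a sound and destroys the actor after a short delay.
; End overlap resets the flag and, if the wall is destroyed, clears the character's ActorRef.
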(event OnComponentBeginOverlap(LeverCollider)
  (params (OverlappedComponent :type Primitive%20Component%20Object%20Reference) (OtherActor :type Actor%20Object%20Reference) (OtherComp :type Primitive%20Component%20Object%20Reference) (OtherBodyIndex :type Integer) (bFromSweep :type Boolean) (SweepResult :type Hit%20Result%20Structure%20%28by%20ref%29))
  (bind _asbp_main_base (Utilities|Casting|CastToBP_MainBase OtherActor))
  (Variables|Default|SetAs%20BP%20Main%20Character _asbp_main_base)
  (Variables|Default|SetisCollision true)
  (Default|NeartheWall _asbp_main_base self))

(event OnComponentEndOverlap(LeverCollider)
  (params (OverlappedComponent :type Primitive%20Component%20Object%20Reference) (OtherActor :type Actor%20Object%20Reference) (OtherComp :type Primitive%20Component%20Object%20Reference) (OtherBodyIndex :type Integer))
  (Utilities|Casting|CastToBP_MainBase OtherActor)
  (Variables|Default|SetisCollision false)
  (if (Variables|Default|GetisDestroy)
    (Variables|/Game/Proto/Main/Blueprint/BP_MainBase.BP_MainBase_C|SetActor_Ref (Variables|Default|GetAs%20BP%20Main%20Character) 0)))

(event Custom|WallDestroy
  (if (Variables|Default|GetisCollision)
    (Variables|Default|SetisDestroy true)
    (Variables|/Game/Proto/Main/Blueprint/BP_MainBase.BP_MainBase_C|SetNear%20Wall (Variables|Default|GetAs%20BP%20Main%20Character) 0)
    (Audio|PlaySoundatLocation "/Game/Proto/Proto_Florian/SFX/SFX_DestructibleWall.SFX_DestructibleWall" (Transformation|GetActorLocation) "0, 0, 0" 1.0 1.0 0.0 0 0 0 0)
    (Utilities|FlowControl|Delay 0.2)
    (Actor|DestroyActor)))

(fn ConstructionScript)