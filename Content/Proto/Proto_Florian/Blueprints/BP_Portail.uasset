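; BP_Portail is a toothed gate that opens via Partie2, or on BeginPlay if the game instance's RopeCut flag is set.
; With BarrierAnim set, it blends the view to itself, plays a sound, then returns the camera and re-enables player input.
; Otherwise it opens without the cutscene.
; Timelines move upper teeth by OpenTop and lower teeth downward, lerping from current location each update, so offsets accumulate.
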(event Custom|Partie2
  (bind _returnvalue (Game|GetPlayerController 0))
  (bind _teeth_up (Variables|Default|GetTeeth_up))
  (bind _teeth_bottom (Variables|Default|GetTeeth_bottom))
  (bind _teeth_up_2 (Variables|Default|GetTeeth_up))
  (bind _teeth_bottom_2 (Variables|Default|GetTeeth_bottom))
  (bind _returnvalue_2 (Transformation|GetWorldLocation _teeth_bottom))
  (bind _returnvalue_3 (Transformation|GetWorldLocation _teeth_up))
  (bind _returnvalue_4 (Transformation|GetWorldLocation _teeth_up_2))
  (bind _returnvalue_5 (Transformation|GetWorldLocation _teeth_bottom_2))
  (if (Variables|/Game/Proto/Main/Blueprint/Save_BFL_GameInstance/BloodTrial_GameInstance.BloodTrial_GameInstance_C|GetBarrierAnim (CallFunction|GetInst))
    (Game|Player|SetViewTargetwithBlend _returnvalue self 2.0 "VTBlend_Linear" 0.0 false)
    (Utilities|FlowControl|Delay 3.0)
    (Audio|PlaySound2D "/Game/Proto/Main/SFX/EnviroSystem/Pressure_Door/DoorOpen.DoorOpen" 1.0 1.0 0.0 0 0)
    (Utilities|FlowControl|Sequence
      (:then_0
        (bind _newtrack_0 (Timeline|Timeline_1 Play)
          (:Update
            (Transformation|SetWorldLocation _teeth_up (Math|Vector|Lerp(Vector) _returnvalue_3 (+ _returnvalue_3 (Math|Vector|MakeVector 0.0 0.0 (Variables|Default|GetOpen_top))) _newtrack_0) false false))))
      (:then_1
        (bind _newtrack_0_2 (Timeline|Timeline_0 Play)
          (:Update
            (Transformation|SetWorldLocation _teeth_bottom (Math|Vector|Lerp(Vector) _returnvalue_2 (+ _returnvalue_2 "0.000000,0,-10.000000") _newtrack_0_2) false false))))
      (:then_2
        (Utilities|FlowControl|Delay 1.0)
        (Game|Player|SetViewTargetwithBlend _returnvalue (Components|GetOwner (Variables|/Game/Proto/Main/Blueprint/BP_MainBase.BP_MainBase_C|GetCamera (stale EventBeginPlay _asbp_main_base))) 2.0 "VTBlend_Linear" 0.0 false)
        (Input|EnableInput (Game|GetPlayerCharacter 0) 0)))
    (else
      (Utilities|FlowControl|Sequence
        (:then_0
          (bind _newtrack_0_3 (Timeline|Timeline_3 Play)
            (:Update
              _)
            (:Finished
              _))
          (Transformation|SetWorldLocation _teeth_up_2 (Math|Vector|Lerp(Vector) _returnvalue_4 (+ _returnvalue_4 (Math|Vector|MakeVector 0.0 0.0 (Variables|Default|GetOpen_top))) _newtrack_0_3) false false))
        (:then_1
          (bind _newtrack_0_4 (Timeline|Timeline_2 Play)
            (:Update
              _)
            (:Finished
              _))
          (Transformation|SetWorldLocation _teeth_bottom_2 (Math|Vector|Lerp(Vector) _returnvalue_5 (+ _returnvalue_5 "0.000000,0,-10.000000") _newtrack_0_4) false false))))))

(event EventBeginPlay
  (bind _asblood_trial_game_instance (CallFunction|GetInst))
  (bind _returnvalue (Game|GetPlayerController 0))
  (bind _teeth_up (Variables|Default|GetTeeth_up))
  (bind _teeth_bottom (Variables|Default|GetTeeth_bottom))
  (bind _teeth_up_2 (Variables|Default|GetTeeth_up))
  (bind _teeth_bottom_2 (Variables|Default|GetTeeth_bottom))
  (bind _returnvalue_2 (Transformation|GetWorldLocation _teeth_bottom))
  (bind _returnvalue_3 (Transformation|GetWorldLocation _teeth_up))
  (bind _returnvalue_4 (Transformation|GetWorldLocation _teeth_up_2))
  (bind _returnvalue_5 (Transformation|GetWorldLocation _teeth_bottom_2))
  (bind _asbp_main_base (Utilities|Casting|CastToBP_MainBase (Game|GetPlayerCharacter 0)))
  (if (Variables|/Game/Proto/Main/Blueprint/Save_BFL_GameInstance/BloodTrial_GameInstance.BloodTrial_GameInstance_C|GetRopeCut? _asblood_trial_game_instance)
    (if (Variables|/Game/Proto/Main/Blueprint/Save_BFL_GameInstance/BloodTrial_GameInstance.BloodTrial_GameInstance_C|GetBarrierAnim _asblood_trial_game_instance)
      (Game|Player|SetViewTargetwithBlend _returnvalue self 2.0 "VTBlend_Linear" 0.0 false)
      (Utilities|FlowControl|Delay 3.0)
      (Audio|PlaySound2D "/Game/Proto/Main/SFX/EnviroSystem/Pressure_Door/DoorOpen.DoorOpen" 1.0 1.0 0.0 0 0)
      (Utilities|FlowControl|Sequence
        (:then_0
          (bind _newtrack_0 (Timeline|Timeline_1 Play)
            (:Update
              (Transformation|SetWorldLocation _teeth_up (Math|Vector|Lerp(Vector) _returnvalue_3 (+ _returnvalue_3 (Math|Vector|MakeVector 0.0 0.0 (Variables|Default|GetOpen_top))) _newtrack_0) false false))))
        (:then_1
          (bind _newtrack_0_2 (Timeline|Timeline_0 Play)
            (:Update
              (Transformation|SetWorldLocation _teeth_bottom (Math|Vector|Lerp(Vector) _returnvalue_2 (+ _returnvalue_2 "0.000000,0,-10.000000") _newtrack_0_2) false false))))
        (:then_2
          (Utilities|FlowControl|Delay 1.0)
          (Game|Player|SetViewTargetwithBlend _returnvalue (Components|GetOwner (Variables|/Game/Proto/Main/Blueprint/BP_MainBase.BP_MainBase_C|GetCamera _asbp_main_base)) 2.0 "VTBlend_Linear" 0.0 false)
          (Input|EnableInput (Game|GetPlayerCharacter 0) 0)))
      (else
        (Utilities|FlowControl|Sequence
          (:then_0
            (bind _newtrack_0_3 (Timeline|Timeline_3 Play)
              (:Update
                _)
              (:Finished
                _))
            (Transformation|SetWorldLocation _teeth_up_2 (Math|Vector|Lerp(Vector) _returnvalue_4 (+ _returnvalue_4 (Math|Vector|MakeVector 0.0 0.0 (Variables|Default|GetOpen_top))) _newtrack_0_3) false false))
          (:then_1
            (bind _newtrack_0_4 (Timeline|Timeline_2 Play)
              (:Update
                _)
              (:Finished
                _))
            (Transformation|SetWorldLocation _teeth_bottom_2 (Math|Vector|Lerp(Vector) _returnvalue_5 (+ _returnvalue_5 "0.000000,0,-10.000000") _newtrack_0_4) false false)))))))

(fn ConstructionScript)