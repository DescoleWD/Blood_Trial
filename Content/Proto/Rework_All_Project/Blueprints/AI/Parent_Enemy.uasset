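; Parent Blueprint for AI enemies that configures stats, armor and weapon from a combat style or custom overrides.
; BeginPlay runs that setup only if the death check passes, but the check is currently hardwired to dead.
; Setup feeds equipment, combat, melee and input components, spawns data-table weapons and messages the AI controller.
; Death only unhides the mesh and drops weapons; ragdoll is disconnected, kill-cam conditions always fail and most getters are stubs.
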(event EventBeginPlay
  (bind _dead (CallFunction|BeginPlayDeathCheck))
  (if (not _dead)
    (CallFunction|SetupStats)
    (CallFunction|SetupArmor)
    (CallFunction|SetupComponents)
    (CallFunction|SetupWeapon)))

(fn ConstructionScript
  (Class|SkinnedMeshComponent|SetMasterPoseComponent (Variables|Default|GetBack) (Variables|Character|GetMesh) false))

(fn SetupDefaultStats
  (params (AICOmbatStyle :type E_AICombatStyle%20Enum :default "NewEnumerator7"))
  (return (Utilities|Select :Index AICOmbatStyle :NewEnumerator1 (Utilities|Struct|MakeS_Custom_AI_Values) :NewEnumerator3 "")))

(fn SetupStats
  ;[1 1 1] Sets Either Custom Stats Or Default Stats
  (if (Utilities|Struct|BreakS_Custom_AI_Values (Variables|Default|GetCustomValues))
    (CallFunction|StoreStats (Variables|Default|GetCustomValues))
    (else
      (bind _customstats (CallFunction|SetupDefaultStats (Variables|Default|GetAICombatStyle)))
      (CallFunction|StoreStats _customstats))))

(fn SetupArmor
  ;[1 1 1] Sets Either Default OR Custom Armor
  (if (Utilities|Struct|BreakS_Custom_AI_Equipment (Variables|Default|GetCustomEquipment))
    (CallFunction|StoreArmor (Variables|Default|GetCustomEquipment))
    (else
      (bind _returnvalue (CallFunction|SetupDefaultArmor (Variables|Default|GetAICombatStyle)))
      (CallFunction|StoreArmor _returnvalue))))

(fn StoreArmor
  (params (S_Custom_AI_Equipment :type S%20Custom%20AI%20Equipment%20Structure%20%28by%20ref%29))
  (bind (_usecustomequipment _chest _hands _legs _boots _back) (Utilities|Struct|BreakS_Custom_AI_Equipment S_Custom_AI_Equipment))
  (Class|SkinnedMeshComponent|SetSkeletalMesh (Variables|Default|GetHands) _hands true)
  (Class|SkinnedMeshComponent|SetSkeletalMesh (Variables|Default|GetBack) _back true))

(fn SetupDefaultArmor
  (params (AICombatStyle :type Byte :default 0))
  (bind _defaulthandsarmor (LocalVariables|GetDefaultHandsArmor))
  (return (Utilities|Select :Index AICombatStyle :Option%200 (Utilities|Struct|MakeS_Custom_AI_Equipment false _defaulthandsarmor) :Option%201 (Utilities|Struct|MakeS_Custom_AI_Equipment false _defaulthandsarmor))))

(fn SetupWeapon
  (bind _customweapon (Variables|Default|GetCustomWeapon))
  (bind (_mainhand _primaryattackstyle _meleeweapontype) (Utilities|Struct|BreakS_Custom_AI_Weapon _customweapon))
  ;[1 1 1] Sets Up The Attack Styles And Weapon Outputs For AI Controller, Combat Component & Mele Component
  (Class|IAIController|UpdateAttackStyle(Message) (AI|GetAIController self) (Utilities|Select :Index (Variables|Default|GetAICombatStyle) :Option%200 "NewEnumerator0" :Option%201 "NewEnumerator0" :Option%202 "NewEnumerator0" :Option%203 "NewEnumerator0" :Option%204 "NewEnumerator0" :Option%205 "NewEnumerator0" :Option%206 "NewEnumerator0") (Utilities|Select :Index (Variables|Default|GetAICombatStyle) :NewEnumerator1 "NewEnumerator1" :NewEnumerator3 "NewEnumerator0" :NewEnumerator5 "NewEnumerator1"))
  ;[1 1 1] Set Range Based On Combat Style
  (Variables|Default|SetMelee%20Weapon%20Range (Utilities|Select :Index (Variables|Default|GetAICombatStyle) :NewEnumerator1 4e+02 :NewEnumerator3 4e+02 :NewEnumerator0 3.5e+02))
  (if (Utilities|Struct|BreakS_Custom_AI_Weapon (Variables|Default|GetCustomWeapon))
    ;[1 1 1] Update With Custom Equipment
    (Variables|Default|SetMain%20Hand _mainhand)
    (CallFunction|SpawnAIWeapon "NewEnumerator18" (Variables|Default|GetMain%20Hand))
    ;[1 1 1] Pass Combat Types Used For Switching Attack Style
    (Class|IAIController|PassCombatTypes(Message) (AI|GetAIController self) (Utilities|Enum|ByteToEnumE_AttackStyle _primaryattackstyle) (Utilities|Enum|ByteToEnumE_WeaponType _meleeweapontype))
    (else
      ;[1 1 1] Create Weapons
      (switch Utilities|FlowControl|Switch|SwitchonE_AICombatStyle (Variables|Default|GetAICombatStyle)
        (:NewEnumerator3
          (CallFunction|SpawnAIWeapon "NewEnumerator18" (Variables|Default|GetMain%20Hand))
          (Class|IAIController|PassCombatTypes(Message) (AI|GetAIController self) "NewEnumerator0" "NewEnumerator0"))))))

(fn Death
  (params (SavedDeath :type Boolean))
  (Utilities|FlowControl|DoOnce false
    (:Completed
      ;[1 1 1] Outline Only Works On Visible Objects
      (Development|SetHiddeninGame (Variables|Character|GetMesh) false false)
      ;[1 1 1] Undo Any Component Actions, Activate Actor (Set in Details), Check If Quest Actor, Detach Weapon
      ;;[1 1 1] Detach Weapon
      (Default|DeathWeaponDrop (Variables|Default|GetCombatStatusComponent)))))

(fn SlowMotionRunning
  (params (Running? :type Boolean))
  (if Running?
    (Variables|Default|SetSlowMotionOccuring true)
    (Input|DisableInput (Game|GetPlayerController 0))
    (else
      (Input|EnableInput (Game|GetPlayerController 0))
      (Variables|Default|SetSlowMotionOccuring false))))

(fn SlowMotionConditions
  (params (IncomingDamage :type Integer))
  (if true
    (LocalVariables|SetCanTriggerKIllCam false :!label _label)
    (else
      ;[1 1 1] Close Enough To Player To Trigger
      (if (Variables|Default|GetInPlayerRange)
        ;[1 1 1] If Incoming Damage is more then current Health
        (if (>= IncomingDamage 0)
          (if (Variables|Default|GetBlockUp)
            (goto _label)
            (else
              (LocalVariables|SetCanTriggerKIllCam true)))
          (else
            (goto _label)))
        (else
          (goto _label)))))
  (return (LocalVariables|GetCanTriggerKIllCam)))

(fn ReportNoise
  (params (NoiseLocation :type Vector) (Instigator :type Actor%20Object%20Reference))
  (Class|AISenseHearing|ReportNoiseEvent NoiseLocation 1.0 Instigator 3e+02 "None")
  (Class|AISenseDamage|ReportDamageEvent self Instigator 1e+01 NoiseLocation "0, 0, 0" "None"))

(fn UpdateWidgetValues
  (bind _equipmentcomponent (Variables|Default|GetEquipmentComponent))
  (bind _maxhealth (Variables|/Game/Proto/Rework_All_Project/Blueprints/Components/EquipmentComponent.EquipmentComponent_C|GetMaxHealth _equipmentcomponent))
  (Default|CallUpdateHealth _equipmentcomponent _maxhealth _maxhealth))

(fn BeginPlayDeathCheck
  ;[1 1 1] Check IF AI Dead, If Yes, Load Loot, Set Transform & Run Death
  (Variables|Default|SetAI-Start-Transform (Transformation|GetActorLocation))
  (LocalVariables|SetAI-Dead false)
  ;;[1 1 1] check hp
  (if true
    (CallFunction|Death false)
    (LocalVariables|SetAI-Dead true)
    (return (LocalVariables|GetAI-Dead))))

(fn InitializeComponents)

(fn SetupComponents
  ;[1 1 1] Setup
  (Default|InitializeCombatStatus (Variables|Default|GetCombatStatusComponent) false)
  (Default|UpdateMaterials (Variables|Default|GetEquipmentComponent))
  (Variables|/Game/Proto/Rework_All_Project/Blueprints/Components/InputBufferComponent.InputBufferComponent_C|SetEnemyAI (Variables|Default|GetInputBufferComponent) true)
  (Variables|/Game/Proto/Rework_All_Project/Blueprints/Components/TakingDamage.TakingDamage_C|SetEnemyAI (Variables|Default|GetTakingDamage) true))

(fn SpawnAIWeapon
  (params (Item%20Type :type E_ItemType%20Enum :default "NewEnumerator18") (Weapon%20Info :type S%20Item%20Setup%20Data%20Structure))
  (bind _datatableinfo (Utilities|Struct|BreakS_ItemSetupData Weapon%20Info))
  (bind (_datatable _rowname) (Utilities|Struct|BreakDataTableRowHandle _datatableinfo))
  (if (Utilities|Name|NotEqual(Name) (.RowName (Utilities|Struct|BreakDataTableRowHandle (.DataTableInfo (Utilities|Struct|BreakS_ItemSetupData Weapon%20Info)))) "None")
    ;[1 1 1] Spawn Set Weapon
    (switch Utilities|FlowControl|Switch|SwitchonE_ItemType Item%20Type
      (:NewEnumerator9
        _)
      (:NewEnumerator12
        _))
    (bind _returnvalue (Game|SpawnActorfromClass "/Game/Proto/Rework_All_Project/Blueprints/Items/PickUpItems/BP_WeaponParent.BP_WeaponParent_C" (Math|Transform|MakeTransform (Transformation|GetActorLocation self) "0, 0, 0" "1.000000,1.000000,1.000000") "Undefined" 0 0))
    (LocalVariables|SetWeaponRef _returnvalue)
    ;[1 1 1] Retreive Item Data
    (bind _returnvalue_2 (Utilities|GetDataTableRow _datatable _rowname)
      (:then
        (bind _structout (Utilities|Struct|SetmembersinS_ItemData (.ItemStructure (Utilities|Struct|BreakS_SlotInfo (Utilities|Struct|MakeS_SlotInfo _datatableinfo _returnvalue_2))) (Utilities|Enum|ByteToEnumE_ItemType Item%20Type)))
        (Utilities|Struct|SetmembersinS_SlotInfo (Utilities|Struct|MakeS_SlotInfo _datatableinfo _returnvalue_2) _structout)
        (Class|IItemInterface|Spawn&Use(Message) (LocalVariables|GetWeaponRef) self)
        (Class|IWeaponInterface|AttachWeapontoHand(Message) (LocalVariables|GetWeaponRef))
        ;[1 1 1] Set Appropriate Variables
        (switch Utilities|FlowControl|Switch|SwitchonE_ItemType (Utilities|Enum|ByteToEnumE_ItemType Item%20Type)
          (:NewEnumerator9
            _)
          (:NewEnumerator12
            _)
          (:NewEnumerator11
            _))
        (Variables|/Game/Proto/Rework_All_Project/Blueprints/Components/CombatStatusComponent.CombatStatusComponent_C|SetEquippedMainHand (Variables|Default|GetCombatStatusComponent) (LocalVariables|GetWeaponRef))
        (Variables|/Game/Proto/Rework_All_Project/Blueprints/Components/MeleeComponent.MeleeComponent_C|SetEquippedMainHand (Variables|Default|GetMeleeComponent) (LocalVariables|GetWeaponRef))))))

(fn DestroySelf&Items
  (Default|DestroyWeapons (Variables|Default|GetCombatStatusComponent))
  (Actor|DestroyActor))

(fn StoreStats
  (params (Custom%20Values :type S%20Custom%20AI%20Values%20Structure))
  (bind (_basehealth _basecritchance _basearmor _baseshieldblock _basemainhanddamage) (Utilities|Struct|BreakS_Custom_AI_Values Custom%20Values))
  (bind _equipmentcomponent (Variables|Default|GetEquipmentComponent))
  (Utilities|FlowControl|Sequence
    (:then_0
      (bind _output_get (Variables|/Game/Proto/Rework_All_Project/Blueprints/Components/EquipmentComponent.EquipmentComponent_C|SetHealth _equipmentcomponent _basehealth))
      (Variables|/Game/Proto/Rework_All_Project/Blueprints/Components/EquipmentComponent.EquipmentComponent_C|SetMaxHealth _equipmentcomponent _output_get))
    (:then_1
      (Variables|/Game/Proto/Rework_All_Project/Blueprints/Components/EquipmentComponent.EquipmentComponent_C|SetCritValue _equipmentcomponent _basecritchance))
    (:then_2
      (Variables|/Game/Proto/Rework_All_Project/Blueprints/Components/EquipmentComponent.EquipmentComponent_C|SetArmor _equipmentcomponent _basearmor))
    (:then_3
      (Variables|/Game/Proto/Rework_All_Project/Blueprints/Components/EquipmentComponent.EquipmentComponent_C|SetShieldBlock _equipmentcomponent _baseshieldblock))
    (:then_4
      (Variables|/Game/Proto/Rework_All_Project/Blueprints/Components/EquipmentComponent.EquipmentComponent_C|SetMainHandWepDamage _equipmentcomponent _basemainhanddamage))))

(fn CanbeAssassinated
  (return false))

(fn FindAvailableAssassinationCam
  (return 0))

(fn GetWeaponRange
  (return 0.0))

(fn IsDead
  (return false))

(fn IsFacingEnemy?
  (return false))

(fn IsMoving?
  (return false))

(fn IsPlayer?
  (return false))

(fn IsWeaponDrawn?
  (return false))

(fn PassArmorMeshes
  (return 0))

(fn PassAssassinationComps
  (return 0 0))

(fn PassAttackStyle
  (return "(INVALID)"))

(fn PassBehaviourTree
  (return 0))

(fn PassBody
  (return 0 0))

(fn PassCamera
  (return 0 0))

(fn PassHealthHUD
  (return 0))

(fn PassMovementMode
  (return "MOVE_None"))

(fn PassSpline
  (return 0))

(fn PassSwitchAttackStyle
  (return false))

(fn PassWarningMesh
  (return 0))

(fn PassWeaponRange
  (return 0.0))

(fn RetrieveOutlineInfo
  (return "" 0 0 0 0 0))

(fn RetrievePlayerStatus
  (return false "(INVALID)" "NewEnumerator0"))

(fn UpdateMovementMode
  (params (MovementMode :type EMovementMode%20Enum :default "MOVE_None"))
  (return false))