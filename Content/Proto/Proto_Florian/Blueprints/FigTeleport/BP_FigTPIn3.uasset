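; Prototype teleporter entrance that sends the main character to the exit point of a BP_FigTPOut actor.
; Box overlap by BP_MainCharacter finds that actor by class and moves the character to its ExitRef location without sweeping.
; It then sets the FigTeleportIn3 flag on the object returned by GetInst.
; The construction script positions its own Teleport and ExitRef components from the TeleportTransform and ExitLocation variables.
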(event OnComponentBeginOverlap(Box)
  (params (OverlappedComponent :type Primitive%20Component%20Object%20Reference) (OtherActor :type Actor%20Object%20Reference) (OtherComp :type Primitive%20Component%20Object%20Reference) (OtherBodyIndex :type Integer) (bFromSweep :type Boolean) (SweepResult :type Hit%20Result%20Structure%20%28by%20ref%29))
  (bind _asbp_main_character (Utilities|Casting|CastToBP_MainCharacter OtherActor))
  (bind _returnvalue (Actor|GetActorOfClass "/Game/Proto/Proto_Florian/Blueprints/FigTeleport/BP_FigTPOut.BP_FigTPOut_C"))
  (Transformation|SetActorLocation _asbp_main_character (Transformation|GetWorldLocation (Variables|/Game/Proto/Proto_Florian/Blueprints/FigTeleport/BP_FigTPOut.BP_FigTPOut_C|GetExit%20Ref _returnvalue)) false false)
  (Variables|/Game/Proto/Main/Blueprint/BloodTrial_GameInstance.BloodTrial_GameInstance_C|SetFigTeleportIn3 (CallFunction|GetInst) true))

(fn ConstructionScript
  ;[1 1 1] Set Enter And Exit Location
  (Transformation|SetRelativeTransform (Variables|Default|GetTeleport) (Variables|Default|GetTeleport%20Transform) false false)
  (Transformation|SetRelativeLocation (Variables|Default|GetExit%20Ref) (Variables|Default|GetExit%20Location) false false))