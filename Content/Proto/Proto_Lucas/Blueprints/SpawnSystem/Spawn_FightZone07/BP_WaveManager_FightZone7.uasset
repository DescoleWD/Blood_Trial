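; Wave manager for Fight Zone 7 that spawns data-table-driven enemy waves at spawn points and starts the next once all spawned enemies are gone.
; BeginPlay sorts spawn points by enemy type, then a timer countdown precedes each wave, whose row is looked up by wave number.
; SpawnEnemies re-rolls random points until one matches the wave number and is free, then frees that type's points afterward.
; Polling checks enemy validity before advancing.
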(event Custom|StartCountdown
  ;[1 1 1] Countdown
  (bind _returnvalue (Utilities|Time|SetTimerbyEvent (delegate Custom|Count) 1.0 true))
  (Variables|Default|SetTime 3))

(event Custom|Count
  ;[1 1 1] Countdown
  (Development|PrintString (Utilities|String|ToString(Integer) (Variables|Default|GetTime)) true true "(R=0.568324,G=0.661458,B=0.000000,A=1.000000)")
  (if (== (Variables|Default|GetTime) 0)
    (Utilities|Time|ClearandInvalidateTimerbyHandle (stale Custom|StartCountdown _returnvalue))
    (CallFunction|BeginWave)
    (else
      (Math|Integer|DecrementInt (Variables|Default|GetTime)))))

(event Custom|BeginWave
  ;[1 1 1] Spawn Enemies for wave
  (bind _returnvalue (Utilities|GetDataTableRow (Variables|Default|GetEnemyDataTable) (Utilities|String|StringToName (Utilities|String|ToString(Integer) (Variables|Default|GetWaveNumber))))
    (:then
      (for _array_element (.EnemyInfos (Utilities|Struct|BreakStruct_WaveInfo _returnvalue))
        (CallFunction|SpawnEnemies _array_element (.waveID (Utilities|Struct|BreakStruct_WaveInfo _returnvalue))))
      (CallFunction|StartCheckingifEnemiesAreDead))
    (:RowNotFound
      (Development|PrintString "Couldn't find row for wave data" true true "(R=0.666667,G=0.000000,B=0.021645,A=1.000000)"))))

(event Custom|StartCheckingIfEnemiesAreDead
  ;[1 1 1] Check if enemies are dead and start new wave
  (bind _aredead_1 (CallFunction|CheckifAllEnemiesAreDead :!label _label))
  (if _aredead_1
    (Audio|SpawnSound2D "/Game/StarterContent/Audio/Fire01.Fire01" 1.0 1.0 0.0 0)
    (Math|Integer|IncrementInt (Variables|Default|GetWaveNumber)
      (:%20%20
        (CallFunction|StartCountdown)))
    (else
      (Utilities|FlowControl|Delay 0.5)
      (goto _label))))

(event EventBeginPlay
  (Utilities|FlowControl|Delay 0.2)
  ;[1 1 1] Sort enemies spawner references
  (bind _outactors (Actor|GetAllActorsOfClass "/Game/Proto/Proto_Lucas/Blueprints/SpawnSystem/BaseSpawnSystem/BP_WaveSpawnPoint.BP_WaveSpawnPoint_C"))
  (bind _output_get (Variables|Default|SetEnemySpawnPoints _outactors))
  (for _array_element _output_get
    (switch Utilities|FlowControl|Switch|SwitchonEnemyTypes (Variables|/Game/Proto/Proto_Lucas/Blueprints/SpawnSystem/BaseSpawnSystem/BP_WaveSpawnPoint.BP_WaveSpawnPoint_C|GetSpawnerType _array_element)
      (:NewEnumerator0
        (Utilities|Array|Add (Variables|Default|GetTzitzimime) _array_element))
      (:NewEnumerator1
        (Utilities|Array|Add (Variables|Default|GetButterfly) _array_element))
      (:NewEnumerator2
        (Utilities|Array|Add (Variables|Default|GetStrongTzitzimime) _array_element))))
  (CallFunction|StartCountdown))

(fn ConstructionScript)

(fn SpawnEnemies
  (params (Struct_EnemyInfo :type Struct%20Enemies%20Infos%20Structure%20%28by%20ref%29) (WaveID :type Array%20of%20Integers))
  ;[1 0.7571 0.3957] Set spawners references according to selected enemies' types
  (LocalVariables|SetEnemyInfoRef Struct_EnemyInfo)
  (LocalVariables|SetCurrentSpawnPoints (Utilities|Select :Index (.EnemyType (Utilities|Struct|BreakStruct_EnemiesInfos Struct_EnemyInfo)) :NewEnumerator0 (Variables|Default|GetTzitzimime) :NewEnumerator1 (Variables|Default|GetButterfly) :NewEnumerator2 (Variables|Default|GetStrongTzitzimime)))
  (for _index (range 1 (.enemynumber (LocalVariables|GetEnemyInfoRef)))
    ;[1 1 1] Get Spawners and spawn enemies on all of them
    (bind _output_get (Variables|Default|SetCurrent%20Spawns (Utilities|Array|Get(acopy) (LocalVariables|GetCurrentSpawnPoints) (Math|Random|RandomIntegerinRange 0 (Utilities|Array|LastIndex (LocalVariables|GetCurrentSpawnPoints)))) :!label _label))
    (if (== (Variables|/Game/Proto/Proto_Lucas/Blueprints/SpawnSystem/BaseSpawnSystem/BP_WaveSpawnPoint.BP_WaveSpawnPoint_C|GetEnemySpawnIDs _output_get) (Variables|Default|GetWaveNumber))
      (if (Variables|/Game/Proto/Proto_Lucas/Blueprints/SpawnSystem/BaseSpawnSystem/BP_WaveSpawnPoint.BP_WaveSpawnPoint_C|GetisAvailable? _output_get)
        (Variables|/Game/Proto/Proto_Lucas/Blueprints/SpawnSystem/BaseSpawnSystem/BP_WaveSpawnPoint.BP_WaveSpawnPoint_C|SetisAvailable? (Variables|Default|GetCurrent%20Spawns) false)
        (bind _returnvalue (AI|SpawnAIFromClass (.enemyclass (LocalVariables|GetEnemyInfoRef)) 0 (.Location (Math|Transform|BreakTransform (Transformation|GetWorldTransform (Variables|/Game/Proto/Proto_Lucas/Blueprints/SpawnSystem/BaseSpawnSystem/BP_WaveSpawnPoint.BP_WaveSpawnPoint_C|GetBillboard _output_get)))) (.Rotation (Math|Transform|BreakTransform (Transformation|GetWorldTransform (Variables|/Game/Proto/Proto_Lucas/Blueprints/SpawnSystem/BaseSpawnSystem/BP_WaveSpawnPoint.BP_WaveSpawnPoint_C|GetBillboard _output_get)))) false 0))
        (Utilities|Array|Add (Variables|Default|GetCurrentEnemies) _returnvalue)
        (else
          (goto _label)))
      (else
        (goto _label))))
  ;[0.5766 1 0.4989] Set "isAvailable?" spawner value to true when all spawners are false after spawning
  (for _array_element (LocalVariables|GetCurrentSpawnPoints)
    (Variables|/Game/Proto/Proto_Lucas/Blueprints/SpawnSystem/BaseSpawnSystem/BP_WaveSpawnPoint.BP_WaveSpawnPoint_C|SetisAvailable? _array_element true)))

(fn CheckifAllEnemiesAreDead
  (LocalVariables|SetAreDead? true)
  (for _array_element (Variables|Default|GetCurrentEnemies)
    (Utilities|IsValid _array_element
      (:Is%20Valid
        (LocalVariables|SetAreDead? false))))
  (return (LocalVariables|GetAreDead?)))