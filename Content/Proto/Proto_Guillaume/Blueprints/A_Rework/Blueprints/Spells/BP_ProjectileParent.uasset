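; Parent Blueprint for projectile magic spells, covering charge, cast, launch and impact, with sounds, effects and animation drawn from SpellInfo.
; Casting plays a montage; the animation-triggered event detaches the projectile and sets its calculated velocity.
; Walls use hit events, while enemies use overlaps so the projectile keeps its velocity against the caster.
; Impacts report AI noise and destroy the spell; overlaps also apply MagicComponent-calculated point damage.
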(event OnComponentBeginOverlap(AbilityCollision)
  (params (OverlappedComponent :type Primitive%20Component%20Object%20Reference) (OtherActor :type Actor%20Object%20Reference) (OtherComp :type Primitive%20Component%20Object%20Reference) (OtherBodyIndex :type Integer) (bFromSweep :type Boolean) (SweepResult :type Hit%20Result%20Structure%20%28by%20ref%29))
  (bind _impactpoint (Collision|BreakHitResult SweepResult))
  ;[1 1 1] Overlap For Enemies (Needs to Overlap Otherwise Projectile Collides with Player Removing Velocity)
  (if (not (== OtherActor (Variables|Default|GetCharacterActorRef)))
    (Utilities|FlowControl|DoOnce false
      (:Completed
        (CallFunction|PlayHitSound _impactpoint)
        (CallFunction|ApplyDamage OtherActor _impactpoint SweepResult)
        (CallFunction|DestroySpell)))))

(event OnComponentHit(AbilityCollision)
  (params (HitComponent :type Primitive%20Component%20Object%20Reference) (OtherActor :type Actor%20Object%20Reference) (OtherComp :type Primitive%20Component%20Object%20Reference) (NormalImpulse :type Vector :default "0, 0, 0") (Hit :type Hit%20Result%20Structure%20%28by%20ref%29))
  (bind _impactpoint (Collision|BreakHitResult Hit))
  ;[1 1 1] Hit For Walls
  (Utilities|FlowControl|DoOnce false
    (:Completed
      (CallFunction|PlayHitSound _impactpoint)
      (Niagara|SpawnSystematLocation (Utilities|Struct|Break (.SpellProjectile (Utilities|Struct|Break (Variables|Default|GetSpellInfo)))) _impactpoint)
      (CallFunction|DestroySpell))))

(event Custom|AttemptSpellAgain
  ;[1 1 1] Send Animation Spell
  (Audio|PlaySoundatLocation (Utilities|Struct|Break (Utilities|Struct|Break (Variables|Default|GetSpellInfo))) (Transformation|GetActorLocation) "0, 0, 0" 1.0 1.0 0.0 0 0 0)
  (CallFunction|CalculateSpellHitLocation)
  (Animation|Montage|PlayMontage (Variables|Default|GetCharacterMesh) (Utilities|Struct|Break (Variables|Default|GetSpellInfo))
    (:OnInterrupted
      (CallFunction|NextSpell (Variables|Default|GetMagicComponent)))))

(event EventBeginMagicCharge
  ;[1 1 1] Begin Charge
  (Audio|PlaySoundatLocation (Utilities|Struct|Break (Utilities|Struct|Break (Variables|Default|GetSpellInfo))) (Transformation|GetActorLocation) "0, 0, 0" 1.0 1.0 0.0 0 0 0)
  (Utilities|FlowControl|Delay 0.2)
  (bind _returnvalue (Audio|SpawnSoundAttached (Utilities|Struct|Break (.SpellSoundFX (Utilities|Struct|Break (Variables|Default|GetSpellInfo)))) (Variables|Default|GetAbilityCollision) "None" "0, 0, 0" "0, 0, 0" "SnapToTarget" false 0.5 1.0 0.0 0 0))
  (Variables|Default|SetLoopSound _returnvalue))

(event EventStopMagicCharge
  (bind _loopsound (Variables|Default|GetLoopSound))
  ;[1 1 1] Release Charge
  (Components|Activation|Deactivate (Variables|Default|GetNiagaraSystem))
  (Utilities|IsValid _loopsound
    (:Is%20Valid
      (Audio|Components|Audio|Stop _loopsound))))

(event EventSendMagicSpell
  ;[1 1 1] Send Animation Spell
  (Audio|PlaySoundatLocation (Utilities|Struct|Break (Utilities|Struct|Break (Variables|Default|GetSpellInfo))) (Transformation|GetActorLocation) "0, 0, 0" 1.0 1.0 0.0 0 0 0)
  (CallFunction|CalculateSpellHitLocation)
  (Animation|Montage|PlayMontage (Variables|Default|GetCharacterMesh) (Utilities|Struct|Break (Variables|Default|GetSpellInfo))
    (:OnInterrupted
      (CallFunction|NextSpell (Variables|Default|GetMagicComponent)))))

(event EventTriggerMagicSpell
  ;[1 1 1] Trigger Spell Attack (Triggered From Animation)
  (Transformation|DetachFromActor "KeepWorld" "KeepWorld" "KeepWorld")
  (CallFunction|CalculateSpellVelocity)
  (Variables|/Script/Engine.MovementComponent|SetVelocity (Variables|Default|GetProjectileMovement) (Variables|Default|GetSpellVelocity)))

(fn ConstructionScript)

(fn ApplyDamage
  (params (HitActor :type Actor%20Object%20Reference) (HitFromDirection :type Vector%20%28by%20ref%29) (HitInfo :type Hit%20Result%20Structure))
  (bind _magiccomponent (Variables|Default|GetMagicComponent))
  (bind _spellinfo (Variables|Default|GetSpellInfo))
  (bind (_damagetype _specialdamageinfo) (Utilities|Struct|Break _spellinfo))
  (bind _returnvalue (Actor|GetComponentbyClass HitActor 0))
  (Utilities|FlowControl|DoOnce false
    (:Completed
      (Utilities|IsValid _magiccomponent
        (:Is%20Valid
          (bind (_spell_damage _critical_hit) (CallFunction|CalculateMagicDamage _magiccomponent (Variables|Default|GetSpellInfo)))
          (Utilities|IsValid _returnvalue
            (:Is%20Valid
              (CallFunction|PassDamageInfo _returnvalue 0 0 _damagetype _critical_hit _specialdamageinfo)
              (Game|Damage|ApplyPointDamage HitActor _spell_damage HitFromDirection (Collision|MakeHitResult false false 0.0 0.0 "0, 0, 0" HitFromDirection "0,0,1" "0,0,1" 0 HitActor) 0 (Variables|Default|GetCharacterActorRef))
              (Niagara|SpawnSystematLocation (Utilities|Struct|Break (.SpellProjectile (Utilities|Struct|Break (Variables|Default|GetSpellInfo)))) HitFromDirection))))))))

(fn PlayHitSound
  (params (Location :type Vector))
  (bind _loopsound (Variables|Default|GetLoopSound))
  (Audio|PlaySoundatLocation (Utilities|Struct|Break (.SpellSoundFX (Utilities|Struct|Break (Variables|Default|GetSpellInfo)))) Location "0, 0, 0" 1.0 1.0 0.0 0 0 0)
  (Class|AISenseHearing|ReportNoiseEvent (Variables|Default|GetSpellPlacementLocation) 1.0 (Variables|Default|GetCharacterActorRef) 5e+02 "None")
  (Utilities|IsValid _loopsound
    (:Is%20Valid
      (Audio|Components|Audio|Stop _loopsound))))