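; BP_FlameThrower is a prototype flame trap that slides its Fire component out when BP_MainBase enters the trigger Box and retracts it on exit.
; Overlapping BoxFire starts damage and shows a Lava_Feedback widget, removed when that overlap ends.
; Tick applies the game instance's LavaDamage through a delayed DoOnce, repeating until the player leaves the outer Box, even after exiting BoxFire.
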(event OnComponentBeginOverlap(Box)
  (params (OverlappedComponent :type Primitive%20Component%20Object%20Reference) (OtherActor :type Actor%20Object%20Reference) (OtherComp :type Primitive%20Component%20Object%20Reference) (OtherBodyIndex :type Integer) (bFromSweep :type Boolean) (SweepResult :type Hit%20Result%20Structure%20%28by%20ref%29))
  (Utilities|Casting|CastToBP_MainBase OtherActor)
  (Utilities|FlowControl|Delay 0.2)
  (Components|MoveComponentTo (Variables|Default|GetFire) (+ (Variables|Default|GetFireOriginLocation) "0,250.000000,0.000000") (Variables|Default|GetFireOriginRotation) true true 0.3 false))

(event OnComponentEndOverlap(Box)
  (params (OverlappedComponent :type Primitive%20Component%20Object%20Reference) (OtherActor :type Actor%20Object%20Reference) (OtherComp :type Primitive%20Component%20Object%20Reference) (OtherBodyIndex :type Integer))
  (Utilities|Casting|CastToBP_MainBase OtherActor)
  (Variables|Default|SetFireActivate false)
  (Utilities|FlowControl|Sequence
    (:then_0
      (if (Variables|Default|GetPlayerIsOnFire)
        _))
    (:then_1
      (Components|MoveComponentTo (Variables|Default|GetFire) (+ (Variables|Default|GetFireOriginLocation) "") (Variables|Default|GetFireOriginRotation) true true 0.5 false))))

(event OnComponentBeginOverlap(BoxFire)
  (params (OverlappedComponent :type Primitive%20Component%20Object%20Reference) (OtherActor :type Actor%20Object%20Reference) (OtherComp :type Primitive%20Component%20Object%20Reference) (OtherBodyIndex :type Integer) (bFromSweep :type Boolean) (SweepResult :type Hit%20Result%20Structure%20%28by%20ref%29))
  (Utilities|Casting|CastToBP_MainBase OtherActor)
  (Variables|Default|SetFireActivate true)
  (Variables|Default|SetPlayerIsOnFire true)
  (Utilities|FlowControl|DoOnce false
    (:Completed
      (bind _returnvalue (Game|ConstructObjectfromClass "/Game/Proto/Main/HUD/Lava_Feedback.Lava_Feedback_C"))
      (UserInterface|Viewport|AddtoViewport _returnvalue 0)
      (Default|LavaEffectHUD _returnvalue))))

(event OnComponentEndOverlap(BoxFire)
  (params (OverlappedComponent :type Primitive%20Component%20Object%20Reference) (OtherActor :type Actor%20Object%20Reference) (OtherComp :type Primitive%20Component%20Object%20Reference) (OtherBodyIndex :type Integer))
  (Utilities|Casting|CastToBP_MainBase OtherActor)
  (Variables|Default|SetPlayerIsOnFire false)
  (Widget|RemovefromParent (stale OnComponentBeginOverlap(BoxFire) _returnvalue))
  (Utilities|FlowControl|DoOnce false) ; enters at Reset
)

(event EventBeginPlay
  (Variables|Default|SetFireOriginLocation (Variables|/Script/Engine.SceneComponent|GetRelativeLocation (Variables|Default|GetFire)))
  (Variables|Default|SetFireOriginRotation (Variables|/Script/Engine.SceneComponent|GetRelativeRotation (Variables|Default|GetFire))))

(event EventTick
  (params (DeltaSeconds :type Float%20%28single-precision%29))
  (bind _returnvalue (Actor|GetActorOfClass "/Game/Proto/Main/Blueprint/BP_MainBase.BP_MainBase_C"))
  (if (Variables|Default|GetFireActivate)
    (Utilities|FlowControl|DoOnce false :!label _label
      (:Completed
        (Game|Damage|ApplyDamage _returnvalue (Variables|/Game/Proto/Main/Blueprint/Save_BFL_GameInstance/BloodTrial_GameInstance.BloodTrial_GameInstance_C|GetLavaDamage (CallFunction|GetInst)) 0 0)
        (Utilities|FlowControl|Delay 0.5)
        (goto _label Reset)))))

(fn ConstructionScript)