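; BP_Papillon is an enemy AI character that chases the player, attacking by montage and spawning projectiles.
; On BeginPlay or sighting, it alerts every Papillon into an AIMoveTo loop that randomly picks attack or strafe (WorldStrafingDirection currently returns zero).
; Damage drains a floating health bar, triggering hit reaction, brief invincibility and optional player vampirism, or death with score.
; Bolas hits immobilize it, then return to the player or explode.
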(event OnSeePawn(PawnSensing)
  (params (Pawn :type Pawn%20Object%20Reference))
  ;[1 1 1] Begin
  (CallFunction|PlayerIsSeen))

(event Custom|Boule2Feu
  ;[1 1 1] General Behavior Logic
  (if (not (or (Variables|Default|GetisHit) (Variables|Default|GetBolas)))
    (CallFunction|SpawnSpell)
    (Utilities|FlowControl|Delay 0.5)
    ;;[1 1 1] General Behavior Logic
    (CallFunction|Weknowurlocation)))

(event Custom|Mort_IA
  (bind _returnvalue (Transformation|GetActorLocation))
  ;[0.08256 1 0] Mort IA
  (Utilities|FlowControl|Sequence
    (:then_0
      (Pawn|Components|CharacterMovement|SetMovementMode (Variables|Character|GetCharacterMovement) "MOVE_None" 0)
      (Utilities|FlowControl|DoOnce false
        (:Completed
          (CallFunction|IncrScore (Variables|/Game/Proto/Main/Blueprint/Save_BFL_GameInstance/BloodTrial_GameInstance.BloodTrial_GameInstance_C|GetScore_Enemy2 (CallFunction|GetInst))))))
    (:then_1
      (Collision|SetCollisionResponsetoChannel (Variables|Default|GetCapsuleComponent) "ECC_GameTraceChannel2" "ECR_Ignore")
      (Audio|PlaySoundatLocation "/Game/Proto/Rework_All_Project/SoundFX/SFX_Player/Death_Tzitzimine/249813__spookymodem__goblin-death.249813__spookymodem__goblin-death" _returnvalue "0, 0, 0" -5.0 1.0 0.0 0 0 0 0)
      (Effects|SpawnEmitteratLocation "/Game/Proto/Proto_Guillaume/Blueprints/DynamicHealthbars/_Demo/FX/EnemyDeath/P_EnemyDeath.P_EnemyDeath" _returnvalue)
      (bind _animplayrate (CallFunction|PlayHighPriorityMontage "/Game/Proto/Rework_All_Project/Animation/Papillon/Animation/papillon_death_Montage.papillon_death_Montage" "None" 1.0))
      (Utilities|FlowControl|Delay _animplayrate)
      (Actor|DestroyActor))))

(event Custom|Begin_2
  (bind _returnvalue (Math|Random|RandomFloatinRange 8e+02 1.2e+03))
  (Variables|/Script/AIModule.PawnSensingComponent|SetSightRadius (Variables|Default|GetPawnSensing) 6e+01)
  (if (Variables|Default|GetFirstLook)
    (CallFunction|PlayerIsSeen)
    (elif (not (Variables|Default|GetHasTarget))
      (CallFunction|ServerFindClosestPLayer)
      (Variables|Default|SetHasTarget true)
      (Variables|Default|SetFirstLook true)
      (if (Math|Boolean|ORBoolean (Variables|Default|GetisHit) (Variables|Default|GetBolas) (Variables|Default|GetIA_Dead))
        (Utilities|FlowControl|Delay 0.7)
        (Variables|Default|SetisHit false)
        (else
          (AI|AIMoveTo self (Transformation|GetWorldLocation (Variables|/Script/Engine.Character|GetMesh (Variables|Default|GetClosestPlayer))) (Variables|Default|GetClosestPlayer) (Math|Random|RandomFloatinRange 7e+02 9e+02) true
            (:OnSuccess
              (if (not (Variables|Default|GetMustAttack))
                (switch int (Math|Random|RandomInteger 3)
                  (:0
                    (AI|AIMoveTo self (Transformation|GetWorldLocation (Variables|/Script/Engine.Character|GetMesh (Variables|Default|GetClosestPlayer))) (Variables|Default|GetClosestPlayer) 4.5e+02 true
                      (:OnSuccess
                        (if (not (Variables|Default|GetIsAttacking))
                          (bind _animplayrate (CallFunction|PlayHighPriorityMontage (Variables|Default|GetAttack01) "None" 1.0))
                          (Utilities|FlowControl|Delay _animplayrate)
                          (Variables|Default|SetMustAttack false)
                          (Variables|Default|SetHasTarget false)
                          (CallFunction|Weknowurlocation :!label _label)))
                      (:OnFail
                        (Utilities|FlowControl|Delay 0.2)
                        (goto _label))))
                  (:1
                    (if (not (Variables|Default|GetMustAttack))
                      (Variables|/Script/Engine.CharacterMovementComponent|SetMaxWalkSpeed (Variables|Character|GetCharacterMovement) (Math|Random|RandomFloatinRange 4e+02 8e+02))
                      (Variables|Default|SetStrafingDirection "NewEnumerator0")
                      (Variables|Default|SetStrafing? true)
                      (Utilities|FlowControl|Delay 1.0 :!label _label_2)
                      (Variables|Default|SetMustAttack true)
                      (Variables|Default|SetStrafing? false)
                      (Variables|/Script/Engine.CharacterMovementComponent|SetMaxWalkSpeed (Variables|Character|GetCharacterMovement) 7.5e+02)
                      (CallFunction|Weknowurlocation)))
                  (:2
                    (if (not (Variables|Default|GetMustAttack))
                      (Variables|/Script/Engine.CharacterMovementComponent|SetMaxWalkSpeed (Variables|Character|GetCharacterMovement) _returnvalue)
                      (Variables|Default|SetStrafingDirection "NewEnumerator1")
                      (Variables|Default|SetStrafing? true)
                      (goto _label_2)))
                  (:3
                    (if (not (Variables|Default|GetMustAttack))
                      (Variables|/Script/Engine.CharacterMovementComponent|SetMaxWalkSpeed (Variables|Character|GetCharacterMovement) _returnvalue)
                      (Variables|Default|SetStrafingDirection "NewEnumerator2")
                      (Variables|Default|SetStrafing? true)
                      (goto _label_2))))))
            (:OnFail
              (Utilities|FlowControl|Delay 0.2)
              (CallFunction|Weknowurlocation))))))))

(event Custom|Event_Death
  ;[0.08256 1 0] Mort IA
  (Actor|DestroyActor))

(event Custom|Weknowurlocation
  (bind _returnvalue (Math|Random|RandomFloatinRange 8e+02 1.2e+03))
  (bind _returnvalue_2 (Game|GetPlayerCharacter 0))
  (if (not (Variables|Default|GetIA_Dead))
    (if (Variables|Default|GetisHit)
      (Utilities|FlowControl|Delay 1.0)
      (Variables|Default|SetisHit false)
      (CallFunction|Weknowurlocation)
      (else
        (AI|AIMoveTo self (Transformation|GetWorldLocation (Variables|/Script/Engine.Character|GetCapsuleComponent (Game|GetPlayerCharacter 0))) (Game|GetPlayerCharacter 0) (Math|Random|RandomFloatinRange 7e+02 9e+02) true
          (:OnSuccess
            (if (Variables|Default|GetMustAttack)
              (AI|AIMoveTo self (Transformation|GetWorldLocation (Variables|/Script/Engine.Character|GetCapsuleComponent _returnvalue_2)) _returnvalue_2 4.5e+02 false :!label _label
                (:OnSuccess
                  (if (not (Variables|Default|GetIsAttacking))
                    (bind _animplayrate (CallFunction|PlayHighPriorityMontage (Variables|Default|GetAttack01) "None" 1.0))
                    (Utilities|FlowControl|Delay _animplayrate)
                    (Variables|Default|SetMustAttack false)
                    (Variables|Default|SetStrafing? true)))
                (:OnFail
                  (Utilities|FlowControl|Delay 0.5)
                  (CallFunction|Weknowurlocation)))
              (else
                (switch int (Math|Random|RandomInteger 3)
                  (:0
                    (goto _label))
                  (:1
                    (if (not (Variables|Default|GetMustAttack))
                      (Variables|/Script/Engine.CharacterMovementComponent|SetMaxWalkSpeed (Variables|Character|GetCharacterMovement) (Math|Random|RandomFloatinRange 4e+02 8e+02))
                      (Variables|Default|SetStrafingDirection "NewEnumerator0")
                      (Variables|Default|SetStrafing? true)
                      (Utilities|FlowControl|Delay 2.0 :!label _label_2)
                      (Variables|Default|SetMustAttack true)
                      (Variables|Default|SetStrafing? false)
                      (Variables|/Script/Engine.CharacterMovementComponent|SetMaxWalkSpeed (Variables|Character|GetCharacterMovement) 7.5e+02)
                      (CallFunction|Weknowurlocation)))
                  (:2
                    (if (not (Variables|Default|GetMustAttack))
                      (Variables|/Script/Engine.CharacterMovementComponent|SetMaxWalkSpeed (Variables|Character|GetCharacterMovement) _returnvalue)
                      (Variables|Default|SetStrafingDirection "NewEnumerator1")
                      (Variables|Default|SetStrafing? true)
                      (goto _label_2)))
                  (:3
                    (if (not (Variables|Default|GetMustAttack))
                      (Variables|/Script/Engine.CharacterMovementComponent|SetMaxWalkSpeed (Variables|Character|GetCharacterMovement) _returnvalue)
                      (Variables|Default|SetStrafingDirection "NewEnumerator2")
                      (Variables|Default|SetStrafing? true)
                      (goto _label_2)))))))
          (:OnFail
            (Utilities|FlowControl|Delay 0.5)
            (CallFunction|Weknowurlocation)))))))

(event Custom|SpawnBolas_T
  (bind _asblood_trial_game_instance (CallFunction|GetInst))
  (bind _capsulecomponent (Variables|Default|GetCapsuleComponent))
  (bind _capsulecomponent_2 (Variables|Default|GetCapsuleComponent))
  (bind _returnvalue (Transformation|GetWorldLocation _capsulecomponent_2))
  (bind _returnvalue_2 (Transformation|GetWorldLocation _capsulecomponent))
  (Variables|Default|SetBolas true)
  (Variables|/Game/Proto/Main/Blueprint/Save_BFL_GameInstance/BloodTrial_GameInstance.BloodTrial_GameInstance_C|SetIsBolas_Attached? _asblood_trial_game_instance true)
  (if (Variables|/Game/Proto/Main/Blueprint/Save_BFL_GameInstance/BloodTrial_GameInstance.BloodTrial_GameInstance_C|GetSacrifice_1_BolasExplosion _asblood_trial_game_instance)
    ;[1 0 0.7542] Step 1 : Bolas s'attache sur l'ennemi
    (Effects|SpawnEmitteratLocation "/Game/Proto/Rework_All_Project/VFX/MeleeVFX/Bolas_Impact_Explosif.Bolas_Impact_Explosif" (Math|Vector|MakeVector (.x _returnvalue_2) (.y _returnvalue_2) (+ (.z _returnvalue_2) 2e+01)))
    (else
      (Effects|SpawnEmitteratLocation "/Game/Proto/Rework_All_Project/VFX/MeleeVFX/Bolas_Impact.Bolas_Impact" (Math|Vector|MakeVector (.x _returnvalue) (.y _returnvalue) (+ (.z _returnvalue) 5e+01)) "0, 0, 0" "1.000000,1.000000,1.000000" true "AutoRelease")))
  ;;[0.9325 1 0] Step 3  :Jouer l'animation d'étranglement - Besoin anim étranglement Tzitzimine
  (Pawn|Components|CharacterMovement|SetMovementMode (Variables|Character|GetCharacterMovement) "MOVE_None" 0)
  (bind _animplayrate (CallFunction|PlayHighPriorityMontage "/Game/Proto/Rework_All_Project/Animation/Papillon/Animation/DW_BlockBreak_Retargeted_Montage.DW_BlockBreak_Retargeted_Montage" "None" 1.0))
  (Utilities|FlowControl|Delay _animplayrate)
  (if (not (Variables|Default|GetExplosion))
    (CallFunction|BolasReturnPlayer)
    (Pawn|Components|CharacterMovement|SetMovementMode (Variables|Character|GetCharacterMovement) "MOVE_NavWalking" 0)))

(event Custom|Explosion_M
  ;[1 0 0.7108] Explosion
  ;;[0.1952 1 0] Step 1 : Déclencher l'explosion + Throw bolas pas valide
  (Variables|Default|SetExplosion true)
  (Variables|/Game/Proto/Main/Blueprint/Save_BFL_GameInstance/BloodTrial_GameInstance.BloodTrial_GameInstance_C|SetCanThrowBolas? (CallFunction|GetInst) false)
  ;;[0.1836 1 0] Step 1.5 : Stop anim being strangled
  (Animation|StopAnimMontage "/Game/Proto/Rework_All_Project/Animation/Papillon/Animation/DW_BlockBreak_Retargeted_Montage.DW_BlockBreak_Retargeted_Montage")
  ;;[0.1621 1 0] Step 3 : Call debug de l'explosion + valide variable explosion
  (CallFunction|CollisionExplosion))

(event Custom|BolasReturn_Player
  (bind _asblood_trial_game_instance (CallFunction|GetInst))
  (bind _returnvalue (Game|GetPlayerCharacter 0))
  (bind _capsulecomponent (Variables|Default|GetCapsuleComponent))
  (bind _returnvalue_2 (Transformation|GetWorldLocation _capsulecomponent))
  (bind _capsulecomponent_2 (Variables|/Script/Engine.Character|GetCapsuleComponent _returnvalue))
  (bind _returnvalue_3 (Transformation|GetWorldLocation _capsulecomponent_2))
  ;[0.8705 1 0] Retour Bolas
  (bind _returnvalue_4 (Game|SpawnActorfromClass "/Game/Proto/Proto_Florian/Blueprints/Bolas/BP_Apparence_Bolas.BP_Apparence_Bolas_C" (Math|Transform|MakeTransform (Math|Vector|MakeVector (.x _returnvalue_2) (.y _returnvalue_2) (+ (.z _returnvalue_2) 2e+02)) "0, 0, 0" "0.300000,0.300000,0.300000") "AlwaysSpawn" 0 0))
  (Components|MoveComponentTo (Variables|/Game/Proto/Proto_Florian/Blueprints/Bolas/BP_Apparence_Bolas.BP_Apparence_Bolas_C|GetStaticMesh _returnvalue_4) (Math|Vector|MakeVector (.x _returnvalue_3) (.y _returnvalue_3) (.z _returnvalue_3)) "0, 0, 0" true true 0.3 true)
  (Variables|/Game/Proto/Main/Blueprint/Save_BFL_GameInstance/BloodTrial_GameInstance.BloodTrial_GameInstance_C|SetIsBolas_Attached? _asblood_trial_game_instance false)
  (Variables|/Game/Proto/Main/Blueprint/Save_BFL_GameInstance/BloodTrial_GameInstance.BloodTrial_GameInstance_C|SetCanThrowBolas? _asblood_trial_game_instance true)
  (Variables|Default|SetExplosion false)
  (Variables|Default|SetBolas false)
  (Actor|DestroyActor _returnvalue_4))

(event Custom|Collision_Explosion
  ;[1 0 0.7108] Explosion
  ;;[1 0.9631 0] Step 1 : Spawn sphere collision pour explosion et identifier les actors touchés
  (Game|SpawnActorfromClass "/Game/Proto/Proto_Guillaume/Blueprints/Player/Explosion.Explosion_C" (Math|Conversions|ToTransform(Vector) (Transformation|GetWorldLocation (Variables|Default|GetBolasAttached))) "Undefined" 0 0)
  (Variables|Default|SetExplosion true)
  (CallFunction|BolasReturnPlayer))

(event Custom|PlayerIsSeen
  ;[1 1 1] General Behavior Logic
  ;;[1 1 1] General Behavior Logic
  ;;;[1 0 0.6379] Initialisation : Le player est vu ==> (Jouer une anim ?)
  (Audio|PlaySoundatLocation "/Game/Proto/Main/SFX/SFXHADES/Enemies/Alerted/Bloodless01_EmoteAlerted_1.Bloodless01_EmoteAlerted_1" (Transformation|GetWorldLocation (Variables|Default|GetCapsuleComponent)) "0, 0, 0" -5.0 1.0 0.0 0 0 0 0)
  (bind _outactors (Actor|GetAllActorsOfClass "BP_Papillon_C"))
  (CallFunction|Weknowurlocation _outactors))

(event Custom|AI_IS_Bolassed
  ;[1 1 1] General Behavior Logic
  ;;[1 1 1] General Behavior Logic
  (Variables|Default|SetbCanBeDamaged true))

(event Game|Damage|EventAnyDamage
  (params (Damage :type Float%20%28single-precision%29) (DamageType :type Damage%20Type%20Object%20Reference) (InstigatedBy :type Controller%20Object%20Reference) (DamageCauser :type Actor%20Object%20Reference))
  (bind _floating_healtbar (CallFunction|GetHealthBarWidget0))
  (bind _capsulecomponent (Variables|Default|GetCapsuleComponent))
  (bind _value (Default|GetCurrentValue _floating_healtbar "NewEnumerator0"))
  (Variables|Default|SetDamage_0 Damage)
  (Variables|Default|SetDamage%20Causer DamageCauser)
  (bind _output_get (Variables|Default|SetDamageCauserRadial (stale Game|Damage|EventRadialDamage DamageCauser)))
  (Variables|Default|SetDamage%20Causer _output_get)
  (Variables|Default|SetImpact%20Normal (Math|Vector|GetForwardVector (Variables|/Script/Engine.Character|GetCapsuleComponent (Game|GetPlayerCharacter 0))))
  (if (Variables|Default|GetIA_Dead)
    (CallFunction|EventDeath)
    (elif (>= _value 1.0)
      (Default|SubtractValue _floating_healtbar "NewEnumerator0" (Variables|Default|GetDamage_0))
      (bind _output_get_2 (Variables|Default|SetValue _value))
      (Math|Float|CompareFloat _output_get_2 0.0
        (:>
          (Utilities|FlowControl|Sequence
            (:then_0
              (bind _animplayrate (CallFunction|PlayHighPriorityMontage "/Game/Proto/Rework_All_Project/Animation/Papillon/Animation/papillon_TakeBigdamage_Montage.papillon_TakeBigdamage_Montage" "None" 1.0))
              (Utilities|FlowControl|Delay _animplayrate))
            (:then_1
              ;[1 1 1] Play mesh Skull move not camera Shake
              (Camera|PlayWorldCameraShake 0 (Transformation|GetActorLocation (Game|GetPlayerCharacter 0)) 0.0 4e+03)
              (CallFunction|KnockBack (Variables|Default|GetDamage%20Causer))
              (Audio|PlaySoundatLocation "/Game/Proto/Main/SFX/SFXHADES/Player/Player_Hurt/EmoteHurt_5.EmoteHurt_5" (Transformation|GetActorLocation) "0, 0, 0" -5.0 1.0 0.0 0 0 0 0)
              (Utilities|FlowControl|Delay 0.2)
              (Variables|/Script/Engine.CharacterMovementComponent|SetGroundFriction (Variables|Character|GetCharacterMovement) 3.0)
              (Variables|Default|SetFirstLook true)
              (Variables|Default|SetisHit true)
              ;[1 1 1] Delay Invincible Frame
              (Utilities|FlowControl|Delay 0.02)
              (Collision|SetCollisionResponsetoChannel _capsulecomponent "ECC_GameTraceChannel4" "ECR_Block")
              (Collision|SetCollisionResponsetoChannel _capsulecomponent "ECC_GameTraceChannel5" "ECR_Block")
              (Variables|Default|SetbCanBeDamaged true)
              (Variables|Default|SetFirstLook true)
              (if (Variables|/Game/Proto/Main/Blueprint/Save_BFL_GameInstance/BloodTrial_GameInstance.BloodTrial_GameInstance_C|GetSacrifice_4_Vampirisme (CallFunction|GetInst))
                (bind _asbp_main_base (Utilities|Casting|CastToBP_MainBase (Game|GetPlayerCharacter 0)))
                (Default|Vampirisme _asbp_main_base)
                (Niagara|SpawnSystematLocation "/Game/TA/Scene/Hugo/BloodDrain/BloodDrainVfxV1.BloodDrainVfxV1" (Transformation|GetWorldLocation (Variables|Default|GetCapsuleComponent)))))))
        (:==
          (CallFunction|MortIA :!label _label)
          (Variables|Default|SetIA_Dead false)
          (CallFunction|KnockBack (Variables|Default|GetDamage%20Causer)))
        (:<
          (goto _label)))
      (else
        (Variables|Default|SetIA_Dead true)
        (CallFunction|MortIA)))))

(event EventTick
  (params (DeltaSeconds :type Float%20%28single-precision%29))
  (bind _returnvalue (Game|GetPlayerCharacter 0))
  (bind _closestplayer (Variables|Default|GetClosestPlayer))
  (bind _capsulecomponent (Variables|/Script/Engine.Character|GetCapsuleComponent _returnvalue))
  ;[1 1 1] Look At Target Player and add movement input for strafing
  (if (Math|Boolean|ORBoolean (Variables|Default|GetisHit) (Variables|Default|GetBolas) (Variables|Default|GetIsAttacking) (Variables|Default|GetIA_Dead))
    (Components|Movement|StopMovementImmediately (Variables|Character|GetCharacterMovement))
    (elif (Variables|Default|GetFirstLook)
      (if (Variables|Default|GetStrafing?) :!label _label
        (Utilities|IsValid _capsulecomponent
          (:Is%20Valid
            (Transformation|SetActorRotation (Math|Rotator|FindLookatRotation (Transformation|GetActorLocation) (Transformation|GetWorldLocation _capsulecomponent)))
            (Pawn|Input|AddMovementInput (CallFunction|WorldStrafingDirection) 1.0 false)
            (Utilities|FlowControl|Delay 0.02)
            (goto _label))))
      (else
        (if (Variables|Default|GetStrafing?) :!label _label_2
          (Utilities|IsValid _closestplayer
            (:Is%20Valid
              (Transformation|SetActorRotation (Math|Rotator|FindLookatRotation (Transformation|GetActorLocation) (Transformation|GetActorLocation _closestplayer)))
              (Pawn|Input|AddMovementInput (CallFunction|WorldStrafingDirection) 1.0 false)
              (Utilities|FlowControl|Delay 0.02)
              (goto _label_2))))))))

(event EventMovement
  (params (On%20/%20Off :type Boolean))
  (if (not (or (Variables|Default|GetisHit) (Variables|Default|GetBolas)))
    (Variables|Default|SetMovementOn On%20/%20Off)
    (Development|PrintString "Hello")))

(event Game|Damage|EventRadialDamage
  (params (DamageReceived :type Float%20%28single-precision%29) (DamageType :type Damage%20Type%20Object%20Reference) (Origin :type Vector :default "0, 0, 0") (HitInfo :type Hit%20Result%20Structure%20%28by%20ref%29) (InstigatedBy :type Controller%20Object%20Reference) (DamageCauser :type Actor%20Object%20Reference))
  (bind _floating_healtbar (CallFunction|GetHealthBarWidget0))
  (bind _capsulecomponent (Variables|Default|GetCapsuleComponent))
  (bind _value (Default|GetCurrentValue _floating_healtbar "NewEnumerator0"))
  (Variables|Default|SetDamage_0 (stale Game|Damage|EventAnyDamage Damage))
  (Variables|Default|SetDamage%20Causer (stale Game|Damage|EventAnyDamage DamageCauser))
  (bind _output_get (Variables|Default|SetDamageCauserRadial DamageCauser))
  (Variables|Default|SetDamage%20Causer _output_get)
  (Variables|Default|SetImpact%20Normal (Math|Vector|GetForwardVector (Variables|/Script/Engine.Character|GetCapsuleComponent (Game|GetPlayerCharacter 0))))
  (if (Variables|Default|GetIA_Dead)
    (CallFunction|EventDeath)
    (elif (>= _value 1.0)
      (Default|SubtractValue _floating_healtbar "NewEnumerator0" (Variables|Default|GetDamage_0))
      (bind _output_get_2 (Variables|Default|SetValue _value))
      (Math|Float|CompareFloat _output_get_2 0.0
        (:>
          (Utilities|FlowControl|Sequence
            (:then_0
              (bind _animplayrate (CallFunction|PlayHighPriorityMontage "/Game/Proto/Rework_All_Project/Animation/Papillon/Animation/papillon_TakeBigdamage_Montage.papillon_TakeBigdamage_Montage" "None" 1.0))
              (Utilities|FlowControl|Delay _animplayrate))
            (:then_1
              ;[1 1 1] Play mesh Skull move not camera Shake
              (Camera|PlayWorldCameraShake 0 (Transformation|GetActorLocation (Game|GetPlayerCharacter 0)) 0.0 4e+03)
              (CallFunction|KnockBack (Variables|Default|GetDamage%20Causer))
              (Audio|PlaySoundatLocation "/Game/Proto/Main/SFX/SFXHADES/Player/Player_Hurt/EmoteHurt_5.EmoteHurt_5" (Transformation|GetActorLocation) "0, 0, 0" -5.0 1.0 0.0 0 0 0 0)
              (Utilities|FlowControl|Delay 0.2)
              (Variables|/Script/Engine.CharacterMovementComponent|SetGroundFriction (Variables|Character|GetCharacterMovement) 3.0)
              (Variables|Default|SetFirstLook true)
              (Variables|Default|SetisHit true)
              ;[1 1 1] Delay Invincible Frame
              (Utilities|FlowControl|Delay 0.02)
              (Collision|SetCollisionResponsetoChannel _capsulecomponent "ECC_GameTraceChannel4" "ECR_Block")
              (Collision|SetCollisionResponsetoChannel _capsulecomponent "ECC_GameTraceChannel5" "ECR_Block")
              (Variables|Default|SetbCanBeDamaged true)
              (Variables|Default|SetFirstLook true)
              (if (Variables|/Game/Proto/Main/Blueprint/Save_BFL_GameInstance/BloodTrial_GameInstance.BloodTrial_GameInstance_C|GetSacrifice_4_Vampirisme (CallFunction|GetInst))
                (bind _asbp_main_base (Utilities|Casting|CastToBP_MainBase (Game|GetPlayerCharacter 0)))
                (Default|Vampirisme _asbp_main_base)
                (Niagara|SpawnSystematLocation "/Game/TA/Scene/Hugo/BloodDrain/BloodDrainVfxV1.BloodDrainVfxV1" (Transformation|GetWorldLocation (Variables|Default|GetCapsuleComponent)))))))
        (:==
          (CallFunction|MortIA :!label _label)
          (Variables|Default|SetIA_Dead false)
          (CallFunction|KnockBack (Variables|Default|GetDamage%20Causer)))
        (:<
          (goto _label)))
      (else
        (Variables|Default|SetIA_Dead true)
        (CallFunction|MortIA)))))

(event EventBeginPlay
  ;[1 1 1] Begin
  (Default|Initialise (CallFunction|GetHealthBarWidget0) self 1.0 (Variables|Default|GetPapillonMaxHP) -1 false false 0 "(R=0.500000,G=0.004823,B=0.000000,A=1.000000)" 0.0 1 false false true true -1.0 3e+03 "")
  (CallFunction|Begin2)
  (CallFunction|PlayerIsSeen))

(fn ConstructionScript
  (|CallParentFunction))

(fn WorldStrafingDirection
  (return "0, 0, 0"))

(fn GetHealthBarWidget0
  (bind _aswidget_floating_healthbar (Utilities|Casting|CastToWidget_FloatingHealthbar (UserInterface|GetUserWidgetObject (Variables|Default|GetWidget))))
  (return _aswidget_floating_healthbar))

(fn SpawnSpell
  (bind _spelldirection (Variables|Default|GetSpellDirection))
  (bind _returnvalue (Transformation|GetWorldTransform _spelldirection))
  (Development|PrintString "0")
  ;[0.05725 1 0] Spell unique
  (bind _returnvalue_2 (Game|SpawnActorfromClass "/Game/Proto/Proto_Florian/Blueprints/Projectile_Papillon/ProjPapillon.ProjPapillon_C" (Math|Transform|MakeTransform (.location _returnvalue) (.rotation _returnvalue) "0.300000,0.300000,0.300000") "AlwaysSpawn" self 0))
  (Physics|AddImpulse (Variables|/Game/Proto/Proto_Florian/Blueprints/Projectile_Papillon/ProjPapillon.ProjPapillon_C|GetBoule _returnvalue_2) (* (Math|Vector|GetForwardVector _spelldirection) 1e+03) "None" false))

(fn PlayHighPriorityMontage
  (params (Montage :type Anim%20Montage%20Object%20Reference) (StartSectionName :type Name) (InPlayRate :type Float%20%28double-precision%29))
  (if (not (Animation|Montage|MontageIsPlaying (Components|SkeletalMesh|GetAnimInstance (Variables|Character|GetMesh)) Montage))
    (bind _output_get (Variables|Default|SetHighPriorityMontage Montage))
    (bind _returnvalue (Animation|PlayAnimMontage _output_get InPlayRate StartSectionName))
    (return _returnvalue)))

(fn KnockBack
  (params (HitActor :type Actor%20Object%20Reference))
  (Variables|Default|SetNewVar_0 (Transformation|GetActorForwardVector HitActor))
  (CallFunction|InvincibleFrame))

(fn InvincibleFrame
  (bind _capsulecomponent (Variables|Default|GetCapsuleComponent))
  (bind _charactermovement (Variables|Character|GetCharacterMovement))
  (Collision|SetCollisionResponsetoChannel _capsulecomponent "ECC_GameTraceChannel4" "ECR_Ignore")
  (Collision|SetCollisionResponsetoChannel _capsulecomponent "ECC_GameTraceChannel5" "ECR_Ignore")
  (Variables|Default|SetbCanBeDamaged false)
  (Variables|/Script/Engine.CharacterMovementComponent|SetGroundFriction _charactermovement 0.0)
  (Variables|/Script/Engine.MovementComponent|SetVelocity _charactermovement "0, 0, 0"))

(fn TakePVEDamage
  (params (HitResult :type Hit%20Result%20Structure) (DamageAmount :type Float%20%28double-precision%29) (Attacker :type Actor%20Object%20Reference) (AttackerID :type Integer)))

(fn BeginPlayDeathCheck
  (Variables|Default|SetIA_Dead false)
  (if (Variables|Default|GetIA_Dead)
    (CallFunction|Death)
    (bind _output_get (Variables|Default|SetIA_Dead true))
    (return _output_get)
    (else
      (return false))))

(fn Death
  (bind _returnvalue (Pawn|GetController))
  (bind _capsulecomponent (Variables|Default|GetCapsuleComponent))
  (bind _mesh (Variables|Character|GetMesh))
  (bind _returnvalue_2 (AI|GetAIController _returnvalue))
  (Default|DeathWeaponDrop (Variables|Default|GetCombatStatusComponent))
  ;[1 1 1] Remove Capsule Collision
  (Utilities|IsValid _capsulecomponent
    (:Is%20Valid
      (Collision|SetCollisionEnabled _capsulecomponent "NoCollision"))
    (:Is%20Not%20Valid
      _))
  ;[1 1 1] Set Overlap For Mesh - Needs to Overlap Pawn For Looting
  (Collision|SetCollisionResponsetoChannel _mesh "ECC_WorldStatic" "ECR_Block")
  (Collision|SetCollisionResponsetoChannel _mesh "ECC_WorldDynamic" "ECR_Block")
  (Collision|SetCollisionResponsetoChannel _mesh "ECC_Pawn" "ECR_Overlap")
  ;[1 1 1] Go Ragdoll
  (Physics|SetSimulatePhysics (Variables|Character|GetMesh) true)
  ;[1 1 1] Stops AI Logic
  (Utilities|IsValid _returnvalue_2
    (:Is%20Valid
      (AI|Logic|StopLogic (Variables|/Script/AIModule.AIController|GetBrainComponent _returnvalue_2) "Death"))
    (:Is%20Not%20Valid
      _))
  ;[1 1 1] Destroy Investigating Mesh & Health Bar
  (Components|DestroyComponent (Variables|Default|GetHealthHUD))
  ;[1 1 1] Stops Running Anim BP
  (Components|Animation|SetAnimationMode (Variables|Character|GetMesh) "AnimationCustomMode"))