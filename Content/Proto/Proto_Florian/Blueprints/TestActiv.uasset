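; Prototype trigger actor that unlocks jumping for the player when they touch its box.
; On overlap by BP_MainCharacter it sets JumpActive on the character every time.
; On the first touch only, guarded by AlreadyTaken, it turns its spotlight green, prints a message, plays a sound and adds JumpPoints to the character's Score.
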(event OnComponentBeginOverlap(Box)
  (params (OverlappedComponent :type Primitive%20Component%20Object%20Reference) (OtherActor :type Actor%20Object%20Reference) (OtherComp :type Primitive%20Component%20Object%20Reference) (OtherBodyIndex :type Integer) (bFromSweep :type Boolean) (SweepResult :type Hit%20Result%20Structure%20%28by%20ref%29))
  (bind _asbp_florian_character (Utilities|Casting|CastToBP_MainCharacter OtherActor))
  (Variables|/Game/Proto/Main/Blueprint/BP_MainCharacter.BP_MainCharacter_C|SetJumpActive _asbp_florian_character true)
  (if (not (Variables|Default|GetAlreadyTaken?))
    (Rendering|Components|Light|SetLightColor (Variables|Default|GetSpotLight) "(R=0.000000,G=1.000000,B=0.211823,A=1.000000)" true)
    (Development|PrintText "Jump Allowed")
    (Audio|PlaySound2D "/Game/Proto/Proto_Florian/SFX/ActiveJump.ActiveJump" 1.0 1.0 0.0 0 0)
    (Variables|Default|SetAlreadyTaken? true)
    (Variables|/Game/Proto/Main/Blueprint/BP_MainCharacter.BP_MainCharacter_C|SetScore _asbp_florian_character (+ (Variables|/Game/Proto/Main/Blueprint/BP_MainCharacter.BP_MainCharacter_C|GetScore _asbp_florian_character) (Variables|Default|GetJumpPoints)))))

(fn ConstructionScript)