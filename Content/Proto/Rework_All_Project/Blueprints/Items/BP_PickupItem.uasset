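; Base world pickup item, built from a data table row with static or skeletal mesh and optionally random quantity.
; Interact adds it to the character's inventory, updates quests and destroys it, or warns when full.
; Pickups are stored via the GameMode by object name plus location, and BeginPlay destroys those already in the save.
; Spawn&Use strips pickup components and calls empty consume or weapon events for children to implement.
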(event Custom|WeaponOnUse
  ;[1 1 1] Use Item, Called From Inventory
  ;;[0.2431 0.696 1] Open For Children To Use
)

(event Custom|ConsumeOnUse
  ;[1 1 1] Use Item, Called From Inventory
  ;;[0.2431 0.696 1] Open For Children To Use
)

(event EventInteract
  (params (Character :type Character%20Object%20Reference))
  (bind _returnvalue (Actor|GetComponentbyClass Character "/Game/FlexibleCombatSystem/Blueprints/Components/InventoryComponent.InventoryComponent_C"))
  (bind _iteminfo (Variables|Status|GetItemInfo))
  (bind (_itemstructure _datatableinfo _quantity _slotnumber _itemid) (Utilities|Struct|BreakS_SlotInfo _iteminfo))
  ;[1 1 1] On Character Interact, Add Item To Inventory
  (if (Variables|/Game/FlexibleCombatSystem/Blueprints/Components/InventoryComponent.InventoryComponent_C|GetInventoryFull _returnvalue)
    (bind _returnvalue_2 (UserInterface|CreateWidget "/Game/FlexibleCombatSystem/Widgets/Combat/WB_PopupText.WB_PopupText_C" 0 "Inventory Full!"))
    (UserInterface|Viewport|AddtoViewport _returnvalue_2 0)
    (Audio|PlaySoundatLocation "/Game/FlexibleCombatSystem/SoundFX/General/SW_Warning.SW_Warning" (Transformation|GetActorLocation) "0, 0, 0" 1.0 1.0 0.0 0 0 0)
    (else
      (Default|AddtoInventory _returnvalue (Utilities|Struct|MakeS_SlotInfo _itemstructure _datatableinfo (select (== _quantity 0) 1 _quantity) _slotnumber _itemid) false false)
      (CallFunction|IsQuestActor (Game|GetPlayerController 0) (.quantity (Variables|Status|GetItemInfo)) (CallFunction|GetQuestName))
      (Audio|PlaySoundatLocation "/Game/FlexibleCombatSystem/SoundFX/General/SW_PickupItem.SW_PickupItem" (Transformation|GetActorLocation) "0, 0, 0" 1.0 1.0 0.0 0 0 0)
      (CallFunction|PassItemforSave)
      (CallFunction|DestroySelf))))

(event EventBeginPlay
  ;[1 1 1] Begin Play Setup
  (CallFunction|InitializeItem)
  (CallFunction|SetMesh)
  (CallFunction|PickedUpCheck))

(event EventSpawn&Use
  (params (CharacterRef :type Character%20Object%20Reference) (ItemInfo :type S%20Slot%20Info%20Structure))
  ;[1 1 1] Use Item, Called From Inventory
  (Variables|References|SetCharacterRef CharacterRef)
  (Variables|Status|SetItemInfo ItemInfo)
  (CallFunction|SpawnSetup)
  (if (Utilities|Enum|Equal(Enum) (.ItemType (Utilities|Struct|BreakS_ItemData (Utilities|Struct|BreakS_SlotInfo (Variables|Status|GetItemInfo)))) "NewEnumerator14")
    (CallFunction|ConsumeonUse)
    (else
      (CallFunction|WeapononUse))))

(fn ConstructionScript
  (bind _itemskeletal (Variables|Default|GetItemSkeletal))
  (bind _itemskeletal_2 (Variables|Default|GetItemSkeletal))
  (bind _datasetup (Variables|Default|GetDataSetup))
  (bind _itemstatic (Variables|Default|GetItemStatic))
  (bind (_datatableinfo _quantity) (Utilities|Struct|BreakS_ItemSetupData _datasetup))
  (bind _relativelocation (Variables|/Script/Engine.SceneComponent|GetRelativeLocation _itemskeletal_2))
  (bind (_datatable _rowname) (Utilities|Struct|BreakDataTableRowHandle _datatableinfo))
  (bind (_quantity_2 _randomizequantity _quantitymin _quantitymax) (Utilities|Struct|BreakS_QuantityOptions _quantity))
  (Utilities|IsValid _datatable
    (:Is%20Valid
      (bind _returnvalue (Utilities|GetDataTableRow _datatable _rowname)
        (:then
          (Utilities|IsValid (.ItemMesh (Utilities|Struct|BreakS_ItemData (.ItemStructure (Utilities|Struct|BreakS_SlotInfo (Utilities|Struct|MakeS_SlotInfo _returnvalue _datatableinfo (select _randomizequantity (Math|Random|RandomIntegerinRange _quantitymin _quantitymax) _quantity_2))))))
            (:Is%20Valid
              (Components|StaticMesh|SetStaticMesh _itemstatic (.ItemMesh (Utilities|Struct|BreakS_ItemData (.ItemStructure (Utilities|Struct|BreakS_SlotInfo (Utilities|Struct|MakeS_SlotInfo _returnvalue _datatableinfo (select _randomizequantity (Math|Random|RandomIntegerinRange _quantitymin _quantitymax) _quantity_2))))))))
            (:Is%20Not%20Valid
              (Rendering|SetVisibility _itemstatic false false)
              (Collision|SetCollisionEnabled _itemstatic "NoCollision")))
          (Utilities|IsValid (.BowArmorSkeletalMesh (Utilities|Struct|BreakS_EquipmentInfo (.EquipmentInfo (Utilities|Struct|BreakS_ItemData (.ItemStructure (Utilities|Struct|BreakS_SlotInfo (Utilities|Struct|MakeS_SlotInfo _returnvalue _datatableinfo (select _randomizequantity (Math|Random|RandomIntegerinRange _quantitymin _quantitymax) _quantity_2))))))))
            (:Is%20Valid
              (Class|SkinnedMeshComponent|SetSkeletalMesh _itemskeletal (.BowArmorSkeletalMesh (Utilities|Struct|BreakS_EquipmentInfo (.EquipmentInfo (Utilities|Struct|BreakS_ItemData (.ItemStructure (Utilities|Struct|BreakS_SlotInfo (Utilities|Struct|MakeS_SlotInfo _returnvalue _datatableinfo (select _randomizequantity (Math|Random|RandomIntegerinRange _quantitymin _quantitymax) _quantity_2)))))))) true)
              (Transformation|SetRelativeLocation _itemskeletal_2 (Math|Vector|MakeVector (- (.x _relativelocation) (.SMZ-Offset (Utilities|Struct|BreakS_EquipmentInfo (.EquipmentInfo (Utilities|Struct|BreakS_ItemData (.ItemStructure (Utilities|Struct|BreakS_SlotInfo (Utilities|Struct|MakeS_SlotInfo _returnvalue _datatableinfo (select _randomizequantity (Math|Random|RandomIntegerinRange _quantitymin _quantitymax) _quantity_2))))))))) (.y _relativelocation) (.z _relativelocation)) false false))
            (:Is%20Not%20Valid
              (Rendering|SetVisibility _itemskeletal false false)
              (Collision|SetCollisionEnabled _itemskeletal "NoCollision"))))))))

(fn PassItemforSave
  ;[1 1 1] We Use Display Name + Actor Location As Display Name Is Unique Per Placed Object. We combine it with Actor Location as it's not Unique Between Levels so this ensures we don't get 2 IDs the same
  (Class|IGameMode|StorePickedItem(Message) (Game|GetGameMode) (Utilities|String|Append (Utilities|GetObjectName self) (Utilities|String|ToString(Vector) (Transformation|GetActorLocation)))))

(fn DestroySelf
  (Default|RemoveActorTag (Variables|Default|GetOutlineComponent))
  (Class|IWeaponInterface|DestroySelf&Attachments(Message) self)
  (Actor|DestroyActor))

(fn SpawnSetup
  (bind _outlinecomponent (Variables|Default|GetOutlineComponent))
  ;[1 1 1] Remove Tag Overlap
  (CallFunction|SetMeshDestroy)
  (Components|DestroyComponent (Variables|Default|GetCapsule))
  (Default|RemoveActorTag _outlinecomponent)
  (Components|DestroyComponent _outlinecomponent)
  ;[1 1 1] Set Equipment Comp Ref
  (Variables|Default|SetEquipmentComponent (Actor|GetComponentbyClass (Variables|References|GetCharacterRef) "/Game/FlexibleCombatSystem/Blueprints/Components/EquipmentComponent.EquipmentComponent_C")))

(fn InitializeItem
  (bind _datasetup (Variables|Default|GetDataSetup))
  (bind (_datatableinfo _quantity) (Utilities|Struct|BreakS_ItemSetupData _datasetup))
  (bind (_datatable _rowname) (Utilities|Struct|BreakDataTableRowHandle _datatableinfo))
  (bind (_quantity_2 _randomizequantity _quantitymin _quantitymax) (Utilities|Struct|BreakS_QuantityOptions _quantity))
  (Utilities|IsValid _datatable
    (:Is%20Valid
      (bind _returnvalue (Utilities|GetDataTableRow _datatable _rowname)
        (:then
          (Variables|Status|SetItemInfo (Utilities|Struct|MakeS_SlotInfo _returnvalue _datatableinfo (select _randomizequantity (Math|Random|RandomIntegerinRange _quantitymin _quantitymax) _quantity_2))))))))

(fn SetMesh
  (bind _itemstatic (Variables|Default|GetItemStatic))
  (bind _itemskeletal (Variables|Default|GetItemSkeletal))
  (bind _iteminfo (Variables|Status|GetItemInfo))
  (bind _itemstructure (Utilities|Struct|BreakS_SlotInfo _iteminfo))
  (bind (_itemmesh _isspawneditem _weaponvfxinfo _equipmentinfo) (Utilities|Struct|BreakS_ItemData _itemstructure))
  (bind _bowarmorskeletalmesh (Utilities|Struct|BreakS_EquipmentInfo _equipmentinfo))
  ;[1 1 1] Set Meshes, Destroy the One Not Used
  (Utilities|IsValid _itemmesh
    (:Is%20Valid
      (Components|StaticMesh|SetStaticMesh _itemstatic _itemmesh)
      (Rendering|SetVisibility _itemstatic true false)
      (Variables|Default|SetSkeletalMesh false))
    (:Is%20Not%20Valid
      (Variables|Default|SetSkeletalMesh true)))
  (Utilities|IsValid _bowarmorskeletalmesh
    (:Is%20Valid
      (Class|SkinnedMeshComponent|SetSkeletalMesh _itemskeletal _bowarmorskeletalmesh true)
      (Rendering|SetVisibility _itemskeletal true false))))

(fn GetQuestName
  (bind _iteminfo (Variables|Status|GetItemInfo))
  (bind _itemstructure (Utilities|Struct|BreakS_SlotInfo _iteminfo))
  (bind _questinfo (Utilities|Struct|BreakS_ItemData _itemstructure))
  (bind _questitem (Utilities|Struct|BreakS_QuestData _questinfo))
  (bind (_datatable _rowname) (Utilities|Struct|BreakDataTableRowHandle _questitem))
  ;[1 1 1] Finds Quest In DT Based Upon Struct
  ;;[1 1 1] Check Incase Item Not Quest Related
  (Utilities|IsValid _datatable
    (:Is%20Valid
      (bind _returnvalue (Utilities|GetDataTableRow _datatable _rowname)
        (:then
          (return (.QuestID (Utilities|Struct|BreakS_QuestInfo _returnvalue))))))))

(fn SetMeshDestroy
  (bind _itemstatic (Variables|Default|GetItemStatic))
  (bind _itemskeletal (Variables|Default|GetItemSkeletal))
  (bind _iteminfo (Variables|Status|GetItemInfo))
  (bind _itemstructure (Utilities|Struct|BreakS_SlotInfo _iteminfo))
  (bind (_itemmesh _isspawneditem _weaponvfxinfo _equipmentinfo) (Utilities|Struct|BreakS_ItemData _itemstructure))
  (bind _bowarmorskeletalmesh (Utilities|Struct|BreakS_EquipmentInfo _equipmentinfo))
  ;[1 1 1] Set Meshes, Destroy the One Not Used
  (Utilities|IsValid _itemmesh
    (:Is%20Valid
      (Components|StaticMesh|SetStaticMesh _itemstatic _itemmesh)
      (Variables|Default|SetSkeletalMesh false))
    (:Is%20Not%20Valid
      (Components|DestroyComponent _itemstatic)
      (Variables|Default|SetSkeletalMesh true)))
  (Utilities|IsValid _bowarmorskeletalmesh
    (:Is%20Valid
      (Class|SkinnedMeshComponent|SetSkeletalMesh _itemskeletal _bowarmorskeletalmesh true))
    (:Is%20Not%20Valid
      (Components|DestroyComponent _itemskeletal))))

(fn PickedUpCheck
  ;[1 1 1] Checks IF Picked Up - Destroys IF Is
  (bind _returnvalue (SaveGame|LoadGamefromSlot "save1"))
  (bind _asbp_save_game (Utilities|Casting|CastToBP_SaveGame _returnvalue))
  (bind _array_element (Utilities|Array|ForEachLoopwithBreak (Variables|/Game/FlexibleCombatSystem/Blueprints/BP_SaveGame.BP_SaveGame_C|GetPickedUpActors _asbp_save_game) :!label _label)
    (:LoopBody
      (if (Utilities|Enum|Equal(Enum) _array_element (Utilities|String|Append (Utilities|GetObjectName self) (Utilities|String|ToString(Vector) (Transformation|GetActorLocation))))
        (Actor|DestroyActor)
        (goto _label Break)))))

(fn RetrieveOutlineInfo
  (bind _itemstatic (Variables|Default|GetItemStatic))
  (bind _itemskeletal (Variables|Default|GetItemSkeletal))
  (bind _iteminfo (Variables|Status|GetItemInfo))
  (bind (_itemstructure _datatableinfo _quantity) (Utilities|Struct|BreakS_SlotInfo _iteminfo))
  (bind (_name _itemrarity) (Utilities|Struct|BreakS_ItemData _itemstructure))
  (return _name _itemrarity "NewEnumerator0" _quantity (select (Utilities|IsValid _itemstatic) _itemstatic 0) 0 (select (Utilities|IsValid _itemskeletal) _itemskeletal 0)))