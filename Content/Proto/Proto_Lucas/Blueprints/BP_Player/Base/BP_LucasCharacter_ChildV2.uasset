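; Prototype player character child Blueprint (Lucas) that adds movement input and test sound playback.
; Four movement axes pass a small dead zone and push the pawn along fixed world diagonals, independent of control rotation, as in isometric-style controls.
; Numpad 1-3 play music or ambience sounds at the character's location.
; BlockCheck compares yaw with the attacking actor, but its condition is true for any difference except exactly 360 degrees.
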(event EventBeginPlay
  (|CallParentFunction) ; This node is disabled and will not be called.\nDrag off pins to build functionality.
)

(event Collision|EventActorBeginOverlap
  (params (OtherActor :type Actor%20Object%20Reference)))

(event EventTick
  (params (DeltaSeconds :type Float%20%28single-precision%29))
  (|CallParentFunction DeltaSeconds) ; This node is disabled and will not be called.\nDrag off pins to build functionality.
)

(event Input|AxisEvents|InputAxisMoveForward
  (params (AxisValue :type Float%20%28single-precision%29))
  ;[1 1 1] Character movement
  (if (>= (Math|Float|Absolute(Float) (* AxisValue 1e+01)) 1.0)
    (Pawn|Input|AddMovementInput (Class|PawnMovementComponent|GetPawnOwner (Variables|Character|GetCharacterMovement)) "1000.000000,-1000.000000, 0" AxisValue false)))

(event Input|AxisEvents|InputAxisMoveBackward
  (params (AxisValue :type Float%20%28single-precision%29))
  ;[1 1 1] Character movement
  (if (>= (Math|Float|Absolute(Float) (* AxisValue 1e+01)) 1.0)
    (Pawn|Input|AddMovementInput (Class|PawnMovementComponent|GetPawnOwner (Variables|Character|GetCharacterMovement)) "1000.000000,-1000.000000, 0" AxisValue false)))

(event Input|AxisEvents|InputAxisMoveLeft
  (params (AxisValue :type Float%20%28single-precision%29))
  ;[1 1 1] Character movement
  (if (>= (Math|Float|Absolute(Float) (* AxisValue 1e+01)) 1.0)
    (Pawn|Input|AddMovementInput (Class|PawnMovementComponent|GetPawnOwner (Variables|Character|GetCharacterMovement)) "1000.000000,1000.000000, 0" AxisValue false)))

(event Input|AxisEvents|InputAxisMoveRight
  (params (AxisValue :type Float%20%28single-precision%29))
  ;[1 1 1] Character movement
  (if (>= (Math|Float|Absolute(Float) (* AxisValue 1e+01)) 1.0)
    (Pawn|Input|AddMovementInput (Class|PawnMovementComponent|GetPawnOwner (Variables|Character|GetCharacterMovement)) "1000.000000,1000.000000, 0" AxisValue false)))

(event Input|KeyboardEvents|NumPadTwo
  (params (Key :type Key%20Structure :default "None"))
  (:Pressed
    (Audio|PlaySoundatLocation "/Game/Proto/Main/SFX/Music/AMBIANCE_V1.AMBIANCE_V1" (Transformation|GetActorLocation) "0, 0, 0" 1.0 1.0 0.0 0 0 0 0)))

(event Input|KeyboardEvents|NumPadOne
  (params (Key :type Key%20Structure :default "None"))
  (:Pressed
    (Audio|PlaySoundatLocation "/Game/Proto/Main/SFX/Music/SALLES_MYST7RE_V1.SALLES_MYST7RE_V1" (Transformation|GetActorLocation) "0, 0, 0" 1.0 1.0 0.0 0 0 0 0)))

(event Input|KeyboardEvents|NumPadThree
  (params (Key :type Key%20Structure :default "None"))
  (:Pressed
    (Audio|PlaySoundatLocation "/Game/Proto/Main/SFX/Music/AmbientTemple.AmbientTemple" (Transformation|GetActorLocation) "0, 0, 0" 1.0 1.0 0.0 0 0 0 0)))

(fn ConstructionScript
  (|CallParentFunction))

(fn BlockCheck
  (bind _returnvalue (Transformation|GetActorRotation))
  (bind _attackingactor_0 (Variables|Default|GetAttackingActor_0))
  (bind _returnvalue_2 (Transformation|GetActorRotation _attackingactor_0))
  (bind _returnvalue_3 (- (.yaw _returnvalue) (.yaw _returnvalue_2)))
  (return (or (> _returnvalue_3 3.6e+02) (< _returnvalue_3 3.6e+02))))