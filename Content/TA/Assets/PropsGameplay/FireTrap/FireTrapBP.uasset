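; Fire trap prop that fires when its trigger box is overlapped, damaging the player and showing a lava HUD feedback.
; After a delay it plays the trap animation and Niagara effect, drives an emissive material pulse by timeline, and slides the FireBox hitbox out and back.
; FireBox overlaps during a burst apply game-instance lava damage through DoOnce gates; the feedback widget is removed on exit.
; The timeline's end re-arms the trap.
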(event OnComponentBeginOverlap(Box)
  (params (OverlappedComponent :type Primitive%20Component%20Object%20Reference) (OtherActor :type Actor%20Object%20Reference) (OtherComp :type Primitive%20Component%20Object%20Reference) (OtherBodyIndex :type Integer) (bFromSweep :type Boolean) (SweepResult :type Hit%20Result%20Structure%20%28by%20ref%29))
  (bind _firetrapanim (Variables|Default|GetFireTrapAnim))
  (if (Variables|Default|Getfinish)
    (Variables|Default|Setfinish false)
    (Utilities|FlowControl|Delay (Variables|Default|Getdelay))
    (Components|Animation|PlayAnimation _firetrapanim "/Game/TA/Assets/PropsGameplay/FireTrap/FireTrapAnim_Anim.FireTrapAnim_Anim" false)
    (Components|Activation|SetActive (Variables|Default|GetNiagara) true true)
    (bind _returnvalue (Rendering|Material|CreateDynamicMaterialInstance _firetrapanim 0 (Rendering|Material|GetMaterial _firetrapanim 0) "None" :!class /Script/Engine.PrimitiveComponent))
    (Utilities|FlowControl|Sequence
      (:then_0
        (bind _newtrack_0 (Timeline|Timeline_0 PlayFromStart)
          (:Update
            (Rendering|Material|SetScalarParameterValue _returnvalue "Emissiv" (* _newtrack_0 15.0) :!class /Script/Engine.MaterialInstanceDynamic))
          (:Finished
            (Variables|Default|Setfinish true))))
      (:then_1
        (Components|MoveComponentTo (Variables|Default|GetFireBox) (+ (Variables|Default|GetFireOriginLocation) "0,400.000000,0.000000") (Variables|Default|GetFireOriginRotation) true true 0.3 false)
        (Utilities|FlowControl|Delay 1.0)
        (Components|MoveComponentTo (Variables|Default|GetFireBox) (+ (Variables|Default|GetFireOriginLocation) "") (Variables|Default|GetFireOriginRotation) true true 0.3 false)))))

(event OnComponentBeginOverlap(FireBox)
  (params (OverlappedComponent :type Primitive%20Component%20Object%20Reference) (OtherActor :type Actor%20Object%20Reference) (OtherComp :type Primitive%20Component%20Object%20Reference) (OtherBodyIndex :type Integer) (bFromSweep :type Boolean) (SweepResult :type Hit%20Result%20Structure%20%28by%20ref%29))
  ;[1 1 1] Need ID BP ==> Damage Player + IA
  (Utilities|Casting|CastToBP_MainBase OtherActor)
  (if (not (Variables|Default|Getfinish))
    (Utilities|FlowControl|DoOnce false
      (:Completed
        (bind _returnvalue (Game|ConstructObjectfromClass "/Game/Proto/Main/HUD/Lava_Feedback.Lava_Feedback_C"))
        (UserInterface|Viewport|AddtoViewport _returnvalue 0)
        (Default|LavaEffectHUD _returnvalue)
        (Variables|Default|Setremovedhud? false)
        (if (not (Variables|Default|Getfinish))
          (bind _asbp_main_base (Utilities|Casting|CastToBP_MainBase (Game|GetPlayerCharacter 0)))
          (Utilities|FlowControl|DoOnce false :!label _label
            (:Completed
              (Game|Damage|ApplyDamage _asbp_main_base (Variables|/Game/Proto/Main/Blueprint/Save_BFL_GameInstance/BloodTrial_GameInstance.BloodTrial_GameInstance_C|GetLavaDamage (CallFunction|GetInst)) 0 self)
              (Utilities|FlowControl|Delay 0.5)
              (goto _label Reset))))))))

(event OnComponentEndOverlap(FireBox)
  (params (OverlappedComponent :type Primitive%20Component%20Object%20Reference) (OtherActor :type Actor%20Object%20Reference) (OtherComp :type Primitive%20Component%20Object%20Reference) (OtherBodyIndex :type Integer))
  (Utilities|Casting|CastToBP_MainBase OtherActor)
  (if (not (Variables|Default|Getremovedhud?))
    (Widget|RemovefromParent (stale OnComponentBeginOverlap(FireBox) _returnvalue))
    (Variables|Default|Setremovedhud? true)
    (Utilities|FlowControl|DoOnce false) ; enters at Reset
  ))

(event EventBeginPlay
  (bind _firebox (Variables|Default|GetFireBox))
  (Input|EnableInput (Game|GetPlayerController 0))
  (Components|Activation|SetActive (Variables|Default|GetNiagara) false false)
  (Variables|Default|SetFireOriginRotation (Variables|/Script/Engine.SceneComponent|GetRelativeRotation _firebox))
  (Variables|Default|SetFireOriginLocation (Variables|/Script/Engine.SceneComponent|GetRelativeLocation _firebox)))

(fn ConstructionScript)