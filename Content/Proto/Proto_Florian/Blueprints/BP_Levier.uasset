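; BP_Levier is a prototype lever actor that sets a portal (BP_Portail) moving when activated.
; Its collider flags InCollision and calls NearTheLever on an overlapping BP_FlorianCharacter_Child tagged Player, and any end overlap clears the flag.
; LeverActive, which nothing in this graph calls, destroys the lever, then calls Movement on the BP_Portail found by GetActorOfClass, with no direct link to a specific portal.
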(event OnComponentBeginOverlap(LeverCollider)
  (params (OverlappedComponent :type Primitive%20Component%20Object%20Reference) (OtherActor :type Actor%20Object%20Reference) (OtherComp :type Primitive%20Component%20Object%20Reference) (OtherBodyIndex :type Integer) (bFromSweep :type Boolean) (SweepResult :type Hit%20Result%20Structure%20%28by%20ref%29))
  (bind _asbp_florian_character_child (Utilities|Casting|CastToBP_FlorianCharacter_Child OtherActor))
  (if (Actor|ActorHasTag _asbp_florian_character_child "Player")
    (Variables|Default|SetInCollision? true)
    (Default|NeartheLever _asbp_florian_character_child)))

(event OnComponentEndOverlap(LeverCollider)
  (params (OverlappedComponent :type Primitive%20Component%20Object%20Reference) (OtherActor :type Actor%20Object%20Reference) (OtherComp :type Primitive%20Component%20Object%20Reference) (OtherBodyIndex :type Integer))
  (Variables|Default|SetInCollision? false))

(event Custom|LeverActive
  (Actor|DestroyActor)
  (bind _returnvalue (Actor|GetActorOfClass "/Game/Proto/Proto_Florian/Blueprints/BP_Portail.BP_Portail_C"))
  (Default|Movement _returnvalue))

(fn ConstructionScript)