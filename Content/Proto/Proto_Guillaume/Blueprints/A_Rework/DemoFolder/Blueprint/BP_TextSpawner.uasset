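; BP_TextSpawner is a trigger volume that shows a tutorial text widget while the player stands inside it.
; When an actor tagged Player begins overlapping the box, a DoOnce creates WB_TutorialText with the configured message and adds it to the viewport.
; On exit, a valid widget receives EventMoveDown and the DoOnce resets, allowing the text to show again.
; The construction script sizes the box from exposed X and Y scales with a fixed height.
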(event OnComponentBeginOverlap(Box)
  (params (OverlappedComponent :type Primitive%20Component%20Object%20Reference) (OtherActor :type Actor%20Object%20Reference) (OtherComp :type Primitive%20Component%20Object%20Reference) (OtherBodyIndex :type Integer) (bFromSweep :type Boolean) (SweepResult :type Hit%20Result%20Structure%20%28by%20ref%29))
  (if (Actor|ActorHasTag OtherActor "Player")
    (Utilities|FlowControl|DoOnce false
      (:Completed
        (bind _returnvalue (UserInterface|CreateWidget "/Game/FlexibleCombatSystem/Widgets/General/WB_TutorialText.WB_TutorialText_C" 0 (Variables|Default|GetText)))
        (UserInterface|Viewport|AddtoViewport _returnvalue 0)
        (Variables|Default|SetTextWidget _returnvalue)))))

(event OnComponentEndOverlap(Box)
  (params (OverlappedComponent :type Primitive%20Component%20Object%20Reference) (OtherActor :type Actor%20Object%20Reference) (OtherComp :type Primitive%20Component%20Object%20Reference) (OtherBodyIndex :type Integer))
  (if (Actor|ActorHasTag OtherActor "Player")
    (Utilities|IsValid (stale OnComponentBeginOverlap(Box) _returnvalue)
      (:Is%20Valid
        (Default|EventMoveDown (stale OnComponentBeginOverlap(Box) _returnvalue))
        (Utilities|FlowControl|DoOnce false) ; enters at Reset
      ))))

(event EventBeginPlay)

(event Collision|EventActorBeginOverlap
  (params (OtherActor :type Actor%20Object%20Reference)))

(event EventTick
  (params (DeltaSeconds :type Float%20%28single-precision%29)))

(fn ConstructionScript
  (Transformation|SetRelativeScale3D (Variables|Default|GetBox) (Math|Vector|MakeVector (Variables|Default|GetCollisionScaleX) (Variables|Default|GetCollisionScaleY) 1e+01)))