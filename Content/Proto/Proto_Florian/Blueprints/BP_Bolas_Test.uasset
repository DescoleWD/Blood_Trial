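; Prototype bolas projectile that flies out, stops on blocking geometry, then returns to the player.
; Each Tick runs a tiny visibility trace: a hit freezes the projectile and triggers Return after 5 seconds, otherwise Return follows a 2-second delay.
; Return glides the root to the character's SpawnBloodWave placeholder, destroys the actor and calls BolasReturn on BP_FlorianCharacter_Child.
; That character bumping it adds an input-direction impulse; enemy hits remain unimplemented.
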(event Custom|Return
  (Utilities|FlowControl|DoOnce false
    (:Completed
      ;[1 1 1] à changer avec le spawn bolas
      (bind _asbp_main_character (Utilities|Casting|CastToBP_MainCharacter (Game|GetPlayerCharacter 0)))
      (Components|MoveComponentTo (Variables|Default|GetDefaultSceneRoot) (.location (Transformation|GetWorldTransform (Variables|/Game/Proto/Main/Blueprint/BP_MainCharacter.BP_MainCharacter_C|GetSpawnBloodWave _asbp_main_character))) (.rotation (Transformation|GetWorldTransform (Variables|/Game/Proto/Main/Blueprint/BP_MainCharacter.BP_MainCharacter_C|GetSpawnBloodWave _asbp_main_character))) false true 0.5 false)
      (Actor|DestroyActor)
      (Variables|Default|SetReturning true)
      (bind _asbp_florian_character_child (Utilities|Casting|CastToBP_FlorianCharacter_Child (Game|GetPlayerCharacter 0)))
      (Default|BolasReturn _asbp_florian_character_child))))

(event EventTick
  (params (DeltaSeconds :type Float%20%28single-precision%29))
  (bind _projectilemovement (Variables|Default|GetProjectileMovement))
  (bind _staticmesh (Variables|Default|GetStaticMesh))
  (bind _returnvalue (Transformation|GetWorldLocation _staticmesh))
  (bind _outhit (Collision|LineTraceByChannel (Transformation|GetWorldLocation _staticmesh) (Math|Vector|MakeVector (+ (.x _returnvalue) 1.0) (.y _returnvalue) (.z _returnvalue)) "TraceTypeQuery1" false 0 "None"))
  (if (.bBlockingHit (Collision|BreakHitResult _outhit))
    ;[1 1 1] Rajouter node pour quand il touche un ennemi
    (Utilities|FlowControl|DoOnce false
      (:Completed
        (Components|Movement|StopMovementImmediately _projectilemovement)
        (Variables|/Script/Engine.ProjectileMovementComponent|SetProjectileGravityScale _projectilemovement 0.0)
        (Utilities|FlowControl|Delay 5.0)
        (CallFunction|Return)))
    (else
      (Utilities|FlowControl|Delay 2.0)
      (CallFunction|Return))))

(event Collision|EventHit
  (params (MyComp :type Primitive%20Component%20Object%20Reference) (Other :type Actor%20Object%20Reference) (OtherComp :type Primitive%20Component%20Object%20Reference) (bSelfMoved :type Boolean) (HitLocation :type Vector :default "0, 0, 0") (HitNormal :type Vector :default "0, 0, 0") (NormalImpulse :type Vector :default "0, 0, 0") (Hit :type Hit%20Result%20Structure%20%28by%20ref%29))
  (bind _asbp_florian_character_child (Utilities|Casting|CastToBP_FlorianCharacter_Child Other))
  (Physics|AddImpulse MyComp (* (Pawn|Components|PawnMovement|GetLastInputVector (Variables|/Script/Engine.Character|GetCharacterMovement _asbp_florian_character_child)) 1.0) "None" false))

(fn ConstructionScript)