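; Arena spawner that runs staged combat rounds, triggered once per reset by the player entering its box.
; It closes the gates and spawns growing waves of randomly styled, stage-levelled BP_EnemyAI at random points in the box, facing the player.
; Enemies report deaths through ActivateActor, which starts the next round or completes the stage, opening gates, updating NPC dialogue and raising difficulty.
; ResetArena destroys spawned mobs and re-arms the trigger.
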(event OnComponentBeginOverlap(Box)
  (params (OverlappedComponent :type Primitive%20Component%20Object%20Reference) (OtherActor :type Actor%20Object%20Reference) (OtherComp :type Primitive%20Component%20Object%20Reference) (OtherBodyIndex :type Integer) (bFromSweep :type Boolean) (SweepResult :type Hit%20Result%20Structure%20%28by%20ref%29))
  ;[1 1 1] Begin Arena & Reset
  (bind _asbp_player_character (Utilities|Casting|CastToBP_PlayerCharacter OtherActor))
  (Utilities|FlowControl|DoOnce false
    (:Completed
      (Default|CloseGates (Variables|Default|GetBP_Gate))
      (Variables|Default|SetCharacterRef _asbp_player_character)
      (CallFunction|BeginArena))))

(event Custom|BeginArena
  (bind _returnvalue (Transformation|GetActorLocation))
  (bind _box (Variables|Default|GetBox))
  (bind _characterref (Variables|Default|GetCharacterRef))
  (bind _returnvalue_2 (Transformation|GetWorldLocation _box))
  (bind _returnvalue_3 (Transformation|GetActorLocation _characterref))
  (bind _boxextent (Variables|/Script/Engine.BoxComponent|GetBoxExtent _box))
  (bind _returnvalue_4 (Math|Random|RandomPointinBoundingBox _returnvalue_2 _boxextent))
  (bind (_x _y) (Math|Vector|BreakVector _returnvalue_4))
  ;[1 1 1] Spawn Enemies
  (for _index (range 1 (+ (Variables|Default|GetCurrentRound) (Variables|Default|GetEnemyIncrementer)))
    (Variables|Default|SetSpawnLocation (Math|Vector|MakeVector _x _y (.z _returnvalue)))
    (bind _returnvalue_5 (Game|SpawnActorfromClass :Class "/Game/FlexibleCombatSystem/Blueprints/AI/BP_EnemyAI.BP_EnemyAI_C" :SpawnTransform (Math|Transform|MakeTransform (Variables|Default|GetSpawnLocation) (Math|Rotator|FindLookatRotation (Variables|Default|GetSpawnLocation) (Math|Vector|MakeVector (.x _returnvalue_3) (.y _returnvalue_3) (.z _returnvalue))) "1,1,1") :CollisionHandlingOverride "AdjustIfPossibleButAlwaysSpawn" :AI%20Combat%20Style (Utilities|Select :Index (Math|Random|RandomIntegerinRange 0 3) :Option%200 "NewEnumerator0" :Option%201 "NewEnumerator1" :Option%202 "NewEnumerator2" :Option%203 "NewEnumerator3" :Option%204 "NewEnumerator4" :Option%205 "NewEnumerator5") :EnemyLevel (Variables|Default|GetCurrentStage) :XP_GivenWhenKilled 50 :BehaviourTree "/Game/FlexibleCombatSystem/Blueprints/AI/BehaviourTrees/BT_MixedCombat.BT_MixedCombat" :CanSwitchAttackStyle (Math|Random|RandomBoolwithWeight 0.25) :EnemyLootInfo (Utilities|Struct|MakeS_LootSetupInfo "Arena Fighter" "NewEnumerator1" 0 true "/Game/FlexibleCombatSystem/DataTables/LootTemplates/DT_Loot-General.DT_Loot-General") :ActivateActorOnDeath self :Quest%20ID "None" :Instigator 0))
    (Niagara|SpawnSystematLocation 0 (Variables|Default|GetSpawnLocation))
    (Utilities|Array|Add (Variables|Default|GetSpawnedMobs) _returnvalue_5)))

(event Custom|ResetArena
  ;[1 1 1] Begin Arena & Reset
  (for _array_element (Variables|Default|GetSpawnedMobs)
    (Utilities|IsValid _array_element
      (:Is%20Valid
        (Actor|DestroyActor _array_element))))
  (Utilities|FlowControl|DoOnce false) ; enters at Reset
)

(event EventActivateActor
  ;[1 1 1] Enemy Killed
  ;;[1 1 1] If All Enemies Slain
  (bind _result (Math|Integer|IncrementInt (Variables|Default|GetDeadEnemies))
    (:%20%20
      (if (== _result (+ (Variables|Default|GetCurrentRound) (Variables|Default|GetEnemyIncrementer)))
        ;;[1 1 1] IF Complete Final Stage
        (if (== (Variables|Default|GetCurrentRound) (Variables|Default|GetRounds%20Per%20Stage))
          ;;[1 1 1] Stage Complete, Open Gates
          (bind _returnvalue (UserInterface|CreateWidget "/Game/FlexibleCombatSystem/Widgets/HUD/WB_PopupTitle.WB_PopupTitle_C" 0 "Stage Complete!"))
          (UserInterface|Viewport|AddtoViewport _returnvalue 0)
          (Default|OpenGates (Variables|Default|GetBP_Gate))
          (Variables|/Game/FlexibleCombatSystem/Blueprints/Components/DialogueComponent.DialogueComponent_C|SetStoredStartLine (Variables|/Game/FlexibleCombatSystem/Blueprints/AI/BP_NPC_Parent.BP_NPC_Parent_C|GetDialogueComponent (Variables|Default|GetNPC)) (Math|Integer|SelectInt 15 13 (== (Variables|Default|GetCurrentStage) 1)))
          (Math|Integer|IncrementInt (Variables|Default|GetCurrentStage)
            (:%20%20
              (Variables|Default|SetCurrentRound 1)
              (Math|Integer|IncrementInt (Variables|Default|GetEnemyIncrementer)
                (:%20%20
                  (Variables|Default|SetDeadEnemies 0)))))
          (else
            ;;[1 1 1] Add Round, Spawn Next
            (Variables|Default|SetDeadEnemies 0)
            (Math|Integer|IncrementInt (Variables|Default|GetCurrentRound)
              (:%20%20
                (Utilities|FlowControl|Delay 1.0)
                (bind _returnvalue_2 (UserInterface|CreateWidget "/Game/FlexibleCombatSystem/Widgets/HUD/WB_PopupTitle.WB_PopupTitle_C" 0 "Round Complete!"))
                (UserInterface|Viewport|AddtoViewport _returnvalue_2 0)
                (Utilities|FlowControl|Delay 2.0)
                (CallFunction|BeginArena)))))))))

(fn ConstructionScript)