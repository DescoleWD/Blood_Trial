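; Parent Blueprint for NPCs with modular outfits and conversations that temporarily take over the player's camera.
; The construction script binds equipment meshes to the body via master pose and optionally applies custom equipment meshes.
; Dialogue runs through DialogueComponent, while helper functions switch to the NPC camera and place the player facing it.
; On return, the player's camera, input, walking, HUD and the NPC's actor tag are restored.
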(fn ConstructionScript
  (bind (_usecustomequipment _chest _hands _legs _boots _back _helmet _shoulder) (Utilities|Struct|Break))
  (Class|SkinnedMeshComponent|SetMasterPoseComponent (Variables|Default|GetHelmet) (Variables|Character|GetMesh) false)
  (if _usecustomequipment
    (for (_array_element _array_index) (Utilities|Array|MakeArray (Variables|Default|GetChest) (Variables|Default|GetHands) (Variables|Default|GetLegs) (Variables|Default|GetBoots) (Variables|Default|GetBack) (Variables|Default|GetHelmet) (Variables|Default|GetShoulder))
      (Class|SkinnedMeshComponent|SetSkeletalMesh _array_element (Utilities|Array|Get(acopy) (Utilities|Array|MakeArray _chest _hands _legs _boots _back _helmet _shoulder) _array_index) true))))

(fn RunDialogue
  (Class|Object|HideHUD(Message) (Game|GetPlayerController 0))
  (CallFunction|BeginDialogue (Variables|Default|GetDialogueComponent) (Variables|SetupInGame|GetNPC%20Dialogue) (Variables|SetupInGame|GetNPC_Name)))

(fn SetupConversationCam
  (bind _returnvalue (Transformation|GetActorRotation))
  ;[1 1 1] Adjust Camera & Player Position
  (Game|Player|SetViewTargetwithBlend (Game|GetPlayerController 0) (Components|GetOwner (Variables|Default|GetCamera)) 0.0 "VTBlend_Linear" 0.0 false)
  (Transformation|SetActorTransform (Variables|Default|GetCharacterRef) (Math|Transform|MakeTransform (+ (Transformation|GetActorLocation) (* (Transformation|GetActorForwardVector) 1.5e+02)) (Math|Rotator|MakeRotator (.roll _returnvalue) (.pitch _returnvalue) (+ (.yaw _returnvalue) 1.8e+02)))))

(fn ReturnCameraandSettings
  (bind _returnvalue (Game|GetPlayerController 0))
  (bind _camera (Class|Object|PassCamera(Message) (Variables|Default|GetCharacterRef)))
  (Game|Player|SetViewTargetwithBlend (Game|GetPlayerController 0) (Components|GetOwner _camera) 0.0 "VTBlend_Linear" 0.0 false)
  (Input|SetInputModeGameOnly _returnvalue)
  (Variables|/Script/Engine.PlayerController|SetbShowMouseCursor _returnvalue false)
  (Pawn|Components|CharacterMovement|SetMovementMode (Variables|/Script/Engine.Character|GetCharacterMovement (Game|GetPlayerCharacter 0)) "MOVE_Walking" 0)
  (Class|Object|ShowHUD(Message) (Game|GetPlayerController 0))
  (CallFunction|ShowActorTag (Variables|Default|GetLootOutlineComponent)))

(fn TransitionCam)