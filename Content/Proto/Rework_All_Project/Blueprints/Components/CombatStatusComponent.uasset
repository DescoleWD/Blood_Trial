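; Character combat status component that tracks attack style, drawn state and equipped weapons, and routes attack and block input to the melee component.
; Equipping derives a weapon animation type from item type and current loadout, then broadcasts it and updates the melee component's anim output.
; Style cycling is throttled by a two-second lockout, and switching clears the input buffer and redraws weapons.
; It also restores stance on initialization for non-AI owners and handles weapon cleanup.
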(event Custom|InitializeCombatStatus
  (params (IgnoreSaveData :type Boolean))
  ;[1 1 1] Setup Save Data & Weapons
  (CallFunction|StoreComponents)
  (if (not IgnoreSaveData)
    ;;[1 1 1] Not Run by AI
    (CallFunction|LoadAttackStance)))

(event Custom|ReleaseBlock
  ;[1 1 1] [RMB] (Block OR Aim)
  (bind _canattack_ (CallFunction|AttackConditions false))
  (if _canattack_
    (switch Utilities|FlowControl|Switch|SwitchonE_AttackStyle (Variables|Default|GetCurrentAttackStyle)
      (:NewEnumerator0
        ;;[1 0.01444 0] Send Melee Release Block
        (Default|ReleaseBlock (Variables|Default|GetMeleeComponent))))))

(event Custom|SwitchAttackStyle
  (params (ForwardCycle :type Boolean))
  ;[1 1 1] Change Attack Style
  (Utilities|FlowControl|DoOnce false :!label _label
    (:Completed
      (bind (_success _attackstyle) (CallFunction|AttackStyleSwitcher ForwardCycle))
      (if _success
        (CallFunction|ChangeAttackStyle _attackstyle false)
        (Utilities|FlowControl|Delay 2.0) ; Prevents Interupting Montage Causing Instant Weapon Equip
        (goto _label Reset)))))

(event Custom|Event%20Unequip%20Weapon
  (params (Item%20Data :type S%20Item%20Data%20Structure))
  ;[1 1 1] Equip/UnEquip Weapon
  ;;[1 1 1] UnEquip Weapon Animation
  (CallFunction|CalculateAnimOutput false Item%20Data)
  ;;[1 1 1] Equip Weapon Animation - Called From Equipment Component When Item Being Equipped
  (CallFunction|UpdateAnimationOutput))

(event Custom|ChangeAttackStyle
  (params (CurrentAttackStyle :type E_AttackStyle%20Enum :default "NewEnumerator0") (AI%20Ignore%20Conditions :type Boolean))
  ;[1 1 1] Change Attack Style
  (if AI%20Ignore%20Conditions
    (CallFunction|UpdateAttackStyle CurrentAttackStyle :!label _label)
    (switch Utilities|FlowControl|Switch|SwitchonE_AttackStyle (Variables|Default|GetCurrentAttackStyle)
      (:NewEnumerator0
        ;;[1 0.07002 0.04539] Change To Mele Attack Style - If Weapon Drawn Pass Weapon Anim Output
        (CallFunction|SetAnimOutput false)
        (if (or (Variables|Default|GetWeaponDrawn) (Variables|Default|GetMagePrevious))
          (if (or (Utilities|IsValid (Variables|Default|GetEquippedMainHand)) (Utilities|IsValid (Variables|Default|GetEquippedOffHand)))
            (Default|ClearBuffer (Variables|Default|GetInputBufferComponent) true)
            (Variables|Default|SetWeaponDrawn false) ; Draw Weapon Condition Is Weapon Drawn = False
            (CallFunction|DrawWeapon)
            ;;;[1 1 1] Used to Instantly Draw Weapon (For Spawn Magic Wep)
            (Variables|Default|SetMagePrevious false :!label _label_2))
          (else
            (goto _label_2)))))
    (elif (Utilities|Enum|NotEqual(Enum) (Variables|Default|GetCurrentAttackStyle) CurrentAttackStyle)
      (if true
        (goto _label)))))

(event Custom|FireAttack
  ;[1 1 1] [LMB] - Attack
  (bind _canattack_ (CallFunction|AttackConditions true))
  (if _canattack_
    (switch Utilities|FlowControl|Switch|SwitchonE_AttackStyle (Variables|Default|GetCurrentAttackStyle)
      (:NewEnumerator0
        ;;[1 0.01444 0] Send Melee Attack
        (Default|EventLightAttack (Variables|Default|GetMeleeComponent))))))

(event Custom|UpdateAnimationOutput
  ;[1 1 1] Equip/UnEquip Weapon
  ;;[1 1 1] Update Animations With "Equipped Weapon Enum"
  (CallFunction|SetAnimOutput false))

(event Custom|FireBlock
  ;[1 1 1] [RMB] (Block OR Aim)
  (bind _canattack_ (CallFunction|AttackConditions true))
  (if _canattack_
    (switch Utilities|FlowControl|Switch|SwitchonE_AttackStyle (Variables|Default|GetCurrentAttackStyle)
      (:NewEnumerator0
        ;;[1 0.01444 0] Send Melee Block
        (Default|SendBlock (Variables|Default|GetMeleeComponent))))))

(event Custom|DrawWeapon
  ;[1 1 1] Draw & Sheathe Weapon
  (Variables|Default|SetWeaponDrawn true))

(event Custom|EquipWeapon
  (params (Weapon%20Actor :type Actor%20Object%20Reference) (Item%20Data :type S%20Item%20Data%20Structure))
  ;[1 1 1] Equip/UnEquip Weapon
  ;;[1 1 1] Equip Weapon Animation - Called From Equipment Component When Item Being Equipped
  (CallFunction|StoreComponents) ; Incase Load Game Triggers before Components Stored
  ;;;[1 1 1] Tells us what Weapon Style We Have Equipped
  (CallFunction|CalculateAnimOutput true Item%20Data)
  (CallFunction|UpdateAnimationOutput))

(fn UpdateAttackStyle
  (params (UpdatedAttackStyle :type E_AttackStyle%20Enum :default "NewEnumerator0"))
  ;[1 1 1] Change Attack Style
  (Variables|Default|SetCurrentAttackStyle UpdatedAttackStyle)
  (Default|CallAttackStyleUpdated UpdatedAttackStyle)
  (Audio|PlaySoundatLocation 0 (Transformation|GetActorLocation (Components|GetOwner)) "0, 0, 0" 1.0 1.0 0.0 0 0 0 0))

(fn CalculateAnimOutput
  (params (EquippingWeapon :type Boolean) (Item%20Data :type S%20Item%20Data%20Structure))
  (bind _itemtype (Utilities|Struct|BreakS_ItemData Item%20Data))
  (LocalVariables|SetTwoHanded (Utilities|Enum|Equal(Enum) _itemtype "NewEnumerator12"))
  (LocalVariables|SetShield (Utilities|Enum|Equal(Enum) _itemtype "(INVALID)"))
  (LocalVariables|SetMainHand (Utilities|Enum|Equal(Enum) _itemtype "NewEnumerator9"))
  (if EquippingWeapon
    ;[1 1 1] If Equipped Item Being Added
    ;;[1 1 1] If Two-Handed Equipped - Set Animation Output = Two-Handed
    (if (LocalVariables|GetTwoHanded)
      (Variables|Default|SetEquippedMeleeWeapon "NewEnumerator1")
      (elif (LocalVariables|GetMainHand)
        ;;[1 1 1] If Fists/TwoHanded/Bow Current & Main-Hand Equipped - Set Anim Output = Mainhand
        (if (or (Utilities|Enum|Equal(Enum) (Variables|Default|GetEquippedMeleeWeapon) "(INVALID)") (Utilities|Enum|Equal(Enum) (Variables|Default|GetEquippedMeleeWeapon) "NewEnumerator1"))
          (Variables|Default|SetEquippedMeleeWeapon "NewEnumerator0")
          (else
            ;;[1 1 1] If Off-Hand Current & Main-Hand Equipped - Set Anim Output = Mainhand And Shield
            (if (Utilities|Enum|Equal(Enum) (Variables|Default|GetEquippedMeleeWeapon) "(INVALID)")
              (Variables|Default|SetEquippedMeleeWeapon "(INVALID)")
              (else
                ;;[1 1 1] If Off-Hand Wep Current & Main-Hand Equipped - Set Anim Output = Dual Wield
                (if (Utilities|Enum|Equal(Enum) (Variables|Default|GetEquippedMeleeWeapon) "(INVALID)")
                  (Variables|Default|SetEquippedMeleeWeapon "(INVALID)"))))))
        (else
          ;;[1 1 1] If TwoHanded/Bow/MainHand Current & Off-Hand Equipped - Set Anim Output = MainHand+Shield/Dual Wield
          (if (Math|Boolean|ORBoolean (Utilities|Enum|Equal(Enum) (Variables|Default|GetEquippedMeleeWeapon) "NewEnumerator0") (Utilities|Enum|Equal(Enum) (Variables|Default|GetEquippedMeleeWeapon) "(INVALID)") (Utilities|Enum|Equal(Enum) (Variables|Default|GetEquippedMeleeWeapon) "(INVALID)"))
            (if (LocalVariables|GetShield)
              (Variables|Default|SetEquippedMeleeWeapon "(INVALID)")
              (else
                (Variables|Default|SetEquippedMeleeWeapon "(INVALID)")))
            (else
              ;;[1 1 1] IF 2H Equip or OffHand Equip - Replace it
              (if (Math|Boolean|ORBoolean (Utilities|Enum|Equal(Enum) (Variables|Default|GetEquippedMeleeWeapon) "(INVALID)") (Utilities|Enum|Equal(Enum) (Variables|Default|GetEquippedMeleeWeapon) "(INVALID)") (Utilities|Enum|Equal(Enum) (Variables|Default|GetEquippedMeleeWeapon) "(INVALID)"))
                ;;[1 1 1] If Fists Current & Off-Hand Equipped - Set Anim Output = OffHand Shield/OffHand Weapon
                (if (LocalVariables|GetShield) :!label _label
                  (Variables|Default|SetEquippedMeleeWeapon "(INVALID)")
                  (else
                    (Variables|Default|SetEquippedMeleeWeapon "(INVALID)")))
                (elif (Utilities|Enum|Equal(Enum) (Variables|Default|GetEquippedMeleeWeapon) "(INVALID)")
                  (goto _label))))))))))

(fn SetAnimOutput
  (params (IgnoreFists :type Boolean))
  (bind _equippedmeleeweapon (Variables|Default|GetEquippedMeleeWeapon))
  (bind _meleecomponent (Variables|Default|GetMeleeComponent))
  (Utilities|IsValid (Variables|Default|GetEquipmentComponent)
    (:Is%20Valid
      (switch Utilities|FlowControl|Switch|SwitchonE_AttackStyle (Variables|Default|GetCurrentAttackStyle)
        (:NewEnumerator0
          (if (or (Variables|Default|GetWeaponDrawn) IgnoreFists)
            ;[1 1 1] Set Anim Output
            (Default|CallWeaponOutputUpdated _equippedmeleeweapon)
            (switch Utilities|FlowControl|Switch|SwitchonE_WeaponType _equippedmeleeweapon
              (:NewEnumerator0
                _)
              (:NewEnumerator1
                _))
            ;[1 1 1] Update Melee Output
            (Utilities|IsValid _meleecomponent
              (:Is%20Valid
                (Default|SetMeleeAnimOutput _meleecomponent (Variables|Default|GetEquippedMeleeWeapon))))))))))

(fn AttackStyleSwitcher
  (params (ForwardCycle :type Boolean))
  (bind _currentattackstyle (Variables|Default|GetCurrentAttackStyle))
  (bind _returnvalue (Utilities|Enum|NotEqual(Enum) _currentattackstyle "NewEnumerator0"))
  (if ForwardCycle :!label _label
    ;[1 1 1] Increment 1 or flip to start if at end
    (Variables|Default|SetAttackStyleCounter (Math|Integer|SelectInt 1 (+ (Variables|Default|GetAttackStyleCounter) 1) (== (Variables|Default|GetAttackStyleCounter) 3)))
    (else
      ;[1 1 1] Decrement 1 or flip to end if at start
      (Variables|Default|SetAttackStyleCounter (Math|Integer|SelectInt 3 (- (Variables|Default|GetAttackStyleCounter) 1) (== (Variables|Default|GetAttackStyleCounter) 1)))))
  (switch Utilities|FlowControl|Switch|SwitchonE_AttackStyle (Utilities|Enum|ByteToEnumE_AttackStyle (Utilities|Array|Get(acopy) (LocalVariables|GetAttackStyles) (- (Variables|Default|GetAttackStyleCounter) 1)))
    (:NewEnumerator0
      ;[1 1 1] Final Condition Checks
      (if _returnvalue
        (return _returnvalue "NewEnumerator0")
        (else
          (Utilities|FlowControl|DoN (- (Utilities|Array|Length (LocalVariables|GetAttackStyles)) 1)
            (:Exit
              (goto _label))))))))

(fn LoadAttackStance
  (bind _equippedmainhand (Variables|Default|GetEquippedMainHand))
  (bind _currentattackstyle (Variables|Default|GetCurrentAttackStyle))
  ;[1 1 1] Loads The Status Of The Character, Combat, Weapons, Spells Selected etc
  ;;[1 1 1] Update Draw/Sheathe & Attack Anims
  (CallFunction|SetAnimOutput false)
  ;;[1 1 1] Based Upon Attack Style, Update Weapons/Magic Accordingly
  (Default|CallAttackStyleUpdated _currentattackstyle)
  (switch Utilities|FlowControl|Switch|SwitchonE_AttackStyle _currentattackstyle
    (:NewEnumerator0
      (if (Variables|Default|GetWeaponDrawn)
        (Utilities|IsValid _equippedmainhand
          (:Is%20Valid
            (Class|IWeaponInterface|AttachWeapontoHand(Message) _equippedmainhand)))))))

(fn AttackConditions
  (params (Attacking :type Boolean))
  (Variables|Default|SetAimHeldDown Attacking)
  (if (AI|Components|NavMovement|IsFalling (Variables|/Script/Engine.Character|GetCharacterMovement (Variables|Components|GetCharacterRef)))
    _
    (elif (Variables|Default|GetDisableControls)
      _
      (else
        (return true))))
  (return false))

(fn StoreComponents
  (bind _returnvalue (Components|GetOwner))
  (Utilities|FlowControl|DoOnce false
    (:Completed
      (Variables|Default|SetMeleeComponent (Actor|GetComponentbyClass _returnvalue "/Game/Proto/Rework_All_Project/Blueprints/Components/MeleeComponent.MeleeComponent_C"))
      (Variables|Default|SetEquipmentComponent (Actor|GetComponentbyClass _returnvalue "/Game/Proto/Rework_All_Project/Blueprints/Components/EquipmentComponent.EquipmentComponent_C"))
      (Variables|Default|SetInputBufferComponent (Actor|GetComponentbyClass _returnvalue "/Game/Proto/Rework_All_Project/Blueprints/Components/InputBufferComponent.InputBufferComponent_C"))
      (Variables|Default|SetTargetingComp (Actor|GetComponentbyClass _returnvalue "/Game/Proto/Rework_All_Project/Blueprints/Components/TargetingComponent.TargetingComponent_C"))
      (bind _ascharacter (Utilities|Casting|CastToCharacter (Components|GetOwner)))
      (Variables|Components|SetCharacterRef _ascharacter)
      (Default|Initialize (Variables|Default|GetMeleeComponent))
      (Default|SetMeleeAnimOutput (Variables|Default|GetMeleeComponent) "(INVALID)"))))

(fn UpdateWeaponStyle
  (params (EquippedWeapon :type E_WeaponType%20Enum :default "NewEnumerator2"))
  (bind _meleecomponent (Variables|Default|GetMeleeComponent))
  ;[1 1 1] Update Weapon Equipped - Passes Info to ABP and Melee Comp to Update Attack Montages
  (bind _output_get (Variables|Default|SetEquippedMeleeWeapon EquippedWeapon))
  (CallFunction|SetAnimOutput true)
  (Utilities|IsValid _meleecomponent
    (:Is%20Valid
      (Default|SetMeleeAnimOutput _meleecomponent _output_get))))

(fn UpdateAnimations
  (CallFunction|SetAnimOutput false))

(fn DestroyWeapons
  (bind _equippedmainhand (Variables|Default|GetEquippedMainHand))
  (bind _equippedoffhand (Variables|Default|GetEquippedOffHand))
  (bind _equippedrangedweapon (Variables|Default|GetEquippedRangedWeapon))
  (bind _equippedquiver (Variables|Default|GetEquippedQuiver))
  (Utilities|IsValid _equippedmainhand
    (:Is%20Valid
      (Actor|DestroyActor _equippedmainhand))
    (:Is%20Not%20Valid
      _))
  (Utilities|IsValid _equippedoffhand
    (:Is%20Valid
      (Actor|DestroyActor _equippedoffhand))
    (:Is%20Not%20Valid
      _))
  (Utilities|IsValid _equippedrangedweapon
    (:Is%20Valid
      (Actor|DestroyActor _equippedrangedweapon))
    (:Is%20Not%20Valid
      _))
  (Utilities|IsValid _equippedquiver
    (:Is%20Valid
      (Actor|DestroyActor _equippedquiver))))

(fn DeathWeaponDrop
  (bind _equippedmainhand (Variables|Default|GetEquippedMainHand))
  (Utilities|IsValid _equippedmainhand
    (:Is%20Valid
      (Class|IWeaponInterface|PlayerDied(Message) _equippedmainhand))))