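; BP_HoleRespawn is a hole trap that damages and respawns any BP_MainBase character entering its Box trigger.
; On overlap it applies environmental damage read from GetInst, calls the character's Respawn, and adds a new Respawn widget that runs FadeInBlackness.
; A DoOnce gate reset after a short delay keeps the 2D fall sound from replaying on rapid overlaps.
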(event OnComponentBeginOverlap(Box)
  (params (OverlappedComponent :type Primitive%20Component%20Object%20Reference) (OtherActor :type Actor%20Object%20Reference) (OtherComp :type Primitive%20Component%20Object%20Reference) (OtherBodyIndex :type Integer) (bFromSweep :type Boolean) (SweepResult :type Hit%20Result%20Structure%20%28by%20ref%29))
  (bind _asbp_main_base (Utilities|Casting|CastToBP_MainBase OtherActor))
  (if (== _asbp_main_base OtherActor)
    (Game|Damage|ApplyDamage _asbp_main_base (Variables|/Game/Proto/Main/Blueprint/Save_BFL_GameInstance/BloodTrial_GameInstance.BloodTrial_GameInstance_C|GetEnviroDamage (CallFunction|GetInst)) (Game|GetPlayerController 0) self)
    (Default|Respawn _asbp_main_base)
    (bind _returnvalue (Game|ConstructObjectfromClass "/Game/Proto/Main/HUD/Respawn.Respawn_C"))
    (UserInterface|Viewport|AddtoViewport _returnvalue 0)
    (Default|FadeinBlackness _returnvalue)
    (Utilities|FlowControl|DoOnce false :!label _label
      (:Completed
        (Audio|PlaySound2D "/Game/Proto/Main/SFX/EnviroSystem/Hole/SFX_Fall.SFX_Fall" 1.0 1.0 0.0 0 0)
        (Utilities|FlowControl|Delay 1.0)
        (goto _label Reset)))))

(fn ConstructionScript)