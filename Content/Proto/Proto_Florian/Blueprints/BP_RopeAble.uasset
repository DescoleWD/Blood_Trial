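; BP_RopeAble is a prototype rope interactable that the character can cut once, using lever-style interaction events.
; Overlapping LeverCollider registers it with the BP_MainBase character through NearTheLever and enables LeverActive.
; Activation resets the character's ActorRef, sets RopeCut on the game instance, flings the Cube upward, then destroys the actor.
; BeginPlay removes the actor if RopeCut is already set; a Player tag check is left disconnected.
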(event OnComponentBeginOverlap(LeverCollider)
  (params (OverlappedComponent :type Primitive%20Component%20Object%20Reference) (OtherActor :type Actor%20Object%20Reference) (OtherComp :type Primitive%20Component%20Object%20Reference) (OtherBodyIndex :type Integer) (bFromSweep :type Boolean) (SweepResult :type Hit%20Result%20Structure%20%28by%20ref%29))
  (bind _asbp_main_base (Utilities|Casting|CastToBP_MainBase OtherActor))
  (Variables|Default|SetAs%20BP%20Main%20Character _asbp_main_base)
  (Variables|Default|SetisCollision true)
  (Default|NeartheLever _asbp_main_base self)
  (Development|PrintString "Call Enter" true false))

(event OnComponentEndOverlap(LeverCollider)
  (params (OverlappedComponent :type Primitive%20Component%20Object%20Reference) (OtherActor :type Actor%20Object%20Reference) (OtherComp :type Primitive%20Component%20Object%20Reference) (OtherBodyIndex :type Integer))
  (bind _as_bp_main_character (Variables|Default|GetAs%20BP%20Main%20Character))
  (Utilities|Casting|CastToBP_MainBase OtherActor)
  (Variables|Default|SetisCollision false)
  (if (Variables|Default|GetisDestroy)
    (Variables|/Game/Proto/Main/Blueprint/BP_MainBase.BP_MainBase_C|SetActor_Ref _as_bp_main_character _as_bp_main_character)
    (Development|PrintString "Call Out" true false)))

(event Custom|LeverActive
  (bind _as_bp_main_character (Variables|Default|GetAs%20BP%20Main%20Character))
  (if (Variables|Default|GetisCollision)
    (Development|PrintString "Call Active" true false)
    (Variables|Default|SetisDestroy true)
    (Variables|/Game/Proto/Main/Blueprint/BP_MainBase.BP_MainBase_C|SetActor_Ref _as_bp_main_character _as_bp_main_character)
    (Utilities|FlowControl|Delay 0.2)
    (Variables|/Game/Proto/Main/Blueprint/Save_BFL_GameInstance/BloodTrial_GameInstance.BloodTrial_GameInstance_C|SetRopeCut? (CallFunction|GetInst) true)
    (Components|MoveComponentTo (Variables|Default|GetCube) "0, 0,2500.000000" "0, 0,270.000000" false false 0.5 false)
    (Utilities|FlowControl|Delay 0.5)
    (Actor|DestroyActor)
    (Development|PrintString "SFX:RopeCut" true false "(R=0.000000,G=1.000000,B=0.090196,A=1.000000)")))

(event EventBeginPlay
  (if (Variables|/Game/Proto/Main/Blueprint/Save_BFL_GameInstance/BloodTrial_GameInstance.BloodTrial_GameInstance_C|GetRopeCut? (CallFunction|GetInst))
    (Actor|DestroyActor)))

(fn ConstructionScript)