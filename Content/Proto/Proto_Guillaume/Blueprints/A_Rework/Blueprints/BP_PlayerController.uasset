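; Player controller that acts as the UI hub, toggling inventory, loot, vendor and container windows, spellbook, quest log, spell trainer and pause menu.
; On setup it caches the character's components and links them to HUD widgets, then exposes references and open states through getters.
; An open-UI counter drives cursor and input mode, while a lock counter blocks toggles during nested popups.
; Opening some windows closes conflicting ones or hides the quest tracker.
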(event EventToggleExternalContainerInv
  (params (Inventory%20Component :type Inventory%20Component%20Object%20Reference) (Actor%20Ref :type Actor%20Object%20Reference))
  ;[1 0.2817 0.1317] Toggle External Container Inventory
  (if (Variables|Default|GetCanToggleWIdget)
    (if (not (and (Variables|MenuStatus|GetInventoryOpen) (not (Variables|MenuStatus|GetExternalInventoryOpen?))))
      (CallFunction|ToggleExternalInventoryGroup Inventory%20Component Actor%20Ref true)
      (Widget|SetVisibility (Variables|/Game/FlexibleCombatSystem/Widgets/HUD/WB_HUD.WB_HUD_C|GetWB_ContainerInventory (Variables|References|GetWB_HUD_Ref)) (select (Variables|MenuStatus|GetExternalInventoryOpen?) "Visible" "Hidden"))
      (Variables|Default|SetInventoryMenuState (select (Variables|MenuStatus|GetExternalInventoryOpen?) "NewEnumerator1" "NewEnumerator0"))
      (Audio|PlaySound2D "/Game/FlexibleCombatSystem/SoundFX/General/SW_OpenMenu.SW_OpenMenu" 1.0 1.0 0.0 0 0)
      (Default|ToggleActorTag (Variables|Default|GetOutline%20Component)))))

(event EventShowHUD
  ;[1 1 1] Toggle HUD
  (Default|EventShowHUD (Variables|References|GetBP_HUD)))

(event EventToggleQuestLog
  ;[0.1644 0.951 1] Toggle Quest Log
  (if (and (Variables|Default|GetCanToggleWIdget) (not (Variables|MenuStatus|GetInventoryOpen)))
    (CallFunction|RemoveExternalWidget false true false)
    (bind _output_get (Variables|MenuStatus|SetQuestLogOpen (not (Variables|MenuStatus|GetQuestLogOpen))))
    (CallFunction|SetUICounter _output_get)
    (Widget|SetVisibility (Variables|/Game/FlexibleCombatSystem/Widgets/HUD/WB_HUD.WB_HUD_C|GetWB_QuestLog (Variables|References|GetWB_HUD_Ref)) (select _output_get "Visible" "Hidden"))
    (Audio|PlaySound2D "/Game/FlexibleCombatSystem/SoundFX/General/SW_OpenSpellbook_01.SW_OpenSpellbook_01" 1.0 1.0 0.0 0 0)))

(event EventToggleSpellTrainer
  (bind _outline_component (Variables|Default|GetOutline%20Component))
  ;[0.2767 0.2388 1] Toggle Spell Trainer
  (if (Variables|Default|GetCanToggleWIdget)
    (CallFunction|RemoveExternalWidget false false true)
    (bind _output_get (Variables|MenuStatus|SetSpellTrainerOpen (not (Variables|MenuStatus|GetSpellTrainerOpen))))
    (CallFunction|SetUICounter _output_get)
    (Widget|SetVisibility (Variables|/Game/FlexibleCombatSystem/Widgets/HUD/WB_HUD.WB_HUD_C|GetWB_AbilityTrainer (Variables|References|GetWB_HUD_Ref)) (select _output_get "Visible" "Hidden"))
    (CallFunction|ToggleQuestTracker _output_get)
    (Audio|PlaySound2D "/Game/FlexibleCombatSystem/SoundFX/General/SW_OpenSpellbook_03.SW_OpenSpellbook_03" 1.0 1.0 0.0 0 0)
    (Utilities|IsValid _outline_component
      (:Is%20Valid
        (Default|ToggleActorTag _outline_component)))))

(event EventToggleExternalInventory
  (params (ExternalInventoryComponent :type Inventory%20Component%20Object%20Reference) (ActorRef :type Actor%20Object%20Reference) (Vendor :type Boolean))
  (bind _wb_hud_ref (Variables|References|GetWB_HUD_Ref))
  (bind _externalinventoryopen_ (Variables|MenuStatus|GetExternalInventoryOpen?))
  (bind _outline_component (Variables|Default|GetOutline%20Component))
  (bind _wb_vendorwindow (Variables|/Game/FlexibleCombatSystem/Widgets/HUD/WB_HUD.WB_HUD_C|GetWB_VendorWindow _wb_hud_ref))
  ;[1 0.6696 0.3033] Toggle External Inventory
  (bind _interact (CallFunction|ExternalInventoryConditions))
  (if _interact
    (CallFunction|ToggleExternalInventoryGroup ExternalInventoryComponent ActorRef false)
    (Variables|/Game/FlexibleCombatSystem/Widgets/InventorySystem/WB_ExternalInventory.WB_ExternalInventory_C|SetNPC-Ref _wb_vendorwindow ActorRef)
    (Widget|SetVisibility _wb_vendorwindow (select (Variables|MenuStatus|GetExternalInventoryOpen?) "Visible" "Hidden"))
    (Default|UpdateValues _wb_vendorwindow)
    (Audio|PlaySound2D "/Game/FlexibleCombatSystem/SoundFX/General/SW_OpenSpellbook_03.SW_OpenSpellbook_03" 1.0 1.0 0.0 0 0)
    (if Vendor
      ;;[1 1 1] Used To Tell Inventory Slot What Inventory Type Is Being Dealt With
      (Variables|Default|SetInventoryMenuState (select _externalinventoryopen_ "NewEnumerator2" "NewEnumerator0"))
      (else
        (Variables|Default|SetInventoryMenuState (select _externalinventoryopen_ "NewEnumerator1" "NewEnumerator0"))))
    (Utilities|IsValid _outline_component
      (:Is%20Valid
        (Default|ToggleActorTag _outline_component)))))

(event EventHideHUD
  ;[1 1 1] Toggle HUD
  (Default|EventHideHUD (Variables|References|GetBP_HUD)))

(event EventToggleInventory
  (bind _wb_hud_ref (Variables|References|GetWB_HUD_Ref))
  (bind _outline_component (Variables|Default|GetOutline%20Component))
  (bind _wb_inventory (Variables|/Game/FlexibleCombatSystem/Widgets/HUD/WB_HUD.WB_HUD_C|GetWB_Inventory _wb_hud_ref))
  ;[0.4773 0.3837 1] Toggle Inventory
  (if (and (Variables|Default|GetCanToggleWIdget) (not (Variables|MenuStatus|GetExternalInventoryOpen?)))
    (if (not (Variables|/Game/FlexibleCombatSystem/Widgets/InventorySystem/WB_Inventory.WB_Inventory_C|GetMidAnimation _wb_inventory))
      (CallFunction|RemoveExternalWidget true false false)
      (Variables|MenuStatus|SetInventoryOpen (not (Variables|MenuStatus|GetInventoryOpen)))
      (Class|ICharacter|ToggleInventoryCamera!(Message) (Variables|References|GetCharacterRef) (Variables|MenuStatus|GetInventoryOpen))
      (CallFunction|SetUICounter (Variables|MenuStatus|GetInventoryOpen))
      (Default|ToggleInventory _wb_inventory (select (Variables|MenuStatus|GetInventoryOpen) "NewEnumerator0" "NewEnumerator1"))
      (CallFunction|ToggleQuestTracker (Variables|MenuStatus|GetInventoryOpen))
      (CallFunction|RemoveLootContainer)
      (Audio|PlaySound2D "/Game/FlexibleCombatSystem/SoundFX/General/SW_OpenSpellbook_02.SW_OpenSpellbook_02" 1.0 1.0 0.0 0 0)
      (Utilities|IsValid _outline_component
        (:Is%20Valid
          (Default|ToggleActorTag _outline_component))))))

(event EventToggleLootMenu
  (params (Loot%20Component :type Loot%20Component%20Object%20Reference))
  (bind _outline_component (Variables|Default|GetOutline%20Component))
  (bind _wb_hud_ref (Variables|References|GetWB_HUD_Ref))
  (bind _wb_lootwindow (Variables|/Game/FlexibleCombatSystem/Widgets/HUD/WB_HUD.WB_HUD_C|GetWB_LootWindow _wb_hud_ref))
  (bind _hidden (CallFunction|GetVisibility _wb_lootwindow))
  ;[0.9152 0.3752 1] Toggle Loot Container
  (Variables|Default|SetLootComponent Loot%20Component)
  (if (not (Variables|MenuStatus|GetInventoryOpen))
    (if (Variables|Default|GetCanToggleWIdget)
      (Variables|MenuStatus|SetLootMenuOpen _hidden)
      (CallFunction|SetUICounter _hidden)
      (Widget|SetVisibility (Variables|/Game/FlexibleCombatSystem/Widgets/HUD/WB_HUD.WB_HUD_C|GetWB_LootWindow (Variables|References|GetWB_HUD_Ref)) (select _hidden "Visible" "Hidden"))
      (Audio|PlaySound2D "/Game/FlexibleCombatSystem/SoundFX/General/SW_OpenMenu.SW_OpenMenu" 1.0 1.0 0.0 0 0)
      (Utilities|IsValid _outline_component
        (:Is%20Valid
          (Default|ToggleActorTag _outline_component))))))

(event EventToggleSpellBook
  (bind _wb_hud_ref (Variables|References|GetWB_HUD_Ref))
  (bind _wb_spellbook (Variables|/Game/FlexibleCombatSystem/Widgets/HUD/WB_HUD.WB_HUD_C|GetWB_Spellbook _wb_hud_ref))
  (bind _hidden (CallFunction|GetVisibility _wb_spellbook))
  ;[0.2562 0.3434 1] Toggle SpellBook
  (if (and (Variables|Default|GetCanToggleWIdget) (not (Variables|MenuStatus|GetInventoryOpen)))
    (CallFunction|RemoveExternalWidget false false false)
    (Variables|MenuStatus|SetSpellBookOpen (not (Variables|MenuStatus|GetSpellBookOpen)))
    (CallFunction|ToggleSpellHotbar)
    (CallFunction|SetUICounter _hidden)
    (Widget|SetVisibility (Variables|/Game/FlexibleCombatSystem/Widgets/HUD/WB_HUD.WB_HUD_C|GetWB_Spellbook (Variables|References|GetWB_HUD_Ref)) (select _hidden "Visible" "Hidden"))
    (CallFunction|ToggleQuestTracker (not _hidden))
    (Audio|PlaySound2D "/Game/FlexibleCombatSystem/SoundFX/General/SW_OpenSpellbook_03.SW_OpenSpellbook_03" 1.0 1.0 0.0 0 0)))

(event EventTogglePauseMenu
  (bind _wb_hud_ref (Variables|References|GetWB_HUD_Ref))
  (bind _wb_pausemenu (Variables|/Game/FlexibleCombatSystem/Widgets/HUD/WB_HUD.WB_HUD_C|GetWB_PauseMenu _wb_hud_ref))
  (bind _hidden (CallFunction|GetVisibility _wb_pausemenu))
  ;[0.1975 1 0.2662] Pause Menu
  (if (Variables|Default|GetCanToggleWIdget)
    (if (not (Variables|/Game/FlexibleCombatSystem/Widgets/General/WB_PauseMenu.WB_PauseMenu_C|GetMidAnimation _wb_pausemenu))
      (CallFunction|SetUICounter _hidden)
      (Game|SetGamePaused _hidden)
      (Default|TogglePauseMenu _wb_pausemenu (select _hidden "Forward" "Reverse"))
      (Audio|PlaySound2D "/Game/FlexibleCombatSystem/SoundFX/General/SW_OpenMenu.SW_OpenMenu" 1.0 1.0 0.0 0 0))))

(event EventSetupReferences
  (params (CharacterRef :type Character%20Object%20Reference) (HUDRef :type BP%20Player%20HUD%20Object%20Reference))
  ;[1 0.8608 0.3588] Initial Setup - Pass HUD & Component References
  (Variables|References|SetCharacterRef CharacterRef)
  (CallFunction|CreateHUDRef HUDRef)
  (CallFunction|CreateComponentRefs)
  (CallFunction|SetupHUD))

(fn ConstructionScript)

(fn GetVisibility
  (params (Widget :type Widget%20Object%20Reference))
  (return (Utilities|Enum|Equal(Enum) (Widget|GetVisibility Widget) "Hidden")))

(fn SetUICounter
  (params (SetVisibile :type Boolean))
  (if SetVisibile
    ;[0.7022 1 0.7104] Increase UI Counter - Show Mouse Cursor - Input Mode Game And UI
    (Math|Integer|IncrementInt (Variables|Default|GetUI_Open)
      (:%20%20
        (if (not (Variables|Default|GetbShowMouseCursor))
          (Input|SetInputModeGameandUI self 0 "DoNotLock" true)
          (Variables|Default|SetbShowMouseCursor true))))
    (else
      ;[1 0.6295 0.6928] Decrament UI Counter - Hide Mouse Cursor - Input Mode Game Only
      (bind _result (Math|Integer|DecrementInt (Variables|Default|GetUI_Open))
        (:%20%20
          (if (== _result 0)
            (Input|SetInputModeGameOnly self)
            (Variables|Default|SetbShowMouseCursor false)))))))

(fn ToggleInventoryVisibility)

(fn RemoveLootContainer
  ;[1 1 1] Remove Loot Container If You Open Inventory
  (if (Variables|MenuStatus|GetLootMenuOpen)
    (Class|IPlayerController|ToggleLootMenu(Message) self (Variables|Default|GetLootComponent))))

(fn CreateHUDRef
  (params (BP_HUD :type BP%20Player%20HUD%20Object%20Reference))
  (Variables|References|SetBP_HUD BP_HUD)
  (Variables|References|SetWB_HUD_Ref (Variables|/Game/FlexibleCombatSystem/Blueprints/BP_PlayerHUD.BP_PlayerHUD_C|GetWG_HUD BP_HUD)))

(fn SetupHUD
  (Utilities|FlowControl|Sequence
    (:then_0
      ;[1 1 1] Pass Inventory Component To Inventory Widgets
      (Variables|/Game/FlexibleCombatSystem/Widgets/InventorySystem/WB_Inventory.WB_Inventory_C|SetInventoryComponent (Variables|/Game/FlexibleCombatSystem/Widgets/HUD/WB_HUD.WB_HUD_C|GetWB_Inventory (Variables|References|GetWB_HUD_Ref)) (Variables|Default|GetInventoryComponent))
      (Default|Setup (Variables|/Game/FlexibleCombatSystem/Widgets/InventorySystem/WB_Inventory.WB_Inventory_C|GetInventoryWindow (Variables|/Game/FlexibleCombatSystem/Widgets/HUD/WB_HUD.WB_HUD_C|GetWB_Inventory (Variables|References|GetWB_HUD_Ref))) (Variables|Default|GetInventoryComponent))
      (Variables|/Game/FlexibleCombatSystem/Widgets/Equipment/WB_Equipment.WB_Equipment_C|SetInventoryComponent (Variables|/Game/FlexibleCombatSystem/Widgets/InventorySystem/WB_Inventory.WB_Inventory_C|GetWB_Equipment (Variables|/Game/FlexibleCombatSystem/Widgets/HUD/WB_HUD.WB_HUD_C|GetWB_Inventory (Variables|References|GetWB_HUD_Ref))) (Variables|Default|GetInventoryComponent))
      (Default|SetupLink (Variables|/Game/FlexibleCombatSystem/Widgets/InventorySystem/WB_Inventory.WB_Inventory_C|GetWB_LevelTracker (Variables|/Game/FlexibleCombatSystem/Widgets/HUD/WB_HUD.WB_HUD_C|GetWB_Inventory (Variables|References|GetWB_HUD_Ref))) (Variables|Default|GetEquipmentComponent))
      (Variables|/Game/FlexibleCombatSystem/Widgets/InventorySystem/WB_Inventory.WB_Inventory_C|SetWB_HUD_Ref (Variables|/Game/FlexibleCombatSystem/Widgets/HUD/WB_HUD.WB_HUD_C|GetWB_Inventory (Variables|References|GetWB_HUD_Ref)) (Variables|References|GetWB_HUD_Ref)))
    (:then_1
      ;[1 1 1] Setup Stats
      (Default|Setup (Variables|/Game/FlexibleCombatSystem/Widgets/InventorySystem/WB_Inventory.WB_Inventory_C|GetWB_CharacterStats (Variables|/Game/FlexibleCombatSystem/Widgets/HUD/WB_HUD.WB_HUD_C|GetWB_Inventory (Variables|References|GetWB_HUD_Ref))) (Variables|Default|GetEquipmentComponent)))
    (:then_2
      ;[1 1 1] Setup Hotbar
      (Default|SetupComponentLink (Variables|/Game/FlexibleCombatSystem/Widgets/HUD/WB_HUD.WB_HUD_C|GetWB_PlayerAttackStyle (Variables|References|GetWB_HUD_Ref)) (Variables|References|GetCharacterRef)))
    (:then_3
      ;[1 1 1] Setup Character Portrait
      (Default|Initialize (Variables|/Game/FlexibleCombatSystem/Widgets/HUD/WB_HUD.WB_HUD_C|GetWB_CharacterPortrait (Variables|References|GetWB_HUD_Ref)) (Variables|References|GetCharacterRef)))
    (:then_4
      ;[1 1 1] Setup Ranged Crosshair
      (Default|Setup (Variables|/Game/FlexibleCombatSystem/Widgets/HUD/WB_HUD.WB_HUD_C|GetWB_Ranged_Crosshair (Variables|References|GetWB_HUD_Ref)) (Variables|References|GetCharacterRef)))
    (:then_5
      ;[1 1 1] Setup Magic Crosshair
      (Default|SetupMagicCross (Variables|/Game/FlexibleCombatSystem/Widgets/HUD/WB_HUD.WB_HUD_C|GetWB_MagicCrosshair (Variables|References|GetWB_HUD_Ref)) (Variables|References|GetCharacterRef)))))

(fn CreateComponentRefs
  (bind _characterref (Variables|References|GetCharacterRef))
  (Variables|Default|SetInventoryComponent (Actor|GetComponentbyClass _characterref "/Game/FlexibleCombatSystem/Blueprints/Components/InventoryComponent.InventoryComponent_C"))
  (Variables|Default|SetEquipmentComponent (Actor|GetComponentbyClass _characterref "/Game/FlexibleCombatSystem/Blueprints/Components/EquipmentComponent.EquipmentComponent_C"))
  (Variables|Default|SetMagicComponent (Actor|GetComponentbyClass _characterref "/Game/FlexibleCombatSystem/Blueprints/Components/MagicComponent.MagicComponent_C")))

(fn SetupInventory
  (params (ExternalInventory :type Inventory%20Component%20Object%20Reference))
  (if (Variables|/Game/FlexibleCombatSystem/Blueprints/Components/InventoryComponent.InventoryComponent_C|GetInventorySetup ExternalInventory)
    (Default|SetupExternalInventory ExternalInventory)
    (else
      (Default|ClearInventory ExternalInventory)
      (Default|InitializeInventory ExternalInventory)
      (Variables|/Game/FlexibleCombatSystem/Blueprints/Components/InventoryComponent.InventoryComponent_C|SetInventorySetup ExternalInventory true))))

(fn ToggleExternalInventoryGroup
  (params (ExternalInventory :type Inventory%20Component%20Object%20Reference) (Actor :type Object%20Object%20Reference) (Container :type Boolean))
  (bind _wb_hud_ref (Variables|References|GetWB_HUD_Ref))
  (bind _wb_inventory (Variables|/Game/FlexibleCombatSystem/Widgets/HUD/WB_HUD.WB_HUD_C|GetWB_Inventory _wb_hud_ref))
  ;[1 1 1] Clear Inventory For Next Container/Vendor OR Setup IF Opening
  (if (Variables|MenuStatus|GetExternalInventoryOpen?)
    (Default|ClearInventory ExternalInventory)
    ;[1 1 1] Open Close Inventory
    (Default|ToggleInventory _wb_inventory (select Container "NewEnumerator5" "NewEnumerator3"))
    (Variables|MenuStatus|SetInventoryOpen false)
    (else
      (Variables|Default|SetExternalInventoryComponent ExternalInventory)
      (CallFunction|SetupInventory ExternalInventory)
      (Default|ToggleInventory _wb_inventory (select Container "NewEnumerator4" "NewEnumerator2"))
      (Variables|MenuStatus|SetInventoryOpen true)))
  (Variables|MenuStatus|SetExternalInventoryOpen? (not (Variables|MenuStatus|GetExternalInventoryOpen?)))
  ;[1 1 1] Increase UI Counter
  (CallFunction|SetUICounter (Variables|MenuStatus|GetExternalInventoryOpen?)))

(fn RemoveExternalWidget
  (params (Inventory :type Boolean) (QuestLog :type Boolean) (RemoveAll :type Boolean))
  ;[1 1 1] Closes Other Widgets IF Another Widget Opens Up
  (if RemoveAll
    (if (Variables|MenuStatus|GetQuestLogOpen) :!label _label
      (CallFunction|ToggleQuestLog))
    (if (Variables|MenuStatus|GetSpellBookOpen)
      (CallFunction|ToggleSpellBook))
    (if (and RemoveAll (Variables|MenuStatus|GetInventoryOpen))
      (CallFunction|ToggleInventory))
    (elif Inventory
      (goto _label)
      (elif QuestLog
        (if (Variables|MenuStatus|GetSpellBookOpen)
          (CallFunction|ToggleSpellBook))
        (elif (Variables|MenuStatus|GetQuestLogOpen)
          (CallFunction|ToggleQuestLog))))))

(fn ToggleSpellHotbar
  (bind _magiccomponent (Variables|Default|GetMagicComponent))
  (bind _magiccomponent_2 (Variables|Default|GetMagicComponent))
  (if (Variables|MenuStatus|GetSpellBookOpen)
    (if (not (Utilities|Enum|Equal(Enum) (Variables|/Game/FlexibleCombatSystem/Blueprints/Components/MagicComponent.MagicComponent_C|GetHotbarVisibility _magiccomponent_2) "Visible"))
      (Default|ToggleAbilityHotbar _magiccomponent_2 "Visible")
      (Variables|Default|SetHotbarSetVisible true))
    (elif (Variables|Default|GetHotbarSetVisible)
      (if (Utilities|Enum|Equal(Enum) (Variables|/Game/FlexibleCombatSystem/Blueprints/Components/MagicComponent.MagicComponent_C|GetHotbarVisibility _magiccomponent) "Visible")
        (Default|ToggleAbilityHotbar _magiccomponent "Hidden")
        (Variables|Default|SetHotbarSetVisible false)))))

(fn ToggleQuestTracker
  (params (OpeningWidget :type Boolean))
  (bind _wb_hud_ref (Variables|References|GetWB_HUD_Ref))
  (bind _wb_questlog (Variables|/Game/FlexibleCombatSystem/Widgets/HUD/WB_HUD.WB_HUD_C|GetWB_QuestLog _wb_hud_ref))
  (bind _wb_questtracker (Variables|/Game/FlexibleCombatSystem/Widgets/NPC/WB_QuestLog.WB_QuestLog_C|GetWB_QuestTracker _wb_questlog))
  ;[1 1 1] Toggle Quest Tracker To Hide During Widget Open
  (if OpeningWidget
    (if (Widget|IsVisible _wb_questtracker)
      (Widget|SetVisibility _wb_questtracker "Hidden"))
    (elif (Variables|/Game/FlexibleCombatSystem/Widgets/NPC/WB_QuestLog.WB_QuestLog_C|GetQuestTrackerVisible _wb_questlog)
      (Widget|SetVisibility _wb_questtracker "Visible"))))

(fn ContainerStatus
  (return (Variables|MenuStatus|GetExternalInventoryOpen?)))

(fn ExternalInventoryConditions
  (return (and (Variables|Default|GetCanToggleWIdget) (not (and (Variables|MenuStatus|GetInventoryOpen) (not (Variables|MenuStatus|GetExternalInventoryOpen?)))))))

(fn ExternalInventoryOpen
  (return (Variables|MenuStatus|GetExternalInventoryOpen?)))

(fn InventoryStatus
  (return (Variables|MenuStatus|GetInventoryOpen)))

(fn LootMenuStatus
  (return (Variables|MenuStatus|GetLootMenuOpen)))

(fn PassContainerWindowWB
  (return (Variables|/Game/FlexibleCombatSystem/Widgets/HUD/WB_HUD.WB_HUD_C|GetWB_ContainerInventory (Variables|References|GetWB_HUD_Ref))))

(fn PassEquipmentComp
  (return (Variables|Default|GetEquipmentComponent)))

(fn PassExternalInventory
  (return (Variables|Default|GetExternalInventoryComponent)))

(fn PassHUDWB
  (return (Variables|References|GetWB_HUD_Ref)))

(fn PassInventoryComp
  (return (Variables|Default|GetInventoryComponent)))

(fn PassInventoryState
  (return (Variables|Default|GetInventoryMenuState)))

(fn PassLootComponent
  (return (Variables|Default|GetLootComponent)))

(fn PassLootWindowWB
  (return (Variables|/Game/FlexibleCombatSystem/Widgets/HUD/WB_HUD.WB_HUD_C|GetWB_LootWindow (Variables|References|GetWB_HUD_Ref))))

(fn PassOptionsMenu
  (return (Variables|References|GetWB_OptionsMenu)))

(fn PassOutlineComponent
  (params (OutlineComponent :type Outline%20Component%20Object%20Reference))
  (Variables|Default|SetOutline%20Component OutlineComponent)
  (return))

(fn PassSkillTrainer
  (return (Variables|/Game/FlexibleCombatSystem/Widgets/HUD/WB_HUD.WB_HUD_C|GetWB_AbilityTrainer (Variables|References|GetWB_HUD_Ref))))

(fn RecieveOptionsMenu
  (params (Options%20Menu :type WB%20Option%20List%20Object%20Reference))
  (Variables|References|SetWB_OptionsMenu Options%20Menu))

(fn SetCanUpdateWidget
  (params (CanUpdateWidget :type Boolean))
  (bind _counter (Variables|Default|GetCounter))
  ;[0.4442 0.9273 1] Prevents Widgets From Opening Closing - Needed for when a widget has created a widget, don't want to close first widget until second widget is removed. E.g. Inventory Open, Drop Item widget created = Prevent Inventory Closing until drop item widget closed
  (if CanUpdateWidget
    (Math|Integer|DecrementInt _counter
      (:%20%20
        _))
    (else
      (Math|Integer|IncrementInt _counter
        (:%20%20
          _))))
  (Variables|Default|SetCanToggleWIdget (== _counter 0))
  (return))

(fn WidgetMenuOpen
  (bind _wb_hud_ref (Variables|References|GetWB_HUD_Ref))
  (return (Math|Boolean|ANDBoolean (CallFunction|GetVisibility (Variables|/Game/FlexibleCombatSystem/Widgets/HUD/WB_HUD.WB_HUD_C|GetWB_Spellbook _wb_hud_ref)) (CallFunction|GetVisibility (Variables|/Game/FlexibleCombatSystem/Widgets/HUD/WB_HUD.WB_HUD_C|GetWB_VendorWindow _wb_hud_ref)) (CallFunction|GetVisibility (Variables|/Game/FlexibleCombatSystem/Widgets/HUD/WB_HUD.WB_HUD_C|GetWB_ContainerInventory _wb_hud_ref)) (CallFunction|GetVisibility (Variables|/Game/FlexibleCombatSystem/Widgets/HUD/WB_HUD.WB_HUD_C|GetWB_QuestLog _wb_hud_ref)) (CallFunction|GetVisibility (Variables|/Game/FlexibleCombatSystem/Widgets/HUD/WB_HUD.WB_HUD_C|GetWB_AbilityTrainer _wb_hud_ref)) (CallFunction|GetVisibility (Variables|/Game/FlexibleCombatSystem/Widgets/HUD/WB_HUD.WB_HUD_C|GetWB_LootWindow _wb_hud_ref)) (not (Variables|MenuStatus|GetInventoryOpen)))))