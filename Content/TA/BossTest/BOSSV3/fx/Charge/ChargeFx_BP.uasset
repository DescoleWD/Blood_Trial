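; ChargeFx_BP is a charge effect Blueprint, apparently for a boss, that feeds trace distance into a Niagara effect.
; Each Tick it line-traces on the Visibility channel from the Niagara component along its forward vector and sets the "Distance" float parameter to the hit distance, without checking for a hit.
; BeginPlay runs the same trace but discards the result, and both traces draw debug lines.
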(event EventBeginPlay
  (bind _niagara (Variables|Default|GetNiagara))
  (bind _returnvalue (Transformation|GetWorldLocation _niagara))
  (Collision|LineTraceByChannel _returnvalue (+ _returnvalue (* (Math|Vector|GetForwardVector (Transformation|GetWorldRotation _niagara)) 4000)) "TraceTypeQuery1" false 0 "ForDuration" true "(R=1.000000,G=0.000000,B=0.000000,A=1.000000)" "(R=0.000000,G=1.000000,B=0.000000,A=1.000000)" 0.5))

(event EventTick
  (params (DeltaSeconds :type Float%20%28single-precision%29))
  (bind _niagara (Variables|Default|GetNiagara))
  (bind _returnvalue (Transformation|GetWorldLocation _niagara))
  (bind _outhit (Collision|LineTraceByChannel _returnvalue (+ _returnvalue (* (Math|Vector|GetForwardVector (Transformation|GetWorldRotation _niagara)) 4000)) "TraceTypeQuery1" false 0 "ForDuration" true "(R=1.000000,G=0.000000,B=0.000000,A=1.000000)" "(R=0.000000,G=1.000000,B=0.000000,A=1.000000)" 0.5))
  (Effects|Components|ParticleSystem|SetFloatParameter (Variables|Default|GetNiagara) "Distance" (.Distance (Collision|BreakHitResult _outhit))))

(fn ConstructionScript)