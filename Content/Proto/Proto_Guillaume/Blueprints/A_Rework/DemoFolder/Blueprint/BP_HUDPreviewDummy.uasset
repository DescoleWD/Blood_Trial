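; BP_HUDPreviewDummy is a stand-in enemy in a demo folder that previews the enemy health widget.
; BeginPlay initializes its WB_EnemyHealth with itself and its combat style, and a sphere overlap shows or hides the widget as the player enters or leaves.
; Most AI and combat query functions are stubs returning fixed or empty values.
; Leftover kill-cam slow-motion and noise-reporting logic remains, while death only sets a flag, with ragdoll disconnected.
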(event OnComponentBeginOverlap(Sphere)
  (params (OverlappedComponent :type Primitive%20Component%20Object%20Reference) (OtherActor :type Actor%20Object%20Reference) (OtherComp :type Primitive%20Component%20Object%20Reference) (OtherBodyIndex :type Integer) (bFromSweep :type Boolean) (SweepResult :type Hit%20Result%20Structure%20%28by%20ref%29))
  (Utilities|Casting|CastToBP_PlayerCharacter OtherActor)
  (Development|SetHiddeninGame (Variables|Default|GetWidget) false false))

(event OnComponentEndOverlap(Sphere)
  (params (OverlappedComponent :type Primitive%20Component%20Object%20Reference) (OtherActor :type Actor%20Object%20Reference) (OtherComp :type Primitive%20Component%20Object%20Reference) (OtherBodyIndex :type Integer))
  (Utilities|Casting|CastToBP_PlayerCharacter OtherActor)
  (Development|SetHiddeninGame (Variables|Default|GetWidget) true false))

(event EventBeginPlay
  (bind _aswb_enemy_health (Utilities|Casting|CastToWB_EnemyHealth (UserInterface|GetUserWidgetObject (Variables|Default|GetWidget))))
  (Default|InitializeEnemyHealth _aswb_enemy_health self (Variables|SetupinGame|GetAI%20Combat%20Style))
  (CallFunction|UpdateWidgetValues))

(fn ConstructionScript)

(fn Death
  (params (SavedDeath :type Boolean))
  (Utilities|FlowControl|DoOnce false
    (:Completed
      (Variables|Character|SetDead true))))

(fn SlowMotionRunning
  (params (Running? :type Boolean))
  (if Running?
    (Variables|AttackVariables|SetSlowMotionOccuring true)
    (Input|DisableInput (Game|GetPlayerController 0))
    (else
      (Input|EnableInput (Game|GetPlayerController 0))
      (Variables|AttackVariables|SetSlowMotionOccuring false))))

(fn SlowMotionConditions
  (params (IncomingDamage :type Integer))
  (if (Variables|Character|GetDead)
    (LocalVariables|SetCanTriggerKIllCam false :!label _label)
    (else
      ;[1 1 1] Close Enough To Player To Trigger
      (if (Variables|AttackVariables|GetInPlayerRange)
        ;[1 1 1] If Incoming Damage is more then current Health
        (if (>= IncomingDamage 0)
          (if (Variables|AttackVariables|GetBlockUp)
            (goto _label)
            (else
              (LocalVariables|SetCanTriggerKIllCam true)))
          (else
            (goto _label)))
        (else
          (goto _label)))))
  (return (LocalVariables|GetCanTriggerKIllCam)))

(fn ReportNoise
  (params (NoiseLocation :type Vector) (Instigator :type Actor%20Object%20Reference))
  (Class|AISenseHearing|ReportNoiseEvent NoiseLocation 1.0 Instigator 2e+02 "None")
  (Class|AISenseDamage|ReportDamageEvent self Instigator 1e+01 NoiseLocation "0, 0, 0" "None"))

(fn UpdateWidgetValues)

(fn BeginPlayDeathCheck)

(fn InitializeComponents)

(fn CanbeAssassinated
  (return false))

(fn FindAvailableAssassinationCam
  (return 0))

(fn GetWeaponRange
  (return (Variables|Default|GetMelee%20Weapon%20Range)))

(fn IsDead
  (return (Variables|Character|GetDead)))

(fn IsFacingEnemy?
  (return false))

(fn IsMoving?
  (return false))

(fn IsPlayer?
  (return false))

(fn IsWeaponDrawn?
  (return false))

(fn PassArmorMeshes
  (return 0 0 0 0 0 0 0 0 0 0 0))

(fn PassAssassinationComps
  (return 0 0))

(fn PassAttackStyle
  (return "NewEnumerator7"))

(fn PassBehaviourTree
  (return 0))

(fn PassBody
  (return 0 0 0 0 0 0 0 0))

(fn PassCamera
  (return 0 0))

(fn PassHealthHUD
  (return 0))

(fn PassMovementMode
  (return "MOVE_None"))

(fn PassSpline
  (return (Variables|SetupInGame|GetPathwaySplineRef)))

(fn PassSwitchAttackStyle
  (return false))

(fn PassWarningMesh
  (return 0))

(fn PassWeaponRange
  (return (Variables|Default|GetMelee%20Weapon%20Range)))

(fn RetrievePlayerStatus
  (return false "NewEnumerator2" "NewEnumerator0"))

(fn SendDeath
  (CallFunction|Death false)
  (return))

(fn SetDisableControls
  (params (DisableMovement :type Boolean) (DisableCamera :type Boolean))
  (return))

(fn UpdateMovementMode
  (params (MovementMode :type EMovementMode%20Enum :default "MOVE_None")))