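; Targeting component that gives the owning character a toggleable enemy lock-on, available in one attack style.
; A camera-forward sphere trace picks a living pawn, then a looping timer eases control rotation toward it.
; Locking disables camera input and makes the character follow controller rotation, except during a roll montage.
; Left/right switching scans nearby living EnemyAI, splits them by camera-right dot product and picks the unobstructed one closest to the current target.
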(event Custom|LockToTargetTick
  ;[1 1 1] Lock To Target - Triggered By Timer
  (CallFunction|LockontoTarget))

(event Custom|LockOnTarget
  (bind (_start _end) (CallFunction|CreateForwardTrace))
  ;[1 1 1] Tab To Target Select Target (All explained in one of my step by step tutorials "Unreal Engine 4 - Enemy Targeting System & Switch Attack Stance" Beardgames)
  (if (Utilities|Enum|Equal(Enum) (Variables|/Game/Proto/Rework_All_Project/Blueprints/Components/CombatStatusComponent.CombatStatusComponent_C|GetCurrentAttackStyle (Variables|Default|GetCombatStatusComponent)) "NewEnumerator0")
    (if (Utilities|IsValid (Variables|Default|GetLockedOnTarget))
      (CallFunction|ToggleLockon false)
      (Utilities|Time|ClearandInvalidateTimerbyHandle (Variables|Default|GetLockOnTick))
      (else
        (bind (_outhit _returnvalue) (Collision|SphereTraceForObjects _start _end 3e+02 (Utilities|Array|MakeArray "ObjectTypeQuery3") false 0 "None"))
        (if _returnvalue
          (bind _dead (Class|ICharacter|IsDead(Message) (.HitActor (Collision|BreakHitResult _outhit))))
          (if _dead
            (CallFunction|ToggleLockon false :!label _label)
            (if (Utilities|Time|IsValidTimerHandle (Variables|Default|GetLockOnTick))
              (Utilities|Time|ClearandInvalidateTimerbyHandle (Variables|Default|GetLockOnTick)))
            (else
              (CallFunction|ToggleLockon true (.HitActor (Collision|BreakHitResult _outhit)))
              (bind _returnvalue_2 (Utilities|Time|SetTimerbyEvent (EventDispatchers|CreateEvent :!event Custom|LockToTargetTick) 0.003 true))
              (Variables|Default|SetLockOnTick _returnvalue_2)))
          (else
            (goto _label)))))))

(event Custom|ToggleLockOn
  ;[1 1 1] Find Enemies In Area
  (CallFunction|ScanActorsinArea false))

(event Custom|RemoveLock
  ;[1 1 1] Tab To Target Select Target (All explained in one of my step by step tutorials "Unreal Engine 4 - Enemy Targeting System & Switch Attack Stance" Beardgames)
  (Utilities|IsValid (Variables|Default|GetLockedOnTarget)
    (:Is%20Valid
      (CallFunction|ToggleLockon false)
      (Utilities|Time|ClearandInvalidateTimerbyHandle (Variables|Default|GetLockOnTick)))))

(event Custom|CheckForNextLock
  (bind (_start _end) (CallFunction|CreateForwardTrace))
  ;[1 1 1] Tab To Target Select Target (All explained in one of my step by step tutorials "Unreal Engine 4 - Enemy Targeting System & Switch Attack Stance" Beardgames)
  (Utilities|IsValid (Variables|Default|GetLockedOnTarget)
    (:Is%20Valid
      (bind (_outhit _returnvalue) (Collision|SphereTraceForObjects _start _end 3e+02 (Utilities|Array|MakeArray "ObjectTypeQuery3") false 0 "None"))
      (if _returnvalue
        (bind _dead (Class|ICharacter|IsDead(Message) (.HitActor (Collision|BreakHitResult _outhit))))
        (if _dead
          (CallFunction|ToggleLockon false :!label _label)
          (if (Utilities|Time|IsValidTimerHandle (Variables|Default|GetLockOnTick))
            (Utilities|Time|ClearandInvalidateTimerbyHandle (Variables|Default|GetLockOnTick)))
          (else
            (CallFunction|ToggleLockon true (.HitActor (Collision|BreakHitResult _outhit)))
            (bind _returnvalue_2 (Utilities|Time|SetTimerbyEvent (EventDispatchers|CreateEvent :!event Custom|LockToTargetTick) 0.003 true))
            (Variables|Default|SetLockOnTick _returnvalue_2)))
        (else
          (goto _label))))))

(event EventBeginPlay
  ;[1 1 1] Setup
  (CallFunction|StoreComponents))

(fn CreateForwardTrace
  (bind _returnvalue (Components|GetOwner))
  (bind _followcamera (Variables|Default|GetFollowCamera))
  (bind _returnvalue_2 (Transformation|GetActorLocation _returnvalue))
  (bind _returnvalue_3 (Math|Vector|GetForwardVector _followcamera))
  (bind _returnvalue_4 (* _returnvalue_3 2.8e+02))
  (bind _returnvalue_5 (+ _returnvalue_2 _returnvalue_4))
  (return _returnvalue_5 (+ _returnvalue_5 (* (Math|Vector|GetForwardVector (Variables|Default|GetFollowCamera)) 2e+03) "0,0,200.000000")))

(fn ScanActorsinArea
  (params (IgnoreReset :type Boolean))
  (bind _returnvalue (Components|GetOwner))
  (bind _returnvalue_2 (Transformation|GetActorLocation _returnvalue))
  ;[1 1 1] Scans All Actors In Area
  (if IgnoreReset
    _
    (else
      (Utilities|Array|Clear (Variables|Default|GetAI_InRange))))
  (bind _outhits (Collision|MultiSphereTraceForObjects _returnvalue_2 _returnvalue_2 (Variables|Default|GetLockOnRadius) (Utilities|Array|MakeArray "ObjectTypeQuery3") false (Utilities|Array|MakeArray (Components|GetOwner)) "None"))
  (for _array_element _outhits
    (if (not (Utilities|Array|ContainsItem (Variables|Default|GetAI_InRange) (.HitActor (Collision|BreakHitResult _array_element))))
      (if (Actor|ActorHasTag (.HitActor (Collision|BreakHitResult _array_element)) "EnemyAI")
        (bind _dead (Class|ICharacter|IsDead(Message) (.HitActor (Collision|BreakHitResult _array_element))))
        (if (not _dead)
          (Utilities|Array|Add (Variables|Default|GetAI_InRange) (.HitActor (Collision|BreakHitResult _array_element)))))))
  (if (not IgnoreReset)
    (CallFunction|LockonTarget)))

(fn ToggleLockon
  (params (LockOn :type Boolean) (LockedOnTarget :type Actor%20Object%20Reference))
  (bind _characterref (Variables|Components|GetCharacterRef))
  (bind _charactermovement (Variables|/Script/Engine.Character|GetCharacterMovement _characterref))
  (if LockOn
    (Variables|Default|SetLockedOnTarget LockedOnTarget)
    (Default|CallUpdateTargetLocked true)
    (Class|ICharacter|SetDisableControls(Message) _characterref false true)
    (Variables|/Script/Engine.CharacterMovementComponent|SetbUseControllerDesiredRotation _charactermovement true)
    (Variables|/Script/Engine.CharacterMovementComponent|SetbOrientRotationToMovement _charactermovement false)
    (else
      (Variables|Default|SetLockedOnTarget 0)
      (Default|CallUpdateTargetLocked false)
      (Class|ICharacter|SetDisableControls(Message) _characterref false false)
      (Variables|/Script/Engine.CharacterMovementComponent|SetbUseControllerDesiredRotation _charactermovement false)
      (Variables|/Script/Engine.CharacterMovementComponent|SetbOrientRotationToMovement _charactermovement true))))

(fn LockontoTarget
  (bind _returnvalue (Utilities|Time|GetWorldDeltaSeconds))
  (bind _returnvalue_2 (Components|GetOwner))
  (bind _returnvalue_3 (Components|GetOwner))
  (bind _lockedontarget (Variables|Default|GetLockedOnTarget))
  (bind _returnvalue_4 (Transformation|GetActorLocation _lockedontarget))
  (bind _returnvalue_5 (Transformation|GetActorLocation _returnvalue_3))
  (bind _instigator (Variables|/Script/Engine.Actor|GetInstigator _returnvalue_2))
  (bind _returnvalue_6 (- (.z _returnvalue_4) 1e+02))
  (bind _returnvalue_7 (Pawn|GetController _instigator))
  (bind _returnvalue_8 (Math|Rotator|FindLookatRotation _returnvalue_5 (Math|Vector|MakeVector (.x _returnvalue_4) (.y _returnvalue_4) _returnvalue_6)))
  (bind _returnvalue_9 (Transformation|GetActorRotation _returnvalue_7))
  (bind _returnvalue_10 (Math|Interpolation|RInterpTo _returnvalue_9 _returnvalue_8 _returnvalue 5.0))
  ;[1 1 1] Set Camera To Location
  (Pawn|SetControlRotation _returnvalue_7 (Math|Rotator|MakeRotator (.Roll (Math|Rotator|BreakRotator _returnvalue_9)) (.pitch _returnvalue_10) (.yaw _returnvalue_10)))
  ;[1 1 1] IF Player Rolls, Don't Lock Character Until Facing Forwards Again
  (if (CallFunction|IsPlayingMontage (Variables|/Script/Engine.Character|GetMesh (Variables|Components|GetCharacterRef)) (CallFunction|PassAnimation "NewEnumerator0"))
    (Variables|/Script/Engine.CharacterMovementComponent|SetbOrientRotationToMovement (Variables|/Script/Engine.Character|GetCharacterMovement (Variables|Components|GetCharacterRef)) true)
    (else
      (CallFunction|ToggleLockon true (Variables|Default|GetLockedOnTarget)))))

(fn SwitchTargetRight
  (bind _characterref (Variables|Components|GetCharacterRef))
  (bind _ai_onright (Variables|Default|GetAI_OnRight))
  (bind _output (Utilities|Array|Get(acopy) _ai_onright))
  (CallFunction|ScanActorsinArea true)
  (Variables|Default|SetClosestAIToLockTarget 0)
  (Utilities|Array|Clear (Variables|Default|GetAI_OnRight))
  ;[1 1 1] Checks for AI on Right Side Of Locked On Target
  (for _array_element (Variables|Default|GetAI_InRange)
    (if (!= _array_element (Variables|Default|GetLockedOnTarget))
      (if (not (> (Math|Vector|DotProduct (Math|Vector|GetRightVector (Variables|Default|GetFollowCamera)) (Math|Vector|Normalize (- (Transformation|GetActorLocation (Variables|Default|GetLockedOnTarget)) (Transformation|GetActorLocation _array_element)))) 0.0))
        ;;[1 1 1] Only Swap Targets If Nothing Inbetween
        (bind _returnvalue (Collision|LineTraceForObjects (Transformation|GetActorLocation _array_element) (Transformation|GetActorLocation _characterref) (Utilities|Array|MakeArray "ObjectTypeQuery1") false (Utilities|Array|MakeArray _characterref (Variables|Default|GetLockedOnTarget)) "None"))
        (if (not _returnvalue)
          (Utilities|Array|Add (Variables|Default|GetAI_OnRight) _array_element)))))
  ;[1 1 1] Finds AI on Right Side, Closest to Locked On Target
  (Utilities|IsValid _output
    (:Is%20Valid
      (Variables|Default|SetClosestAIToLockTarget _output)
      (for _array_element_2 (Variables|Default|GetAI_OnRight)
        (if (!= (Variables|Default|GetLockedOnTarget) _array_element_2)
          (if (< (Transformation|GetDistanceTo _array_element_2 (Variables|Default|GetLockedOnTarget)) (Transformation|GetDistanceTo (Variables|Default|GetClosestAIToLockTarget) (Variables|Default|GetLockedOnTarget)))
            (Variables|Default|SetClosestAIToLockTarget _array_element_2))))
      (Variables|Default|SetLockedOnTarget (Variables|Default|GetClosestAIToLockTarget))
      (Animation|PlayAnimMontage (Variables|Components|GetCharacterRef) 0 1.0 "None"))))

(fn SwitchTargetLeft
  (bind _characterref (Variables|Components|GetCharacterRef))
  (bind _ai_onleft (Variables|Default|GetAI_OnLeft))
  (bind _output (Utilities|Array|Get(acopy) _ai_onleft))
  (CallFunction|ScanActorsinArea true)
  (Variables|Default|SetClosestAIToLockTarget 0)
  (Utilities|Array|Clear (Variables|Default|GetAI_OnLeft))
  (LocalVariables|SetSuccess false)
  ;[1 1 1] Checks for AI on Left Side Of Locked On Target
  (for _array_element (Variables|Default|GetAI_InRange)
    (if (!= (Variables|Default|GetLockedOnTarget) _array_element)
      (if (> (Math|Vector|DotProduct (Math|Vector|GetRightVector (Variables|Default|GetFollowCamera)) (Math|Vector|Normalize (- (Transformation|GetActorLocation (Variables|Default|GetLockedOnTarget)) (Transformation|GetActorLocation _array_element)))) 0.0)
        ;;[1 1 1] Only Swap Targets If Nothing Inbetween
        (bind _returnvalue (Collision|LineTraceForObjects (Transformation|GetActorLocation _array_element) (Transformation|GetActorLocation _characterref) (Utilities|Array|MakeArray "ObjectTypeQuery1") false (Utilities|Array|MakeArray _characterref (Variables|Default|GetLockedOnTarget)) "None"))
        (if (not _returnvalue)
          (Utilities|Array|Add (Variables|Default|GetAI_OnLeft) _array_element)
          (LocalVariables|SetSuccess true)))))
  ;[1 1 1] Finds AI on Left Side, Closest to Locked On Target
  (if (LocalVariables|GetSuccess)
    (Utilities|IsValid _output
      (:Is%20Valid
        (Variables|Default|SetClosestAIToLockTarget _output)
        (for _array_element_2 (Variables|Default|GetAI_OnLeft)
          (if (!= (Variables|Default|GetLockedOnTarget) _array_element_2)
            (if (< (Transformation|GetDistanceTo _array_element_2 (Variables|Default|GetLockedOnTarget)) (Transformation|GetDistanceTo (Variables|Default|GetClosestAIToLockTarget) (Variables|Default|GetLockedOnTarget)))
              (Variables|Default|SetClosestAIToLockTarget _array_element_2))))
        (Variables|Default|SetLockedOnTarget (Variables|Default|GetClosestAIToLockTarget))
        (Animation|PlayAnimMontage (Variables|Components|GetCharacterRef) 0 1.0 "None")))))

(fn StoreComponents
  (bind _returnvalue (Components|GetOwner))
  (Variables|Default|SetCombatStatusComponent (Actor|GetComponentbyClass _returnvalue "/Game/Proto/Rework_All_Project/Blueprints/Components/CombatStatusComponent.CombatStatusComponent_C"))
  (bind _ascharacter (Utilities|Casting|CastToCharacter _returnvalue))
  (Variables|Components|SetCharacterRef _ascharacter))