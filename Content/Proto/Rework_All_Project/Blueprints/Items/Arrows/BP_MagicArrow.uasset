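; BP_MagicArrow is an arrow item that carries magic damage and is tinted by its damage type.
; InitializeArrow stores the damage type and special damage info on its ArrowComponent, then creates a dynamic material on each mesh slot, always sourced from the first material.
; Each instance gets a fixed Value and a Colour picked by damage type, with bright HDR colours for Fire, Frost, Electric and Poison and black for the rest.
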(event Collision|EventActorBeginOverlap
  (params (OtherActor :type Actor%20Object%20Reference)))

(event EventTick
  (params (DeltaSeconds :type Float%20%28single-precision%29))
  (|CallParentFunction DeltaSeconds) ; This node is disabled and will not be called.\nDrag off pins to build functionality.
)

(event EventInitializeArrow
  (params (DamageType :type E_DamageType%20Enum :default "NewEnumerator0") (SpecialDamage :type S%20Special%20Damage%20Info%20Structure))
  (bind _arrow (Variables|Default|GetArrow))
  (bind _arrowcomponent (Variables|Default|GetArrowComponent))
  ;[1 1 1] Retrieve Magic Values
  (bind _output_get (Variables|/Game/FlexibleCombatSystem/Blueprints/Components/ArrowComponent.ArrowComponent_C|SetDamageType _arrowcomponent DamageType))
  (Variables|/Game/FlexibleCombatSystem/Blueprints/Components/ArrowComponent.ArrowComponent_C|SetSpecialDamageInfo _arrowcomponent SpecialDamage)
  ;[1 1 1] Setup Magic Arrow Materials
  (for (_ _array_index) (Rendering|Material|GetMaterials _arrow)
    (bind _returnvalue (Rendering|Material|CreateDynamicMaterialInstance _arrow _array_index (Rendering|Material|GetMaterial _arrow 0) "None" :!class /Script/Engine.PrimitiveComponent))
    (Rendering|Material|SetScalarParameterValue _returnvalue "Value" 0.1 :!class /Script/Engine.MaterialInstanceDynamic)
    (Rendering|Material|SetVectorParameterValue _returnvalue "Colour" (Utilities|Select :Index _output_get :NewEnumerator0 "" :NewEnumerator1 "(R=300.000000,G=33.448704,B=0.000000,A=1.000000)" :NewEnumerator2 "" :NewEnumerator8 "(R=0.000000,G=242.207047,B=300.000000,A=1.000000)" :NewEnumerator3 "(R=300.000000,G=209.420441,B=0.000000,A=1.000000)" :NewEnumerator4 "(R=97.154366,G=300.000000,B=0.000000,A=1.000000)" :NewEnumerator5 "" :NewEnumerator6 "" :NewEnumerator7 "" :NewEnumerator9 "") :!class /Script/Engine.MaterialInstanceDynamic)))

(fn ConstructionScript
  (|CallParentFunction))