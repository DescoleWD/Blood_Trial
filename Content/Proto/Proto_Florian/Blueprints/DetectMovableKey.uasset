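; Prototype key-gated platform that moves its static mesh when the player enters a trigger box.
; With HaveKey set, chained eased MoveComponentTo calls carry the mesh through preset locations, applying a 180-degree rotation on the last leg.
; Without the key, it prints a warning and plays a refusal sound.
; Leaving the box after a move sends the mesh back along the waypoints after a short delay; HaveMoved is never cleared.
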(event OnComponentBeginOverlap(Box)
  (params (OverlappedComponent :type Primitive%20Component%20Object%20Reference) (OtherActor :type Actor%20Object%20Reference) (OtherComp :type Primitive%20Component%20Object%20Reference) (OtherBodyIndex :type Integer) (bFromSweep :type Boolean) (SweepResult :type Hit%20Result%20Structure%20%28by%20ref%29))
  (bind _asbp_main_character (Utilities|Casting|CastToBP_MainCharacter OtherActor))
  (if (Actor|ActorHasTag _asbp_main_character "Player")
    (if (Variables|Default|GetHaveKey?)
      (Variables|Default|SetHaveMoved true)
      (Components|MoveComponentTo (Variables|Default|GetStaticMesh) (Variables|Default|GetPlatLocation2) "0, 0, 0" true true (Variables|Default|GetDuration) false)
      (Components|MoveComponentTo (Variables|Default|GetStaticMesh) (Variables|Default|GetPlatLocation3) "0, 0, 0" true true (Variables|Default|GetDuration) false)
      (Components|MoveComponentTo (Variables|Default|GetStaticMesh) (Variables|Default|GetPlatLocation4) "0,180.000000, 0" true true 2.0 false)
      (else
        (Development|PrintText "NEED KEY" true true "(R=1.000000,G=0.000000,B=0.030401,A=1.000000)")
        (Audio|PlaySound2D "/Game/Proto/Proto_Florian/SFX/PlatformNoMove.PlatformNoMove" 1.0 1.0 0.0 0 0)))))

(event OnComponentEndOverlap(Box)
  (params (OverlappedComponent :type Primitive%20Component%20Object%20Reference) (OtherActor :type Actor%20Object%20Reference) (OtherComp :type Primitive%20Component%20Object%20Reference) (OtherBodyIndex :type Integer))
  (bind _asbp_main_character (Utilities|Casting|CastToBP_MainCharacter OtherActor))
  (if (Actor|ActorHasTag _asbp_main_character "Player")
    (if (Variables|Default|GetHaveMoved)
      (Utilities|FlowControl|Delay 0.5)
      (Components|MoveComponentTo (Variables|Default|GetStaticMesh) (Variables|Default|GetPlatLocation3) "0, 0, 0" true true 1.0 false)
      (Components|MoveComponentTo (Variables|Default|GetStaticMesh) (Variables|Default|GetPlatLocation2) "0, 0, 0" true true 1.0 false)
      (Components|MoveComponentTo (Variables|Default|GetStaticMesh) (Variables|Default|GetPlatLocation1) "0, 0, 0" true true 2.0 false))))

(fn ConstructionScript)