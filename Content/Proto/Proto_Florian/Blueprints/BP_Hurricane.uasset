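; Prototype hurricane hazard with four rotating wings that damage Master_Enemy actors on overlap and can be launched outward in a dash.
; DashActive stops the rotation, slides each wing along its own timeline to point 1 of its spline, and scales up DashEffect as a growing blast.
; Wing boxes deal light damage while spinning and heavy damage once launched; DashEffect only damages after launch.
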(event OnComponentBeginOverlap(Box)
  (params (OverlappedComponent :type Primitive%20Component%20Object%20Reference) (OtherActor :type Actor%20Object%20Reference) (OtherComp :type Primitive%20Component%20Object%20Reference) (OtherBodyIndex :type Integer) (bFromSweep :type Boolean) (SweepResult :type Hit%20Result%20Structure%20%28by%20ref%29))
  ;[0.1444 1 0.1815] Damage Ennemi
  (bind _asmaster_enemy (Utilities|Casting|CastToMaster_Enemy OtherActor))
  (if (Variables|Default|GetLaunch?)
    (Game|Damage|ApplyDamage _asmaster_enemy 15.0 0 0)
    (else
      (Game|Damage|ApplyDamage _asmaster_enemy 3.0 0 0))))

(event OnComponentBeginOverlap(Box1)
  (params (OverlappedComponent :type Primitive%20Component%20Object%20Reference) (OtherActor :type Actor%20Object%20Reference) (OtherComp :type Primitive%20Component%20Object%20Reference) (OtherBodyIndex :type Integer) (bFromSweep :type Boolean) (SweepResult :type Hit%20Result%20Structure%20%28by%20ref%29))
  ;[0.1444 1 0.1815] Damage Ennemi
  (bind _asmaster_enemy (Utilities|Casting|CastToMaster_Enemy OtherActor))
  (if (Variables|Default|GetLaunch?)
    (Game|Damage|ApplyDamage _asmaster_enemy 15.0 0 0)
    (else
      (Game|Damage|ApplyDamage _asmaster_enemy 3.0 0 0))))

(event OnComponentBeginOverlap(Box3)
  (params (OverlappedComponent :type Primitive%20Component%20Object%20Reference) (OtherActor :type Actor%20Object%20Reference) (OtherComp :type Primitive%20Component%20Object%20Reference) (OtherBodyIndex :type Integer) (bFromSweep :type Boolean) (SweepResult :type Hit%20Result%20Structure%20%28by%20ref%29))
  ;[0.1444 1 0.1815] Damage Ennemi
  (bind _asmaster_enemy (Utilities|Casting|CastToMaster_Enemy OtherActor))
  (if (Variables|Default|GetLaunch?)
    (Game|Damage|ApplyDamage _asmaster_enemy 15.0 0 0)
    (else
      (Game|Damage|ApplyDamage _asmaster_enemy 3.0 0 0))))

(event OnComponentBeginOverlap(Box2)
  (params (OverlappedComponent :type Primitive%20Component%20Object%20Reference) (OtherActor :type Actor%20Object%20Reference) (OtherComp :type Primitive%20Component%20Object%20Reference) (OtherBodyIndex :type Integer) (bFromSweep :type Boolean) (SweepResult :type Hit%20Result%20Structure%20%28by%20ref%29))
  ;[0.1444 1 0.1815] Damage Ennemi
  (bind _asmaster_enemy (Utilities|Casting|CastToMaster_Enemy OtherActor))
  (if (Variables|Default|GetLaunch?)
    (Game|Damage|ApplyDamage _asmaster_enemy 15.0 0 0)
    (else
      (Game|Damage|ApplyDamage _asmaster_enemy 3.0 0 0))))

(event OnComponentBeginOverlap(DashEffect)
  (params (OverlappedComponent :type Primitive%20Component%20Object%20Reference) (OtherActor :type Actor%20Object%20Reference) (OtherComp :type Primitive%20Component%20Object%20Reference) (OtherBodyIndex :type Integer) (bFromSweep :type Boolean) (SweepResult :type Hit%20Result%20Structure%20%28by%20ref%29))
  (bind _asmaster_enemy (Utilities|Casting|CastToMaster_Enemy OtherActor))
  (if (Variables|Default|GetLaunch?)
    (Game|Damage|ApplyDamage _asmaster_enemy 15.0 0 0)))

(event Custom|DashActive
  ;[0.0196 1 0.03739] Launch
  (Variables|Default|SetLaunch? true)
  (Utilities|FlowControl|Sequence
    (:then_0
      (Components|Activation|SetActive (Variables|Default|GetRotatingMovement) false false)
      (Utilities|FlowControl|Sequence
        (:then_0
          (Variables|Default|SetWing1_Location (Variables|/Script/Engine.SceneComponent|GetRelativeLocation (Variables|Default|GetWing1)))
          (Components|Timeline|SetPlayRate (Variables|Default|GetDashWing_1) (/ 1.0 (Variables|Default|GetTimeToComplete)))
          (bind _movetrack (Timeline|DashWing_1 Play)
            (:Update
              (Transformation|SetRelativeLocation (Variables|Default|GetWing1) (Math|Vector|Lerp(Vector) (Variables|Default|GetWing1_Location) (Spline|GetLocationatSplinePoint (Variables|Default|GetSpline1) 1 "Local") _movetrack) false false))))
        (:then_1
          (Variables|Default|SetWing2_Location (Variables|/Script/Engine.SceneComponent|GetRelativeLocation (Variables|Default|GetWing2)))
          (Components|Timeline|SetPlayRate (Variables|Default|GetTimeline_0) (/ 1.0 (Variables|Default|GetTimeToComplete)))
          (bind _movetrack_2 (Timeline|Timeline_0 Play)
            (:Update
              (Transformation|SetRelativeLocation (Variables|Default|GetWing2) (Math|Vector|Lerp(Vector) (Variables|Default|GetWing2_Location) (Spline|GetLocationatSplinePoint (Variables|Default|GetSpline2) 1 "Local") _movetrack_2) false false))))
        (:then_2
          (Variables|Default|SetWing3_Location (Variables|/Script/Engine.SceneComponent|GetRelativeLocation (Variables|Default|GetWing3)))
          (Components|Timeline|SetPlayRate (Variables|Default|GetTimeline_1) (/ 1.0 (Variables|Default|GetTimeToComplete)))
          (bind _movetrack_3 (Timeline|Timeline_1 Play)
            (:Update
              (Transformation|SetRelativeLocation (Variables|Default|GetWing3) (Math|Vector|Lerp(Vector) (Variables|Default|GetWing3_Location) (Spline|GetLocationatSplinePoint (Variables|Default|GetSpline3) 1 "Local") _movetrack_3) false false))))
        (:then_3
          (Variables|Default|SetWing4_Location (Variables|/Script/Engine.SceneComponent|GetRelativeLocation (Variables|Default|GetWing)))
          (Components|Timeline|SetPlayRate (Variables|Default|GetTimeline_2) (/ 1.0 (Variables|Default|GetTimeToComplete)))
          (bind _movetrack_4 (Timeline|Timeline_2 Play)
            (:Update
              (Transformation|SetRelativeLocation (Variables|Default|GetWing) (Math|Vector|Lerp(Vector) (Variables|Default|GetWing4_Location) (Spline|GetLocationatSplinePoint (Variables|Default|GetSpline) 1 "Local") _movetrack_4) false false))))))
    (:then_1
      (bind _movetrack_5 (Timeline|Timeline_3 Play)
        (:Update
          (Transformation|SetWorldScale3D (Variables|Default|GetDashEffect) (Math|Vector|Lerp(Vector) "1.000000,1.000000,1.000000" "50.000000,50.000000,50.000000" _movetrack_5)))))))

(fn ConstructionScript)