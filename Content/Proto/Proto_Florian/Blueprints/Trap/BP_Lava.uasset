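; BP_Lava is a prototype lava trap that slows and burns the player.
; Box overlaps with BP_MainBase subtract or restore walk speed and toggle a CharacterIn flag.
; While the flag is set, Brulure runs from Tick and damages player character 0 using the game instance's LavaDamage; its DoOnce resets immediately, so damage lands every frame.
; The Lava_Feedback HUD widget logic is disconnected and never runs.
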(event OnComponentBeginOverlap(Box)
  (params (OverlappedComponent :type Primitive%20Component%20Object%20Reference) (OtherActor :type Actor%20Object%20Reference) (OtherComp :type Primitive%20Component%20Object%20Reference) (OtherBodyIndex :type Integer) (bFromSweep :type Boolean) (SweepResult :type Hit%20Result%20Structure%20%28by%20ref%29))
  (bind _asbp_main_base (Utilities|Casting|CastToBP_MainBase OtherActor))
  (CallFunction|Brulure)
  (Variables|/Script/Engine.CharacterMovementComponent|SetMaxWalkSpeed (Variables|/Script/Engine.Character|GetCharacterMovement _asbp_main_base) (- (Variables|/Script/Engine.CharacterMovementComponent|GetMaxWalkSpeed (Variables|/Script/Engine.Character|GetCharacterMovement _asbp_main_base)) (Variables|Default|GetMainChara_SpeedReduction)))
  (Variables|Default|SetCharacterIn? true))

(event OnComponentEndOverlap(Box)
  (params (OverlappedComponent :type Primitive%20Component%20Object%20Reference) (OtherActor :type Actor%20Object%20Reference) (OtherComp :type Primitive%20Component%20Object%20Reference) (OtherBodyIndex :type Integer))
  (bind _asbp_main_base (Utilities|Casting|CastToBP_MainBase OtherActor))
  (CallFunction|Brulure)
  (Variables|/Script/Engine.CharacterMovementComponent|SetMaxWalkSpeed (Variables|/Script/Engine.Character|GetCharacterMovement _asbp_main_base) (+ (Variables|/Script/Engine.CharacterMovementComponent|GetMaxWalkSpeed (Variables|/Script/Engine.Character|GetCharacterMovement _asbp_main_base)) (Variables|Default|GetMainChara_SpeedReduction)))
  (Variables|Default|SetCharacterIn? false))

(event EventTick
  (params (DeltaSeconds :type Float%20%28single-precision%29))
  (CallFunction|Brulure))

(fn ConstructionScript)

(fn Brulure
  (if (Variables|Default|GetCharacterIn?)
    (Utilities|FlowControl|DoOnce false :!label _label
      (:Completed
        (bind _asbp_main_base (Utilities|Casting|CastToBP_MainBase (Game|GetPlayerCharacter 0)))
        (Game|Damage|ApplyDamage _asbp_main_base (Variables|/Game/Proto/Main/Blueprint/Save_BFL_GameInstance/BloodTrial_GameInstance.BloodTrial_GameInstance_C|GetLavaDamage (CallFunction|GetInst)) 0 self)
        (goto _label Reset)))))