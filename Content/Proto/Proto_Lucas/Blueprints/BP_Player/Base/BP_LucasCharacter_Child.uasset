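; Prototype player character Blueprint that handles movement input and pause menu toggling.
; Four axis inputs move the pawn along fixed world diagonals, independent of control rotation, with a small dead zone.
; The pause action lazily creates and caches WBP_PauseMenu, then toggles game pause, cursor and input mode.
; The bolas explosion input is unfinished: it only casts the bolas reference, and its interface call is disconnected.
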(event EventBeginPlay)

(event Collision|EventActorBeginOverlap
  (params (OtherActor :type Actor%20Object%20Reference)))

(event EventTick
  (params (DeltaSeconds :type Float%20%28single-precision%29)))

(event Input|ActionEvents|InputActionPauseMenu
  (params (Key :type Key%20Structure :default "None"))
  (bind _returnvalue (Game|GetPlayerController 0))
  ;[1 1 1] Pause/Unpause Game
  (:Pressed
    (Utilities|IsValid (Variables|Default|GetPauseMenuRef)
      (:Is%20Valid
        _)
      (:Is%20Not%20Valid
        (bind _returnvalue_2 (UserInterface|CreateWidget "/Game/Proto/Proto_Lucas/Blueprints/Menus/Widgets/WBP_PauseMenu.WBP_PauseMenu_C"))
        (Variables|Default|SetPauseMenuRef _returnvalue_2)))
    (if (Game|IsGamePaused)
      (Widget|RemovefromParent (Variables|Default|GetPauseMenuRef))
      (Game|SetGamePaused false)
      (Variables|/Script/Engine.PlayerController|SetbShowMouseCursor _returnvalue false)
      (Input|SetInputModeGameOnly _returnvalue)
      (else
        (UserInterface|Viewport|AddtoViewport (Variables|Default|GetPauseMenuRef) 0)
        (Game|SetGamePaused true)
        (Variables|/Script/Engine.PlayerController|SetbShowMouseCursor _returnvalue true)
        (Input|SetInputModeGameandUI _returnvalue (Variables|Default|GetPauseMenuRef) "LockInFullscreen" false)))))

(event Input|ActionEvents|InputActionBolasExplosion
  (params (Key :type Key%20Structure :default "None"))
  ;[0.5896 0.2389 1] Bolas Explosion
  (:Pressed
    (Utilities|Casting|CastToBP_Bolas (Variables|Default|GetBolasRef))))

(event Input|AxisEvents|InputAxisMoveForward
  (params (AxisValue :type Float%20%28single-precision%29))
  ;[1 1 1] Character movement
  (if (>= (Math|Float|Absolute(Float) (* AxisValue 1e+01)) 1.0)
    (Pawn|Input|AddMovementInput (Class|PawnMovementComponent|GetPawnOwner (Variables|Character|GetCharacterMovement)) "1000.000000,-1000.000000, 0" AxisValue false)))

(event Input|AxisEvents|InputAxisMoveBackward
  (params (AxisValue :type Float%20%28single-precision%29))
  ;[1 1 1] Character movement
  (if (>= (Math|Float|Absolute(Float) (* AxisValue 1e+01)) 1.0)
    (Pawn|Input|AddMovementInput (Class|PawnMovementComponent|GetPawnOwner (Variables|Character|GetCharacterMovement)) "1000.000000,-1000.000000, 0" AxisValue false)))

(event Input|AxisEvents|InputAxisMoveLeft
  (params (AxisValue :type Float%20%28single-precision%29))
  ;[1 1 1] Character movement
  (if (>= (Math|Float|Absolute(Float) (* AxisValue 1e+01)) 1.0)
    (Pawn|Input|AddMovementInput (Class|PawnMovementComponent|GetPawnOwner (Variables|Character|GetCharacterMovement)) "1000.000000,1000.000000, 0" AxisValue false)))

(event Input|AxisEvents|InputAxisMoveRight
  (params (AxisValue :type Float%20%28single-precision%29))
  ;[1 1 1] Character movement
  (if (>= (Math|Float|Absolute(Float) (* AxisValue 1e+01)) 1.0)
    (Pawn|Input|AddMovementInput (Class|PawnMovementComponent|GetPawnOwner (Variables|Character|GetCharacterMovement)) "1000.000000,1000.000000, 0" AxisValue false)))

(fn ConstructionScript
  (|CallParentFunction))