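; Blueprint interface for the player controller, the contract other objects use to drive the player's HUD and menus.
; Toggle calls cover inventory, loot, containers, external and vendor inventories, pause, spell book, quest log and spell trainer.
; Getters expose widgets, components and open-menu states, while setters hand over character, HUD, options menu and outline component references.
; All functions are empty declarations, leaving behavior to the implementing class.
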(fn ShowHUD)

(fn HideHUD)

(fn ToggleInventory)

(fn ToggleContainerMenu
  (params (LootComponent :type Loot%20Component%20Object%20Reference) (ToggleTag :type Boolean)))

(fn TogglePauseMenu)

(fn ToggleSpellBook)

(fn SetupReferences
  (params (CharacterRef :type Character%20Object%20Reference) (HUDRef :type BP%20Player%20HUD%20Object%20Reference)))

(fn SetCanUpdateWidget
  (params (CanUpdateWidget :type Boolean))
  (return))

(fn PassHUDWB
  (return 0))

(fn PassLootWindowWB
  (return 0))

(fn LootMenuStatus
  (return false))

(fn InventoryStatus
  (return false))

(fn PassEquipmentComp
  (return 0))

(fn PassInventoryComp
  (return 0))

(fn ContainerStatus
  (return false))

(fn PassContainerWindowWB
  (return 0))

(fn ToggleLootMenu
  (params (Loot%20Component :type Loot%20Component%20Object%20Reference)))

(fn PassLootComponent
  (return 0))

(fn PassExternalInventory
  (return 0))

(fn ToggleExternalInventory
  (params (ExternalInventoryComponent :type Inventory%20Component%20Object%20Reference) (ActorRef :type Actor%20Object%20Reference) (Vendor :type Boolean))
  (return))

(fn ToggleExternalContainerInv
  (params (Inventory%20Component :type Inventory%20Component%20Object%20Reference) (Actor%20Ref :type Actor%20Object%20Reference)))

(fn PassInventoryState
  (return "NewEnumerator0"))

(fn RecieveOptionsMenu
  (params (Options%20Menu :type WB%20Option%20List%20Object%20Reference))
  (return))

(fn PassOptionsMenu
  (return 0))

(fn ToggleQuestLog)

(fn ToggleSpellTrainer)

(fn PassSkillTrainer
  (return 0))

(fn WidgetMenuOpen
  (return false))

(fn ExternalInventoryOpen
  (return false))

(fn PassOutlineComponent
  (params (OutlineComponent :type Outline%20Component%20Object%20Reference))
  (return))

(fn ExternalInventoryConditions
  (return false))