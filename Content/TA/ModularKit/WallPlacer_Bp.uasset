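; Modular wall placer Blueprint that lays static mesh pieces along an editable spline at construction time.
; The construction script makes spline points linear, applies the closed-loop setting, and derives piece spacing from mesh bounding-box X size plus an offset.
; It adds a mesh component at each interval, aligned to the spline, with a mesh picked randomly from an array.
; Spacing and piece count sample the array randomly too, assuming similarly sized meshes.
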(event EventBeginPlay)

(event Collision|EventActorBeginOverlap
  (params (OtherActor :type Actor%20Object%20Reference)))

(event EventTick
  (params (DeltaSeconds :type Float%20%28single-precision%29)))

(fn ConstructionScript
  (bind _target (Variables|Default|GetTarget))
  (bind _offset (Variables|Default|GetOffset))
  (bind _spline (Variables|Default|GetSpline))
  (bind _spline_2 (Variables|Default|GetSpline))
  (bind _returnvalue (Utilities|Array|Length _target))
  (bind _returnvalue_2 (- _returnvalue 1))
  (bind _returnvalue_3 (Math|Random|RandomIntegerinRange 0 _returnvalue_2))
  (bind _output (Utilities|Array|Get(acopy) _target _returnvalue_3))
  (bind _returnvalue_4 (StaticMesh|GetBoundingBox _output))
  (bind _returnvalue_5 (- (.max _returnvalue_4) (.min _returnvalue_4)))
  (bind _returnvalue_6 (+ (.x _returnvalue_5) _offset))
  (for _index (range 0 (- (Spline|GetNumberOfSplinePoints _spline_2) 1))
    (Spline|SetSplinePointType _spline_2 _index "Linear" true))
  (Variables|Default|SetLenght _returnvalue_6)
  (for _index_2 (range 0 (Math|Float|Floor (/ (Spline|GetSplineLength (Variables|Default|GetSpline)) _returnvalue_6)))
    (Spline|SetClosedLoop (Variables|Default|GetSpline) (Variables|Default|GetIn%20Closed%20Loop) true)
    (bind _returnvalue_7 (AddComponent|AddStaticMeshComponent false (Math|Transform|MakeTransform (Math|Vector|MakeVector (.X (Math|Vector|BreakVector (Spline|GetLocationatDistanceAlongSpline _spline (* _index_2 (Variables|Default|GetLenght)) "Local"))) (.Y (Math|Vector|BreakVector (Spline|GetLocationatDistanceAlongSpline _spline (* _index_2 (Variables|Default|GetLenght)) "Local"))) (.Z (Math|Vector|BreakVector (Spline|GetLocationatDistanceAlongSpline _spline (* _index_2 (Variables|Default|GetLenght)) "Local")))) (Math|Rotator|MakeRotator (.Roll (Math|Rotator|BreakRotator (Spline|GetRotationatDistanceAlongSpline _spline (* _index_2 (Variables|Default|GetLenght)) "Local"))) (.Pitch (Math|Rotator|BreakRotator (Spline|GetRotationatDistanceAlongSpline _spline (* _index_2 (Variables|Default|GetLenght)) "Local"))) (.Yaw (Math|Rotator|BreakRotator (Spline|GetRotationatDistanceAlongSpline _spline (* _index_2 (Variables|Default|GetLenght)) "Local")))) "1.000000,1.000000,1.000000")))
    (Components|StaticMesh|SetStaticMesh _returnvalue_7 _output)))