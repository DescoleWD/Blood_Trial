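; Actor component that handles incoming point and radial damage for player and AI characters, from block checks to death.
; It stores hit info, skips hits during certain montages unless frozen, then tries AI auto-block or a raised block through MeleeComponent.
; Unblocked physical hits update EquipmentComponent health, show combat text, and play impact effects and direction-based stun montages.
; AI auto-block chance grows with consecutive hits and resets after success or a lull.
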(event Custom|TakeDamage
  (bind _enemyai (Variables|Default|GetEnemyAI))
  (bind _enemyhit_playrate (Variables|Default|GetEnemyHit-PlayRate))
  (bind _returnvalue (Math|Float|SelectFloat _enemyhit_playrate 1.0 _enemyai))
  ;[1 1 1] Taking Damage
  (CallFunction|SpawnEmitterPS)
  ;;[1 1 1] Reset Melee AI Attack CD
  (CallFunction|UpdateCombatStatuses)
  (Variables|Default|SetDamage%20Over%20Time false)
  (CallFunction|PlayHitSound)
  (switch Utilities|FlowControl|Switch|SwitchonE_DamageType (Variables|IncomingAttackInfo|GetDamageType)
    (:NewEnumerator0
      ;;[1 1 1] Take Physical Damage
      (CallFunction|DamageHealth 0.0 "NewEnumerator0")
      (bind _hitanimation (CallFunction|CalculateHitAnim))
      (bind _ignorehitanim (CallFunction|IgnoreHitAnim))
      (if (not _ignorehitanim)
        (Default|SendStunCalculation (Variables|Default|GetMeleeComponent) (Variables|/Script/Engine.AnimSequenceBase|GetSequenceLength _hitanimation) _returnvalue)
        (Animation|Montage|PlayMontage (Variables|Default|GetCharacterMesh) _hitanimation _returnvalue)))))

(event Custom|PassDamageInfo
  (params (Particle%20System :type Particle%20System%20Object%20Reference) (AttackType :type E_CharacterAction%20Enum :default "NewEnumerator4") (Damage%20Type :type E_DamageType%20Enum :default "NewEnumerator0") (CriticalHit :type Boolean))
  ;[1 1 1] Damage Triggers
  (Variables|IncomingAttackInfo|SetEnemyWeaponPS Particle%20System)
  (Variables|IncomingAttackInfo|SetAttackType AttackType)
  (Variables|IncomingAttackInfo|SetDamageType Damage%20Type)
  (Variables|IncomingAttackInfo|SetCriticalHit CriticalHit))

(event Custom|EventPointDamage
  (params (DamagedActor :type Actor%20Object%20Reference) (Damage :type Float%20%28single-precision%29) (InstigatedBy :type Controller%20Object%20Reference) (HitLocation :type Vector) (FHitComponent :type Primitive%20Component%20Object%20Reference) (BoneName :type Name) (ShotFromDirection :type Vector) (DamageType :type Damage%20Type%20Object%20Reference) (DamageCauser :type Actor%20Object%20Reference))
  (bind _meleecomponent (Variables|Default|GetMeleeComponent))
  ;[1 1 1] Damage Triggers
  (CallFunction|StoreDamageInfo Damage HitLocation DamageCauser)
  (CallFunction|AIReport)
  (bind _damage (CallFunction|CanTakeDamage))
  (if _damage
    (CallFunction|PlayShakeIFPlayer)
    (bind (_success _ignorestack) (CallFunction|AIBlockChance))
    (if _success
      (Default|EventBlock _meleecomponent (Variables|IncomingAttackInfo|GetAttackType) :!label _label)
      (Default|SendBlock _meleecomponent)
      (else
        (bind _block_success (CallFunction|CanBlockAttack))
        (if _block_success
          (goto _label)
          (else
            (CallFunction|TakeDamage)
            (if (not _ignorestack)
              (Utilities|IncrementAutoBlock))))))))

(event Custom|EventRadialDamage
  (params (DamagedActor :type Actor%20Object%20Reference) (Damage :type Float%20%28single-precision%29) (DamageType :type Damage%20Type%20Object%20Reference) (Origin :type Vector) (HitInfo :type Hit%20Result%20Structure) (InstigatedBy :type Controller%20Object%20Reference) (DamageCauser :type Actor%20Object%20Reference))
  (bind _meleecomponent (Variables|Default|GetMeleeComponent))
  ;[1 1 1] Damage Triggers
  (CallFunction|StoreDamageInfo Damage Origin DamageCauser)
  (CallFunction|AIReport)
  (bind _damage (CallFunction|CanTakeDamage))
  (if _damage
    (CallFunction|PlayShakeIFPlayer)
    (bind (_success _ignorestack) (CallFunction|AIBlockChance))
    (if _success
      (Default|EventBlock _meleecomponent (Variables|IncomingAttackInfo|GetAttackType) :!label _label)
      (Default|SendBlock _meleecomponent)
      (else
        (bind _block_success (CallFunction|CanBlockAttack))
        (if _block_success
          (goto _label)
          (else
            (CallFunction|TakeDamage)
            (if (not _ignorestack)
              (Utilities|IncrementAutoBlock))))))))

(event EventBeginPlay
  ;[1 1 1] Setup
  (CallFunction|StoreComponents))

(fn CalculateHitAnim
  (bind _returnvalue (Components|GetOwner))
  (bind _returnvalue_2 (Components|GetOwner))
  (bind _impactpoint (Variables|IncomingAttackInfo|GetImpactPoint))
  (bind _attackingactor (Variables|IncomingAttackInfo|GetAttackingActor))
  (bind _returnvalue_3 (Transformation|GetActorLocation _returnvalue))
  (bind _returnvalue_4 (Transformation|GetActorRotation _returnvalue))
  (bind _returnvalue_5 (Transformation|GetActorRotation _attackingactor))
  (bind _returnvalue_6 (Math|Vector|GetForwardVector _returnvalue_4))
  (bind _returnvalue_7 (Math|Vector|GetForwardVector _returnvalue_5))
  (bind _returnvalue_8 (+ _returnvalue_3 _returnvalue_6))
  (bind _returnvalue_9 (+ _impactpoint _returnvalue_7))
  (bind _returnvalue_10 (- _returnvalue_3 _returnvalue_8))
  (bind _returnvalue_11 (- _impactpoint _returnvalue_9))
  (bind _returnvalue_12 (Math|Vector|Normalize _returnvalue_10))
  (bind _returnvalue_13 (Math|Vector|Normalize _returnvalue_11))
  (bind _returnvalue_14 (Math|Vector|DotProduct _returnvalue_13 _returnvalue_12))
  ;[1 1 1] Hit Back - Determine IF The Attack Is Coming From The Front Or Back
  (if (Math|Float|InRange(Float) _returnvalue_14 0.7 1.0)
    (LocalVariables|SetHitAnim (CallFunction|PassAnimation "NewEnumerator0"))
    (return (LocalVariables|GetHitAnim))
    (elif (Math|Float|InRange(Float) _returnvalue_14 -1.0 -0.7)
      ;[1 1 1] Hit Front - Detects If The Front Of The Enemy Is Hit From The Left OR Right
      (if (< (Math|Vector|DotProduct (Math|Transform|InverseTransformLocation (Transformation|GetActorTransform _returnvalue_2) (Variables|IncomingAttackInfo|GetImpactPoint)) (Transformation|GetActorForwardVector _returnvalue_2)) 0.0)
        (LocalVariables|SetHitAnim (CallFunction|PassAnimation "NewEnumerator0"))
        (else
          (LocalVariables|SetHitAnim (CallFunction|PassAnimation "NewEnumerator0"))))
      (return (LocalVariables|GetHitAnim))
      (else
        ;[1 1 1] Hit Left/Right - Determine if the Impact Point is on the Left Or Right Side
        (if (> (Math|Vector|DotProduct (Transformation|GetActorRightVector (Components|GetOwner)) (Math|Vector|Normalize (- (Transformation|GetActorLocation (Components|GetOwner)) (Transformation|GetActorLocation (Variables|IncomingAttackInfo|GetAttackingActor))))) 0.0)
          (LocalVariables|SetHitAnim (CallFunction|PassAnimation "NewEnumerator0"))
          (else
            (LocalVariables|SetHitAnim (CallFunction|PassAnimation "NewEnumerator0"))))
        (return (LocalVariables|GetHitAnim))))))

(fn DamageHealth
  (params (Damage :type Float%20%28double-precision%29) (DamageType :type E_DamageType%20Enum :default "NewEnumerator0"))
  (bind _equipmentcomponent (Variables|Default|GetEquipmentComponent))
  (bind _equipmentcomponent_2 (Variables|Default|GetEquipmentComponent))
  ;[1 1 1] Lowers Health
  (bind _output_get (Variables|/Game/Proto/Rework_All_Project/Blueprints/Components/EquipmentComponent.EquipmentComponent_C|SetHealth _equipmentcomponent_2 (select (<= (- (Variables|/Game/Proto/Rework_All_Project/Blueprints/Components/EquipmentComponent.EquipmentComponent_C|GetHealth (Variables|Default|GetEquipmentComponent)) Damage) 0.0) 0.0 (- (Variables|/Game/Proto/Rework_All_Project/Blueprints/Components/EquipmentComponent.EquipmentComponent_C|GetHealth (Variables|Default|GetEquipmentComponent)) Damage))))
  (Default|CallUpdateWidgetHealthDisplay _output_get (Variables|/Game/Proto/Rework_All_Project/Blueprints/Components/EquipmentComponent.EquipmentComponent_C|GetMaxHealth _equipmentcomponent_2))
  ;[1 1 1] Damage Popup
  (CallFunction|DamagePopup Damage DamageType)
  ;[1 1 1] IF Health Equals Or Less Than 0.9 = Death
  (Utilities|IsValid _equipmentcomponent
    (:Is%20Valid
      (if (<= (Variables|/Game/Proto/Rework_All_Project/Blueprints/Components/EquipmentComponent.EquipmentComponent_C|GetHealth _equipmentcomponent) 0.9)
        ;[1 1 1] Kill Target If Alive
        (bind _dead (Class|ICharacter|IsDead(Message) (Components|GetOwner)))
        (if _dead
          (return true)
          (else
            (Class|ICharacter|SendDeath(Message) (Components|GetOwner)))))
      (return (<= (Variables|/Game/Proto/Rework_All_Project/Blueprints/Components/EquipmentComponent.EquipmentComponent_C|GetHealth _equipmentcomponent) 0.9)))
    (:Is%20Not%20Valid
      (return false))))

(fn DamagePopup
  (params (Damage :type Float%20%28double-precision%29) (DamageType :type E_DamageType%20Enum :default "NewEnumerator0"))
  (bind _returnvalue (Components|GetOwner))
  (bind _attackingactor (Variables|IncomingAttackInfo|GetAttackingActor))
  (bind _returnvalue_2 (Actor|ActorHasTag _returnvalue "Player"))
  (bind _returnvalue_3 (select _returnvalue_2 _returnvalue _attackingactor))
  (bind _returnvalue_4 (Actor|GetComponentbyClass _returnvalue_3 "/Game/Proto/Rework_All_Project/Blueprints/Components/CombatTextComponent.CombatTextComponent_C"))
  (Utilities|IsValid _returnvalue_4
    (:Is%20Valid
      (Default|CombatTextPopup _returnvalue_4 (Math|Vector|SelectVector (Transformation|GetActorLocation (Components|GetOwner)) (Variables|IncomingAttackInfo|GetImpactPoint) (Variables|Default|GetDamage%20Over%20Time)) (Math|Float|Round Damage) (Utilities|Select :Index DamageType :Option%200 0 :Option%201 0 :Option%202 0 :Option%203 0 :Option%204 0 :Option%205 0 :Option%206 0 :Option%207 0 :Option%208 0 :Option%209 0) (Variables|IncomingAttackInfo|GetCriticalHit) (Variables|Default|GetDamage%20Over%20Time) (Actor|ActorHasTag (Components|GetOwner) "Player")))))

(fn SpawnEmitterPS
  (Effects|SpawnEmitteratLocation (Variables|IncomingAttackInfo|GetEnemyWeaponPS) (Variables|IncomingAttackInfo|GetImpactPoint)))

(fn StoreDamageInfo
  (params (DamageInc :type Float%20%28double-precision%29) (HitLocation :type Vector) (AttackingActor :type Actor%20Object%20Reference))
  (bind _meleecomponent (Variables|Default|GetMeleeComponent))
  (Utilities|FlowControl|Sequence
    (:then_0
      (Variables|IncomingAttackInfo|SetDamageIncoming DamageInc)
      (Variables|IncomingAttackInfo|SetAttackingActor AttackingActor)
      (Variables|IncomingAttackInfo|SetImpactPoint HitLocation))
    (:then_1
      (Utilities|IsValid _meleecomponent
        (:Is%20Valid
          (Variables|/Game/Proto/Rework_All_Project/Blueprints/Components/MeleeComponent.MeleeComponent_C|SetDamageInc _meleecomponent DamageInc)
          (Variables|/Game/Proto/Rework_All_Project/Blueprints/Components/MeleeComponent.MeleeComponent_C|SetAttackingActor _meleecomponent 0)
          (Variables|/Game/Proto/Rework_All_Project/Blueprints/Components/MeleeComponent.MeleeComponent_C|SetImpactPoint _meleecomponent HitLocation))))))

(fn CanTakeDamage
  (bind _dead (Class|ICharacter|IsDead(Message) (Components|GetOwner)))
  (if _dead
    (return false)
    (else
      (Utilities|IsValid 0
        (:Is%20Valid
          (if (or (CallFunction|IsPlayingMontage (Variables|Default|GetCharacterMesh) (CallFunction|PassAnimation "NewEnumerator0")) (CallFunction|IsPlayingMontage (Variables|Default|GetCharacterMesh) (CallFunction|PassAnimation "NewEnumerator0")))
            ;[1 1 1] If Frozen Take Damage Even if Mid Roll
            (if (Variables|Default|GetIsFrozen)
              _
              (else
                (return false))))
          (return true))
        (:Is%20Not%20Valid
          (CallFunction|TakeDamage))))))

(fn StoreComponents
  (bind _returnvalue (Components|GetOwner))
  (EventDispatchers|BindEventtoOnTakePointDamage _returnvalue (EventDispatchers|CreateEvent :!event Custom|EventPointDamage))
  (EventDispatchers|BindEventtoOnTakeRadialDamage _returnvalue (EventDispatchers|CreateEvent :!event Custom|EventRadialDamage))
  (Variables|Default|SetEquipmentComponent (Actor|GetComponentbyClass _returnvalue "/Game/Proto/Rework_All_Project/Blueprints/Components/EquipmentComponent.EquipmentComponent_C"))
  (Variables|Default|SetMeleeComponent (Actor|GetComponentbyClass _returnvalue "/Game/Proto/Rework_All_Project/Blueprints/Components/MeleeComponent.MeleeComponent_C"))
  (Variables|Default|SetInputBufferComp (Actor|GetComponentbyClass _returnvalue "/Game/Proto/Rework_All_Project/Blueprints/Components/InputBufferComponent.InputBufferComponent_C"))
  (Variables|Default|SetCombatStatusComp (Actor|GetComponentbyClass _returnvalue "/Game/Proto/Rework_All_Project/Blueprints/Components/CombatStatusComponent.CombatStatusComponent_C"))
  (bind _ascharacter (Utilities|Casting|CastToCharacter _returnvalue))
  (Variables|Components|SetCharacterRef _ascharacter)
  (Variables|Default|SetCharacterMesh (Variables|/Script/Engine.Character|GetMesh _ascharacter))
  (Variables|ElementalEffects|SetSkeletalMeshRef (Variables|/Script/Engine.SkinnedMeshComponent|GetSkeletalMesh (Variables|/Script/Engine.Character|GetMesh (Variables|Components|GetCharacterRef))))
  (Variables|Default|SetAnimationSet (Utilities|GetClass (Components|SkeletalMesh|GetAnimInstance (Variables|Default|GetCharacterMesh)))))

(fn AIBlockChance
  (bind _attacktype (Variables|IncomingAttackInfo|GetAttackType))
  (if (Variables|Default|GetPolymorphed)
    ;[1 1 1] Block Chance Conditions
    (return false true)
    (else
      ;;[1 1 1] If Not AI - No Random Block Chance
      (if (Variables|Default|GetEnemyAI)
        ;;[1 1 1] If Not Melee AI
        (if (Utilities|Enum|NotEqual(Enum) (Variables|/Game/Proto/Rework_All_Project/Blueprints/Components/CombatStatusComponent.CombatStatusComponent_C|GetCurrentAttackStyle (Variables|Default|GetCombatStatusComp)) "NewEnumerator0")
          (return false true)
          (else
            ;;[1 1 1] IF Attack Is Spell, Arrow Or Reflect
            (if (Math|Boolean|ORBoolean (Utilities|Enum|Equal(Enum) _attacktype "NewEnumerator15") (Utilities|Enum|Equal(Enum) _attacktype "NewEnumerator18") (Utilities|Enum|Equal(Enum) _attacktype "NewEnumerator16"))
              (return false true)
              (else
                ;;[1 1 1] IF Block On CD
                (bind _blockcd (Class|IAIController|PassBlockCD(Message) (AI|GetAIController (Components|GetOwner))))
                (if _blockcd
                  (return false true)
                  (else
                    ;;[1 1 1] Random Block Chance
                    (if (Math|Random|RandomBoolwithWeight (Variables|Default|GetAutoBlockChance))
                      ;;[1 1 1] Reset Block Chance - Block Success
                      (Variables|Default|SetAutoBlockChance 0.05)
                      (return true false)
                      (else
                        ;;[1 1 1] Failed Block - Increase Block Chance
                        (return false false)))))))))
        (else
          (return false true))))))

(fn UpdateCombatStatuses
  (bind _attacktype (Variables|IncomingAttackInfo|GetAttackType))
  ;[1 1 1] Only Reset Melee Attack IF Attack Not Barrier Reflect
  (if (not (or (Utilities|Enum|Equal(Enum) _attacktype "NewEnumerator16") (Utilities|Enum|Equal(Enum) _attacktype "NewEnumerator19")))
    (Default|ResetMeleeAttack (Variables|Default|GetMeleeComponent))
    (Class|IAIController|EndAttackTimer(Message) (AI|GetAIController (Components|GetOwner)))))

(fn IgnoreHitAnim
  (bind _charactermesh (Variables|Default|GetCharacterMesh))
  (bind _returnvalue (Components|SkeletalMesh|GetAnimInstance _charactermesh))
  (bind _movementmode (Class|ICharacter|PassMovementMode(Message) (Components|GetOwner)))
  (if (Utilities|Enum|Equal(Enum) _movementmode "MOVE_Flying")
    (return true)
    (else
      (Utilities|IsValid _returnvalue
        (:Is%20Valid
          (Animation|Montage|MontageStop _returnvalue 0.0 0))
        (:Is%20Not%20Valid
          _))
      (Default|ClearBuffer (Variables|Default|GetInputBufferComp) false)
      (return false))))

(fn AIReport)

(fn PlayShakeIFPlayer
  (bind _characterref (Variables|Components|GetCharacterRef))
  (Utilities|IsValid _characterref
    (:Is%20Valid
      (if (Actor|ActorHasTag _characterref "Player")
        (Camera|PlayWorldCameraShake 0 (Transformation|GetActorLocation _characterref) 0.0 1e+03 0.0)))))

(fn PlayHitSound
  (bind _attacktype (Variables|IncomingAttackInfo|GetAttackType))
  (if (Utilities|Enum|Equal(Enum) (Variables|IncomingAttackInfo|GetAttackType) "NewEnumerator17")
    (Audio|PlaySoundatLocation (.OutItem (Utilities|Array|Random (Utilities|Array|MakeArray "/Game/Proto/Rework_All_Project/SoundFX/Melee/SW_FistHit_01.SW_FistHit_01" "/Game/Proto/Rework_All_Project/SoundFX/Melee/SW_FistHit_02.SW_FistHit_02" "/Game/Proto/Rework_All_Project/SoundFX/Melee/SW_FistHit_03.SW_FistHit_03" "/Game/Proto/Rework_All_Project/SoundFX/Melee/SW_FistHit_04.SW_FistHit_04"))) (Variables|IncomingAttackInfo|GetImpactPoint) "0, 0, 0" 1.0 1.0 0.0 0 0 0 0)
    (elif (not (Math|Boolean|ORBoolean (Utilities|Enum|Equal(Enum) _attacktype "NewEnumerator15") (Utilities|Enum|Equal(Enum) _attacktype "NewEnumerator19") (Utilities|Enum|Equal(Enum) _attacktype "NewEnumerator18")))
      (Audio|PlaySoundatLocation (.OutItem (Utilities|Array|Random (Utilities|Array|MakeArray "/Game/Proto/Rework_All_Project/SoundFX/Melee/SW_MeleeHit_01.SW_MeleeHit_01" "/Game/Proto/Rework_All_Project/SoundFX/Melee/SW_MeleeHit_02.SW_MeleeHit_02" "/Game/Proto/Rework_All_Project/SoundFX/Melee/SW_MeleeHit_03.SW_MeleeHit_03" "/Game/Proto/Rework_All_Project/SoundFX/Melee/SW_MeleeHit_04.SW_MeleeHit_04"))) (Variables|IncomingAttackInfo|GetImpactPoint) "0, 0, 0" 1.0 1.0 0.0 0 0 0 0))))

(fn CanBlockAttack
  (bind _attacktype (Variables|IncomingAttackInfo|GetAttackType))
  (bind _combatstatuscomp (Variables|Default|GetCombatStatusComp))
  (bind _equippedmeleeweapon (Variables|/Game/Proto/Rework_All_Project/Blueprints/Components/CombatStatusComponent.CombatStatusComponent_C|GetEquippedMeleeWeapon _combatstatuscomp))
  (if (Variables|Default|GetPolymorphed)
    ;[1 1 1] Block Conditions
    (return false)
    (else
      ;;[1 1 1] Can't Block Sky/Eruption Spell
      (if (Utilities|Enum|Equal(Enum) (Variables|IncomingAttackInfo|GetAttackType) "NewEnumerator18")
        (return false)
        (else
          ;;[1 1 1] Is Block Up
          (if (Variables|/Game/Proto/Rework_All_Project/Blueprints/Components/MeleeComponent.MeleeComponent_C|GetBlockUp (Variables|Default|GetMeleeComponent))
            ;;[1 1 1] If Shield Equip Can Block Anything
            (if (or (Utilities|Enum|Equal(Enum) _equippedmeleeweapon "NewEnumerator6") (Utilities|Enum|Equal(Enum) _equippedmeleeweapon "NewEnumerator7"))
              (return true)
              (else
                ;;[1 1 1] Cant Block Spells or Arrows (Unless Shield Equip)
                (if (or (Utilities|Enum|Equal(Enum) _attacktype "NewEnumerator15") (Utilities|Enum|Equal(Enum) _attacktype "NewEnumerator16"))
                  (return false)
                  (else
                    (return true)))))
            (else
              (return false))))))))

(fn StatusPopup
  (params (DamageType :type E_DamageType%20Enum :default "NewEnumerator0") (StatusEnd :type Boolean))
  (bind _returnvalue (Components|GetOwner))
  (bind _attackingactor (Variables|IncomingAttackInfo|GetAttackingActor))
  (bind _returnvalue_2 (Actor|ActorHasTag _returnvalue "Player"))
  (bind _returnvalue_3 (select _returnvalue_2 _returnvalue _attackingactor))
  (bind _returnvalue_4 (Actor|GetComponentbyClass _returnvalue_3 "/Game/Proto/Rework_All_Project/Blueprints/Components/CombatTextComponent.CombatTextComponent_C"))
  (Utilities|IsValid _returnvalue_4
    (:Is%20Valid
      (Default|CreateStatusCombatText _returnvalue_4 (Variables|IncomingAttackInfo|GetImpactPoint) (Utilities|Select :Index DamageType :NewEnumerator0 0 :NewEnumerator1 0 :NewEnumerator4 0 :NewEnumerator6 0 :NewEnumerator9 0) StatusEnd))))