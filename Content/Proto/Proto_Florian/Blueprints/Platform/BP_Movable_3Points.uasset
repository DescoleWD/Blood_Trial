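; Prototype moving platform that endlessly shuttles its static mesh between three relative locations held in variables.
; From BeginPlay, chained latent MoveComponentTo nodes send the mesh to point 3, back through point 2 to point 1, then to point 2 again before looping.
; It pauses briefly at the two end points and passes through the middle one without a delay.
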(event EventBeginPlay
  (Components|MoveComponentTo (Variables|Default|GetStaticMesh) (Variables|Default|GetPlatLocation3) "0, 0, 0" false false 2.0 false :!label _label)
  (Utilities|FlowControl|Delay 1.0)
  (Components|MoveComponentTo (Variables|Default|GetStaticMesh) (Variables|Default|GetPlatLocation2) "0, 0,0.000000" false false 2.0 false)
  (Components|MoveComponentTo (Variables|Default|GetStaticMesh) (Variables|Default|GetPlatLocation1) "0, 0, 0" false false 2.0 false)
  (Utilities|FlowControl|Delay 1.0)
  (Components|MoveComponentTo (Variables|Default|GetStaticMesh) (Variables|Default|GetPlatLocation2) "0, 0, 0" false false 2.0 false)
  (goto _label))

(fn ConstructionScript)