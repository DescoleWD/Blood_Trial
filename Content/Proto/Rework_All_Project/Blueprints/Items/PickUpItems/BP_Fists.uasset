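; BP_Fists is the unarmed melee weapon, snapping two fist components to the character's hand sockets.
; StartAttack runs a fast looping timer that sphere-traces Pawns at both fists, handled here rather than in WeaponCollision because there are two traces.
; Each actor hit once per attack gets randomized EquipmentComponent-based point damage, plus effect info if it has TakingDamage; StopAttack resets both.
; A rebuilt HitResult works around wrong UE5 impact locations.
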(event Custom|AttachToPlayer
  (params (CharacterRef :type Character%20Object%20Reference))
  (bind _mesh (Variables|/Script/Engine.Character|GetMesh CharacterRef))
  ;[1 1 1] Attach Fists To Player
  (bind _output_get (Variables|Default|SetCharacterRef CharacterRef))
  (Variables|Default|SetEquipmentComponent (Actor|GetComponentbyClass _output_get "/Game/Proto/Rework_All_Project/Blueprints/Components/EquipmentComponent.EquipmentComponent_C"))
  (Transformation|AttachComponentToComponent (Variables|Default|GetFist1Ref) _mesh "hand_L" "SnapToTarget" "SnapToTarget" "KeepRelative" true)
  (Transformation|AttachComponentToComponent (Variables|Default|GetFist2Ref) _mesh "hand_R" "SnapToTarget" "SnapToTarget" "KeepRelative" true))

(event Custom|Trace
  ;[1 1 1] Attack AND Generate LineTrace For Hit - We do this in the Fist and not Weapon Collision because the Fists have 2 traces
  (CallFunction|FistLineTraceHit (Variables|Default|GetFist1Ref))
  (CallFunction|FistLineTraceHit (Variables|Default|GetFist2Ref)))

(event EventStartAttack
  ;[1 1 1] Attack AND Generate LineTrace For Hit - We do this in the Fist and not Weapon Collision because the Fists have 2 traces
  (bind _returnvalue (Utilities|Time|SetTimerbyEvent (delegate Custom|Trace) 0.01 true)))

(event EventStopAttack
  ;[1 1 1] Attack AND Generate LineTrace For Hit - We do this in the Fist and not Weapon Collision because the Fists have 2 traces
  (Utilities|Time|ClearandInvalidateTimerbyHandle (stale EventStartAttack _returnvalue))
  (Utilities|Array|Clear (Variables|Default|GetAlreadyDamagedEnemy)))

(fn ConstructionScript)

(fn FistLineTraceHit
  (params (Fist :type Scene%20Component%20Object%20Reference))
  (bind _weaponcollision (Variables|Default|GetWeaponCollision))
  (bind (_outhit _returnvalue) (Collision|SphereTraceForObjects (Transformation|GetWorldLocation Fist) (Transformation|GetWorldLocation Fist) 4e+01 (Utilities|Array|MakeArray "ObjectTypeQuery3") false (Utilities|Array|MakeArray (Variables|Default|GetCharacterRef)) "None"))
  (if _returnvalue
    (if (not (Utilities|Array|ContainsItem (Variables|Default|GetAlreadyDamagedEnemy) (.HitActor (Collision|BreakHitResult _outhit))))
      (Utilities|Array|Add (Variables|Default|GetAlreadyDamagedEnemy) (.HitActor (Collision|BreakHitResult _outhit)))
      (Utilities|IsValid (Actor|GetComponentbyClass (.HitActor (Collision|BreakHitResult _outhit)) "/Game/Proto/Rework_All_Project/Blueprints/Components/TakingDamage.TakingDamage_C")
        (:Is%20Valid
          (Default|PassDamageInfo (Actor|GetComponentbyClass (.HitActor (Collision|BreakHitResult _outhit)) "/Game/Proto/Rework_All_Project/Blueprints/Components/TakingDamage.TakingDamage_C") (Variables|Default|GetWeaponPS _weaponcollision) "NewEnumerator17" "NewEnumerator0" (Variables|Default|GetCriticalHit _weaponcollision))
          ;[0.3211 1 0.9359] Bug in UE5 means that the default Hit Info doesn't give the correct Impact Location. Tweaked this to work for UE5, UE4 can plug Normal Hit Info in
          (Game|Damage|ApplyPointDamage (.HitActor (Collision|BreakHitResult _outhit)) (CallFunction|RandomMinMaxValue (Variables|/Game/Proto/Rework_All_Project/Blueprints/Components/EquipmentComponent.EquipmentComponent_C|GetMaxFistDmg (Variables|Default|GetEquipmentComponent))) (.Location (Collision|BreakHitResult _outhit)) (Collision|MakeHitResult false false 0.0 0.0 "0, 0, 0" (.Location (Collision|BreakHitResult _outhit)) "0,0,1" "0,0,1" 0 0) 0 (Variables|Default|GetCharacterRef)))))))