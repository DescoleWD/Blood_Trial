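; BP_Rope is a prototype rope that works as a one-shot lever to move a linked portal.
; Its collider detects the main character, stores the reference and registers the rope through NearTheLever.
; When LeverActive fires during overlap, it clears the character's NearRope, waits briefly, calls Movement on the referenced BP_Portail and destroys itself.
; Debug prints trace these steps, and a Player tag check is left unconnected.
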(event OnComponentBeginOverlap(LeverCollider)
  (params (OverlappedComponent :type Primitive%20Component%20Object%20Reference) (OtherActor :type Actor%20Object%20Reference) (OtherComp :type Primitive%20Component%20Object%20Reference) (OtherBodyIndex :type Integer) (bFromSweep :type Boolean) (SweepResult :type Hit%20Result%20Structure%20%28by%20ref%29))
  (bind _asbp_main_character (Utilities|Casting|CastToBP_MainCharacter OtherActor))
  (Variables|Default|SetAs%20BP%20Main%20Character _asbp_main_character)
  (Variables|Default|SetisCollision true)
  (Default|NeartheLever _asbp_main_character self)
  (Development|PrintString "Call Enter"))

(event OnComponentEndOverlap(LeverCollider)
  (params (OverlappedComponent :type Primitive%20Component%20Object%20Reference) (OtherActor :type Actor%20Object%20Reference) (OtherComp :type Primitive%20Component%20Object%20Reference) (OtherBodyIndex :type Integer))
  (Utilities|Casting|CastToBP_MainCharacter OtherActor)
  (Variables|Default|SetisCollision false)
  (if (Variables|Default|GetisDestroy)
    (Variables|/Game/Proto/Main/Blueprint/BP_MainCharacter.BP_MainCharacter_C|SetNearRope (Variables|Default|GetAs%20BP%20Main%20Character) 0)
    (Development|PrintString "Call Out")))

(event Custom|LeverActive
  (if (Variables|Default|GetisCollision)
    (Development|PrintString "Call Active")
    (Variables|Default|SetisDestroy true)
    (Variables|/Game/Proto/Main/Blueprint/BP_MainCharacter.BP_MainCharacter_C|SetNearRope (Variables|Default|GetAs%20BP%20Main%20Character) 0)
    (Utilities|FlowControl|Delay 0.2)
    (bind _asbp_portail (Utilities|Casting|CastToBP_Portail (Variables|Default|GetPortail_REF)))
    (Default|Movement _asbp_portail)
    (Actor|DestroyActor)))

(fn ConstructionScript)