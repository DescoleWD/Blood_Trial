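; ProjPapillon is a prototype enemy projectile that damages the player and plays a looping 2D sound from spawn.
; On sphere overlap, a sphere trace for pawns ignoring "IA"-tagged actors applies SpellDamage if it hits the player character; any hit destroys the projectile.
; LockOn enables ProjectileMovement homing using FindHomingTarget's scan of "Player"-tagged BP_MainBase actors by horizontal distance, but its repeating half-second caller is disconnected.
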(event OnComponentBeginOverlap(Sphere)
  (params (OverlappedComponent :type Primitive%20Component%20Object%20Reference) (OtherActor :type Actor%20Object%20Reference) (OtherComp :type Primitive%20Component%20Object%20Reference) (OtherBodyIndex :type Integer) (bFromSweep :type Boolean) (SweepResult :type Hit%20Result%20Structure%20%28by%20ref%29))
  (bind _sphere (Variables|Default|GetSphere))
  (bind _returnvalue (Transformation|GetWorldLocation _sphere))
  (Development|PrintString (Utilities|GetDisplayName OtherActor))
  (bind _outactors (Actor|GetAllActorsOfClasswithTag "/Script/Engine.Actor" "IA"))
  (bind (_outhit _returnvalue_2) (Collision|SphereTraceForObjects _returnvalue _returnvalue 1e+02 (Utilities|Array|MakeArray "ObjectTypeQuery3") false _outactors "None"))
  (if _returnvalue_2
    (Variables|Default|SetHit%20Actor (.HitActor (Collision|BreakHitResult _outhit)))
    (Variables|Default|SetHit%20Component (.HitComponent (Collision|BreakHitResult _outhit)))
    (if (== (Game|GetPlayerCharacter 0) (Variables|Default|GetHit%20Actor))
      (Game|Damage|ApplyDamage (Variables|Default|GetHit%20Actor) (Variables|Default|GetSpellDamage) 0 self)
      (Actor|DestroyActor)
      (else
        (Actor|DestroyActor)))
    (else
      (Variables|Default|SetHit%20Actor 0)
      (Variables|Default|SetHit%20Component 0))))

(event Custom|LockOn
  (bind _projectilemovement (Variables|Default|GetProjectileMovement))
  (bind _arrayelement (CallFunction|FindHomingTarget))
  (Variables|/Script/Engine.ProjectileMovementComponent|SetHomingTargetComponent _projectilemovement _arrayelement)
  (Variables|/Script/Engine.ProjectileMovementComponent|SetbIsHomingProjectile _projectilemovement true))

(event EventBeginPlay
  (Audio|PlaySound2D "/Game/Proto/Main/SFX/SFXHADES/Enemies/Enemies_Projectile/EnemyProjectileLoop.EnemyProjectileLoop" 0.3 1.0 0.0 0 0))

(event Collision|EventActorBeginOverlap
  (params (OtherActor :type Actor%20Object%20Reference)))

(fn ConstructionScript)

(fn FindHomingTarget
  (bind _returnvalue (Transformation|GetActorLocation))
  (bind _outactors (Actor|GetAllActorsOfClasswithTag "/Game/Proto/Main/Blueprint/BP_MainBase.BP_MainBase_C" "Player"))
  (for _array_element _outactors
    (if (< (Math|Vector|VectorLength (Math|Vector|MakeVector (.x (- (Math|Vector|MakeVector (.x (Transformation|GetActorLocation _array_element)) (.y (Transformation|GetActorLocation _array_element)) 0.0) (Math|Vector|MakeVector (.x _returnvalue) (.y _returnvalue) 0.0))) (.y (- (Math|Vector|MakeVector (.x (Transformation|GetActorLocation _array_element)) (.y (Transformation|GetActorLocation _array_element)) 0.0) (Math|Vector|MakeVector (.x _returnvalue) (.y _returnvalue) 0.0))) 0.0)) (Variables|Default|GetClosestDistance))
      (Variables|Default|SetClosestDistance (Math|Vector|VectorLength (Math|Vector|MakeVector (.x (- (Math|Vector|MakeVector (.x (Transformation|GetActorLocation _array_element)) (.y (Transformation|GetActorLocation _array_element)) 0.0) (Math|Vector|MakeVector (.x _returnvalue) (.y _returnvalue) 0.0))) (.y (- (Math|Vector|MakeVector (.x (Transformation|GetActorLocation _array_element)) (.y (Transformation|GetActorLocation _array_element)) 0.0) (Math|Vector|MakeVector (.x _returnvalue) (.y _returnvalue) 0.0))) 0.0)))
      (Variables|Default|SetArray%20Element _array_element)))
  (return (Actor|GetComponentbyClass (Variables|Default|GetArray%20Element) "/Script/Engine.SceneComponent")))