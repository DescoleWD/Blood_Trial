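; BP_PlayerHUD is the player's HUD, creating the WB_HUD widget and drawing a lock-on marker.
; NewSpawn stores the character, adds the widget and binds events from its ranged, melee and targeting components.
; Ranged executions and melee assassinations hide the widget until they end.
; Targeting updates cache the locked actor, whose projected screen position DrawHUD uses each frame to draw a small target texture.
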(event Custom|NewSpawn
  (params (CharacterRef :type Character%20Object%20Reference))
  ;[1 1 1] Create HUD WG, Create References To Each Element + Character
  (Variables|Default|SetCharacterRef CharacterRef)
  ;;[1 1 1] Create HUD - Add To Viewport
  (bind _returnvalue (UserInterface|CreateWidget "/Game/FlexibleCombatSystem/Widgets/HUD/WB_HUD.WB_HUD_C"))
  (bind _output_get (Variables|Default|SetWG_HUD _returnvalue))
  (UserInterface|Viewport|AddtoViewport _output_get 0)
  (CallFunction|BindEvents))

(event Custom|EventHideHUD
  ;[1 1 1] Show/Hide HUD
  (Widget|SetVisibility (Variables|Default|GetWG_HUD) "Hidden"))

(event Custom|EventShowHUD
  ;[1 1 1] Show/Hide HUD
  (Widget|SetVisibility (Variables|Default|GetWG_HUD) "Visible"))

(event Custom|BindEvents
  (bind _characterref (Variables|Default|GetCharacterRef))
  ;[1 1 1] Bind Event Dispatchers
  ;;[1 1 1] Ranged Events
  (EventDispatchers|BindEventtoExecuteOccuring (Actor|GetComponentbyClass _characterref "/Game/FlexibleCombatSystem/Blueprints/Components/RangedComponent.RangedComponent_C") (delegate Custom|RangedAssassinationUpdate))
  ;;[1 1 1] Targeting System Events
  (EventDispatchers|BindEventtoUpdateTargetLocked (Actor|GetComponentbyClass _characterref "/Game/FlexibleCombatSystem/Blueprints/Components/TargetingComponent.TargetingComponent_C") (delegate Custom|UpdateTargetLocked))
  ;;[1 1 1] Mele Component
  (EventDispatchers|BindEventtoAssassinationOccuring (Actor|GetComponentbyClass _characterref "/Game/FlexibleCombatSystem/Blueprints/Components/MeleeComponent.MeleeComponent_C") (delegate Custom|MeleeAssassinationUpdate)))

(event Custom|RangedAssassinationUpdate
  (params (ExecuteOccuring :type Boolean))
  ;[1 1 1] Bind Event Dispatchers
  ;;[1 1 1] Ranged Events
  (if ExecuteOccuring
    (CallFunction|EventHideHUD)
    (else
      (CallFunction|EventShowHUD))))

(event Custom|UpdateTargetLocked
  (params (TargetLocked :type Boolean))
  ;[1 1 1] Bind Event Dispatchers
  ;;[1 1 1] Targeting System Events
  (Variables|Default|SetLockedOnTarget (Variables|/Game/FlexibleCombatSystem/Blueprints/Components/TargetingComponent.TargetingComponent_C|GetLockedOnTarget (Actor|GetComponentbyClass (Variables|Default|GetCharacterRef) "/Game/FlexibleCombatSystem/Blueprints/Components/TargetingComponent.TargetingComponent_C")))
  (bind _output_get (Variables|Default|SetTargetLocked TargetLocked))
  (if _output_get
    (Variables|Default|SetTargetScale 8.0)
    (else
      (Variables|Default|SetTargetScale 0.0))))

(event Custom|MeleeAssassinationUpdate
  (params (AssassinationOccuring :type Boolean))
  ;[1 1 1] Bind Event Dispatchers
  ;;[1 1 1] Mele Component
  (if AssassinationOccuring
    (CallFunction|EventHideHUD)
    (else
      (CallFunction|EventShowHUD))))

(event EventDrawHUD
  (params (SizeX :type Integer) (SizeY :type Integer))
  (bind _returnvalue (Game|GetPlayerController 0))
  (bind _targetscale (Variables|Default|GetTargetScale))
  (bind _lockedontarget (Variables|Default|GetLockedOnTarget))
  (bind _returnvalue_2 (Transformation|GetActorLocation _lockedontarget))
  (bind _screenlocation (Class|PlayerController|ProjectWorldLocationtoScreen _returnvalue _returnvalue_2 false))
  ;[1 1 1] Draw HUD Is Constantly Firing like a tick. When the taget is locked we are drawing a texture (a small circle) onto the screen to represent the locked on target
  (Utilities|IsValid (Variables|Default|GetCharacterRef)
    (:Is%20Valid
      (if (Variables|Default|GetTargetLocked)
        (Canvas|DrawTexture "/Game/FlexibleCombatSystem/Widgets/Textures/General/T_target.T_target" (- (.x _screenlocation) 7.0) (- (.y _screenlocation) 12.0) _targetscale _targetscale 0.0 0.0 1.0 1.0 "(R=1.000000,G=1.000000,B=1.000000,A=1.000000)" "BLEND_Translucent" 2.0)))))

(fn ConstructionScript)