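; BP_Fruit is a prototype fig pickup that triggers fig tree regeneration on the player base class, BP_MainBase.
; From BeginPlay, the Fig component bobs endlessly through two looping, eased MoveComponentTo calls.
; Box overlap checks FigThere, calls RegenFigueTree, then destroys the actor after a short delay, clearing the flag only afterwards.
; An older direct, clamped life-increase path remains disconnected.
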(event OnComponentBeginOverlap(Box)
  (params (OverlappedComponent :type Primitive%20Component%20Object%20Reference) (OtherActor :type Actor%20Object%20Reference) (OtherComp :type Primitive%20Component%20Object%20Reference) (OtherBodyIndex :type Integer) (bFromSweep :type Boolean) (SweepResult :type Hit%20Result%20Structure%20%28by%20ref%29))
  (if (Variables|Default|GetFigThere?)
    (bind _asbp_main_base (Utilities|Casting|CastToBP_MainBase OtherActor))
    (Default|RegenFigueTree _asbp_main_base)
    (Utilities|FlowControl|Delay 0.2)
    (Actor|DestroyActor)
    (Variables|Default|SetFigThere? false)))

(event EventBeginPlay
  (Components|MoveComponentTo (Variables|Default|GetFig) "0.000000,0.000000,75.000000" "0, 0, 0" true true 1.0 false :!label _label)
  (Components|MoveComponentTo (Variables|Default|GetFig) "0,0.000000,25.000000" "0, 0, 0" true true 1.0 false)
  (goto _label))

(fn ConstructionScript)