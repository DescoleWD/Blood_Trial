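; Prototype enemy character that takes damage with knockback, a hit reaction and a health bar widget, and is destroyed when HP runs out.
; AnyDamage launches it backward and upward, reveals the cached bar, updates HP and plays a head-hit montage while HP remains.
; The CanBeDamaged flag around the montage resets as soon as playback starts.
; InterfaceMelee delegates attacks to ACMeleeEnemy; a player Regen call is left unwired.
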(event Game|Damage|EventAnyDamage
  (params (Damage :type Float%20%28single-precision%29) (DamageType :type Damage%20Type%20Object%20Reference) (InstigatedBy :type Controller%20Object%20Reference) (DamageCauser :type Actor%20Object%20Reference))
  (CallFunction|KnockBack)
  (Rendering|SetVisibility (Variables|Default|GetHP_Bar) true false)
  (bind _output_get (Variables|Default|SetCurrent_HP (- (Variables|Default|GetCurrent_HP) Damage)))
  (bind _output_get_2 (Variables|/Game/Proto/Proto_Guillaume/Blueprints/Enemy/HP_Bar.HP_Bar_C|SetUI_HP (Variables|Default|GetAs%20HP%20Bar) _output_get))
  (Progress|SetPercent (Variables|/Game/Proto/Proto_Guillaume/Blueprints/Enemy/HP_Bar.HP_Bar_C|GetProgressBar_33 (stale EventBeginPlay _output_get)) (Math|Float|SafeDivide _output_get_2 (Variables|Default|GetMax_HP)))
  (Math|Float|CompareFloat (Variables|Default|GetCurrent_HP) 0.0
    (:>
      (if (Variables|Default|GetbCanBeDamaged)
        (Variables|Default|SetbCanBeDamaged false)
        (Animation|Montage|PlayMontage (Variables|Character|GetMesh) "/Game/Proto/Proto_Guillaume/Blueprints/Anim_Mixamo/30FPS/MediumHitToHead_UE_Montage.MediumHitToHead_UE_Montage"
          (:then
            _)
          (:OnNotifyBegin
            _))
        (Variables|Default|SetbCanBeDamaged true)))
    (:==
      (Utilities|FlowControl|Sequence :!label _label
        (:then_1
          (Actor|DestroyActor))))
    (:<
      (goto _label))))

(event EventBeginPlay
  (bind _ashp_bar (Utilities|Casting|CastToHP_Bar (UserInterface|GetUserWidgetObject (Variables|Default|GetHP_Bar))))
  (bind _output_get (Variables|Default|SetAs%20HP%20Bar _ashp_bar)))

(event EventInterfaceMelee
  (Default|AttaqueEnemyMelee (Variables|Default|GetAC_Melee_Enemy)))

(fn ConstructionScript
  (|CallParentFunction))

(fn UpdateHealthBar
  (bind _ashp_bar (Utilities|Casting|CastToHP_Bar (UserInterface|GetUserWidgetObject (Variables|Default|GetHP_Bar))))
  (Variables|/Game/Proto/Proto_Guillaume/Blueprints/Enemy/HP_Bar.HP_Bar_C|SetUI_HP _ashp_bar (Variables|Default|GetCurrent_HP))
  (return))

(fn KnockBack
  (bind _returnvalue (Transformation|GetActorRotation))
  (bind _returnvalue_2 (Math|Vector|GetForwardVector _returnvalue))
  (bind _returnvalue_3 (* _returnvalue_2 -1e+02))
  (bind (_x _y _z) (Math|Vector|BreakVector _returnvalue_3))
  (Character|LaunchCharacter (Math|Vector|MakeVector _x _y (+ _z 5e+01)) false false))