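; Actor component for lootable items, containers and slain enemies that shows an outline and pickup tag when the player overlaps the owner.
; It pulls name, rarity, quantity and meshes from the owner, then uses custom depth stencil for the outline and a looping timer to track the HUD tag.
; Overlap hides other tags unless the inventory status check diverts it to the controller; leaving restores another overlapped tag and its loot widget.
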(event Custom|SendActorLooted
  ;[1 1 1] Display Outline & Tag
  (Variables|ObjectLoot|SetActorLooted true)
  (ActorTag|RemoveActorTag))

(event Custom|EventOverlap
  (params (OverlappedActor :type Actor%20Object%20Reference) (OtherActor :type Actor%20Object%20Reference))
  ;[1 1 1] Display Outline & Tag
  (Utilities|IsValid OtherActor
    (:Is%20Valid
      (if (Actor|ActorHasTag OtherActor "Player")
        (bind _lootready (CallFunction|AICheck))
        (if _lootready
          (bind _inventoryopen (Class|IPlayerController|InventoryStatus(Message) (Game|GetPlayerController 0)))
          (if _inventoryopen
            (Class|IPlayerController|PassOutlineComponent(Message) (Game|GetPlayerController 0) self)
            (Variables|Default|SetOverlapped true)
            (else
              (CallFunction|RemoveOtherTags OtherActor)
              (Utilities|DataUpdatedCheck
                (:Output
                  (ActorTag|ShowActorTag)
                  (Variables|Default|SetOverlapped true))))))))))

(event Custom|EventEndOverlap
  (params (OverlappedActor :type Actor%20Object%20Reference) (OtherActor :type Actor%20Object%20Reference))
  ;[1 1 1] Display Outline & Tag
  (if (Actor|ActorHasTag OtherActor "Player")
    (ActorTag|RemoveActorTag)
    (Variables|Default|SetOverlapped false)
    (CallFunction|ShowOtherTags OtherActor)))

(event EventBeginPlay
  (bind _returnvalue (Components|GetOwner))
  ;[1 1 1] Display Outline & Tag
  (Collision|BindEventtoOnActorBeginOverlap _returnvalue (delegate Custom|EventOverlap))
  (Collision|BindEventtoOnActorEndOverlap _returnvalue (delegate Custom|EventEndOverlap))
  (Utilities|FlowControl|Delay 0.01) ; Time for Items Placed In Level To Update Data
  (ActorTag|SetupOutlineVariables))

(fn SetTagPosition
  (bind _returnvalue (Game|GetPlayerController 0))
  (bind _returnvalue_2 (Components|GetOwner))
  (bind _mesh (ActorTag|DetermineMesh))
  (bind _ischaracter (Variables|Default|GetIsCharacter))
  (bind _returnvalue_3 (Transformation|GetWorldLocation _mesh))
  (bind _returnvalue_4 (Transformation|GetActorLocation _returnvalue_2))
  (bind _returnvalue_5 (select _ischaracter _returnvalue_4 _returnvalue_3))
  (bind _screenposition (Class|WidgetLayoutLibrary|ProjectWorldLocationtoWidgetPosition _returnvalue _returnvalue_5 false))
  (Utilities|IsValid (Variables|AnyLoot|GetTagCanvas)
    (:Is%20Valid
      (Class|CanvasPanelSlot|SetPosition (Variables|AnyLoot|GetTagCanvas) (Math|Vector2D|MakeVector2D (+ (.x _screenposition) 1e+01) (+ (.y _screenposition) 1e+01))))))

(fn SetupOutlineVariables
  ;[1 1 1] Set Variables For Item/Container/Loot
  (bind (_actor_name _actor_rarity _actor_tag_type _quantity _mesh_1 _mesh_2 _skeletal_mesh) (Class|IOutlineInterface|RetrieveOutlineInfo(Message) (Components|GetOwner)))
  (Variables|LootInfo|SetLoot%20Name _actor_name)
  (Variables|LootInfo|SetRarity%20Of%20Loot%20%28Colour%29 _actor_rarity)
  (Variables|Default|SetActor%20Tag%20Type _actor_tag_type)
  (Variables|Default|SetQuantity _quantity)
  (Variables|LootInfo|SetItemMesh _mesh_1)
  (Variables|Default|SetItem%20Mesh%202 _mesh_2)
  (Variables|LootInfo|SetItemSkeletalMesh _skeletal_mesh)
  (Variables|Default|SetDataUpdated true)
  ;[1 1 1] If Character We Want Tag to Show On Actor Not Mesh
  (Utilities|Casting|CastToCharacter (Components|GetOwner))
  (Variables|Default|SetIsCharacter true))

(fn DetermineMesh
  (bind _itemmesh (Variables|LootInfo|GetItemMesh))
  (Utilities|IsValid (Variables|Default|GetItem%20Mesh%202)
    (:Is%20Valid
      (return (Variables|LootInfo|GetItemMesh) (Variables|Default|GetItem%20Mesh%202)))
    (:Is%20Not%20Valid
      (Utilities|IsValid _itemmesh
        (:Is%20Valid
          (if (Rendering|IsVisible _itemmesh)
            (return (Variables|LootInfo|GetItemMesh) 0)
            (else
              _)))
        (:Is%20Not%20Valid
          _))
      (return (Variables|LootInfo|GetItemSkeletalMesh) 0))))

(fn ShowActorTag
  (bind _returnvalue (Components|GetOwner))
  (bind _mesh (ActorTag|DetermineMesh))
  (bind _returnvalue_2 (Game|GetPlayerController 0))
  (bind _mesh_2 (ActorTag|DetermineMesh))
  (bind _returnvalue_3 (Transformation|GetActorLocation _returnvalue))
  (bind _screenposition (Class|WidgetLayoutLibrary|ProjectWorldLocationtoWidgetPosition _returnvalue_2 _returnvalue_3 false))
  (if (not (Variables|ObjectLoot|GetActorLooted))
    (if (not (Variables|Default|GetActorTagVisible))
      (Class|IPlayerController|PassOutlineComponent(Message) (Game|GetPlayerController 0) self)
      (Variables|Default|SetActorTagVisible true)
      (Utilities|IsValid _mesh
        (:Is%20Valid
          (Rendering|SetRenderCustomDepth _mesh true)
          (Rendering|SetCustomDepthStencilValue _mesh 2))
        (:Is%20Not%20Valid
          _))
      (Utilities|IsValid _mesh_2
        (:Is%20Valid
          (Rendering|SetRenderCustomDepth _mesh_2 true)
          (Rendering|SetCustomDepthStencilValue _mesh_2 2))
        (:Is%20Not%20Valid
          _))
      ;[1 1 1] Create Actor Tag
      (bind _returnvalue_4 (UserInterface|CreateWidget "/Game/FlexibleCombatSystem/Widgets/Looting/WB_ActorPickupTag.WB_ActorPickupTag_C" 0 (Variables|LootInfo|GetLoot%20Name) (Variables|LootInfo|GetRarity%20Of%20Loot%20%28Colour%29) (Variables|Default|GetQuantity) (Variables|Default|GetActor%20Tag%20Type)))
      (bind _output_get (Variables|AnyLoot|SetActorPickupTag _returnvalue_4))
      (bind _hudref (Class|IPlayerController|PassHUDWB(Message) (Game|GetPlayerController 0)))
      (bind _returnvalue_5 (Class|CanvasPanel|AddChildtoCanvas (Variables|/Game/FlexibleCombatSystem/Widgets/HUD/WB_HUD.WB_HUD_C|GetHUD_Screen _hudref) _output_get))
      (bind _output_get_2 (Variables|AnyLoot|SetTagCanvas _returnvalue_5))
      (Utilities|IsValid (.Mesh (ActorTag|DetermineMesh))
        (:Is%20Valid
          (Class|CanvasPanelSlot|SetPosition _output_get_2 (Math|Vector2D|MakeVector2D (+ (.x _screenposition) 1e+01) (+ (.y _screenposition) 1e+01)))
          ;[1 1 1] Create Tick To Update Tag Location
          (bind _returnvalue_6 (Utilities|Time|SetTimerbyEvent (EventDispatchers|CreateEvent :!event SetTagPosition) 0.01 true))
          (Variables|AnyLoot|SetSetTagLocationTick _returnvalue_6))))))

(fn RemoveActorTag
  (bind _mesh_2 (ActorTag|DetermineMesh))
  (bind _mesh (ActorTag|DetermineMesh))
  (bind _actorpickuptag (Variables|AnyLoot|GetActorPickupTag))
  (if (Variables|Default|GetActorTagVisible)
    (Variables|Default|SetActorTagVisible false)
    (Utilities|IsValid _mesh
      (:Is%20Valid
        (Rendering|SetRenderCustomDepth _mesh false))
      (:Is%20Not%20Valid
        _))
    (Utilities|IsValid _mesh_2
      (:Is%20Valid
        (Rendering|SetRenderCustomDepth _mesh_2 false))
      (:Is%20Not%20Valid
        _))
    (Utilities|IsValid _actorpickuptag
      (:Is%20Valid
        (Widget|RemovefromParent _actorpickuptag))
      (:Is%20Not%20Valid
        _))
    (Utilities|Time|ClearandInvalidateTimerbyHandle (Variables|AnyLoot|GetSetTagLocationTick))))

(fn ToggleActorTag
  (if (Variables|Default|GetOverlapped)
    (if (Variables|ObjectLoot|GetActorLooted)
      (ActorTag|RemoveActorTag)
      (elif (Variables|Default|GetActorTagVisible)
        (ActorTag|RemoveActorTag)
        (else
          (ActorTag|ShowActorTag))))))

(fn AICheck
  (bind _returnvalue (Components|GetOwner))
  ;[1 1 1] Makes Sure IF the Loot is from an enemy, the enemy is slain
  (if (Actor|ActorHasTag _returnvalue "EnemyAI")
    (bind _dead (Class|ICharacter|IsDead(Message) _returnvalue))
    (return _dead)
    (else
      (return true))))

(fn RemoveOtherTags
  (params (Actor :type Actor%20Object%20Reference))
  ;[1 1 1] Remove Tag For All Other Actors
  (bind _ascharacter (Utilities|Casting|CastToCharacter Actor))
  (bind _array_element (Utilities|Array|ForEachLoopwithBreak (Collision|GetOverlappingActors (Variables|/Script/Engine.Character|GetCapsuleComponent _ascharacter) "/Script/Engine.Actor" :!class /Script/Engine.PrimitiveComponent))
    (:LoopBody
      (Utilities|IsValid (Actor|GetComponentbyClass _array_element "OutlineComponent_C")
        (:Is%20Valid
          (if (!= (Actor|GetComponentbyClass _array_element "OutlineComponent_C") self)
            (ActorTag|RemoveActorTag (Actor|GetComponentbyClass _array_element "OutlineComponent_C"))))))))

(fn ShowOtherTags
  (params (Actor :type Actor%20Object%20Reference))
  ;[1 1 1] Remove Tag For All Other Actors
  (bind _ascharacter (Utilities|Casting|CastToCharacter Actor))
  (bind _array_element (Utilities|Array|ForEachLoopwithBreak (Collision|GetOverlappingActors (Variables|/Script/Engine.Character|GetCapsuleComponent _ascharacter) "/Script/Engine.Actor" :!class /Script/Engine.PrimitiveComponent) :!label _label)
    (:LoopBody
      (Utilities|IsValid (Actor|GetComponentbyClass _array_element "OutlineComponent_C")
        (:Is%20Valid
          (if (!= (Actor|GetComponentbyClass _array_element "OutlineComponent_C") self)
            (ActorTag|ShowActorTag (Actor|GetComponentbyClass _array_element "OutlineComponent_C"))
            (Utilities|IsValid (Actor|GetComponentbyClass _array_element "/Game/FlexibleCombatSystem/Blueprints/Components/LootComponent.LootComponent_C")
              (:Is%20Valid
                (Default|CreateLootWidget (Actor|GetComponentbyClass _array_element "/Game/FlexibleCombatSystem/Blueprints/Components/LootComponent.LootComponent_C"))
                (goto _label Break))
              (:Is%20Not%20Valid
                (goto _label Break)))))))))