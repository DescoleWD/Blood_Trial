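; BP_UpDownButton is a floor-style button that the player triggers by overlapping its box, with a material chosen by melee, ranged or magic type.
; A timeline lerps the mesh to the LowerCube position, set from MoveLocation at construction, while a Playing flag blocks retriggering.
; When the move finishes, it resets FloorButton and an inactive RangedPractise, or messages ActorToActivate if no RangedPractise is valid.
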(event OnComponentBeginOverlap(Box)
  (params (OverlappedComponent :type Primitive%20Component%20Object%20Reference) (OtherActor :type Actor%20Object%20Reference) (OtherComp :type Primitive%20Component%20Object%20Reference) (OtherBodyIndex :type Integer) (bFromSweep :type Boolean) (SweepResult :type Hit%20Result%20Structure%20%28by%20ref%29))
  (Utilities|Casting|CastToBP_PlayerCharacter OtherActor)
  (if (not (Variables|Default|GetPlaying))
    (Variables|Default|SetPlaying true)
    (Variables|Default|SetRelative%20Location (Variables|/Script/Engine.SceneComponent|GetRelativeLocation (Variables|Default|GetStaticMesh)))
    (bind _newtrack_0 (Timeline|MoveButton PlayFromStart)
      (:Update
        (Transformation|SetRelativeLocation (Variables|Default|GetStaticMesh) (Math|Vector|Lerp(Vector) (Variables|Default|GetRelative%20Location) (Variables|/Script/Engine.SceneComponent|GetRelativeLocation (Variables|Default|GetLowerCube)) _newtrack_0) false false))
      (:Finished
        (CallFunction|Activate)
        (Variables|Default|SetPlaying false)))))

(event Custom|Activate
  (bind _ranged_practise (Variables|Default|GetRanged%20Practise))
  (Utilities|IsValid _ranged_practise
    (:Is%20Valid
      (if (not (Variables|/Game/FlexibleCombatSystem/DemoFolder/Blueprint/BP_RangedPractise.BP_RangedPractise_C|GetActive _ranged_practise))
        (Default|Reset (Variables|Default|GetFloorButton))
        (Default|Reset (Variables|Default|GetRanged%20Practise))))
    (:Is%20Not%20Valid
      (Class|IItemInterface|ActivateActor(Message) (Variables|Default|GetActorToActivate)))))

(fn ConstructionScript
  (Transformation|SetRelativeLocation (Variables|Default|GetLowerCube) (Variables|Default|GetMoveLocation) false false)
  (Rendering|Material|SetMaterial (Variables|Default|GetStaticMesh) 0 (Utilities|Select :Index (Variables|Default|GetButtonType) :NewEnumerator0 "/Game/FlexibleCombatSystem/DemoFolder/Materials/MI_MeleeTraining.MI_MeleeTraining" :NewEnumerator1 "/Game/FlexibleCombatSystem/DemoFolder/Materials/MI_RangedButton.MI_RangedButton" :NewEnumerator2 "/Game/FlexibleCombatSystem/DemoFolder/Materials/MI_MagicButton.MI_MagicButton")))