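; Demo-folder spawner that keeps a group of combat AI dummies available, respawning the whole wave once all are dead.
; On BeginPlay it spawns a BP_DamageTakingDummy at each spawn-point component, running BT_MixedCombat, granting no XP, with attack style set to prevent blocking.
; Each dummy references the spawner as its ActivateActorOnDeath target; ActivateActor checks for survivors and, if none remain, waits briefly, destroys the bodies and respawns.
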(event EventBeginPlay
  (for _array_element (Utilities|Array|MakeArray (Variables|Default|GetSpawn_35) (Variables|Default|GetSpawn_20) (Variables|Default|GetSpawn_21) (Variables|Default|GetSpawn_22) (Variables|Default|GetSpawn_23) (Variables|Default|GetSpawn_24) (Variables|Default|GetSpawn_25) (Variables|Default|GetSpawn_26) (Variables|Default|GetSpawn_27) (Variables|Default|GetSpawn_28) (Variables|Default|GetSpawn_29) (Variables|Default|GetSpawn_30) (Variables|Default|GetSpawn_31) (Variables|Default|GetSpawn_32) (Variables|Default|GetSpawn_33) (Variables|Default|GetSpawn_34))
    (bind _returnvalue (Game|SpawnActorfromClass :Class "/Game/FlexibleCombatSystem/DemoFolder/Blueprint/BP_DamageTakingDummy.BP_DamageTakingDummy_C" :SpawnTransform (Math|Transform|MakeTransform (Transformation|GetWorldLocation _array_element) (Transformation|GetWorldRotation _array_element) "1,1,1") :CollisionHandlingOverride "Undefined" :BehaviourTree "/Game/FlexibleCombatSystem/Blueprints/AI/BehaviourTrees/BT_MixedCombat.BT_MixedCombat" :XP_GivenWhenKilled 0 :ActivateActorOnDeath self :Instigator 0))
    (Utilities|Array|Add (Variables|Default|GetAI) _returnvalue)
    ;[1 1 1] Prevents Block
    (Variables|/Game/FlexibleCombatSystem/Blueprints/Components/CombatStatusComponent.CombatStatusComponent_C|SetCurrentAttackStyle (Variables|/Game/FlexibleCombatSystem/DemoFolder/Blueprint/BP_DamageTakingDummy.BP_DamageTakingDummy_C|GetCombatStatusComponent _returnvalue) "NewEnumerator2")))

(event EventActivateActor
  (bind _ai (Variables|Default|GetAI))
  (Variables|Default|SetAllDead true)
  (bind _array_element (Utilities|Array|ForEachLoopwithBreak (Variables|Default|GetAI) :!label _label)
    (:LoopBody
      (if (not (Variables|/Game/FlexibleCombatSystem/DemoFolder/Blueprint/BP_DamageTakingDummy.BP_DamageTakingDummy_C|GetDead _array_element))
        (Variables|Default|SetAllDead false)
        (goto _label Break)))
    (:Completed
      (if (Variables|Default|GetAllDead)
        (Utilities|FlowControl|Delay 2.0)
        (for _array_element_2 _ai
          (Actor|DestroyActor _array_element_2))
        (Utilities|Array|Clear _ai)
        (for _array_element_3 (Utilities|Array|MakeArray (Variables|Default|GetSpawn_35) (Variables|Default|GetSpawn_20) (Variables|Default|GetSpawn_21) (Variables|Default|GetSpawn_22) (Variables|Default|GetSpawn_23) (Variables|Default|GetSpawn_24) (Variables|Default|GetSpawn_25) (Variables|Default|GetSpawn_26) (Variables|Default|GetSpawn_27) (Variables|Default|GetSpawn_28) (Variables|Default|GetSpawn_29) (Variables|Default|GetSpawn_30) (Variables|Default|GetSpawn_31) (Variables|Default|GetSpawn_32) (Variables|Default|GetSpawn_33) (Variables|Default|GetSpawn_34))
          (bind _returnvalue (Game|SpawnActorfromClass :Class "/Game/FlexibleCombatSystem/DemoFolder/Blueprint/BP_DamageTakingDummy.BP_DamageTakingDummy_C" :SpawnTransform (Math|Transform|MakeTransform (Transformation|GetWorldLocation _array_element_3) (Transformation|GetWorldRotation _array_element_3) "1,1,1") :CollisionHandlingOverride "Undefined" :BehaviourTree "/Game/FlexibleCombatSystem/Blueprints/AI/BehaviourTrees/BT_MixedCombat.BT_MixedCombat" :XP_GivenWhenKilled 0 :ActivateActorOnDeath self :Instigator 0))
          (Utilities|Array|Add (Variables|Default|GetAI) _returnvalue)
          ;[1 1 1] Prevents Block
          (Variables|/Game/FlexibleCombatSystem/Blueprints/Components/CombatStatusComponent.CombatStatusComponent_C|SetCurrentAttackStyle (Variables|/Game/FlexibleCombatSystem/DemoFolder/Blueprint/BP_DamageTakingDummy.BP_DamageTakingDummy_C|GetCombatStatusComponent _returnvalue) "NewEnumerator2"))))))

(fn ConstructionScript)