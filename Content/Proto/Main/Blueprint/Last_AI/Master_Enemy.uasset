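; Master enemy Blueprint that provides player targeting and melee attacks for AI enemies.
; A server-named event scans all BP_MainBase actors and stores the nearest within a large distance cap as ClosestPlayer.
; The melee event, gated by IsAttacking, plays a random montage from up to five attack slots, limited by MaxAttack.
; Health bar widget and knockback functions are empty stubs, as is the construction script.
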(event Custom|Server_FindClosestPLayer
  ;[1 1 1] Find Player
  (Variables|Default|SetClosestPlayerDistance 2e+05)
  (bind _outactors (Actor|GetAllActorsOfClass "/Game/Proto/Main/Blueprint/BP_MainBase.BP_MainBase_C"))
  (for _array_element _outactors
    (if (< (Transformation|GetDistanceTo _array_element self) (Variables|Default|GetClosestPlayerDistance))
      (Variables|Default|SetClosestPlayerDistance (Transformation|GetDistanceTo _array_element self))
      (Variables|Default|SetClosestPlayer _array_element))))

(event Custom|ServerNPCMeleeAttack
  ;[1 1 1] Attack Move set
  (if (not (Variables|Default|GetIsAttacking))
    (Animation|PlayAnimMontage (Utilities|Select :Index (Math|Random|RandomIntegerinRange 0 (- (Variables|Default|GetMaxAttack) 1)) :Option%200 (Variables|AnimAttack|GetAttack01) :Option%201 (Variables|AnimAttack|GetAttack02) :Option%202 (Variables|AnimAttack|GetAttack03) :Option%203 (Variables|AnimAttack|GetAttack04) :Option%204 (Variables|AnimAttack|GetAttack05)) 1.0 "None")))

(fn ConstructionScript)

(fn GetHealthBarWidget)

(fn KnockBackVF)