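; Base Blueprint for bow pick-up items, providing a common set of functions for child bows.
; GetBowAttachments exposes the skeletal mesh, buff particle system, prediction path spline and execute camera.
; The quiver and arrow functions are stubs returning empty or zero values, with no logic here.
; The construction script only calls its parent.
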(fn ConstructionScript
  (|CallParentFunction))

(fn ArrowsinQuiver
  (return 0))

(fn GetArrowName&Quantity
  (return "" 0))

(fn GetBowAttachments
  (return (Variables|Default|GetItemSkeletal) (Variables|Default|GetBowBuffPS) (Variables|Default|GetPredictionPathSpline) 0 (Variables|Default|GetExecuteCamera)))

(fn GetQuiverRef
  (return 0))

(fn PassArrowRef
  (return 0))