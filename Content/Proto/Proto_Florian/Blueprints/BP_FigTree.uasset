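; BP_FigTree is a prototype fig tree healing pickup for the main character.
; A latent MoveComponentTo loop bobs the Fig component up and down from BeginPlay.
; Box overlap applies the clamped, raised life total as negative damage, stores it in game instance ChooseLife, and destroys only the Fig, leaving the trigger.
; Tick prints ChooseLife for debugging, and leftover HP bar update nodes never run.
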(event OnComponentBeginOverlap(Box)
  (params (OverlappedComponent :type Primitive%20Component%20Object%20Reference) (OtherActor :type Actor%20Object%20Reference) (OtherComp :type Primitive%20Component%20Object%20Reference) (OtherBodyIndex :type Integer) (bFromSweep :type Boolean) (SweepResult :type Hit%20Result%20Structure%20%28by%20ref%29))
  (bind _asblood_trial_game_instance (CallFunction|GetInst))
  (bind _asblood_trial_game_instance_2 (CallFunction|GetInst))
  (bind _asbp_main_character (Utilities|Casting|CastToBP_MainCharacter OtherActor))
  (Game|Damage|ApplyDamage _asbp_main_character (* (Math|Float|Clamp(Float) (+ (Variables|/Game/Proto/Main/Blueprint/BloodTrial_GameInstance.BloodTrial_GameInstance_C|GetChoose_Life _asblood_trial_game_instance) 3e+02) 0.0 (Variables|/Game/Proto/Main/Blueprint/BloodTrial_GameInstance.BloodTrial_GameInstance_C|GetMaxLife _asblood_trial_game_instance)) -1.0) 0 0)
  (bind _output_get (Variables|/Game/Proto/Main/Blueprint/BloodTrial_GameInstance.BloodTrial_GameInstance_C|SetChoose_Life _asblood_trial_game_instance_2 (Math|Float|Clamp(Float) (+ (Variables|/Game/Proto/Main/Blueprint/BloodTrial_GameInstance.BloodTrial_GameInstance_C|GetChoose_Life _asblood_trial_game_instance_2) 3e+02) 0.0 (Variables|/Game/Proto/Main/Blueprint/BloodTrial_GameInstance.BloodTrial_GameInstance_C|GetMaxLife _asblood_trial_game_instance_2))))
  (Components|DestroyComponent (Variables|Default|GetFig)))

(event EventBeginPlay
  (Components|MoveComponentTo (Variables|Default|GetFig) "0.000000,210.000000,75.000000" "0, 0, 0" true true 1.0 false :!label _label)
  (Components|MoveComponentTo (Variables|Default|GetFig) "0,210.000000,25.000000" "0, 0, 0" true true 1.0 false)
  (goto _label))

(event EventTick
  (params (DeltaSeconds :type Float%20%28single-precision%29))
  (Development|PrintString (Utilities|String|ToString(Float) (stale OnComponentBeginOverlap(Box) _output_get))))

(fn ConstructionScript)