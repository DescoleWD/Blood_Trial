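; Resource component that drains and regenerates stamina and mana, with the values stored in EquipmentComponent.
; DamageResource applies either a one-off cost or a looping timer drain, which pauses stamina loss while sprinting without positive X/Y velocity.
; Retriggerable delays behind gates start timed regeneration, and value changes fire update calls.
; An empty resource during constant drain shows a "Not Enough" popup, and empty stamina also releases sprint.
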(event Custom|DamageResource
  (params (ResourceReduction :type Float%20%28double-precision%29) (ConstantReduction :type Boolean) (Resource :type Byte :default 0))
  ;[1 1 1] Damage Resource - Drain Constantly OR Damage A Set Amount
  (if ConstantReduction
    (switch Utilities|FlowControl|Switch|Switchon Resource
      (:NewEnumerator0
        (CallFunction|DrainStaminaConstant))
      (:NewEnumerator1
        (CallFunction|DrainManaConstant)))
    (else
      (switch Utilities|FlowControl|Switch|Switchon Resource
        (:NewEnumerator0
          (CallFunction|DamageStaminaOnce ResourceReduction))
        (:NewEnumerator1
          (CallFunction|DamageManaOnce ResourceReduction))))))

(event Custom|BeginManaRecoverTimer
  ;[0.5793 1 0.5424] 2 Seconds Without Losing Stamina - Start Recovering
  ;;[1 1 1] Reset Recover Timer Everytime Called
  (Utilities|FlowControl|Sequence
    (:then_0
      (Utilities|FlowControl|RetriggerableDelay 2.0)
      (Utilities|FlowControl|Gate true :!label _label
        (:Exit
          (CallFunction|RecoverMana))))
    (:then_1
      (goto _label Open))))

(event Custom|DrainStamTick
  ;[1 0.7329 0.7329] Drain Stamina Tick
  (bind _staminadrained (CallFunction|StaminaDrained?))
  (if _staminadrained
    (CallFunction|NotEnoughResource)
    (else
      (bind _drain (CallFunction|SprintCheck))
      (if _drain
        (CallFunction|ReduceStamina)))))

(event Custom|DrainManaTick
  ;[1 0.7329 0.7329] Drain Stamina Tick
  (bind _manadrained (CallFunction|ManaDrained?))
  (if _manadrained
    (CallFunction|NotEnoughResource 0)
    (else
      (CallFunction|ReduceMana))))

(event Custom|ClearDrainStamina
  ;[0.3953 0.5746 1] Clear Stamina Drain Begin Recover
  (Utilities|Time|ClearandInvalidateTimerbyHandle (Variables|TimerInfo|GetDrainStaminaTimer))
  (CallFunction|BeginStamRecoverTimer))

(event Custom|DrainStaminaConstant
  ;[1 0.7329 0.7329] Drain Stamina Tick
  ;;[1 1 1] Clear Recover Timer, Begin Drain
  (CallFunction|StopStamRecoverTimer)
  (bind _returnvalue (Utilities|Time|SetTimerbyEvent (EventDispatchers|CreateEvent :!event Custom|DrainStamTick) (Variables|TimerInfo|GetDrainStaminaTick) true))
  (Variables|TimerInfo|SetDrainStaminaTimer _returnvalue))

(event Custom|StopManaRecoverTimer
  ;[0.5793 1 0.5424] 2 Seconds Without Losing Stamina - Start Recovering
  (Utilities|Time|ClearandInvalidateTimerbyHandle (Variables|TimerInfo|GetRecoverManaTimer))
  ;;[1 1 1] Reset Recover Timer Everytime Called
  (Utilities|FlowControl|Gate true) ; enters at Close
)

(event Custom|RecoverMana
  ;[0.5793 1 0.5424] 2 Seconds Without Losing Stamina - Start Recovering
  ;;[1 1 1] RecoverMana
  (bind _returnvalue (Utilities|Time|SetTimerbyEvent (delegate Custom|RecoverMana) (Variables|TimerInfo|GetIncreaseManaTick) true))
  (Variables|TimerInfo|SetRecoverManaTimer _returnvalue)
  (CallFunction|IncreaseMana))

(event Custom|DrainManaConstant
  ;[1 0.7329 0.7329] Drain Stamina Tick
  ;;[1 1 1] Clear Recover Timer, Begin Drain
  (Utilities|Time|ClearandInvalidateTimerbyHandle (Variables|TimerInfo|GetRecoverManaTimer))
  (bind _returnvalue (Utilities|Time|SetTimerbyEvent (EventDispatchers|CreateEvent :!event Custom|DrainStamTick) (Variables|TimerInfo|GetDrainManaTickF) true))
  (Variables|TimerInfo|SetDrainManaTimer _returnvalue))

(event Custom|RecoverStamina
  ;[0.5793 1 0.5424] 2 Seconds Without Losing Stamina - Start Recovering
  ;;[1 1 1] RecoverStamina
  (bind _returnvalue (Utilities|Time|SetTimerbyEvent (delegate Custom|RecoverStamina) (Variables|TimerInfo|GetIncreaseStaminaTick) true))
  (Variables|TimerInfo|SetRecoverStaminaTimer _returnvalue)
  (CallFunction|IncreaseStamina))

(event Custom|BeginStamRecoverTimer
  ;[0.5793 1 0.5424] 2 Seconds Without Losing Stamina - Start Recovering
  ;;[1 1 1] Reset Recover Timer Everytime Called
  (Utilities|FlowControl|Sequence
    (:then_0
      (Utilities|FlowControl|RetriggerableDelay (Variables|Default|GetStaminaRegainDelay))
      (Utilities|FlowControl|Gate true :!label _label
        (:Exit
          (CallFunction|RecoverStamina))))
    (:then_1
      (goto _label Open))))

(event Custom|StopStamRecoverTimer
  ;[0.5793 1 0.5424] 2 Seconds Without Losing Stamina - Start Recovering
  (Utilities|Time|ClearandInvalidateTimerbyHandle (Variables|TimerInfo|GetRecoverStaminaTimer))
  ;;[1 1 1] Reset Recover Timer Everytime Called
  (Utilities|FlowControl|Gate true) ; enters at Close
)

(event Custom|NotEnoughResource
  (params (Resource :type Byte :default 0))
  (bind _movementcomponent (Variables|Components|GetMovementComponent))
  ;[1 1 1] Damage Resource - Drain Constantly OR Damage A Set Amount
  ;;[1 1 1] Widget - Not Enough Stamina
  (bind _returnvalue (UserInterface|CreateWidget 0 0 (Utilities|Text|ToText(String) (Utilities|String|Append "Not Enough " (Utilities|String|EnumtoString Resource)))))
  (UserInterface|Viewport|AddtoViewport _returnvalue 0)
  (switch Utilities|FlowControl|Switch|Switchon Resource
    (:NewEnumerator0
      (if (Variables|Default|GetSprint _movementcomponent)
        (CallFunction|EventReleaseSprint _movementcomponent)))))

(event EventBeginPlay
  ;[1 1 1] Setup
  (CallFunction|StoreComponents))

(fn DamageStaminaOnce
  (params (DamageAmount :type Float%20%28double-precision%29))
  (bind _equipmentcomponent (Variables|Default|GetEquipmentComponent))
  ;[1 1 1] If Stamina Less Than 0
  (if (< (Variables|Default|GetStamina (.EquipmentComponent (Variables|Default|GetEquipmentComponent))) DamageAmount)
    ;[1 1 1] Set Stamina 0
    (Variables|Default|SetStamina (.EquipmentComponent (Variables|Default|GetEquipmentComponent)) 0.0)
    (else
      ;[1 1 1] Damage Stamina
      (Variables|Default|SetStamina _equipmentcomponent (- (Variables|Default|GetStamina _equipmentcomponent) DamageAmount))))
  (CallFunction|UpdateStaminaF)
  (CallFunction|StopStamRecoverTimer)
  ;[1 1 1] Begin Recover Timer
  (CallFunction|BeginStamRecoverTimer))

(fn StaminaDrained?
  (return (<= (Variables|Default|GetStamina (.EquipmentComponent (Variables|Default|GetEquipmentComponent))) 0.0)))

(fn IncreaseStamina
  (bind _equipmentcomponent (Variables|Default|GetEquipmentComponent))
  (bind _equipmentcomponent_2 (Variables|Default|GetEquipmentComponent))
  ;[1 1 1] If Stamina Is Full
  (if (>= (Variables|Default|GetStamina _equipmentcomponent) (Variables|Default|GetMaxStamina _equipmentcomponent))
    ;[1 1 1] Stop Regenerating
    (Utilities|Time|ClearandInvalidateTimerbyHandle (Variables|TimerInfo|GetRecoverStaminaTimer))
    (else
      ;[1 1 1] Regenerate
      (Variables|Default|SetStamina _equipmentcomponent_2 (+ (Variables|Default|GetStamina _equipmentcomponent_2) 1.0 0.0))
      (CallFunction|UpdateStaminaF))))

(fn ReduceStamina
  (bind _equipmentcomponent (Variables|Default|GetEquipmentComponent))
  (Variables|Default|SetStamina _equipmentcomponent (- (Variables|Default|GetStamina _equipmentcomponent) 1.0))
  (CallFunction|UpdateStaminaF))

(fn UpdateStaminaF
  (bind _equipmentcomponent (Variables|Default|GetEquipmentComponent))
  (Default|CallUpdateStamina (Variables|Default|GetStamina _equipmentcomponent) (Variables|Default|GetMaxStamina _equipmentcomponent)))

(fn ManaDrained?
  (return (<= (Variables|Default|GetMana (.EquipmentComponent (Variables|Default|GetEquipmentComponent))) 0.0)))

(fn DamageManaOnce
  (params (DamageAmount :type Float%20%28double-precision%29))
  (bind _equipmentcomponent (Variables|Default|GetEquipmentComponent))
  ;[1 1 1] Damage Mana
  (bind _output_get (Variables|Default|SetMana _equipmentcomponent (- (Variables|Default|GetMana _equipmentcomponent) DamageAmount)))
  ;[1 1 1] Mana Under 0 Check
  (if (< _output_get 0.0)
    (Variables|Default|SetMana _equipmentcomponent 0.0))
  (CallFunction|UpdateManaF)
  (Utilities|Time|ClearandInvalidateTimerbyHandle (Variables|TimerInfo|GetRecoverManaTimer))
  ;[1 1 1] Begin Recover Timer
  (CallFunction|BeginManaRecoverTimer))

(fn UpdateManaF
  (bind _equipmentcomponent (Variables|Default|GetEquipmentComponent))
  (Default|CallUpdateMana (Variables|Default|GetMana _equipmentcomponent) (Variables|Default|GetMaxMana _equipmentcomponent)))

(fn ReduceMana
  (bind _equipmentcomponent (Variables|Default|GetEquipmentComponent))
  (Variables|Default|SetMana _equipmentcomponent (- (Variables|Default|GetMana _equipmentcomponent) 1.0))
  (CallFunction|UpdateManaF))

(fn IncreaseMana
  (bind _equipmentcomponent (Variables|Default|GetEquipmentComponent))
  (bind _equipmentcomponent_2 (Variables|Default|GetEquipmentComponent))
  ;[1 1 1] If Stamina Is Full
  (if (>= (Variables|Default|GetMana _equipmentcomponent) (Variables|Default|GetMaxMana _equipmentcomponent))
    ;[1 1 1] Stop Regenerating
    (Utilities|Time|ClearandInvalidateTimerbyHandle (Variables|TimerInfo|GetRecoverManaTimer))
    (else
      ;[1 1 1] Regenerate
      (Variables|Default|SetMana _equipmentcomponent_2 (+ (Variables|Default|GetMana _equipmentcomponent_2) 1.0 0.0))
      (CallFunction|UpdateManaF))))

(fn StoreComponents
  (bind _returnvalue (Components|GetOwner))
  (Variables|Default|SetEquipmentComponent 0 (Actor|GetComponentbyClass _returnvalue 0))
  (Variables|Components|SetMovementComponent 0 (Actor|GetComponentbyClass _returnvalue 0)))

(fn UpdateStaminaDispatch
  (bind _equipmentcomponent (Variables|Default|GetEquipmentComponent))
  (Default|CallUpdateStamina (Variables|Default|GetStamina _equipmentcomponent) (Variables|Default|GetMaxStamina _equipmentcomponent)))

(fn UpdateManaDispatch
  (bind _equipmentcomponent (Variables|Default|GetEquipmentComponent))
  (Default|CallUpdateMana (Variables|Default|GetMana _equipmentcomponent) (Variables|Default|GetMaxMana _equipmentcomponent)))

(fn SprintCheck
  (bind _movementcomponent (Variables|Components|GetMovementComponent))
  (bind _charactermovement (Variables|Default|GetCharacterMovement _movementcomponent))
  (bind _velocity (Variables|/Script/Engine.MovementComponent|GetVelocity _charactermovement))
  ;[1 1 1] Only Drain Stamina From Sprint IF Moving
  (if (Variables|Default|GetSprint _movementcomponent)
    (if (or (> (.x _velocity) 0.0) (> (.y _velocity) 0.0))
      (return true)
      (else
        (return false)))
    (else
      (return true))))