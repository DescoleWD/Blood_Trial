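; Key pickup that records possession in a HaveKey flag on the object returned by GetInst.
; When BP_MainBase overlaps the sphere, it sets the flag, plays a sound and disables collision on mesh and sphere.
; The mesh then swaps material and rises while rotating through MoveComponentTo before the actor destroys itself.
; On BeginPlay the key destroys itself if HaveKey is already set, so a collected key does not reappear.
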(event OnComponentBeginOverlap(Sphere)
  (params (OverlappedComponent :type Primitive%20Component%20Object%20Reference) (OtherActor :type Actor%20Object%20Reference) (OtherComp :type Primitive%20Component%20Object%20Reference) (OtherBodyIndex :type Integer) (bFromSweep :type Boolean) (SweepResult :type Hit%20Result%20Structure%20%28by%20ref%29))
  (Utilities|Casting|CastToBP_MainBase OtherActor)
  (Variables|/Game/Proto/Main/Blueprint/BloodTrial_GameInstance.BloodTrial_GameInstance_C|SetHaveKey? (CallFunction|GetInst) true)
  (Audio|PlaySound2D "/Game/Proto/Proto_Florian/SFX/Key.Key" 1.0 1.0 0.0 0 0)
  (Collision|SetCollisionEnabled (Variables|Default|GetStaticMesh) "NoCollision")
  (Rendering|Material|SetMaterial (Variables|Default|GetStaticMesh) 0 "/Game/Core/Textures/Key_Mat_Inst1.Key_Mat_Inst1")
  (Components|MoveComponentTo (Variables|Default|GetStaticMesh) "0, 0, 0" "0, 0, 0" true true 0.01 false)
  (Components|MoveComponentTo (Variables|Default|GetStaticMesh) "0, 0,180.000000" "0,180.000000, 0" true true 0.5 false)
  (Actor|DestroyActor))

(event EventBeginPlay
  (if (Variables|/Game/Proto/Main/Blueprint/BloodTrial_GameInstance.BloodTrial_GameInstance_C|GetHaveKey? (CallFunction|GetInst))
    (Actor|DestroyActor)))

(fn ConstructionScript)