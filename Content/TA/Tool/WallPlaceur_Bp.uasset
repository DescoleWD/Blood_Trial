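; Editor wall-building tool that generates a modular building from a spline in its construction script, using instanced meshes.
; Wall mesh width plus an offset sets the module size used to stack walls along the spline up to Height.
; Optional passes add pillars at spline points, a base row and a roof with optional bottom face.
; Roof tiles use random variants on a bounding-box grid, filtered by a ray-crossing point-in-polygon test.
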(event EventBeginPlay)

(event Collision|EventActorBeginOverlap
  (params (OtherActor :type Actor%20Object%20Reference)))

(event EventTick
  (params (DeltaSeconds :type Float%20%28single-precision%29)))

(fn ConstructionScript
  (bind _offset (Variables|MainParameter|GetOffset))
  (bind _wallshape (Variables|Default|GetWallShape))
  (bind _spline (Variables|Default|GetSpline))
  (bind _returnvalue (Spline|GetSplineLength _spline))
  (bind _staticmesh (Variables|/Script/Engine.StaticMeshComponent|GetStaticMesh _wallshape))
  (bind _returnvalue_2 (StaticMesh|GetBoundingBox _staticmesh))
  (bind _returnvalue_3 (- (.max _returnvalue_2) (.min _returnvalue_2)))
  (bind _returnvalue_4 (+ (.x _returnvalue_3) _offset))
  (bind _returnvalue_5 (/ _returnvalue _returnvalue_4))
  (bind _returnvalue_6 (Math|Float|Truncate _returnvalue_5))
  (CallFunction|TypeOfCurve) ; Set linear or curve
  (for _array_element (Utilities|Array|MakeArray (Variables|Default|GetGroundShape) _wallshape (Variables|Default|GetPillardShape) (Variables|Default|GetDownShape) (Variables|Default|GetGroundShapeVar1) (Variables|Default|GetGroundShaoeVar2) (Variables|Default|GetGroundShapeVar3))
    (Components|InstancedStaticMesh|SetCullDistances _array_element (Variables|Default|GetStart%20Cull%20Distance) (Variables|Default|GetEnd%20Cull%20Distance)))
  (Spline|SetClosedLoop (Variables|Default|GetSpline) (Variables|MainParameter|GetIn%20Closed%20Loop) true)
  (Variables|Default|SetLenght _returnvalue_4)
  (Variables|Default|SetLoopByLengthCurve _returnvalue_6)
  (CallFunction|WallGeneration _returnvalue_6)
  (if (Variables|MainParameter|GetRoof)
    (CallFunction|RoofGenerator))
  (if (Variables|CustomParameter|GetPillard?)
    (CallFunction|PillardFuction))
  (if (Variables|CustomParameter|GetDownShape?)
    (CallFunction|BaseShapeFuction)))

(fn TypeOfCurve
  (bind _spline (Variables|Default|GetSpline))
  (bind _spline_2 (Variables|Default|GetSpline))
  (for _index (range 0 (+ (Spline|GetNumberOfSplinePoints _spline) 2))
    (if (> (Spline|GetSplineLength _spline_2) 201.0)
      (Spline|SetSplinePointType _spline _index "Linear" true)
      (else
        (Spline|SetSplinePointType _spline_2 _index "Curve" true))))
  (return))

(fn WallGeneration
  (params (LastIndex :type Integer))
  (bind _spline (Variables|Default|GetSpline))
  (for _index (range 0 LastIndex)
    (for _index_2 (range 0 (- (Variables|MainParameter|GetHeight) 1))
      (Components|InstancedStaticMesh|AddInstance (Variables|Default|GetWallShape) (Math|Transform|MakeTransform (Math|Vector|MakeVector (.X (Class|KismetMathLibrary|BreakVector3f (Spline|GetLocationatDistanceAlongSpline _spline (* _index (Variables|Default|GetLenght)) "Local"))) (.Y (Class|KismetMathLibrary|BreakVector3f (Spline|GetLocationatDistanceAlongSpline _spline (* _index (Variables|Default|GetLenght)) "Local"))) (* (Variables|Default|GetLenght) _index_2)) (Spline|GetRotationatDistanceAlongSpline _spline (* _index (Variables|Default|GetLenght)) "Local") (Math|Vector|MakeVector 1.0 1.0 1.0)) false)))
  (return))

(fn Orientation
  (params (P :type Vector) (Q :type Vector) (R :type Vector))
  (bind (_x _y) (Class|KismetMathLibrary|BreakVector3f P))
  (bind (_x_2 _y_2) (Class|KismetMathLibrary|BreakVector3f Q))
  (bind (_x_3 _y_3) (Class|KismetMathLibrary|BreakVector3f R))
  (bind _returnvalue (- _y_2 _y))
  (bind _returnvalue_2 (- _x_2 _x))
  (bind _returnvalue_3 (- _x_3 _x_2))
  (bind _returnvalue_4 (- _y_3 _y_2))
  (bind _returnvalue_5 (* _returnvalue_2 _returnvalue_4))
  (bind _returnvalue_6 (* _returnvalue _returnvalue_3))
  (bind _returnvalue_7 (- _returnvalue_6 _returnvalue_5))
  (if (== _returnvalue_7 0.0)
    (return 0)
    (elif (> _returnvalue_7 0.0)
      (return 1)
      (else
        (return 2)))))

(fn DoIntersect
  (params (P1 :type Vector) (Q1 :type Vector) (P2 :type Vector) (Q2 :type Vector))
  (bind _orientation (CallFunction|Orientation P1 Q1 P2))
  (bind _output_get (LocalVariables|SetO1 _orientation))
  (bind _orientation_2 (CallFunction|Orientation P1 Q1 Q2))
  (bind _output_get_2 (LocalVariables|SetO2 _orientation_2))
  (bind _orientation_3 (CallFunction|Orientation P2 Q2 P1))
  (bind _output_get_3 (LocalVariables|SetO3 _orientation_3))
  (bind _orientation_4 (CallFunction|Orientation P2 Q2 Q1))
  (bind _output_get_4 (LocalVariables|SetO4 _orientation_4))
  (return (and (!= _output_get _output_get_2) (!= _output_get_3 _output_get_4))))

(fn IsInside
  (params (P :type Vector))
  (bind _spline (Variables|Default|GetSpline))
  (bind _returnvalue (Spline|GetNumberOfSplinePoints _spline))
  (for _index (range 0 (- _returnvalue 1))
    (bind _intersect (CallFunction|DoIntersect P (+ (Variables|Default|GetPmin) "-100.000000,0,0") (Spline|GetLocationatSplinePoint _spline _index "Local") (Spline|GetLocationatSplinePoint _spline (Math|Integer|%(Integer) (+ _index 1) _returnvalue) "Local")))
    (if _intersect
      (Math|Integer|IncrementInt (LocalVariables|GetCount))))
  (return (!= (Math|Integer|%(Integer) (LocalVariables|GetCount) 2) 0)))

(fn GetMinMaxPoint
  (bind _spline (Variables|Default|GetSpline))
  (bind _returnvalue (Spline|GetLocationatSplinePoint _spline 0 "Local"))
  ;[0 0 0] le but est de determiner le point le plus haut et le plus bas de la shape, minPoint = le point le plus bas, MaxPoint = le plus haut
  (LocalVariables|SetMinPoint _returnvalue)
  (LocalVariables|SetMaxPoint _returnvalue)
  (for _index (range 0 (- (Spline|GetNumberOfSplinePoints _spline) 1))
    (LocalVariables|SetMinPoint (Math|Vector|VectorComponentMin (Math|Vector|VectorComponentMin (Spline|GetLocationatSplinePoint _spline _index "Local") (Spline|GetLocationatSplinePoint _spline (+ _index 1) "Local")) (LocalVariables|GetMinPoint)))
    (LocalVariables|SetMaxPoint (Math|Vector|VectorComponentMax (Math|Vector|VectorComponentMax (Spline|GetLocationatSplinePoint _spline _index "Local") (Spline|GetLocationatSplinePoint _spline (+ _index 1) "Local")) (LocalVariables|GetMaxPoint))))
  ;[0 0 0] On a donc la diagonal du cube entourant notre shape
  (return (LocalVariables|GetMinPoint) (LocalVariables|GetMaxPoint)))

(fn RoofGenerator
  (bind _groundshapevar1 (Variables|Default|GetGroundShapeVar1))
  (bind _groundshape (Variables|Default|GetGroundShape))
  (bind _rotatetile (Variables|CustomParameter|GetRotateTile))
  (bind _lenght (Variables|Default|GetLenght))
  (bind _height (Variables|MainParameter|GetHeight))
  (bind _groundshaoevar2 (Variables|Default|GetGroundShaoeVar2))
  (bind _groundshapevar3 (Variables|Default|GetGroundShapeVar3))
  (bind _returnvalue (Math|Float|SelectFloat 0.0 9e+01 _rotatetile))
  (bind _array (Utilities|Array|MakeArray _groundshape _groundshapevar1 _groundshaoevar2 _groundshapevar3))
  (bind _returnvalue_2 (* _height _lenght))
  (bind _returnvalue_3 (Utilities|Array|Length _array))
  (bind _returnvalue_4 (- _returnvalue_3 1))
  (bind _returnvalue_5 (Math|Random|RandomIntegerinRange 0 _returnvalue_4))
  (bind _output (Utilities|Array|Get(acopy) _array _returnvalue_5))
  (bind (_minpoint1 _maxpoint1) (CallFunction|GetMinMaxPoint))
  (Variables|Default|SetPmin _minpoint1)
  (Variables|Default|SetPmax _maxpoint1)
  (for _index (range 0 (- (Math|Float|Floor (+ (/ (.x (- (Variables|Default|GetPmax) (Variables|Default|GetPmin))) _lenght) 0.1)) 1))
    (for _index_2 (range 0 (- (Math|Float|Floor (+ (/ (.y (- (Variables|Default|GetPmax) (Variables|Default|GetPmin))) _lenght) 0.1)) 1))
      (bind _isinside (CallFunction|IsInside (Math|Vector|MakeVector (+ (* (Variables|Default|GetLenght) _index) (.x (Variables|Default|GetPmin))) (+ (* (Variables|Default|GetLenght) _index_2) (.y (Variables|Default|GetPmin))) _returnvalue_2)))
      (if _isinside
        (Components|InstancedStaticMesh|AddInstance _output (Math|Transform|MakeTransform (Math|Vector|MakeVector (+ (+ (* (Variables|Default|GetLenght) _index) (.x (Variables|Default|GetPmin))) (Math|Float|SelectFloat 0.0 2e+02 _rotatetile) 0.0) (+ (* (Variables|Default|GetLenght) _index_2) (.y (Variables|Default|GetPmin))) _returnvalue_2) (Math|Rotator|MakeRotator 0.0 0.0 _returnvalue) "1.000000,1.000000,1.000000") false)
        (if (Variables|CustomParameter|GetDownFace?)
          (Components|InstancedStaticMesh|AddInstance _output (Math|Transform|MakeTransform (Math|Vector|MakeVector (+ (+ (* (Variables|Default|GetLenght) _index) (.x (Variables|Default|GetPmin))) (Math|Float|SelectFloat 0.0 2e+02 _rotatetile) 0.0) (+ (* (Variables|Default|GetLenght) _index_2) (.y (Variables|Default|GetPmin))) 0.0) (Math|Rotator|MakeRotator 0.0 0.0 _returnvalue) "1.000000,1.000000,1.000000") false)))))
  (return))

(fn PointSnapping
  (bind _spline (Variables|Default|GetSpline))
  (bind _lenght (Variables|Default|GetLenght))
  (bind _returnvalue (Spline|GetNumberOfSplinePoints _spline))
  (bind _returnvalue_2 (/ _lenght 2.0))
  (bind _returnvalue_3 (- _returnvalue 1))
  (bind _returnvalue_4 (Spline|GetLocationatSplinePoint _spline _returnvalue_3 "Local"))
  (Spline|SetLocationatSplinePoint _spline _returnvalue_3 (Math|Vector|MakeVector (+ (.x _returnvalue_4) (Math|Integer|SelectInt 0 100 (== (Math|Integer|%(Integer) (Math|Float|Round (/ (.x _returnvalue_4) _returnvalue_2)) 2) 0))) (+ (.y _returnvalue_4) (Math|Integer|SelectInt 0 100 (== (Math|Integer|%(Integer) (Math|Float|Round (/ (.y _returnvalue_4) _returnvalue_2)) 2) 0))) 0.0) "Local" true)
  (return))

(fn PillardFuction
  (bind _spline (Variables|Default|GetSpline))
  (for _index (range 0 (- (Spline|GetNumberOfSplinePoints _spline) 1))
    (for _index_2 (range 0 (- (Variables|MainParameter|GetHeight) 1))
      (Components|InstancedStaticMesh|AddInstance (Variables|Default|GetPillardShape) (Math|Transform|MakeTransform (Math|Vector|MakeVector (.x (Spline|GetLocationatSplinePoint _spline _index "Local")) (.y (Spline|GetLocationatSplinePoint _spline _index "Local")) (* _index_2 (Variables|Default|GetLenght))) (Spline|GetRotationatSplinePoint _spline _index "Local") "1.000000,1.000000,1.000000") false)))
  (return))

(fn BaseShapeFuction
  (bind _flipface (Variables|Default|GetFlipFace))
  (bind _spline (Variables|Default|GetSpline))
  (for _index (range 0 (Variables|Default|GetLoopByLengthCurve))
    (Components|InstancedStaticMesh|AddInstance (Variables|Default|GetDownShape) (Math|Transform|MakeTransform (Math|Vector|MakeVector (Math|Float|SelectFloat (+ (.X (Class|KismetMathLibrary|BreakVector3f (Spline|GetLocationatDistanceAlongSpline _spline (* _index (Variables|Default|GetLenght)) "Local"))) 2e+02) (.X (Class|KismetMathLibrary|BreakVector3f (Spline|GetLocationatDistanceAlongSpline _spline (* _index (Variables|Default|GetLenght)) "Local"))) _flipface) (.Y (Class|KismetMathLibrary|BreakVector3f (Spline|GetLocationatDistanceAlongSpline _spline (* _index (Variables|Default|GetLenght)) "Local"))) 0.0) (Math|Rotator|MakeRotator (.Roll (Math|Rotator|BreakRotator (Spline|GetRotationatDistanceAlongSpline _spline (* _index (Variables|Default|GetLenght)) "Local"))) (.Pitch (Math|Rotator|BreakRotator (Spline|GetRotationatDistanceAlongSpline _spline (* _index (Variables|Default|GetLenght)) "Local"))) (Math|Float|SelectFloat (+ (.Yaw (Math|Rotator|BreakRotator (Spline|GetRotationatDistanceAlongSpline _spline (* _index (Variables|Default|GetLenght)) "Local"))) 1.8e+02) (.Yaw (Math|Rotator|BreakRotator (Spline|GetRotationatDistanceAlongSpline _spline (* _index (Variables|Default|GetLenght)) "Local"))) _flipface)) (Math|Vector|MakeVector 1.0 1.0 1.0)) false))
  (return))