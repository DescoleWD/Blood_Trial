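; BPMB_EDistance is a ranged enemy character that fires Bullet_Distance projectiles and can be caught by the player's bolas.
; The bolas strangle montage applies damage, uses notifies to halt movement and update AI_Controler_Melee, then returns the bolas and triggers a counterattack, unless an explosion interrupts it.
; Damage events drive hit reactions or death with score and vampirism, sharing state through GetInst.
; It also carries melee combo, block and turn-to-nearest-enemy logic.
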(event Custom|BolasReturnPlayer
  (bind _asblood_trial_game_instance (CallFunction|GetInst))
  (bind _mesh (Variables|Character|GetMesh))
  (bind _returnvalue (Transformation|GetWorldLocation _mesh))
  ;[0.8705 1 0] Bolas en cours
  (Rendering|SetVisibility (Variables|Default|GetBolas_Attached) false false)
  (bind _returnvalue_2 (Game|SpawnActorfromClass "/Game/Proto/Proto_Florian/Blueprints/BP_Apparence_Bolas.BP_Apparence_Bolas_C" (Math|Transform|MakeTransform (Math|Vector|MakeVector (.x _returnvalue) (.y _returnvalue) (+ (.z _returnvalue) 2e+02)) (Transformation|GetWorldRotation _mesh) "0.300000,0.300000,0.300000") "AlwaysSpawn" 0 0))
  (bind _returnvalue_3 (Actor|GetActorOfClass "/Game/Proto/Main/Blueprint/BP_MainBase.BP_MainBase_C"))
  (Components|MoveComponentTo (Variables|/Game/Proto/Proto_Florian/Blueprints/BP_Apparence_Bolas.BP_Apparence_Bolas_C|GetStaticMesh _returnvalue_2) (Math|Vector|MakeVector (.x (Transformation|GetWorldLocation (Variables|/Script/Engine.Character|GetMesh _returnvalue_3))) (.y (Transformation|GetWorldLocation (Variables|/Script/Engine.Character|GetMesh _returnvalue_3))) (.z (Transformation|GetWorldLocation (Variables|/Script/Engine.Character|GetMesh _returnvalue_3)))) "0, 0, 0" true true 0.3 true)
  (Variables|/Game/Proto/Main/Blueprint/BloodTrial_GameInstance.BloodTrial_GameInstance_C|SetBolas_Attache _asblood_trial_game_instance false)
  (Variables|/Game/Proto/Main/Blueprint/BloodTrial_GameInstance.BloodTrial_GameInstance_C|SetThrowBolas _asblood_trial_game_instance true)
  (Actor|DestroyActor _returnvalue_2))

(event Custom|Distance_Attack
  ;[0 1 0.721] Cast Spell
  (Default|AttaqueEnemyDistance (Variables|Default|GetAC_Distance_Enemy)))

(event Custom|Mort_IA
  ;[0.08256 1 0] Mort IA
  (Utilities|FlowControl|Sequence
    (:then_0
      (Utilities|FlowControl|DoOnce false
        (:Completed
          (CallFunction|IncrScore (Variables|/Game/Proto/Main/Blueprint/BloodTrial_GameInstance.BloodTrial_GameInstance_C|GetScore_Enemy1 (CallFunction|GetInst))))))
    (:then_1
      (if (Variables|/Game/Proto/Main/Blueprint/BloodTrial_GameInstance.BloodTrial_GameInstance_C|GetSacrifice_5 (CallFunction|GetInst))
        (bind _returnvalue (Actor|GetActorOfClass "/Game/Proto/Main/Blueprint/BP_MainBase.BP_MainBase_C"))
        (Default|VampirismeonDeath _returnvalue)))
    (:then_2
      (Utilities|FlowControl|DoOnce false
        (:Completed
          (bind _notifyname (Animation|Montage|PlayMontage (Variables|Character|GetMesh) "/Game/Proto/Proto_Guillaume/Blueprints/Anim_Mixamo/30FPS/Mort_1_Montage.Mort_1_Montage")
            (:then
              (Variables|/Game/Proto/Main/Blueprint/BloodTrial_GameInstance.BloodTrial_GameInstance_C|SetAI_Dead (CallFunction|GetInst) true))
            (:OnCompleted
              (Actor|DestroyActor))
            (:OnNotifyBegin
              (switch name _notifyname
                (:Dead
                  (Pawn|Components|CharacterMovement|SetMovementMode (Variables|Character|GetCharacterMovement) "MOVE_None" 0))))))))))

(event Custom|Anim_Damage
  ;[0.1591 1 0] Si pas bolassed then play hit and set can be damaged
  (Animation|Montage|PlayMontage (Variables|Character|GetMesh) "/Game/Proto/Proto_Guillaume/Blueprints/Anim_Mixamo/30FPS/MediumHitToHead_UE_Montage.MediumHitToHead_UE_Montage"
    (:then
      (Variables|Actor|SetbCanBeDamaged true))))

(event Custom|AI_IS_Bolassed
  ;[1 1 1] Si is get bolassed then
  (Variables|Actor|SetbCanBeDamaged true))

(event Custom|Collision_Explosion
  ;[1 0 0.7108] Explosion
  ;;[1 0.9631 0] Step 1 : Spawn sphere collision pour explosion et identifier les actors touchés
  (Game|SpawnActorfromClass "/Game/Proto/Proto_Guillaume/Blueprints/Player/Explosion.Explosion_C" (Math|Conversions|ToTransform(Vector) (Transformation|GetWorldLocation (Variables|Default|GetBolas_Attached))) "Undefined" 0 0)
  (CallFunction|BolasReturnPlayer))

(event Custom|SpawnBolas_M
  ;[1 0 0.7542] Step 1 : Bolas s'attache sur l'ennemi
  ;;[0.2174 1 0] Step 1 : Faire spawn 1 fois le bolas attaché + Validation bolas attached.
  ;; Bolas attached condition ==> Lead to explosion if 2nd input
  (Variables|/Game/Proto/Main/Blueprint/BloodTrial_GameInstance.BloodTrial_GameInstance_C|SetBolas_Attache (CallFunction|GetInst) true)
  ;;[0.1339 1 0] Step 2 : set bolas attached visible
  (Rendering|SetVisibility (Variables|Default|GetBolas_Attached) true false)
  ;;[0.9325 1 0] Step 3  :Jouer l'animation d'étranglement
  (bind _notifyname (Animation|Montage|PlayMontage (Variables|Character|GetMesh) "/Game/Proto/Proto_Guillaume/Blueprints/Anim_Mixamo/30FPS/BeingStrangled_UE_Montage.BeingStrangled_UE_Montage")
    (:then
      ;;[1 0 0] Step 4 : Appliquer les dégâts sur la durée de l'animation
      (CallFunction|Damage self (Variables|/Game/Proto/Main/Blueprint/BloodTrial_GameInstance.BloodTrial_GameInstance_C|GetDamageBolas (CallFunction|GetInst))))
    (:OnCompleted
      ;;[0.2224 1 0] Step 5 : Si animation étranglement completed / interrupted alors bolas return player + Cast contre attaque
      (CallFunction|BolasReturnPlayer :!label _label)
      (bind _asai_controler_melee (Utilities|Casting|CastToAI_Controler_Melee (AI|GetAIController 0)))
      (Default|CounterAttaque _asai_controler_melee))
    (:OnInterrupted
      (goto _label))
    (:OnNotifyBegin
      (switch name _notifyname :!label _label_2
        (:GetBolassed_1
          ;;[1 0.6248 0] Step 6 : Notify begin then stop mvt AI + Cast AI state bolassed
          (Pawn|Components|CharacterMovement|SetMovementMode (Variables|Character|GetCharacterMovement) "MOVE_None" 0)
          (bind _asai_controler_melee_2 (Utilities|Casting|CastToAI_Controler_Melee (AI|GetAIController 0)))
          (Default|GetBolassed _asai_controler_melee_2))
        (:GetBolassed_2
          ;;[1 0.6248 0] Step 7 : Notify end then stop mvt AI + Cast AI state bolassed
          (Pawn|Components|CharacterMovement|SetMovementMode (Variables|Character|GetCharacterMovement) "MOVE_Walking" 0)
          (bind _asai_controler_melee_3 (Utilities|Casting|CastToAI_Controler_Melee (AI|GetAIController 0)))
          (Default|EndGetBolassed _asai_controler_melee_3))))
    (:OnNotifyEnd
      (goto _label_2))))

(event Custom|Explosion_M
  ;[1 0 0.7108] Explosion
  ;;[0.1952 1 0] Step 1 : Déclencher l'explosion + Throw bolas pas valide
  (Variables|/Game/Proto/Main/Blueprint/BloodTrial_GameInstance.BloodTrial_GameInstance_C|SetThrowBolas (CallFunction|GetInst) false)
  ;;[0.1836 1 0] Step 1.5 : Stop anim being strangled
  (Animation|StopAnimMontage "/Game/Proto/Proto_Guillaume/Blueprints/Anim_Mixamo/30FPS/BeingStrangled_UE_Montage.BeingStrangled_UE_Montage")
  ;;[0.1621 1 0] Step 3 : Call debug de l'explosion + valide variable explosion
  (CallFunction|CollisionExplosion)
  (Variables|Default|SetExplosion true))

(event Custom|Cast_Spell
  (bind _charactermovement (Variables|Character|GetCharacterMovement))
  (bind _spawn_spells (Variables|Default|GetSpawn_Spells))
  (bind _returnvalue (Transformation|GetWorldLocation _spawn_spells))
  (bind _returnvalue_2 (Class|CharacterMovementComponent|GetLastUpdateRotation _charactermovement))
  (bind _returnvalue_3 (Math|Transform|MakeTransform _returnvalue _returnvalue_2 "0.300000,0.300000,0.300000"))
  ;[0 1 0.721] Cast Spell
  (bind _returnvalue_4 (Game|SpawnActorfromClass "/Game/Proto/Proto_Guillaume/Blueprints/Enemy/IA_V2/Distance/Bullet_Distance.Bullet_Distance_C" (Math|Transform|MakeTransform (Math|Vector|MakeVector (.x (.location _returnvalue_3)) (.y (.location _returnvalue_3)) (.z (.location _returnvalue_3))) (.rotation _returnvalue_3) (.scale _returnvalue_3)) "AdjustIfPossibleButAlwaysSpawn" self 0))
  (Physics|AddImpulse (Variables|/Game/Proto/Proto_Guillaume/Blueprints/Enemy/IA_V2/Distance/Bullet_Distance.Bullet_Distance_C|GetSphere _returnvalue_4) (* (Math|Vector|GetForwardVector (Variables|Default|GetSpawn_Spells)) 2e+03) "None" true)
  (Utilities|Attack))

(event Custom|Ai_Damage
  ;[1 1 1] Si attaquée ==> Anim
  (if (Variables|Actor|GetbCanBeDamaged)
    (Variables|Actor|SetbCanBeDamaged false)
    (if (Variables|/Game/Proto/Main/Blueprint/BloodTrial_GameInstance.BloodTrial_GameInstance_C|GetBolas_Attache (CallFunction|GetInst))
      (CallFunction|AIISBolassed)
      (else
        (CallFunction|AnimDamage)))))

(event Custom|Finito
  ;[1 0 0.7542] Step 1 : Bolas s'attache sur l'ennemi
  (Utilities|FlowControl|DoOnce false ; enters at Reset
    (:Completed
      ;;[0.2174 1 0] Step 1 : Faire spawn 1 fois le bolas attaché + Validation bolas attached.
      ;; Bolas attached condition ==> Lead to explosion if 2nd input
      (Variables|/Game/Proto/Main/Blueprint/BloodTrial_GameInstance.BloodTrial_GameInstance_C|SetBolas_Attache (CallFunction|GetInst) true)
      ;;[0.1339 1 0] Step 2 : set bolas attached visible
      (Rendering|SetVisibility (Variables|Default|GetBolas_Attached) true false)
      ;;[0.9325 1 0] Step 3  :Jouer l'animation d'étranglement
      (bind _notifyname (Animation|Montage|PlayMontage (Variables|Character|GetMesh) "/Game/Proto/Proto_Guillaume/Blueprints/Anim_Mixamo/30FPS/BeingStrangled_UE_Montage.BeingStrangled_UE_Montage")
        (:then
          ;;[1 0 0] Step 4 : Appliquer les dégâts sur la durée de l'animation
          (CallFunction|Damage self (Variables|/Game/Proto/Main/Blueprint/BloodTrial_GameInstance.BloodTrial_GameInstance_C|GetDamageBolas (CallFunction|GetInst))))
        (:OnCompleted
          ;;[0.2224 1 0] Step 5 : Si animation étranglement completed / interrupted alors bolas return player + Cast contre attaque
          (CallFunction|BolasReturnPlayer :!label _label)
          (bind _asai_controler_melee (Utilities|Casting|CastToAI_Controler_Melee (AI|GetAIController 0)))
          (Default|CounterAttaque _asai_controler_melee))
        (:OnInterrupted
          (goto _label))
        (:OnNotifyBegin
          (switch name _notifyname :!label _label_2
            (:GetBolassed_1
              ;;[1 0.6248 0] Step 6 : Notify begin then stop mvt AI + Cast AI state bolassed
              (Pawn|Components|CharacterMovement|SetMovementMode (Variables|Character|GetCharacterMovement) "MOVE_None" 0)
              (bind _asai_controler_melee_2 (Utilities|Casting|CastToAI_Controler_Melee (AI|GetAIController 0)))
              (Default|GetBolassed _asai_controler_melee_2))
            (:GetBolassed_2
              ;;[1 0.6248 0] Step 7 : Notify end then stop mvt AI + Cast AI state bolassed
              (Pawn|Components|CharacterMovement|SetMovementMode (Variables|Character|GetCharacterMovement) "MOVE_Walking" 0)
              (bind _asai_controler_melee_3 (Utilities|Casting|CastToAI_Controler_Melee (AI|GetAIController 0)))
              (Default|EndGetBolassed _asai_controler_melee_3))))
        (:OnNotifyEnd
          (goto _label_2))))))

(event Game|Damage|EventAnyDamage
  (params (Damage :type Float%20%28single-precision%29) (DamageType :type Damage%20Type%20Object%20Reference) (InstigatedBy :type Controller%20Object%20Reference) (DamageCauser :type Actor%20Object%20Reference))
  (bind _widget (CallFunction|GetHealthBarWidget))
  ;[0.1879 1 0] Takes damages
  (Default|SubtractValue _widget "NewEnumerator0" 0.0)
  (Math|Float|CompareFloat (Default|GetCurrentValue _widget "NewEnumerator0") 0.0
    (:>
      (CallFunction|AiDamage))
    (:==
      (CallFunction|MortIA :!label _label))
    (:<
      (goto _label))))

(event EventBeginPlay
  (Default|Initialise :self (CallFunction|GetHealthBarWidget) :Parent self :MaxValue 2e+02 :OptionalName "Name" :OptionalMultiplayerSettings (Utilities|Struct|MakeSTRUCT_OtherTeamInfo 0 true "(R=0.755208,G=0.252563,B=0.000000,A=1.000000)" true "Enemy")))

(event EventMovement
  (params (On%20/%20Off :type Boolean))
  (Variables|Character|SetMovementOn On%20/%20Off))

(fn ConstructionScript)

(fn NotifyBegin)

(fn TriggerComplexeHit)

(fn TriggerSimpleHit
  (bind _returnvalue (Transformation|GetActorLocation))
  (bind _returnvalue_2 (Transformation|GetActorForwardVector))
  (Class|KismetSystemLibrary|BoxTraceSingleforObjects _returnvalue (+ _returnvalue (* _returnvalue_2 1.2e+02)) "20.000000,100.000000,50.000000" (Math|Conversions|RotationFromXVector _returnvalue_2) (Utilities|Array|MakeArray "ObjectTypeQuery3") false 0 "None" true))

(fn GetHealthBarWidget
  (bind _aswidget_floating_healthbar_player (Utilities|Casting|CastToWidget_FloatingHealthbar_Player (UserInterface|GetUserWidgetObject (Variables|Default|GetWidget))))
  (return _aswidget_floating_healthbar_player))

(fn GetNearestEnemy
  (bind _returnvalue (Transformation|GetActorLocation))
  (bind (_x _y _z) (Math|Vector|BreakVector _returnvalue))
  (bind _outhits (Collision|MultiSphereTraceForObjects _returnvalue (Math|Vector|MakeVector (+ _x 0.1) (+ _y 0.1) (+ _z 0.1)) 2.5e+02 (Utilities|Array|MakeArray "ObjectTypeQuery3") true 0 "None"))
  (for _array_element _outhits
    (Utilities|IsValid (Variables|Code|GetNearestEnemy)
      (:Is%20Valid
        (if (not (< (Transformation|GetDistanceTo (Variables|Code|GetNearestEnemy) self) (Transformation|GetDistanceTo self (Variables|Code|GetNearestEnemy))))
          (Variables|Code|SetNearestEnemy (.hitactor _array_element) :!label _label)))
      (:Is%20Not%20Valid
        (goto _label))))
  (return (Variables|Code|GetNearestEnemy)))

(event EventOnHit
  (params (ActorHited :type Actor%20Object%20Reference))
  (Animation|PlayAnimMontage "/Game/Proto/Proto_Guillaume/Blueprints/Anim_Mixamo/30FPS/MediumHitToHead_UE_Montage.MediumHitToHead_UE_Montage" 1.0 "None")
  (Utilities|ChangeHealth (Variables|/Game/Proto/Main/Blueprint/BloodTrial_GameInstance.BloodTrial_GameInstance_C|GetEnemyDamage_Melee (CallFunction|GetInst))
    (:True
      (Physics|AddImpulse (Variables|Character|GetCharacterMovement) (* (Transformation|GetActorForwardVector self) -8e+02) true)
      (Utilities|FlowControl|Delay 0.5)
      (Utilities|TurntoActor ActorHited))))