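; Ranged combat component for player and AI characters, covering bow and quiver setup, aim, arrow loading and firing, trajectory prediction, and execute shots.
; An arrow switcher widget cycles inventory ammo and its equipment.
; Nearly all graphs are empty stubs here.
; CalculateBowExecute is implemented: it traces past the predicted impact for head or neck hits on assassinable, RangedComponent-owning targets whose AI has no target.
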(event Custom|ShowArrowOptions
  ;[1 1 1] Create Arrow Switcher
)

(event Custom|FireExecuteArrow
  ;[1 1 1] Fire Arrow & Execute
)

(event Custom|SetupBow
  (params (Bow%20Actor :type Actor%20Object%20Reference))
  ;[1 1 1] Create Bow & Quiver References
)

(event Custom|SendRangedAttack
  ;[1 1 1] Fire Arrow
)

(event Custom|ReleaseBowAim
  ;[1 1 1] Bow Aim (Camera Zoom)
)

(event Custom|TogglePredictionPath
  ;[1 1 1] Used To make 1st Predict, from Camera To Destination (Velocity Might Be Incorrect)
  ;;[1 1 1] Toggle Prediction, Enable/Disable
)

(event Custom|SendBowAim
  ;[1 1 1] Bow Aim (Camera Zoom)
)

(event Custom|MoveDownArrowSelect
  ;[1 1 1] Move Through Arrow Switcher
  ;;[1 1 1] Move Up/Down Through Array, Called From Player Character
)

(event Custom|RemoveArrowOptions
  ;[1 1 1] Close Arrow Switcher Widget
)

(event Custom|EnablePredictionPath
  ;[1 1 1] Used To make 1st Predict, from Camera To Destination (Velocity Might Be Incorrect)
  ;;[1 1 1] Toggle Prediction, Enable/Disable
)

(event Custom|CalculatePredictionPath
  ;[1 1 1] Used To make 1st Predict, from Camera To Destination (Velocity Might Be Incorrect)
  ;;[1 1 1] Calculate Prediction Path
)

(event Custom|OwnerDied
  ;[1 1 1] Send String To Location
)

(event Custom|NextArrowSelect
  (params (MoveUp :type Boolean))
  ;[1 1 1] Move Through Arrow Switcher
  ;;[1 1 1] Begin Animation, Update Array, Update Equipment, Repopulate Widget With New Array Order
)

(event Custom|UpdateStringStatus
  ;[1 1 1] Send String To Location
)

(event Custom|ForceDestroyArrow
  ;[1 1 1] Unload Arrow
)

(event Custom|SetupArrow
  ;[1 1 1] Load Arrow (Triggered By Anim Notify)
)

(event Custom|RemoveTrajectoryPrediction
  ;[1 1 1] Used To make 1st Predict, from Camera To Destination (Velocity Might Be Incorrect)
  ;;[1 1 1] Toggle Prediction, Enable/Disable
)

(event Custom|ExecuteOver
  ;[1 1 1] ExecuteOver
)

(event Custom|RangedCalculations
  ;[1 1 1] Used To make 1st Predict, from Camera To Destination (Velocity Might Be Incorrect)
)

(event Custom|MoveUpArrowSelect
  ;[1 1 1] Move Through Arrow Switcher
  ;;[1 1 1] Move Up/Down Through Array, Called From Player Character
)

(event Custom|UnloadArrow
  ;[1 1 1] Unload Arrow
)

(event Custom|Setup%20Quiver
  (params (Quiver%20Actor :type Actor%20Object%20Reference))
  ;[1 1 1] Create Bow & Quiver References
)

(event Custom|ReceiveExecute
  ;[1 1 1] Sent From Arrow Component Hit - Changes Camera To Enemy Camera
)

(event EventBeginPlay
  ;[1 1 1] Create Bow & Quiver References
)

(fn LaunchArrow)

(fn CreateArrow)

(fn CalculateRangedDamage
  (return 0.0 false))

(fn AimSetup)

(fn ReleaseAimSetup)

(fn LaunchConditions)

(fn AddEmptySpaceWidget)

(fn SwitchArrowOpacityMath
  (params (Index :type Integer)))

(fn ScrolltoNextWidget
  (params (MoveUpwards :type Boolean)))

(fn SwitchUpArray
  (params (MoveUpwards :type Boolean)))

(fn SwitchScale&Opacity)

(fn SwitchAmmoEquipment)

(fn PopulateArrowSwitcher)

(fn SetMiddleResetCounter)

(fn CreateArrayfromInventory)

(fn CreateAmmoEquipElement)

(fn SlotAmmoEquipIntoArray)

(fn SetCameraUpdatedRelative)

(fn GetCameraArrowLevel
  (return "0, 0, 0"))

(fn GetVectorInfrontOfCamera
  ;[1 1 1] Gets A Vector Forward From The Control Rotation (Player Pawn)
  (return "0, 0, 0"))

(fn SpawnPredictionPSs)

(fn SetupPredictionMaterials)

(fn SetPredictionPSs)

(fn RemoveArrowData)

(fn ExecuteConditions)

(fn StoreComponents)

(fn PassAIArrow)

(fn SetArrowVelocity
  (params (EndLocation :type Vector)))

(fn DestroyArrow)

(fn SetupAICustomArrows)

(fn UpdateArrowSwitchQuantity)

(fn FindAssassinationAngle)

(fn IsMagicArrow
  (return false))

(fn UpdateEnemyTarget(AI)
  (params (EnemyTarget :type Actor%20Object%20Reference)))

(fn AttachStringConditions)

(fn UpdateArrowSwitcher)

(fn ArrowLoadedNewBow)