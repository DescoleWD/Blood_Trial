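; BP_CameraPawn is the main menu camera pawn, which moves between main menu, character select and settings viewpoints.
; On BeginPlay it creates the menu widget with references to itself and the character spinner, sets UI-only input with a visible cursor, and is possessed with input disabled.
; CameraTransition plays a timeline that lerps from the current transform to the selected view's stored location and rotation, rotating by the shortest path.
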(event Custom|CameraTransition
  (params (Transition :type E_CameraTransitions%20Enum :default "NewEnumerator0"))
  (Variables|Default|SetCurrentLocation (Transformation|GetActorLocation))
  (Variables|Default|SetCurrentRotation (Transformation|GetActorRotation))
  (bind _newtrack_0 (Timeline|Move PlayFromStart)
    (:Update
      (Transformation|SetActorLocation (Math|Vector|Lerp(Vector) (Variables|Default|GetCurrentLocation) (Utilities|Select :Index Transition :NewEnumerator0 (Variables|Default|GetStartLocation) :NewEnumerator1 (Variables|Default|GetCharacterSelectLocation) :NewEnumerator2 (Variables|Default|GetSettingsLocation)) _newtrack_0) false false)
      (Transformation|SetActorRotation (Math|Rotator|Lerp(Rotator) (Variables|Default|GetCurrentRotation) (Utilities|Select :Index Transition :NewEnumerator0 (Variables|Default|GetStartRotation) :NewEnumerator1 (Variables|Default|GetCharacterSelectRotation) :NewEnumerator2 (Variables|Default|GetSettingsRotation)) _newtrack_0 true)))))

(event EventBeginPlay
  (bind _returnvalue (Game|GetPlayerController 0))
  (bind _returnvalue_2 (Game|GetPlayerController 0))
  (bind _returnvalue_3 (UserInterface|CreateWidget "/Game/FlexibleCombatSystem/Widgets/General/WB_MainMenu.WB_MainMenu_C" 0 self (Variables|Default|GetCharacterSpinner)))
  (UserInterface|Viewport|AddtoViewport _returnvalue_3 0)
  (Variables|/Script/Engine.PlayerController|SetbShowMouseCursor _returnvalue_2 true)
  (Input|SetInputModeUIOnly _returnvalue_2 0 "DoNotLock")
  (Pawn|Possess _returnvalue self)
  (Input|DisableInput _returnvalue))

(fn ConstructionScript)