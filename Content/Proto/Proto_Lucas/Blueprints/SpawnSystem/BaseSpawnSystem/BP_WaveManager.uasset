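; BP_WaveManager runs wave-based enemy fights, spawning AI at the current wave's spawners by their type.
; A short looping-timer countdown starts each wave, with the first also switching the player's audio to fight music.
; A half-second delay loop polls the spawned enemies' validity and advances the wave once all are gone.
; After the last wave it calls FightOver on every BP_WaveWalls, stops fight music and restores player audio.
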(event Custom|StartCountdown
  ;[1 1 1] Countdown
  (bind _returnvalue (Utilities|Time|SetTimerbyEvent (delegate Custom|Count) 1.0 true))
  (Variables|Default|SetTime 1)
  (Utilities|FlowControl|DoOnce false
    (:Completed
      (Utilities|FlowControl|Sequence
        (:then_0
          (bind _asbp_main_base (Utilities|Casting|CastToBP_MainBase (Game|GetPlayerCharacter 0)))
          (Default|Stop1Fight _asbp_main_base))
        (:then_1
          (bind _returnvalue_2 (Audio|SpawnSound2D "/Game/Proto/Main/SFX/Music/Test_Son_Guillaume/Fight_Ambiance_Music.Fight_Ambiance_Music" 1.0 1.0 0.0 0))
          (Variables|Default|SetSOundFight _returnvalue_2))))))

(event Custom|Count
  ;[1 1 1] Countdown
  (Development|PrintString (Utilities|String|ToString(Integer) (Variables|Default|GetTime)) true true "(R=0.568324,G=0.661458,B=0.000000,A=1.000000)")
  (if (== (Variables|Default|GetTime) 0)
    (Utilities|Time|ClearandInvalidateTimerbyHandle (stale Custom|StartCountdown _returnvalue))
    (Development|PrintString (Utilities|String|Append "starting wave : " (Utilities|String|ToString(Integer) (Variables|Default|GetWaveNumber))) true true "(R=0.568324,G=0.661458,B=0.000000,A=1.000000)")
    (CallFunction|BeginWave)
    (else
      (Math|Integer|DecrementInt (Variables|Default|GetTime)))))

(event Custom|BeginWave
  ;[1 1 1] Spawn Enemies for wave
  (if (|IsWaveNumberLesserorEqualtoMaxWaveNumber)
    (for _array_element (|Waves)
      (bind _returnvalue (AI|SpawnAIFromClass (Utilities|Select :Index (Variables|/Game/Proto/Proto_Lucas/Blueprints/SpawnSystem/BaseSpawnSystem/BP_WaveSpawnPoint.BP_WaveSpawnPoint_C|GetSpawnerType _array_element) :NewEnumerator0 "/Game/Proto/Main/Blueprint/Last_AI/ChildEnemies/Tzitzimine.Tzitzimine_C" :NewEnumerator1 "/Game/Proto/Main/Blueprint/Last_AI/Papillon/BP_Papillon.BP_Papillon_C" :NewEnumerator2 "/Game/Proto/Main/Blueprint/Last_AI/ChildEnemies/Tzitzimine.Tzitzimine_C") 0 (.location (Transformation|GetActorTransform _array_element)) (.rotation (Transformation|GetActorTransform _array_element)) true 0))
      (Utilities|Array|Add (Variables|Default|GetCurrentEnemies) _returnvalue))
    (CallFunction|StartCheckingifEnemiesAreDead)
    (else
      (bind _outactors (Actor|GetAllActorsOfClass "/Game/Proto/Proto_Lucas/Blueprints/SpawnSystem/BP_WaveWalls.BP_WaveWalls_C"))
      (for _array_element_2 _outactors
        (bind _asbp_wave_walls (Utilities|Casting|CastToBP_WaveWalls _array_element_2))
        (Default|FightOver _asbp_wave_walls)
        (Audio|Components|Audio|Stop (Variables|Default|GetSOundFight))
        (bind _asbp_main_base (Utilities|Casting|CastToBP_MainBase (Game|GetPlayerCharacter 0)))
        (Default|AllSOund _asbp_main_base)))))

(event Custom|StartCheckingIfEnemiesAreDead
  ;[1 1 1] Check if enemies are dead and start new wave
  (bind _aredead_1 (CallFunction|CheckifAllEnemiesAreDead :!label _label))
  (if _aredead_1
    (Audio|SpawnSound2D 0 1.0 1.0 0.0 0)
    (Math|Integer|IncrementInt (Variables|Default|GetWaveNumber)
      (:%20%20
        (CallFunction|StartCountdown)))
    (else
      (Utilities|FlowControl|Delay 0.5)
      (goto _label))))

(fn ConstructionScript)

(fn CheckifAllEnemiesAreDead
  (LocalVariables|SetAreDead? true)
  (for _array_element (Variables|Default|GetCurrentEnemies)
    (Utilities|IsValid _array_element
      (:Is%20Valid
        (LocalVariables|SetAreDead? false))))
  (return (LocalVariables|GetAreDead?)))