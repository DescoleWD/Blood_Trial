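; Parent pickup item for consumables such as potions, applying their effect when the character uses them.
; ConsumeonUse reads power, duration and type from ItemInfo, waits on the animation length, applies the effect, plays a drink sound and destroys the actor.
; Health, stamina and mana restores clamp to max, show combat text and fire update dispatches.
; Buff, barrier and heal-over-time types route to ActivateBuff, which is empty here.
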(event EventConsumeonUse
  (bind _iteminfo (Variables|Default|GetItemInfo))
  (bind _itemstructure (Utilities|Struct|BreakS_SlotInfo _iteminfo))
  (bind _consumableinfo (Utilities|Struct|BreakS_ItemData _itemstructure))
  (bind (_consumablepower _consumableduration) (Utilities|Struct|BreakS_ConsumableInfo _consumableinfo))
  ;[1 1 1] Consumable Usage
  (Variables|Default|SetConsumable%20Power _consumablepower)
  (Variables|Default|SetConsumable%20Duration _consumableduration)
  (Variables|Default|SetBuffComponent (Actor|GetComponentbyClass (Variables|Default|GetCharacterRef) "/Game/FlexibleCombatSystem/Blueprints/Components/BuffComponent.BuffComponent_C"))
  (bind _output_get (Variables|Default|SetConsumable%20Type (Utilities|Struct|BreakS_ConsumableInfo (.ConsumableInfo (Utilities|Struct|BreakS_ItemData (Utilities|Struct|BreakS_SlotInfo (Variables|Default|GetItemInfo)))))))
  (Utilities|FlowControl|Delay (- (Variables|Default|GetConsumeAnimLength) 2.0))
  (switch Utilities|FlowControl|Switch|SwitchonE_ConsumableType _output_get
    (:NewEnumerator0
      (CallFunction|RestoreHealth))
    (:NewEnumerator1
      (CallFunction|RestoreStamina))
    (:NewEnumerator2
      (CallFunction|RestoreMana))
    (:NewEnumerator3
      (CallFunction|ActivateBuff :!label _label))
    (:NewEnumerator4
      (goto _label))
    (:NewEnumerator5
      (goto _label))
    (:NewEnumerator6
      (goto _label))
    (:NewEnumerator7
      (goto _label))
    (:NewEnumerator8
      (goto _label))
    (:NewEnumerator9
      (goto _label)))
  ;[1 1 1] Animation Finish, Destroy
  (Audio|PlaySoundatLocation (.OutItem (Utilities|Array|Random (Utilities|Array|MakeArray "/Game/FlexibleCombatSystem/SoundFX/General/SW_PotionDrink_01.SW_PotionDrink_01" "/Game/FlexibleCombatSystem/SoundFX/General/SW_PotionDrink_02.SW_PotionDrink_02"))) (Transformation|GetActorLocation (Variables|Default|GetCharacterRef)) "0, 0, 0" 1.0 1.0 0.0 0 0 0)
  (Utilities|FlowControl|Delay 1.5)
  (Actor|DestroyActor))

(fn ConstructionScript
  (|CallParentFunction))

(fn ActivateBuff)

(fn RestoreHealth
  (bind _characterref (Variables|Default|GetCharacterRef))
  (bind _equipmentcomponent (Variables|Default|GetEquipmentComponent))
  (bind _maxhealth (Variables|/Game/FlexibleCombatSystem/Blueprints/Components/EquipmentComponent.EquipmentComponent_C|GetMaxHealth _equipmentcomponent))
  ;[1 1 1] Increase Health
  (bind _output_get (Variables|/Game/FlexibleCombatSystem/Blueprints/Components/EquipmentComponent.EquipmentComponent_C|SetHealth _equipmentcomponent (+ (Variables|/Game/FlexibleCombatSystem/Blueprints/Components/EquipmentComponent.EquipmentComponent_C|GetHealth _equipmentcomponent) (Variables|Default|GetConsumable%20Power))))
  ;;[1 1 1] Set Health Back To Max Health If Goes Above
  (if (> _output_get _maxhealth)
    (Variables|/Game/FlexibleCombatSystem/Blueprints/Components/EquipmentComponent.EquipmentComponent_C|SetHealth _equipmentcomponent _maxhealth))
  (Default|CombatTextPopup (Actor|GetComponentbyClass _characterref "/Game/FlexibleCombatSystem/Blueprints/Components/CombatTextComponent.CombatTextComponent_C") (Transformation|GetActorLocation _characterref) (Math|Float|Round (Variables|Default|GetConsumable%20Power)) "NewEnumerator13" false false false)
  (Default|UpdateHealthDispatch (Variables|Default|GetEquipmentComponent)))

(fn RestoreStamina
  (bind _equipmentcomponent (Variables|Default|GetEquipmentComponent))
  (bind _characterref (Variables|Default|GetCharacterRef))
  (bind _maxstamina (Variables|/Game/FlexibleCombatSystem/Blueprints/Components/EquipmentComponent.EquipmentComponent_C|GetMaxStamina _equipmentcomponent))
  ;[1 1 1] Restore Stamina
  (bind _output_get (Variables|/Game/FlexibleCombatSystem/Blueprints/Components/EquipmentComponent.EquipmentComponent_C|SetStamina _equipmentcomponent (+ (Variables|/Game/FlexibleCombatSystem/Blueprints/Components/EquipmentComponent.EquipmentComponent_C|GetStamina _equipmentcomponent) (Variables|Default|GetConsumable%20Power))))
  ;;[1 1 1] Set Stamina Back To Max Stamina If Goes Above
  (if (> _output_get _maxstamina)
    (Variables|/Game/FlexibleCombatSystem/Blueprints/Components/EquipmentComponent.EquipmentComponent_C|SetStamina _equipmentcomponent _maxstamina))
  (Default|CombatTextPopup (Actor|GetComponentbyClass _characterref "/Game/FlexibleCombatSystem/Blueprints/Components/CombatTextComponent.CombatTextComponent_C") (Transformation|GetActorLocation _characterref) (Math|Float|Round (Variables|Default|GetConsumable%20Power)) "NewEnumerator13" false false false)
  (Default|UpdateStaminaDispatch (Actor|GetComponentbyClass (Variables|Default|GetCharacterRef) "/Game/FlexibleCombatSystem/Blueprints/Components/ResourceComponent.ResourceComponent_C")))

(fn RestoreMana
  (bind _equipmentcomponent (Variables|Default|GetEquipmentComponent))
  (bind _characterref (Variables|Default|GetCharacterRef))
  (bind _maxmana (Variables|/Game/FlexibleCombatSystem/Blueprints/Components/EquipmentComponent.EquipmentComponent_C|GetMaxMana _equipmentcomponent))
  ;[1 1 1] Restore Mana
  (bind _output_get (Variables|/Game/FlexibleCombatSystem/Blueprints/Components/EquipmentComponent.EquipmentComponent_C|SetMana _equipmentcomponent (+ (Variables|/Game/FlexibleCombatSystem/Blueprints/Components/EquipmentComponent.EquipmentComponent_C|GetMana _equipmentcomponent) (Variables|Default|GetConsumable%20Power))))
  ;;[1 1 1] Set Mana Back To Max Mana If Goes Above
  (if (> _output_get _maxmana)
    (Variables|/Game/FlexibleCombatSystem/Blueprints/Components/EquipmentComponent.EquipmentComponent_C|SetMana _equipmentcomponent _maxmana))
  (Default|CombatTextPopup (Actor|GetComponentbyClass _characterref "/Game/FlexibleCombatSystem/Blueprints/Components/CombatTextComponent.CombatTextComponent_C") (Transformation|GetActorLocation _characterref) (Math|Float|Round (Variables|Default|GetConsumable%20Power)) "NewEnumerator13" false false false)
  (Default|UpdateManaDispatch (Actor|GetComponentbyClass (Variables|Default|GetCharacterRef) "/Game/FlexibleCombatSystem/Blueprints/Components/ResourceComponent.ResourceComponent_C")))