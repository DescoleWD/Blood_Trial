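; BP_Teleport is a paired teleporter that moves a BP_MainBase actor overlapping its box to a linked teleporter's exit point.
; Each overlap searches all BP_Teleport actors for one with the same TeleportIndex and the opposite Entrance flag, so travel works both ways.
; The actor is then set to that partner's ExitRef location without sweeping.
; The construction script positions the Teleport component and ExitRef from instance variables.
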(event OnComponentBeginOverlap(Box)
  (params (OverlappedComponent :type Primitive%20Component%20Object%20Reference) (OtherActor :type Actor%20Object%20Reference) (OtherComp :type Primitive%20Component%20Object%20Reference) (OtherBodyIndex :type Integer) (bFromSweep :type Boolean) (SweepResult :type Hit%20Result%20Structure%20%28by%20ref%29))
  (bind _asbp_main_character (Utilities|Casting|CastToBP_MainBase OtherActor))
  (if (Variables|Default|GetEntrance?)
    (bind _outactors (Actor|GetAllActorsOfClass "BP_Teleport_C"))
    (bind _array_element (Utilities|Array|ForEachLoopwithBreak _outactors :!label _label)
      (:LoopBody
        (if (and (== (Variables|BP_Teleport_C|GetTeleport%20Index _array_element) (Variables|Default|GetTeleport%20Index)) (not (Variables|BP_Teleport_C|GetEntrance? _array_element)))
          (goto _label Break)))
      (:Completed
        (Transformation|SetActorLocation _asbp_main_character (Transformation|GetWorldLocation (Variables|BP_Teleport_C|GetExit%20Ref _array_element)) false false)))
    (else
      (bind _outactors_2 (Actor|GetAllActorsOfClass "BP_Teleport_C"))
      (bind _array_element_2 (Utilities|Array|ForEachLoopwithBreak _outactors_2 :!label _label_2)
        (:LoopBody
          (if (and (== (Variables|BP_Teleport_C|GetTeleport%20Index _array_element_2) (Variables|Default|GetTeleport%20Index)) (and (not (Variables|Default|GetEntrance?)) (Variables|BP_Teleport_C|GetEntrance? _array_element_2)))
            (goto _label_2 Break)))
        (:Completed
          (Transformation|SetActorLocation _asbp_main_character (Transformation|GetWorldLocation (Variables|BP_Teleport_C|GetExit%20Ref _array_element_2)) false false))))))

(fn ConstructionScript
  ;[1 1 1] Set Enter And Exit Location
  (Transformation|SetRelativeTransform (Variables|Default|GetTeleport) (Variables|Default|GetTeleport%20Transform) false false)
  (Transformation|SetRelativeLocation (Variables|Default|GetExit%20Ref) (Variables|Default|GetExit%20Location) false false))