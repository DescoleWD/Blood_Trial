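; BP_TargetingDummy is a demo Blueprint that, going by its name, serves as an inert dummy for targeting.
; It stubs a set of character query functions covering combat state, assassination, movement and component access, which look like interface implementations.
; Each returns a false, zero, empty or fixed default, so the dummy reports itself as alive, non-player, stationary, unarmed and unassassinable.
; Its event graph and construction script contain no logic.
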(event EventBeginPlay)

(event Collision|EventActorBeginOverlap
  (params (OtherActor :type Actor%20Object%20Reference)))

(event EventTick
  (params (DeltaSeconds :type Float%20%28single-precision%29)))

(fn ConstructionScript)

(fn CanbeAssassinated
  (return false))

(fn FindAvailableAssassinationCam
  (return 0))

(fn GetWeaponRange
  (return 0.0))

(fn IsDead
  (return false))

(fn IsFacingEnemy?
  (return false))

(fn IsMoving?
  (return false))

(fn IsPlayer?
  (return false))

(fn IsWeaponDrawn?
  (return false))

(fn PassArmorMeshes
  (return 0 0 0 0 0 0 0 0 0 0 0))

(fn PassAssassinationComps
  (return 0 0))

(fn PassCamera
  (return 0 0))

(fn PassMovementMode
  (return "MOVE_None"))

(fn RetrievePlayerStatus
  (return false "NewEnumerator2" "NewEnumerator0"))

(fn UpdateMovementMode
  (params (MovementMode :type EMovementMode%20Enum :default "MOVE_None"))
  (return false))