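; Blueprint interface for AI in a prototype rework, declaring getter-style "Pass" functions through which other Blueprints can query an implementer without casting.
; Its functions cover the behaviour tree, warning mesh, spline, health HUD, weapon range, attack style and attack-style switching.
; It holds only default stubs; range returns a float, attack style an enum and the switch a boolean, with actual behaviour left to implementers.
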(fn PassBehaviourTree
  (return 0))

(fn PassWarningMesh
  (return 0))

(fn PassSpline
  (return 0))

(fn PassHealthHUD
  (return 0))

(fn PassWeaponRange
  (return 0.0))

(fn PassAttackStyle
  (return "NewEnumerator7"))

(fn PassSwitchAttackStyle
  (return false))