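; Boss-test projectile actor that receives particle positions from its Shoot Niagara effect to test for hits on the player.
; BeginPlay registers the actor as the effect's "BPcallBack" object, so exported particle data arrives in the ParticleData event.
; Each particle position gets a small debug-drawn sphere trace, compared against the player character.
; The hit branch is empty, so no damage or other response happens yet.
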(event EventBeginPlay
  (Niagara|SetNiagaraVariable(Object) (Variables|Default|GetShoot) "BPcallBack" self))

(event Collision|EventActorBeginOverlap
  (params (OtherActor :type Actor%20Object%20Reference)))

(event EventTick
  (params (DeltaSeconds :type Float%20%28single-precision%29)))

(event EventParticleData
  (params (Data :type Array%20of%20Basic%20Particle%20Data%20Structures) (NiagaraSystem :type Niagara%20System%20Object%20Reference) (SimulationPositionOffset :type Vector%20%28by%20ref%29 :default "0, 0, 0"))
  (for _array_element Data
    (bind _outhit (Collision|SphereTraceByChannel (.Position (Utilities|Struct|BreakBasicParticleData _array_element)) (.Position (Utilities|Struct|BreakBasicParticleData _array_element)) 25.0 "TraceTypeQuery4" false 0 "ForDuration" true "(R=1.000000,G=0.000000,B=0.000000,A=1.000000)" "(R=0.000000,G=1.000000,B=0.000000,A=1.000000)" 0.2))
    (if (== (.HitActor (Collision|BreakHitResult _outhit)) (Game|GetPlayerCharacter 0))
      _)))

(fn ConstructionScript)