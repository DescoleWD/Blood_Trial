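; BP_FlorianCharacter_Child is a prototype child character that adds a ranged basic attack and lever interaction.
; Pressing BasicAttack spawns an actor at the SpawnBloodWaves component, rotated to the movement component's last update rotation.
; The same press calls LeverActive on the BP_Levier found by GetActorOfClass if InLever is set.
; NearTheLever sets InLever to true, and nothing in this file clears it.
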(event Custom|NearTheLever
  (Variables|Default|SetInLever? true))

(event Input|ActionEvents|InputActionBasicAttack
  (params (Key :type Key%20Structure :default "None"))
  (:Pressed
    (Utilities|FlowControl|Sequence
      (:then_0
        (Game|SpawnActorfromClass "/Game/Proto/Proto_Florian/Blueprints/BP_Blood_Waves.BP_Blood_Waves_C" (Math|Transform|MakeTransform (Transformation|GetWorldLocation (Variables|Default|GetSpawnBloodWaves)) (Class|CharacterMovementComponent|GetLastUpdateRotation (Variables|Character|GetCharacterMovement))) "Undefined" 0 0))
      (:then_1
        (if (Variables|Default|GetInLever?)
          (bind _returnvalue (Actor|GetActorOfClass "/Game/Proto/Proto_Florian/Blueprints/BP_Levier.BP_Levier_C"))
          (Default|LeverActive _returnvalue))))))

(fn ConstructionScript
  (|CallParentFunction))