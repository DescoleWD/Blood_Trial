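; Prototype difficulty selector actor that lets the player trigger the Menu_Paris_Sang menu from inside a trigger zone.
; Box overlap begin and end toggle the Widget's visibility and the CanTrial flag, without filtering the overlapping actor.
; Pressing R1 prints a debug "Hello", then creates the menu widget if CanTrial is set, though it never adds it to the viewport here.
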(event OnComponentBeginOverlap(Box)
  (params (OverlappedComponent :type Primitive%20Component%20Object%20Reference) (OtherActor :type Actor%20Object%20Reference) (OtherComp :type Primitive%20Component%20Object%20Reference) (OtherBodyIndex :type Integer) (bFromSweep :type Boolean) (SweepResult :type Hit%20Result%20Structure%20%28by%20ref%29))
  (Rendering|SetVisibility (Variables|Default|GetWidget) true false)
  (Variables|Default|SetCanTrial true))

(event OnComponentEndOverlap(Box)
  (params (OverlappedComponent :type Primitive%20Component%20Object%20Reference) (OtherActor :type Actor%20Object%20Reference) (OtherComp :type Primitive%20Component%20Object%20Reference) (OtherBodyIndex :type Integer))
  (Rendering|SetVisibility (Variables|Default|GetWidget) false false)
  (Variables|Default|SetCanTrial false))

(event EventBeginPlay)

(event Collision|EventActorBeginOverlap
  (params (OtherActor :type Actor%20Object%20Reference)))

(event EventTick
  (params (DeltaSeconds :type Float%20%28single-precision%29)))

(event Input|ActionEvents|InputActionR1
  (params (Key :type Key%20Structure :default "None"))
  (:Pressed
    (Development|PrintString "Hello")
    (if (Variables|Default|GetCanTrial)
      (UserInterface|CreateWidget "/Game/Proto/Proto_Guillaume/Blueprints/DifficultySystem/Menu_Paris_Sang.Menu_Paris_Sang_C"))))

(fn ConstructionScript)