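; Base NPC Blueprint for interactive characters that offer dialogue, vendor trading, skill training and quests.
; Interact fades through a black-screen widget, locks player movement, runs DialogueComponent and faces the player toward the NPC under its camera.
; Events open shop, trainer or quest components, activate linked actors, play montages and move the camera along transition paths.
; Construction script drives modular equipment meshes via master pose, with optional custom meshes.
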(event Custom|BeginDialogue
  (bind _returnvalue (Game|GetPlayerController 0))
  ;[1 1 1] Update Camera & Player Position - Initiate Dialogue
  (Variables|/Script/Engine.PlayerController|SetbShowMouseCursor _returnvalue true)
  (Input|SetInputModeUIOnly _returnvalue 0 "DoNotLock")
  (Pawn|Components|CharacterMovement|DisableMovement (Variables|/Script/Engine.Character|GetCharacterMovement (Game|GetPlayerCharacter 0)))
  (Utilities|TransitionScreen
    (:Completed
      (CallFunction|RunDialogue)
      (CallFunction|SetupConversationCam))))

(event Custom|SetupQuest
  ;[1 1 1 1 30] NPC Quest
  ;;[1 1 1] Called On Begin Play - Loads The Correct Mesh For Quest Givers/Receivers
  (Default|SetupQuest (Variables|Default|GetQuestComponent) self (Variables|SetupinGame|GetQuestsToOffer)))

(event EventBeginPlay
  ;[1 1 1] Begin Play
  (Utilities|IsValid (Variables|Default|GetQuestComponent)
    (:Is%20Valid
      (Utilities|FlowControl|Delay 0.2)
      (CallFunction|SetupQuest))))

(event EventBeginTraining
  ;[1 1 1 1 30] NPC Skill Trainer
  (Default|Setup (Variables|Default|GetSkillTrainerComponent) (Variables|Default|GetCharacterRef) (Variables|SetupInGame|GetAbilityTrainerInfo))
  (Class|IPlayerController|ToggleSpellTrainer(Message) (Game|GetPlayerController 0))
  (Class|IPlayerController|ShowHUD(Message) (Game|GetPlayerController 0)))

(event EventEndTrading
  ;[1 1 1 1 30] NPC Shop
  (Utilities|TransitionScreen
    (:Completed
      (Class|IPlayerController|ToggleExternalInventory(Message) (Game|GetPlayerController 0) (Variables|Default|GetInventoryComponent) self true)
      (CallFunction|ReturnCameraandSettings))))

(event EventActivateActor
  (params (ActorToActivate :type Integer))
  ;[1 1 1 1 30] NPC Activate Actor
  (Class|IItemInterface|ActivateActor(Message) (Utilities|Array|Get(acopy) (Variables|SetupInGame|GetActorsToActivate) (- ActorToActivate 1))))

(event EventPlayAnimation
  (params (Montage :type Anim%20Montage%20Object%20Reference))
  ;[1 1 1] Play Montage
  (Animation|Montage|PlayMontage (Variables|Character|GetMesh) Montage))

(event EventEndTraining
  ;[1 1 1 1 30] NPC Skill Trainer
  (Utilities|TransitionScreen
    (:Completed
      (Class|IPlayerController|ToggleSpellTrainer(Message) (Game|GetPlayerController 0))
      (CallFunction|ReturnCameraandSettings))))

(event EventTransitionCamera
  (params (Transition :type Integer))
  (bind _camerastartlocation (Variables|Default|GetCameraStartLocation))
  ;[1 1 1] Camera Transitions
  (if (not (Variables|Default|GetMidCameraMovement))
    (Variables|Default|SetCameraTransition Transition)
    (if (Variables|/Game/FlexibleCombatSystem/Blueprints/Miscellaneous/BP_PatrolPath.BP_PatrolPath_C|GetComplete (Utilities|Array|Get(acopy) (Variables|SetupInGame|GetCameraTransitionPath) (Variables|Default|GetCameraTransition)))
      (Utilities|FlowControl|Sequence
        (:then_0
          (Components|MoveComponentTo (Variables|Default|GetCamera) (.location _camerastartlocation) (.rotation _camerastartlocation) true true (Variables|Default|GetOver%20Time) true))
        (:then_1
          ;;[1 1 1] In case Camera Bugs out, Guarantee Dialogue End
          (Utilities|FlowControl|Delay (Variables|Default|GetOver%20Time))
          (Variables|/Game/FlexibleCombatSystem/Blueprints/Components/DialogueComponent.DialogueComponent_C|SetMidCameraTransition (Variables|Default|GetDialogueComponent) false)))
      (else
        (Variables|Default|SetCameraCurrentTransform (Transformation|GetWorldTransform (Variables|Default|GetCamera)))
        (Variables|Default|SetMidCameraMovement true)
        (bind _newtrack_0 (Timeline|MoveCamera PlayFromStart)
          (:Update
            (Transformation|SetWorldTransform (Variables|Default|GetCamera) (Math|Transform|Lerp(Transform) (Variables|Default|GetCameraCurrentTransform) (Variables|/Game/FlexibleCombatSystem/Blueprints/Miscellaneous/BP_PatrolPath.BP_PatrolPath_C|GetSplinePointTransform (Utilities|Array|Get(acopy) (Variables|SetupInGame|GetCameraTransitionPath) (Variables|Default|GetCameraTransition))) _newtrack_0) false false))
          (:Finished
            (Default|UpdatePatrolSequence (Utilities|Array|Get(acopy) (Variables|SetupInGame|GetCameraTransitionPath) (Variables|Default|GetCameraTransition)))
            (Variables|Default|SetMidCameraMovement false)
            (Class|INPC|ActivateActor(Message) self (Utilities|Struct|BreakS_DialogueInfo (Variables|/Game/FlexibleCombatSystem/Blueprints/Components/DialogueComponent.DialogueComponent_C|GetDialogueLineInfo (Variables|Default|GetDialogueComponent))))))))))

(event EventTriggerQuest
  ;[1 1 1 1 30] NPC Quest
  ;;[1 1 1] Triggered From Dialogue Component
  (Default|OpenQuest (Variables|Default|GetQuestComponent) (Utilities|Array|Get(acopy) (Variables|SetupInGame|GetActorsToActivate) (- (Variables|Default|GetActor%20to%20Activate) 1))))

(event EventInteract
  (params (Character :type Character%20Object%20Reference))
  ;[1 1 1] Interact
  (Variables|Default|SetCharacterRef Character)
  (CallFunction|BeginDialogue)
  (CallFunction|IsQuestActor (Game|GetPlayerController 0) 1))

(event EventEndConversation
  ;[1 1 1] End Chat
  (Utilities|TransitionScreen
    (:Completed
      (CallFunction|ReturnCameraandSettings)
      (Class|IPlayerController|ShowHUD(Message) (Game|GetPlayerController 0)))))

(event EventBeginTrading
  ;[1 1 1 1 30] NPC Shop
  (Class|IPlayerController|ToggleExternalInventory(Message) (Game|GetPlayerController 0) (Variables|Default|GetInventoryComponent) self true)
  (Class|IPlayerController|ShowHUD(Message) (Game|GetPlayerController 0)))

(fn ConstructionScript
  (bind _customequipment (Variables|SetupInGame|GetCustomEquipment))
  (bind (_usecustomequipment _chest _hands _legs _boots _back _helmet _shoulder) (Utilities|Struct|BreakS_Custom_AI_Equipment _customequipment))
  (Class|SkinnedMeshComponent|SetMasterPoseComponent (Variables|Default|GetHelmet) (Variables|Character|GetMesh) false)
  (if _usecustomequipment
    (for (_array_element _array_index) (Utilities|Array|MakeArray (Variables|Default|GetChest) (Variables|Default|GetHands) (Variables|Default|GetLegs) (Variables|Default|GetBoots) (Variables|Default|GetBack) (Variables|Default|GetHelmet) (Variables|Default|GetShoulder))
      (Class|SkinnedMeshComponent|SetSkeletalMesh _array_element (Utilities|Array|Get(acopy) (Utilities|Array|MakeArray _chest _hands _legs _boots _back _helmet _shoulder) _array_index) true))))

(fn RunDialogue
  (Class|IPlayerController|HideHUD(Message) (Game|GetPlayerController 0))
  (Default|BeginDialogue (Variables|Default|GetDialogueComponent) (Variables|SetupInGame|GetNPC%20Dialogue) (Variables|SetupInGame|GetNPC_Name)))

(fn SetupConversationCam
  (bind _returnvalue (Transformation|GetActorRotation))
  ;[1 1 1] Adjust Camera & Player Position
  (Game|Player|SetViewTargetwithBlend (Game|GetPlayerController 0) (Components|GetOwner (Variables|Default|GetCamera)) 0.0 "VTBlend_Linear" 0.0 false)
  (Transformation|SetActorTransform (Variables|Default|GetCharacterRef) (Math|Transform|MakeTransform (+ (Transformation|GetActorLocation) (* (Transformation|GetActorForwardVector) 1.5e+02)) (Math|Rotator|MakeRotator (.roll _returnvalue) (.pitch _returnvalue) (+ (.yaw _returnvalue) 1.8e+02)))))

(fn ReturnCameraandSettings
  (bind _returnvalue (Game|GetPlayerController 0))
  (bind _camera (Class|ICharacter|PassCamera(Message) (Variables|Default|GetCharacterRef)))
  (Game|Player|SetViewTargetwithBlend (Game|GetPlayerController 0) (Components|GetOwner _camera) 0.0 "VTBlend_Linear" 0.0 false)
  (Input|SetInputModeGameOnly _returnvalue)
  (Variables|/Script/Engine.PlayerController|SetbShowMouseCursor _returnvalue false)
  (Pawn|Components|CharacterMovement|SetMovementMode (Variables|/Script/Engine.Character|GetCharacterMovement (Game|GetPlayerCharacter 0)) "MOVE_Walking" 0)
  (Class|IPlayerController|ShowHUD(Message) (Game|GetPlayerController 0))
  (Default|ShowActorTag (Variables|Default|GetLootOutlineComponent)))

(fn TransitionCam)

(fn PassActorActivateNo
  (params (ActorToActivate :type Integer))
  (Variables|Default|SetActor%20to%20Activate ActorToActivate))

(fn RetrieveInventoryInfo
  (bind _traderinfo (Variables|SetupInGame|GetTraderInfo))
  (return "NewEnumerator2" (.shopname _traderinfo) (.traderimage _traderinfo) (Variables|InventoryData|GetInventoryData) true (.traderstockdata _traderinfo) 0))

(fn RetrieveLootInfo
  (return ""))

(fn RetrieveOutlineInfo
  (return (Variables|SetupInGame|GetNPC_Name) "NewEnumerator1" (Variables|SetupInGame|GetActor%20Tag%20Type) 0 0 0 (Variables|Character|GetMesh)))