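; BP_Lava is a hazard zone that slows and damages the main character (BP_MainBase) while inside its box.
; Box overlaps subtract and restore a walk speed reduction, set an inside flag, and show or remove a Lava_Feedback HUD widget.
; While the flag is set, Tick applies the game instance's lava damage about every half second through a DoOnce reset after a delay.
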(event OnComponentBeginOverlap(Box)
  (params (OverlappedComponent :type Primitive%20Component%20Object%20Reference) (OtherActor :type Actor%20Object%20Reference) (OtherComp :type Primitive%20Component%20Object%20Reference) (OtherBodyIndex :type Integer) (bFromSweep :type Boolean) (SweepResult :type Hit%20Result%20Structure%20%28by%20ref%29))
  (bind _asbp_main_base (Utilities|Casting|CastToBP_MainBase OtherActor))
  (Variables|/Script/Engine.CharacterMovementComponent|SetMaxWalkSpeed (Variables|/Script/Engine.Character|GetCharacterMovement _asbp_main_base) (- (Variables|/Script/Engine.CharacterMovementComponent|GetMaxWalkSpeed (Variables|/Script/Engine.Character|GetCharacterMovement _asbp_main_base)) (Variables|Default|GetMainChara_SpeedReduction)))
  (Development|PrintString "Speed is reduced" true false "(R=1.000000,G=0.014468,B=0.000000,A=1.000000)")
  (Variables|Default|SetCharacterIn? true)
  (bind _returnvalue (Game|ConstructObjectfromClass "/Game/Proto/Main/HUD/Lava_Feedback.Lava_Feedback_C"))
  (UserInterface|Viewport|AddtoViewport _returnvalue 0)
  (Default|LavaEffectHUD _returnvalue))

(event OnComponentEndOverlap(Box)
  (params (OverlappedComponent :type Primitive%20Component%20Object%20Reference) (OtherActor :type Actor%20Object%20Reference) (OtherComp :type Primitive%20Component%20Object%20Reference) (OtherBodyIndex :type Integer))
  (bind _asbp_main_base (Utilities|Casting|CastToBP_MainBase OtherActor))
  (Variables|/Script/Engine.CharacterMovementComponent|SetMaxWalkSpeed (Variables|/Script/Engine.Character|GetCharacterMovement _asbp_main_base) (+ (Variables|/Script/Engine.CharacterMovementComponent|GetMaxWalkSpeed (Variables|/Script/Engine.Character|GetCharacterMovement _asbp_main_base)) (Variables|Default|GetMainChara_SpeedReduction)))
  (Development|PrintString "Speed is back to normal" true false "(R=0.000000,G=1.000000,B=0.016063,A=1.000000)")
  (Variables|Default|SetCharacterIn? false)
  (Widget|RemovefromParent (stale OnComponentBeginOverlap(Box) _returnvalue)))

(event EventTick
  (params (DeltaSeconds :type Float%20%28single-precision%29))
  (bind _returnvalue (Actor|GetActorOfClass "/Game/Proto/Main/Blueprint/BP_MainBase.BP_MainBase_C"))
  (if (Variables|Default|GetCharacterIn?)
    (Utilities|FlowControl|DoOnce false :!label _label
      (:Completed
        (Game|Damage|ApplyDamage _returnvalue (Variables|/Game/Proto/Main/Blueprint/Save_BFL_GameInstance/BloodTrial_GameInstance.BloodTrial_GameInstance_C|GetLavaDamage (CallFunction|GetInst)) 0 0)
        (Utilities|FlowControl|Delay 0.5)
        (Development|PrintString "SFX:Lave" true false "(R=0.000000,G=1.000000,B=0.090196,A=1.000000)")
        (goto _label Reset)))))

(fn ConstructionScript)