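; Player melee component that plays a cycling series of attack montages on its owning Character.
; Montage notifies open and close the combo window through CanAttaque and fire the hit check.
; Hits use a sphere trace between weapon sockets, then report AI damage, apply damage and spawn Niagara FX.
; A separate combo counter resets after a retriggerable delay; jump-attack and box-trace logic are disconnected.
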(event Custom|Attaque
  (if (Variables|Default|GetCanAttaque)
    (Variables|Default|SetCanAttaque false)
    ;[1 0 0] Si et seulement si on prévoit des saut et donc des attattaques aériennes
    (if true
      (bind _notifyname (Animation|Montage|PlayMontage (Variables|/Script/Engine.Character|GetMesh (Variables|Default|GetOwner)) (Utilities|Array|Get(acopy) (Variables|Default|GetAnimationAttaque_V2) (Variables|Default|GetAttaqueIndexCurrent)))
        (:then
          ;[1 1 1] Increment Int attack + Compare to Max attack
          (Variables|Default|SetAttaqueIndexCurrent (Math|Integer|SelectInt (+ (Variables|Default|GetAttaqueIndexCurrent) 1) 0 (< (Variables|Default|GetAttaqueIndexCurrent) (Variables|Default|GetAttaqueIndexMax)))))
        (:OnCompleted
          ;[1 1 1] Can Attaque again - set index =0 (wtf with le set ?)
          (Variables|Default|SetCanAttaque true :!label _label))
        (:OnInterrupted
          (goto _label))
        (:OnNotifyBegin
          ;[1 1 1] Call Notify
          (switch name _notifyname
            (:Hit
              (CallFunction|TriggerComplexeHit))
            (:CanCombo
              (Variables|Default|SetCanAttaque true))
            (:Recovery
              (Variables|Default|SetCanAttaque false))))))))

(event Custom|GroundCheck
  ;[1 0 0] Si et seulement si on prévoit des saut et donc des attattaques aériennes
  (if (AI|Components|NavMovement|IsMovingonGround (Variables|/Script/Engine.Character|GetCharacterMovement (Variables|Default|GetOwner)))
    (Animation|StopAnimMontage (Variables|Default|GetOwner) (Variables|Default|GetJumpAttaqueAnim))
    (Variables|Default|SetCanAttaque true)
    (Utilities|Time|ClearandInvalidateTimerbyHandle (Variables|Default|GetTimeGroundCheck))))

(event Custom|IncrementCombo
  (Math|Integer|IncrementInt (Variables|Default|GetComboCount)
    (:%20%20
      (Utilities|FlowControl|RetriggerableDelay 2.0)
      (Variables|Default|SetComboCount 0))))

(event EventBeginPlay
  ;[1 1 1] Check dans la liste des attaques -1 (comparaison tableau)
  (bind _ascharacter (Utilities|Casting|CastToCharacter (Components|GetOwner)))
  (Variables|Default|SetOwner _ascharacter)
  (Variables|Default|SetAttaqueIndexMax (- (Utilities|Array|Length (Variables|Default|GetAnimationAttaque_V2)) 1)))

(fn TriggerSimpleHit)

(fn TriggerComplexeHit
  (bind _damageplayer (Variables|Default|GetDamagePlayer))
  (bind _asbp_guillaume_character_child (Utilities|Casting|CastToBP_GuillaumeCharacter_Child (Variables|Default|GetOwner)))
  (bind (_outhit _returnvalue) (Collision|SphereTraceForObjects (Transformation|GetSocketLocation (Variables|/Game/Proto/Proto_Guillaume/Blueprints/Player/BP_GuillaumeCharacter_Child.BP_GuillaumeCharacter_Child_C|GetWeapon _asbp_guillaume_character_child) "SocketMelee_Start") (Transformation|GetSocketLocation (Variables|/Game/Proto/Proto_Guillaume/Blueprints/Player/BP_GuillaumeCharacter_Child.BP_GuillaumeCharacter_Child_C|GetWeapon _asbp_guillaume_character_child) "SocketMelee_End") 1e+02 (Utilities|Array|MakeArray "ObjectTypeQuery3") false 0 "None"))
  (if _returnvalue
    (if (Variables|/Script/Engine.Actor|GetbCanBeDamaged (.HitActor (Collision|BreakHitResult _outhit)))
      (Class|AISenseDamage|ReportDamageEvent (.HitActor (Collision|BreakHitResult _outhit)) _asbp_guillaume_character_child _damageplayer (.ImpactPoint (Collision|BreakHitResult _outhit)) "0, 0, 0" "None")
      (Game|Damage|ApplyDamage (.HitActor (Collision|BreakHitResult _outhit)) _damageplayer 0 0)
      ;[1 1 1] Syst template = niagara blood.etc
      (Niagara|SpawnSystematLocation "/Game/Core/Cursor/FX_Cursor.FX_Cursor" (.ImpactPoint (Collision|BreakHitResult _outhit))))))