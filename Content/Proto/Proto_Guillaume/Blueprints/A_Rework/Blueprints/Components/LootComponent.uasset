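; Loot component for chests, dead enemies and dropped containers that opens a pickup window when the player overlaps its owner.
; On BeginPlay it restores contents from the save, keyed by owner class plus start location, or builds them from a drop-chance DataTable or fixed list.
; Items fill slot widgets; emptying them marks the owner looted, destroying dropped containers and removing their saves.
; Save changes route through the GameMode.
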(event Custom|CreateLootWidget
  ;[1 1 1] Add Children To Loot Widget
  ;;[1 1 1] Remove Any Tooltips if they exist
  (for _array_element (Variables|Setup|GetWB_ItemsCreated)
    (Default|RemoveTooltip _array_element))
  ;;[1 1 1] Clear Old Loot
  (bind _loot_window (Class|IPlayerController|PassLootWindowWB(Message) (Game|GetPlayerController 0)))
  (bind _output_get (Variables|Setup|SetWB_LootWindow _loot_window))
  (Default|ClearChildren _output_get)
  (LootActor|AddItemstoLoot)
  (Utilities|FlowControl|Delay 0.1) ; When Save Game Loading Dropped Containers, Let Player Position Update
  (LootActor|SetLootWidgetPosition))

(event Custom|EventOverlap
  (params (OverlappedActor :type Actor%20Object%20Reference) (OtherActor :type Actor%20Object%20Reference))
  ;[1 1 1] Setup
  (Utilities|IsValid OtherActor
    (:Is%20Valid
      (if (Actor|ActorHasTag OtherActor "Player")
        (bind _ascharacter (Utilities|Casting|CastToCharacter OtherActor))
        (Variables|Setup|SetCharacterRef _ascharacter)
        (bind _lootready (CallFunction|LootConditions))
        (if _lootready
          (CallFunction|CreateLootWidget)
          (CallFunction|PassLoottoInventory true))))))

(event Custom|EventEndOverlap
  (params (OverlappedActor :type Actor%20Object%20Reference) (OtherActor :type Actor%20Object%20Reference))
  ;[1 1 1] Setup
  (if (Actor|ActorHasTag OtherActor "Player")
    (LootActor|CloseWindows)
    (CallFunction|PassLoottoInventory false)))

(event Custom|RemoveItem
  (params (RemoveItem :type WB%20Pickup%20Item%20Slot%20Object%20Reference%20%28by%20ref%29))
  ;[1 1 1] When Item Picked Up - Remove
  (Utilities|Array|RemoveItem (Variables|Setup|GetWB_ItemsCreated) RemoveItem)
  (Utilities|Array|RemoveItem (Variables|Setup|GetLoot%20Data) (Variables|/Game/FlexibleCombatSystem/Widgets/Looting/WB_PickupItemSlot.WB_PickupItemSlot_C|GetSlotContents RemoveItem))
  (if (== (Utilities|Array|Length (Variables|Setup|GetWB_ItemsCreated)) 0)
    (CallFunction|SetActorLooted)
    (Class|IPlayerController|ToggleLootMenu(Message) (Game|GetPlayerController 0) self)
    (Saving|RemoveLootSave)
    (LootActor|DestroyDroppedItems)))

(event EventBeginPlay
  (bind _returnvalue (Components|GetOwner))
  ;[1 1 1] Setup
  (Collision|BindEventtoOnActorBeginOverlap _returnvalue (delegate Custom|EventOverlap))
  (Collision|BindEventtoOnActorEndOverlap _returnvalue (delegate Custom|EventEndOverlap))
  (bind _lootdataexists (Saving|LoadLootSaveData))
  (if (not _lootdataexists)
    (LootActor|RetrieveLootData)))

(fn LootWorthSaving
  (CallFunction|UpdateLootData)
  ;[1 1 1] Only Add Actor To Save Once
  (if (not (Variables|SaveInfo|GetLootSaved))
    (Variables|SaveInfo|SetLootSaved true)
    ;[1 1 1] Pass Item To Game Mode For Save
    (Class|IGameMode|SaveLootChanges(Message) (Game|GetGameMode) (Components|GetOwner) (select (Variables|Status|GetDroppedLoot) "NewEnumerator3" "NewEnumerator1"))))

(fn RemoveLootSave
  ;[1 1 1] We only want to remove "Dropped Loot" Save Data. Even if an Enemy/Actor is looted we need to Save that it's been Looted. Unlike Dropped Loot which we destroy when its looted
  (if (Variables|Status|GetDroppedLoot)
    (Class|IGameMode|RemoveLootChangesSave(Message) (Game|GetGameMode) (Components|GetOwner))
    (else
      (CallFunction|UpdateLootData))))

(fn SetLootWidgetPosition
  (bind _returnvalue (Game|GetPlayerController 0))
  (bind _wb_lootwindow (Variables|Setup|GetWB_LootWindow))
  (bind _characterref (Variables|Setup|GetCharacterRef))
  (bind _returnvalue_2 (Transformation|GetActorLocation _characterref))
  (bind _screenposition (Class|WidgetLayoutLibrary|ProjectWorldLocationtoWidgetPosition _returnvalue _returnvalue_2 false))
  (Utilities|IsValid _characterref
    (:Is%20Valid
      ;[1 1 1] Character Ref Exists, Display At Character Location With Offset
      (Class|CanvasPanelSlot|SetPosition (Class|WidgetLayoutLibrary|SlotasCanvasSlot _wb_lootwindow) (Math|Vector2D|MakeVector2D (+ (.x _screenposition) 2e+02) (+ (.y _screenposition) -3e+02))))
    (:Is%20Not%20Valid
      ;[1 1 1] If Character Ref Doesn't Exist (Dropped Container) - Show In Middle of Screen
      (bind _returnvalue_3 (Settings|GetGameUserSettings))
      (Class|UserWidget|SetPositioninViewport _wb_lootwindow (Math|Vector2D|MakeVector2D (Math|Conversions|ToFloat(Integer) (/ (.x (Class|GameUserSettings|GetScreenResolution _returnvalue_3)) 4)) (Math|Conversions|ToFloat(Integer) (/ (.y (Class|GameUserSettings|GetScreenResolution _returnvalue_3)) 4))) true))))

(fn AddItemstoLoot
  ;[1 1 1] Add Pieces Of Loot
  (Utilities|Array|Clear (Variables|Setup|GetWB_ItemsCreated))
  (for _array_element (Variables|Setup|GetLoot%20Data)
    (bind _returnvalue (UserInterface|CreateWidget "/Game/FlexibleCombatSystem/Widgets/Looting/WB_PickupItemSlot.WB_PickupItemSlot_C" 0 (Variables|Setup|GetCharacterRef) self))
    (Variables|/Game/FlexibleCombatSystem/Widgets/Looting/WB_PickupItemSlot.WB_PickupItemSlot_C|SetSlotContents _returnvalue _array_element)
    (Utilities|Array|Add (Variables|Setup|GetWB_ItemsCreated) _returnvalue)
    (Class|VerticalBox|AddChildtoVerticalBox (Variables|/Game/FlexibleCombatSystem/Widgets/Looting/WB_LootWindow.WB_LootWindow_C|GetInventoryGrid (Variables|Setup|GetWB_LootWindow)) _returnvalue)))

(fn CloseWindows
  (bind _lootmenuopen (Class|IPlayerController|LootMenuStatus(Message) (Game|GetPlayerController 0)))
  (if _lootmenuopen
    (Class|IPlayerController|ToggleLootMenu(Message) (Game|GetPlayerController 0) self)
    (Class|ILootInterface|ToggleAnimation(Message) (Components|GetOwner))))

(fn LoadLootSaveData
  ;[1 1 1] Updates Data Over To Save Data If Data Exists
  (Variables|Default|SetStartLocation (Transformation|GetActorLocation (Components|GetOwner)))
  (Variables|Default|SetLootOutlineComp (Actor|GetComponentbyClass (Components|GetOwner) "/Game/FlexibleCombatSystem/Blueprints/Components/OutlineComponent.OutlineComponent_C"))
  (bind _returnvalue (SaveGame|LoadGamefromSlot "save1"))
  (bind _asbp_save_game (Utilities|Casting|CastToBP_SaveGame _returnvalue))
  (for _array_element (Variables|/Game/FlexibleCombatSystem/Blueprints/BP_SaveGame.BP_SaveGame_C|GetLootSaveData _asbp_save_game)
    (if (Utilities|Enum|Equal(Enum) (.uniqueidentifier _array_element) (Utilities|String|Append (Utilities|GetClassDisplayName (Utilities|GetClass (Components|GetOwner))) (Utilities|String|ToString(Vector) (Variables|Default|GetStartLocation))))
      (LocalVariables|SetLootDataExist true)
      (Variables|Setup|SetLoot%20Data (.lootinfo _array_element))))
  (if (LocalVariables|GetLootDataExist)
    (if (== (Utilities|Array|Length (Variables|Setup|GetLoot%20Data)) 0)
      (CallFunction|SetActorLooted))
    (return true)
    (else
      (return false))))

(fn AddLootDataRemake
  (params (NewItem :type S%20Slot%20Info%20Structure%20%28by%20ref%29))
  (bind (_itemstructure _datatableinfo _quantity _slotnumber _itemid) (Utilities|Struct|BreakS_SlotInfo NewItem))
  ;[1 1 1] Comment
  (Utilities|Array|Add (Variables|Setup|GetLoot%20Data) (Utilities|Struct|MakeS_SlotInfo _itemstructure "(DataTable=None,RowName=\"\")" _quantity (- (Utilities|Array|Length (Variables|Setup|GetLoot%20Data)) 1) _itemid))
  (CallFunction|CreateLootWidget))

(fn DestroyDroppedItems
  (if (Variables|Status|GetDroppedLoot)
    (if (== (Utilities|Array|Length (Variables|Setup|GetLoot%20Data)) 0)
      (Actor|DestroyActor (Components|GetOwner)))))

(fn SetActorLooted
  (bind _lootoutlinecomp (Variables|Default|GetLootOutlineComp))
  ;[1 1 1] Whether the Actor Tag Can Pop up - Don't Show if Looted
  (Utilities|IsValid _lootoutlinecomp
    (:Is%20Valid
      (Default|SendActorLooted _lootoutlinecomp))
    (:Is%20Not%20Valid
      _))
  (Variables|Status|SetActorLooted true))

(fn LootConditions
  (bind _returnvalue (Components|GetOwner))
  (if (Variables|Status|GetActorLooted)
    (return false)
    (elif (Actor|ActorHasTag _returnvalue "EnemyAI")
      (bind _dead (Class|ICharacter|IsDead(Message) _returnvalue))
      (return _dead)
      (else
        (return true)))))

(fn RetrieveLootData
  (bind _returnvalue (Components|GetOwner))
  (Utilities|Array|Clear (Variables|Setup|GetLoot%20Data))
  (Variables|Default|SetLootOutlineComp (Actor|GetComponentbyClass _returnvalue "/Game/FlexibleCombatSystem/Blueprints/Components/OutlineComponent.OutlineComponent_C"))
  (bind _lootsetupinfo (Class|ILootInterface|RetrieveLootInfo(Message) _returnvalue))
  (if (.UseDataTable (Utilities|Struct|BreakS_LootSetupInfo _lootsetupinfo))
    ;[1 1 1] Sets Pre-Set Items From Data Table
    ;;[1 1 1] Scan through every DataTable Row
    (bind _outrownames (DataTable|GetDataTableRowNames (.DataTableLoot (Utilities|Struct|BreakS_LootSetupInfo _lootsetupinfo))))
    (for _array_element _outrownames
      ;;[1 1 1] Output Data Row Information
      (bind _returnvalue_2 (Utilities|GetDataTableRow (.DataTableLoot (Utilities|Struct|BreakS_LootSetupInfo _lootsetupinfo)) _array_element)
        (:then
          ;;[1 1 1] Output ItemData Info
          (bind _returnvalue_3 (Utilities|GetDataTableRow (.DataTable (Utilities|Struct|BreakDataTableRowHandle (.DataTableInfo (Utilities|Struct|BreakS_ItemSetupData _returnvalue_2)))) (.RowName (Utilities|Struct|BreakDataTableRowHandle (.DataTableInfo (Utilities|Struct|BreakS_ItemSetupData _returnvalue_2)))))
            (:then
              ;;[1 1 1] IF Loot Drop Chance Is Success, Add To Loot
              (if (< (Math|Random|RandomFloatinRange 0.0 1e+02) (Utilities|Struct|BreakS_LootingInfo (Utilities|Struct|BreakS_ItemData _returnvalue_3)))
                (Utilities|Array|Add (Variables|Setup|GetLoot%20Data) (Utilities|Struct|MakeS_SlotInfo _returnvalue_3 (.DataTableInfo (Utilities|Struct|BreakS_ItemSetupData _returnvalue_2)) (select (.RandomizeQuantity (Utilities|Struct|BreakS_QuantityOptions (.Quantity (Utilities|Struct|BreakS_ItemSetupData _returnvalue_2)))) (Math|Random|RandomIntegerinRange (.QuantityMin (Utilities|Struct|BreakS_QuantityOptions (.Quantity (Utilities|Struct|BreakS_ItemSetupData _returnvalue_2)))) (.QuantityMax (Utilities|Struct|BreakS_QuantityOptions (.Quantity (Utilities|Struct|BreakS_ItemSetupData _returnvalue_2))))) (.Quantity (Utilities|Struct|BreakS_QuantityOptions (.Quantity (Utilities|Struct|BreakS_ItemSetupData _returnvalue_2)))))))))))))
    ;;[1 1 1] Set Looted If No Data
    (if (== (Utilities|Array|Length (Variables|Setup|GetLoot%20Data)) 0)
      (CallFunction|SetActorLooted))
    (else
      ;[1 1 1] Sets Specific Loot (Set In Details)
      ;;[1 1 1] For Each Piece Of Loot Listed
      (bind _output_get (Variables|Setup|SetLootSetup (.PiecesOfLoot (Utilities|Struct|BreakS_LootSetupInfo _lootsetupinfo))))
      (for _array_element_2 _output_get
        ;;[1 1 1] Get Actual Data From ItemData Storage DT
        (Utilities|IsValid (.DataTable (Utilities|Struct|BreakDataTableRowHandle (.DataTableInfo (Utilities|Struct|BreakS_ItemSetupData _array_element_2))))
          (:Is%20Valid
            (bind _returnvalue_4 (Utilities|GetDataTableRow (.DataTable (Utilities|Struct|BreakDataTableRowHandle (.DataTableInfo (Utilities|Struct|BreakS_ItemSetupData _array_element_2)))) (.RowName (Utilities|Struct|BreakDataTableRowHandle (.DataTableInfo (Utilities|Struct|BreakS_ItemSetupData _array_element_2)))))
              (:then
                (Utilities|Array|Add (Variables|Setup|GetLoot%20Data) (Utilities|Struct|MakeS_SlotInfo _returnvalue_4 (.DataTableInfo (Utilities|Struct|BreakS_ItemSetupData _array_element_2)) (select (.RandomizeQuantity (Utilities|Struct|BreakS_QuantityOptions (.Quantity (Utilities|Struct|BreakS_ItemSetupData _array_element_2)))) (Math|Random|RandomIntegerinRange (.QuantityMin (Utilities|Struct|BreakS_QuantityOptions (.Quantity (Utilities|Struct|BreakS_ItemSetupData _array_element_2)))) (.QuantityMax (Utilities|Struct|BreakS_QuantityOptions (.Quantity (Utilities|Struct|BreakS_ItemSetupData _array_element_2))))) (.Quantity (Utilities|Struct|BreakS_QuantityOptions (.Quantity (Utilities|Struct|BreakS_ItemSetupData _array_element_2))))))))))))
      ;;[1 1 1] Set Looted If No Data
      (if (== (Utilities|Array|Length (Variables|Setup|GetLoot%20Data)) 0)
        (CallFunction|SetActorLooted)))))

(fn PassLoottoInventory
  (params (ToggleOn :type Boolean))
  (bind _asbp_loot_actor_parent (Utilities|Casting|CastToBP_LootActorParent (Components|GetOwner)))
  (Utilities|IsValid _asbp_loot_actor_parent
    (:Is%20Valid
      (Default|DroppedItemToggle _asbp_loot_actor_parent ToggleOn))))

(fn UpdateLootData
  ;[1 1 1] Setup Loot Variable For Game Mode To Save With
  (Variables|SaveInfo|SetLootSaveData (Utilities|Struct|MakeS_LootSaveData (Utilities|String|Append (Utilities|GetClassDisplayName (Utilities|GetClass (Components|GetOwner))) (Utilities|String|ToString(Vector) (Variables|Default|GetStartLocation))) (Variables|Setup|GetLoot%20Data))))