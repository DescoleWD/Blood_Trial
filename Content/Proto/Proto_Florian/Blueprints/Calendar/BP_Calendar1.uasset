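; BP_Calendar1 is a one-time calendar piece pickup that adds to score and calendar piece count.
; Its mesh rotates back and forth continuously through looping MoveComponentTo calls.
; When BP_MainBase overlaps the sphere, it plays a sound, disables collision, swaps material, animates and destroys itself, while notifying that actor.
; A CalendarObtain1 flag on the game instance records collection, so BeginPlay removes the pickup if already obtained.
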(event OnComponentBeginOverlap(Sphere)
  (params (OverlappedComponent :type Primitive%20Component%20Object%20Reference) (OtherActor :type Actor%20Object%20Reference) (OtherComp :type Primitive%20Component%20Object%20Reference) (OtherBodyIndex :type Integer) (bFromSweep :type Boolean) (SweepResult :type Hit%20Result%20Structure%20%28by%20ref%29))
  (bind _asblood_trial_game_instance (CallFunction|GetInst))
  (bind _asbp_main_base (Utilities|Casting|CastToBP_MainBase OtherActor))
  (Utilities|FlowControl|Sequence
    (:then_0
      (Audio|PlaySound2D "/Game/Proto/Proto_Florian/SFX/Calendar.Calendar" 1.0 1.0 0.0 0 0)
      (Collision|SetCollisionEnabled (Variables|Default|GetStaticMesh) "NoCollision")
      (Rendering|Material|SetMaterial (Variables|Default|GetStaticMesh) 0 "/Game/Core/Textures/Key_Mat_Inst1.Key_Mat_Inst1")
      (Components|MoveComponentTo (Variables|Default|GetStaticMesh) "0, 0, 0" "0, 0, 0" true true 0.01 false)
      (Components|MoveComponentTo (Variables|Default|GetStaticMesh) "0, 0,180.000000" "0,180.000000, 0" true true 0.5 false)
      (Actor|DestroyActor))
    (:then_1
      (CallFunction|IncrScore (Variables|/Game/Proto/Main/Blueprint/Save_BFL_GameInstance/BloodTrial_GameInstance.BloodTrial_GameInstance_C|GetScore_Calendar _asblood_trial_game_instance))
      (CallFunction|IncrCalendarPieces (Variables|/Game/Proto/Main/Blueprint/Save_BFL_GameInstance/BloodTrial_GameInstance.BloodTrial_GameInstance_C|GetCalendar_Pieces _asblood_trial_game_instance))
      (Default|CalendarReceived _asbp_main_base)
      (Variables|/Game/Proto/Main/Blueprint/Save_BFL_GameInstance/BloodTrial_GameInstance.BloodTrial_GameInstance_C|SetCalendarObtain1 _asblood_trial_game_instance true))))

(event EventBeginPlay
  (Utilities|FlowControl|Sequence
    (:then_0
      (Components|MoveComponentTo (Variables|Default|GetStaticMesh) "0, 0, 0" "0,180.000000, 0" false false 5.0 false :!label _label)
      (Components|MoveComponentTo (Variables|Default|GetStaticMesh) "0, 0, 0" "0, 0, 0" false false 5.0 false)
      (goto _label))
    (:then_1
      (if (Variables|/Game/Proto/Main/Blueprint/Save_BFL_GameInstance/BloodTrial_GameInstance.BloodTrial_GameInstance_C|GetCalendarObtain1 (CallFunction|GetInst))
        (Actor|DestroyActor)))))

(fn ConstructionScript)