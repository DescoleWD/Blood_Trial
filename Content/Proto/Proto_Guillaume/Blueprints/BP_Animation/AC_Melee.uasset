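; Prototype melee combo component for a Character, playing the next montage from an attack list each time Attaque fires.
; Montage notifies trigger hits and open or close the combo window; the index wraps after the last attack.
; Hits use a forward box trace on Pawns that applies damage and spawns Niagara FX.
; Jump attack, index reset on completion and input toggling are unwired; Tick prints the index for debugging.
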(event Custom|Attaque
  (if (Variables|Default|GetCanAttaque)
    (Variables|Default|SetCanAttaque false)
    ;[1 0 0] Si et seulement si on prévoit des saut et donc des attattaques aériennes
    (if true
      (bind _notifyname (Animation|Montage|PlayMontage (Variables|/Script/Engine.Character|GetMesh (Variables|Default|GetOwner)) (Utilities|Array|Get(acopy) (Variables|Default|GetAnimationAttaque) (Variables|Default|GetAttaqueIndexCurrent)))
        (:then
          ;[1 1 1] Increment Int attack + Compare to Max attack
          (Variables|Default|SetAttaqueIndexCurrent (Math|Integer|SelectInt (+ (Variables|Default|GetAttaqueIndexCurrent) 1) 0 (< (Variables|Default|GetAttaqueIndexCurrent) (Variables|Default|GetAttaqueIndexMax)))))
        (:OnCompleted
          ;[1 1 1] Can Attaque again - set index =0 (wtf with le set ?)
          (Variables|Default|SetCanAttaque true))
        (:OnNotifyBegin
          ;[1 1 1] Call Notify
          (switch name _notifyname
            (:Hit
              (CallFunction|TriggerSimpleHit))
            (:CanCombo
              (Variables|Default|SetCanAttaque true))
            (:Recovery
              (Variables|Default|SetCanAttaque false))))))))

(event Custom|GroundCheck
  ;[1 0 0] Si et seulement si on prévoit des saut et donc des attattaques aériennes
  (if (AI|Components|NavMovement|IsMovingonGround (Variables|/Script/Engine.Character|GetCharacterMovement (Variables|Default|GetOwner)))
    (Animation|StopAnimMontage (Variables|Default|GetOwner) (Variables|Default|GetJumpAttaqueAnim))
    (Variables|Default|SetCanAttaque true)
    (Utilities|Time|ClearandInvalidateTimerbyHandle (Variables|Default|GetTimeGroundCheck))))

(event EventBeginPlay
  ;[1 1 1] Check dans la liste des attaques -1 (comparaison tableau)
  (bind _ascharacter (Utilities|Casting|CastToCharacter (Components|GetOwner)))
  (Variables|Default|SetOwner _ascharacter)
  (Variables|Default|SetAttaqueIndexMax (- (Utilities|Array|Length (Variables|Default|GetAnimationAttaque)) 1)))

(event EventTick
  (params (DeltaSeconds :type Float%20%28single-precision%29))
  (Development|PrintString (Utilities|String|ToString(Integer) (Variables|Default|GetAttaqueIndexCurrent))))

(fn TriggerSimpleHit
  (bind _owner (Variables|Default|GetOwner))
  (bind _returnvalue (Transformation|GetActorLocation _owner))
  (bind _returnvalue_2 (Transformation|GetActorForwardVector _owner))
  (bind (_outhit _returnvalue_3) (Class|KismetSystemLibrary|BoxTraceSingleforObjects _returnvalue (+ _returnvalue (* _returnvalue_2 3e+02)) "50.000000,100.000000,50.000000" (Math|Conversions|RotationFromXVector _returnvalue_2) (Utilities|Array|MakeArray "ObjectTypeQuery3") true 0 "ForDuration" true))
  (if _returnvalue_3
    (Game|Damage|ApplyDamage (.HitActor (Collision|BreakHitResult _outhit)) (Variables|Default|GetDamagePlayer) 0 0)
    ;[1 1 1] Syst template = niagara blood.etc
    (Niagara|SpawnSystematLocation "/Game/Core/Cursor/FX_Cursor.FX_Cursor" (.ImpactPoint (Collision|BreakHitResult _outhit)) (Transformation|GetActorRotation (.HitActor (Collision|BreakHitResult _outhit))))))