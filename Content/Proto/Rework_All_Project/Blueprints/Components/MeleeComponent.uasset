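; Melee combat component for player and AI characters, handling light and heavy attack combos, blocking, parrying and stuns.
; Attacks pass the input buffer, queue follow-ups, and push combo- and crit-scaled damage to the weapon's collision component.
; Blocks check facing, then break or notify the attacker's MeleeComponent of a block or timed-window parry.
; Montage lengths set stun durations, after which attack state resets; AI controllers receive combat messages.
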(event Custom|SendLightAttack
  ;[1 1 1] Send Off Attack - Left Click (Attack) - Left Click Again (Save Attack For When First Attack Is Finished) - Attack Combo Triggered in Anim Notify When the Attack Anim almost over
  (if (== (Variables|Default|GetLightAttackCount) (Variables|Default|GetNumberOfLightAttacks))
    (CallFunction|ResetMeleeAttack)
    (CallFunction|ResetAIAttack)
    (else
      (Default|OnActionBegin (Variables|Default|GetInputBufferComponent) "NewEnumerator0")
      (bind _attackno (CallFunction|CalculateLightAttack))
      (CallFunction|SendAttack)
      (Animation|Montage|PlayMontage (Variables|Default|GetCharacterMesh) (Utilities|Select :Index _attackno :Option%200 (Variables|Animations|GetLightAttack1Anim) :Option%201 (Variables|Animations|GetLightAttack2Anim) :Option%202 (Variables|Animations|GetLightAttack3Anim) :Option%203 (Variables|Animations|GetLightAttack4Anim))))))

(event Custom|SendHeavyAttack
  ;[1 1 1] Heavy Attack
  (if (== (Variables|Default|GetHeavyAttackCount) (Variables|Default|GetNumberOfHeavyAttacks))
    (CallFunction|ResetMeleeAttack)
    (CallFunction|ResetAIAttack)
    (else
      (Default|OnActionBegin (Variables|Default|GetInputBufferComponent) "NewEnumerator4")
      (bind _attackno (CallFunction|CalculateHeavyAttack))
      (CallFunction|CalculateSpecialAttackDmg 1.75 "NewEnumerator4")
      (Animation|Montage|PlayMontage (Variables|Default|GetCharacterMesh) (Utilities|Select :Index _attackno :Option%200 (Variables|Animations|GetHeavyAttack1Anim) :Option%201 (Variables|Animations|GetHeavyAttack2Anim))))))

(event Custom|TriggerStun
  (params (StunTimer :type Float%20%28double-precision%29))
  ;[1 1 1] Stun
  (Variables|Default|SetStunned true)
  (Default|ClearBuffer (Variables|Default|GetInputBufferComponent) true)
  (Utilities|FlowControl|RetriggerableDelay StunTimer)
  (Variables|Default|SetStunned false)
  (CallFunction|ResetMeleeAttack))

(event Custom|Initialize
  ;[1 1 1] Setup Components
  (CallFunction|StoreComponents))

(event Custom|AttackCombo
  ;[1 1 1] Send Off Attack - Left Click (Attack) - Left Click Again (Save Attack For When First Attack Is Finished) - Attack Combo Triggered in Anim Notify When the Attack Anim almost over
  (if (Variables|Default|GetSaveAttack)
    (Variables|Default|SetSaveAttack false)
    (if (Variables|Default|GetHeavyAttack)
      (CallFunction|SendHeavyAttack)
      (else
        (CallFunction|SendLightAttack)))
    (else
      (CallFunction|ResetMeleeAttack)
      (CallFunction|ResetAIAttack))))

(event Custom|ReleaseBlock
  ;[1 1 1] Blocking
  (if (Variables|Default|GetBlockUp)
    (Variables|Default|SetBlockUp false)
    (Default|CallUpdateBlock false)
    (Default|ChangeMovementSpeed (Variables|Default|GetMovementComponent) "NewEnumerator0")
    (Default|ConsumeBuffer (Variables|Default|GetInputBufferComponent))
    (else
      (Default|ClearLowPriority (Variables|Default|GetInputBufferComponent)))))

(event Custom|SendBlock
  ;[1 1 1] Blocking
  (if (not (Variables|Default|GetBlockUp))
    (bind _runanimation (Default|CanAnimationPlay (Variables|Default|GetInputBufferComponent) "NewEnumerator2"))
    (if _runanimation
      (Default|OnActionBegin (Variables|Default|GetInputBufferComponent) "NewEnumerator2")
      (Default|CallUpdateBlock true)
      (Default|ChangeMovementSpeed (Variables|Default|GetMovementComponent) "NewEnumerator0")
      (Variables|Default|SetBlockUp true)
      (Variables|Default|SetParryUp true)
      (Utilities|FlowControl|Delay (Variables|Default|GetParryOpening))
      (Variables|Default|SetParryUp false))))

(event Custom|BlockBroken
  (bind _blockbreakanim (Variables|Animations|GetBlockBreakAnim))
  ;[1 1 1] Your Block Has Broken
  (CallFunction|PlaySound)
  (CallFunction|CombatText "NewEnumerator0")
  (CallFunction|BlockBreakWB)
  (Class|IAIController|BlockBreak(Message) (AI|GetAIController (Components|GetOwner)))
  (Default|ChangeMovementSpeed (Variables|Default|GetMovementComponent) "NewEnumerator0")
  (Variables|Default|SetBlockUp false)
  (Default|CallUpdateBlock false)
  (Utilities|IsValid _blockbreakanim
    (:Is%20Valid
      (CallFunction|SendStunCalculation (Variables|/Script/Engine.AnimSequenceBase|GetSequenceLength _blockbreakanim) 1.0)
      (Animation|Montage|PlayMontage (Variables|Default|GetCharacterMesh) (Variables|Animations|GetBlockBreakAnim)))))

(event Custom|AttackParried
  (bind _attackblockedanim (Variables|Animations|GetAttackBlockedAnim))
  ;[1 1 1] Attack Parried
  (CallFunction|PlaySound)
  (CallFunction|StopAttackTrace)
  (CallFunction|ResetAIAttack)
  (Utilities|IsValid _attackblockedanim ; Fists Don't have Attack Blocked Anim
    (:Is%20Valid
      (CallFunction|SendStunCalculation (Variables|/Script/Engine.AnimSequenceBase|GetSequenceLength _attackblockedanim) 0.7)
      (Animation|Montage|PlayMontage (Variables|Default|GetCharacterMesh) (Variables|Animations|GetAttackBlockedAnim) 0.7))))

(event Custom|EventHeavyAttack
  ;[1 1 1] Heavy Attack
  (Utilities|IsValid (Variables|Animations|GetHeavyAttack1Anim)
    (:Is%20Valid
      (if (Utilities|Enum|Equal(Enum) (Variables|/Game/Proto/Rework_All_Project/Blueprints/Components/CombatStatusComponent.CombatStatusComponent_C|GetCurrentAttackStyle (Variables|Default|GetCombatStatusComp)) "NewEnumerator0")
        (bind _runanimation (Default|CanAnimationPlay (Variables|Default|GetInputBufferComponent) "NewEnumerator4"))
        (if _runanimation
          (if (Variables|Default|GetAttacking?)
            (Variables|Default|SetSaveAttack true)
            (Variables|Default|SetHeavyAttack true)
            (else
              (Variables|Default|SetAttacking? true)
              (Variables|Default|SetHeavyAttack true)
              (Default|OnActionBegin (Variables|Default|GetInputBufferComponent) "NewEnumerator4")
              (bind _attackno (CallFunction|CalculateHeavyAttack))
              (CallFunction|CalculateSpecialAttackDmg 1.75 "NewEnumerator4")
              (Animation|Montage|PlayMontage (Variables|Default|GetCharacterMesh) (Utilities|Select :Index _attackno :Option%200 (Variables|Animations|GetHeavyAttack1Anim) :Option%201 (Variables|Animations|GetHeavyAttack2Anim))))))))))

(event Custom|EventLightAttack
  ;[1 1 1] Send Off Attack - Left Click (Attack) - Left Click Again (Save Attack For When First Attack Is Finished) - Attack Combo Triggered in Anim Notify When the Attack Anim almost over
  (bind _runanimation (Default|CanAnimationPlay (Variables|Default|GetInputBufferComponent) "NewEnumerator4"))
  (if _runanimation
    (if (Variables|Default|GetAttacking?)
      (Variables|Default|SetSaveAttack true)
      (Variables|Default|SetHeavyAttack false)
      (else
        (Variables|Default|SetAttacking? true)
        (Variables|Default|SetHeavyAttack false)
        (Default|OnActionBegin (Variables|Default|GetInputBufferComponent) "NewEnumerator0")
        (bind _attackno (CallFunction|CalculateLightAttack))
        (CallFunction|SendAttack)
        (Animation|Montage|PlayMontage (Variables|Default|GetCharacterMesh) (Utilities|Select :Index _attackno :Option%200 (Variables|Animations|GetLightAttack1Anim) :Option%201 (Variables|Animations|GetLightAttack2Anim) :Option%202 (Variables|Animations|GetLightAttack3Anim) :Option%203 (Variables|Animations|GetLightAttack4Anim)))))))

(event Custom|EventBlock
  (params (Attack%20Type :type E_CharacterAction%20Enum :default "NewEnumerator4"))
  ;[1 1 1] Blocked Damage
  ;;[1 1 1] Check If Blocking Facing Attacker
  (bind _facingattackor (CallFunction|CheckAngleforBlock))
  (if _facingattackor
    (if (CallFunction|BreakBlockConditions Attack%20Type)
      (CallFunction|BreakBlockTakeDamage true (Variables|Default|GetDamageInc)) ; Block Broken
      (else
        ;;[1 1 1] Check IF You Have Enough Stamina For Block
        (if true
          (Class|IAIController|BlockedAttack(Message) (AI|GetAIController (Components|GetOwner)))
          (CallFunction|EnemyBlockHit)
          (CallFunction|BlockEmitterandText)
          (CallFunction|SendStunCalculation (Variables|/Script/Engine.AnimSequenceBase|GetSequenceLength (Variables|Animations|GetBlockImpactAnim)) 1.0)
          (Animation|Montage|PlayMontage (Variables|Default|GetCharacterMesh) (Variables|Animations|GetBlockImpactAnim)))))
    (else
      (Default|TakeDamage (Variables|Default|GetTakingDamageComponent)))))

(event Custom|AttackBlocked
  (bind _attackblockedanim (Variables|Animations|GetAttackBlockedAnim))
  ;[1 1 1] Your Attack Has Been Blocked
  (CallFunction|PlaySound)
  (CallFunction|StopAttackTrace)
  (bind _play_rate (CallFunction|CalculateKnockTime))
  (Utilities|IsValid _attackblockedanim
    (:Is%20Valid
      (CallFunction|SendStunCalculation (Variables|/Script/Engine.AnimSequenceBase|GetSequenceLength _attackblockedanim) _play_rate))
    (:Is%20Not%20Valid
      _))
  (Animation|Montage|PlayMontage (Variables|Default|GetCharacterMesh) (Variables|Animations|GetAttackBlockedAnim) _play_rate))

(fn CalculateLightAttack
  (if (== (Variables|Default|GetLightAttackCount) (Variables|Default|GetNumberOfLightAttacks))
    (Variables|Default|SetLightAttackCount 1)
    (else
      (bind _output_get (Variables|Default|SetLightAttackCount (Utilities|Select :Index (Variables|Default|GetLightAttackCount) :Option%200 1 :Option%201 2 :Option%202 3 :Option%203 4)))
      (if (>= (Variables|Default|GetNumberOfLightAttacks) _output_get)
        _
        (else
          (Variables|Default|SetLightAttackCount 1)))))
  (Math|Integer|IncrementInt (Variables|Default|GetComboNumber)
    (:%20%20
      (return (- (Variables|Default|GetLightAttackCount) 1)))))

(fn SendAttack
  (Variables|Default|SetAttackType "NewEnumerator0")
  ;[1 1 1] Calculates Weapon Damage
  (bind (_mainhanddamage _mainhandcritical) (CallFunction|CalculateMeleeDamage))
  ;[1 1 1] Sends Newly Calculated Damage To Weapon/Fists
  (CallFunction|SendAttackInfo (Variables|WeaponRef|GetEquippedMainHand) _mainhanddamage _mainhandcritical))

(fn CalculateMeleeDamage
  ;[1 1 1] Calculates Damaged Based Upon Mele Damage, Combo Attack & Crit Chance
  (LocalVariables|SetComboDamageMultiplier (Utilities|Select :Index (Variables|Default|GetComboNumber) :Option%200 1.0 :Option%201 1.0 :Option%202 1.2 :Option%203 1.4 :Option%204 1.6 :Option%205 1.8 :Option%206 2.0))
  (return (.Damage (CallFunction|CalculateDamage (Variables|/Game/Proto/Rework_All_Project/Blueprints/Components/EquipmentComponent.EquipmentComponent_C|GetMaxMainHandDmg (Variables|Default|GetEquipmentComponent)) (LocalVariables|GetComboDamageMultiplier))) (.CriticalHit (CallFunction|CalculateDamage (Variables|/Game/Proto/Rework_All_Project/Blueprints/Components/EquipmentComponent.EquipmentComponent_C|GetMaxMainHandDmg (Variables|Default|GetEquipmentComponent)) (LocalVariables|GetComboDamageMultiplier)))))

(fn CalculateDamage
  (params (WeaponDamage :type Float%20%28double-precision%29) (ComboAttackNo :type Float%20%28double-precision%29))
  (bind _returnvalue (Math|Random|RandomFloatinRange 0.0 1e+02))
  (bind _equipmentcomponent (Variables|Default|GetEquipmentComponent))
  (bind _critchance (Variables|/Game/Proto/Rework_All_Project/Blueprints/Components/EquipmentComponent.EquipmentComponent_C|GetCritChance _equipmentcomponent))
  (bind _returnvalue_2 (< _returnvalue _critchance))
  ;[1 1 1] Increase Damage Based Upon Combo
  (return (* (* (CallFunction|RandomMinMaxValue WeaponDamage) ComboAttackNo) (Math|Float|SelectFloat 2.0 1.0 _returnvalue_2)) _returnvalue_2))

(fn SetMeleeAnimOutput
  (params (Selection :type E_WeaponType%20Enum :default "NewEnumerator2"))
  (Utilities|FlowControl|Sequence
    (:then_0
      (switch Utilities|FlowControl|Switch|SwitchonE_WeaponType Selection))
    (:then_1
      (CallFunction|CalculateWeaponAttackNumber))))

(fn SendAttackInfo
  (params (Weapon :type Actor%20Object%20Reference) (WeaponDmg :type Float%20%28double-precision%29) (CriticalHit :type Boolean))
  (bind _returnvalue (Actor|GetComponentbyClass Weapon "/Game/Proto/Rework_All_Project/Blueprints/Components/WeaponCollision.WeaponCollision_C"))
  (Utilities|IsValid Weapon
    (:Is%20Valid
      (Variables|/Game/Proto/Rework_All_Project/Blueprints/Components/WeaponCollision.WeaponCollision_C|SetWeaponOutputDamage _returnvalue WeaponDmg)
      (Variables|/Game/Proto/Rework_All_Project/Blueprints/Components/WeaponCollision.WeaponCollision_C|SetCriticalHit _returnvalue CriticalHit)
      (Variables|/Game/Proto/Rework_All_Project/Blueprints/Components/WeaponCollision.WeaponCollision_C|SetAttackType _returnvalue (Variables|Default|GetAttackType)))))

(fn ResetMeleeAttack
  ;[1 1 1] Resets All Attack Variables & Stops Weapon Line Trace (For Generating Hit Results)
  (Variables|Default|SetAttacking? false)
  (Variables|Default|SetSaveAttack false)
  (Variables|Default|SetLightAttackCount 0)
  (Variables|Default|SetHeavyAttackCount 0)
  (Variables|Default|SetComboNumber 0)
  (CallFunction|StopAttack (Utilities|Array|MakeArray (Variables|WeaponRef|GetEquippedMainHand) 0 0)))

(fn StopAttack
  (params (Weapon%20Array :type Array%20of%20Actor%20Object%20References))
  (for _array_element Weapon%20Array
    (Utilities|IsValid _array_element
      (:Is%20Valid
        (Default|StopAttack (Actor|GetComponentbyClass _array_element "/Game/Proto/Rework_All_Project/Blueprints/Components/WeaponCollision.WeaponCollision_C"))))))

(fn CheckAngleforBlock
  (bind _returnvalue (Components|GetOwner))
  (return (Math|Float|NearlyEqual(Float) (.Yaw (Math|Rotator|BreakRotator (Transformation|GetActorRotation _returnvalue))) (.Yaw (Math|Rotator|BreakRotator (Math|Rotator|FindLookatRotation (Transformation|GetActorLocation _returnvalue) (Transformation|GetActorLocation (Variables|Default|GetAttackingActor))))) 3e+01)))

(fn CalculateSpecialAttackDmg
  (params (DamageMultiplier :type Float%20%28double-precision%29) (AttackType :type E_CharacterAction%20Enum :default "NewEnumerator4"))
  (Variables|Default|SetAttackType AttackType)
  (bind (_mainhanddamage _mainhandcritical) (CallFunction|CalculateMeleeDamage))
  ;[1 1 1] IF Dual-Wield Combine Damage
  (if (and (Utilities|IsValid (Variables|WeaponRef|GetEquippedMainHand)) (Utilities|IsValid (Variables|WeaponRef|GetEquippedMainHand)))
    (CallFunction|SendAttackInfo (Variables|WeaponRef|GetEquippedMainHand) (* (+ _mainhanddamage 1.0) (- DamageMultiplier 0.25)) (or _mainhandcritical false))
    (CallFunction|SendAttackInfo 0 0.0 false)
    (else
      ;[1 1 1] Send Damage To Either Main Hand OR Off-Hand
      (Utilities|FlowControl|Sequence
        (:then_0
          (Utilities|IsValid (Variables|WeaponRef|GetEquippedMainHand)
            (:Is%20Valid
              (CallFunction|SendAttackInfo (Variables|WeaponRef|GetEquippedMainHand) (* _mainhanddamage DamageMultiplier) _mainhandcritical))))
        (:then_1
          (Utilities|IsValid 0
            (:Is%20Valid
              (CallFunction|SendAttackInfo 0 (* 0.0 DamageMultiplier) _mainhandcritical))))))))

(fn IsPlayingMontage
  (return (Animation|Montage|MontageIsPlaying (Components|SkeletalMesh|GetAnimInstance (Variables|Default|GetCharacterMesh)) 0)))

(fn IsSpecificPlayingMontage
  (params (Montage :type Anim%20Montage%20Object%20Reference))
  (return (Animation|Montage|MontageIsPlaying (Components|SkeletalMesh|GetAnimInstance (Variables|Default|GetCharacterMesh)) Montage)))

(fn StoreComponents
  (bind _returnvalue (Components|GetOwner))
  (Variables|Default|SetMovementComponent (Actor|GetComponentbyClass _returnvalue "/Game/Proto/Rework_All_Project/Blueprints/Components/MovementStatusComponent.MovementStatusComponent_C"))
  (Variables|Default|SetEquipmentComponent (Actor|GetComponentbyClass _returnvalue "/Game/Proto/Rework_All_Project/Blueprints/Components/EquipmentComponent.EquipmentComponent_C"))
  (Variables|Default|SetInputBufferComponent (Actor|GetComponentbyClass _returnvalue "/Game/Proto/Rework_All_Project/Blueprints/Components/InputBufferComponent.InputBufferComponent_C"))
  (Variables|Default|SetTakingDamageComponent (Actor|GetComponentbyClass _returnvalue "/Game/Proto/Rework_All_Project/Blueprints/Components/TakingDamage.TakingDamage_C"))
  (Variables|Default|SetCombatStatusComp (Actor|GetComponentbyClass _returnvalue "/Game/Proto/Rework_All_Project/Blueprints/Components/CombatStatusComponent.CombatStatusComponent_C"))
  (bind _ascharacter (Utilities|Casting|CastToCharacter _returnvalue))
  (Variables|Components|SetCharacterRef _ascharacter)
  (Variables|Default|SetCharacterMesh (Variables|/Script/Engine.Character|GetMesh _ascharacter))
  (Variables|Default|SetCapsuleComponent (Variables|/Script/Engine.Character|GetCapsuleComponent _ascharacter)))

(fn CalculateWeaponAttackNumber
  ;[1 1 1] Increments 1 Value Every Valid Animation
  (Utilities|FlowControl|Sequence
    (:then_0
      (Variables|Default|SetNumberOfLightAttacks 0)
      (Utilities|IsValid (Variables|Animations|GetLightAttack1Anim)
        (:Is%20Valid
          (Math|Integer|IncrementInt (Variables|Default|GetNumberOfLightAttacks)
            (:%20%20
              _)))
        (:Is%20Not%20Valid
          _))
      (Utilities|IsValid (Variables|Animations|GetLightAttack2Anim)
        (:Is%20Valid
          (Math|Integer|IncrementInt (Variables|Default|GetNumberOfLightAttacks)
            (:%20%20
              _)))
        (:Is%20Not%20Valid
          _))
      (Utilities|IsValid (Variables|Animations|GetLightAttack3Anim)
        (:Is%20Valid
          (Math|Integer|IncrementInt (Variables|Default|GetNumberOfLightAttacks)
            (:%20%20
              _)))
        (:Is%20Not%20Valid
          _))
      (Utilities|IsValid (Variables|Animations|GetLightAttack4Anim)
        (:Is%20Valid
          (Math|Integer|IncrementInt (Variables|Default|GetNumberOfLightAttacks)))))
    (:then_1
      (Variables|Default|SetNumberOfHeavyAttacks 0)
      (Utilities|IsValid (Variables|Animations|GetHeavyAttack1Anim)
        (:Is%20Valid
          (Math|Integer|IncrementInt (Variables|Default|GetNumberOfHeavyAttacks)
            (:%20%20
              _)))
        (:Is%20Not%20Valid
          _))
      (Utilities|IsValid (Variables|Animations|GetHeavyAttack2Anim)
        (:Is%20Valid
          (Math|Integer|IncrementInt (Variables|Default|GetNumberOfHeavyAttacks)))))))

(fn CalculateHeavyAttack
  (if (== (Variables|Default|GetHeavyAttackCount) (Variables|Default|GetNumberOfHeavyAttacks))
    (Variables|Default|SetHeavyAttackCount 1)
    (else
      (bind _output_get (Variables|Default|SetHeavyAttackCount (Utilities|Select :Index (Variables|Default|GetHeavyAttackCount) :Option%200 1 :Option%201 2 :Option%202 3 :Option%203 4)))
      (if (>= (Variables|Default|GetNumberOfHeavyAttacks) _output_get)
        _
        (else
          (Variables|Default|SetHeavyAttackCount 1)))))
  (Math|Integer|IncrementInt (Variables|Default|GetComboNumber)
    (:%20%20
      (return (- (Variables|Default|GetHeavyAttackCount) 1)))))

(fn CalculateKnockTime
  (return (Utilities|Select :Index (Variables|Default|GetAttackType) :Option%200 0.0 :Option%201 0.0 :Option%202 0.0 :Option%203 0.0 :Option%204 0.0 :Option%205 0.0 :Option%206 0.0 :Option%207 0.0 :Option%208 0.0 :Option%209 0.0 :Option%2010 0.0 :Option%2011 0.0 :Option%2012 0.0 :Option%2013 0.0 :Option%2014 0.0 :Option%2015 0.0 :Option%2016 0.0 :Option%2017 0.0 :Option%2018 0.0)))

(fn StopAttackTrace
  (CallFunction|StopAttack (Utilities|Array|MakeArray (Variables|WeaponRef|GetEquippedMainHand) 0 0)))

(fn ResetAIAttack
  (Class|IAIController|BeginAttackTimer(Message) (AI|GetAIController (Components|GetOwner))))

(fn BreakBlockTakeDamage
  (params (BlockBreakAnim :type Boolean) (StaminaDrained :type Float%20%28double-precision%29))
  (if BlockBreakAnim
    ;[1 1 1] Takes Damage then players Block Break Anim
    (Default|TakeDamage (Variables|Default|GetTakingDamageComponent))
    (CallFunction|BlockBroken)
    (else
      ;[1 1 1] Block Break Anim Overwritten By Damage
      (CallFunction|BlockBroken)
      (Default|TakeDamage (Variables|Default|GetTakingDamageComponent)))))

(fn BreakBlockConditions
  (params (AttackType :type E_CharacterAction%20Enum :default "NewEnumerator4"))
  (return (or (Utilities|Enum|Equal(Enum) AttackType "NewEnumerator4") (and (Utilities|Enum|Equal(Enum) AttackType "NewEnumerator4") (not (Variables|Default|GetParryUp))))))

(fn BlockEmitterandText
  ;[1 1 1] Combat Text & PS
  (CallFunction|CombatText (select (Variables|Default|GetParryUp) "NewEnumerator11" "NewEnumerator10"))
  (Effects|SpawnEmitteratLocation 0 (Variables|Default|GetImpactPoint)))

(fn CombatText
  (params (CombatTextType :type E_CombatTextType%20Enum :default "NewEnumerator0"))
  (bind _returnvalue (Components|GetOwner))
  (bind _attackingactor (Variables|Default|GetAttackingActor))
  (bind _returnvalue_2 (Actor|ActorHasTag _returnvalue "Player"))
  (bind _returnvalue_3 (select _returnvalue_2 _returnvalue _attackingactor))
  (bind _returnvalue_4 (Actor|GetComponentbyClass _returnvalue_3 "/Game/Proto/Rework_All_Project/Blueprints/Components/CombatTextComponent.CombatTextComponent_C"))
  (Utilities|IsValid _returnvalue_4
    (:Is%20Valid
      (Default|CombatTextPopup _returnvalue_4 (Transformation|GetActorLocation (Components|GetOwner)) 0 CombatTextType false false (Actor|ActorHasTag (Components|GetOwner) "Player")))))

(fn SendStunCalculation
  (params (AnimLength :type Float%20%28double-precision%29) (PlayRate :type Float%20%28double-precision%29))
  (bind _characterref (Variables|Components|GetCharacterRef))
  (Utilities|IsValid _characterref
    (:Is%20Valid
      (CallFunction|TriggerStun (- (/ AnimLength PlayRate) (Math|Float|SelectFloat 0.2 (LocalVariables|GetStunAdjuster) (Actor|ActorHasTag _characterref "EnemyAI")))))))

(fn EnemyBlockHit
  (bind _attackingactor (Variables|Default|GetAttackingActor))
  (bind _returnvalue (Actor|GetComponentbyClass _attackingactor "MeleeComponent_C"))
  (if (Utilities|Enum|Equal(Enum) (Variables|/Game/Proto/Rework_All_Project/Blueprints/Components/CombatStatusComponent.CombatStatusComponent_C|GetCurrentAttackStyle (Actor|GetComponentbyClass (Variables|Default|GetAttackingActor) "/Game/Proto/Rework_All_Project/Blueprints/Components/CombatStatusComponent.CombatStatusComponent_C")) "NewEnumerator0")
    (if (Variables|Default|GetParryUp)
      (CallFunction|AttackParried _returnvalue)
      (else
        (CallFunction|AttackBlocked _returnvalue)))))

(fn BlockBreakWB
  (if (Actor|ActorHasTag (Components|GetOwner) "Player")
    (bind _returnvalue (UserInterface|CreateWidget "/Game/Proto/Rework_All_Project/Widgets/Combat/WB_BlockBreak.WB_BlockBreak_C"))
    (UserInterface|Viewport|AddtoViewport _returnvalue 0)))

(fn RemoveAssassinationWep
  (bind _combatstatuscomp (Variables|Default|GetCombatStatusComp))
  (Utilities|IsValid _combatstatuscomp
    (:Is%20Valid
      (Actor|DestroyActor (Variables|/Game/Proto/Rework_All_Project/Blueprints/Components/CombatStatusComponent.CombatStatusComponent_C|GetEquippedMainHand _combatstatuscomp)))))

(fn PlaySound
  (params (Sound :type Sound%20Base%20Object%20Reference))
  (Audio|PlaySoundatLocation Sound (Transformation|GetActorLocation (Components|GetOwner)) "0, 0, 0" 1.0 1.0 0.0 0 0 0 0))

(fn Add/RemoveCollision
  (params (Remove :type Boolean))
  ;[1 1 1] Add any more Collision channels on the end!
  (Collision|SetCollisionResponsetoChannel (Variables|Default|GetCapsuleComponent) "ECC_Pawn" (select Remove "ECR_Ignore" "ECR_Block"))
  (Collision|SetCollisionResponsetoChannel (Variables|Default|GetCapsuleComponent) "ECC_WorldStatic" (select Remove "ECR_Ignore" "ECR_Block"))
  (Collision|SetCollisionResponsetoChannel (Variables|Default|GetCapsuleComponent) "ECC_WorldDynamic" (select Remove "ECR_Ignore" "ECR_Block")))