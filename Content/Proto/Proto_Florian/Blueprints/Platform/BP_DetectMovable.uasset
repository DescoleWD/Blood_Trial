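; Prototype moving platform that reacts to the main character, tagged Player, overlapping its Box.
; Entering the box eases the static mesh to a second relative location with MoveComponentTo, then flags the move as finished.
; Leaving the box or the PlayerFall event sends it back after a short delay, but only if the outbound move has finished.
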(event OnComponentBeginOverlap(Box)
  (params (OverlappedComponent :type Primitive%20Component%20Object%20Reference) (OtherActor :type Actor%20Object%20Reference) (OtherComp :type Primitive%20Component%20Object%20Reference) (OtherBodyIndex :type Integer) (bFromSweep :type Boolean) (SweepResult :type Hit%20Result%20Structure%20%28by%20ref%29))
  (bind _asbp_main_character (Utilities|Casting|CastToBP_MainCharacter OtherActor))
  (if (Actor|ActorHasTag _asbp_main_character "Player")
    (Variables|Default|SetHaveMoved true)
    (Components|MoveComponentTo (Variables|Default|GetStaticMesh) (Variables|Default|GetPlatLocation2) "0, 0, 0" true true 1.5 false)
    (Variables|Default|SetFinishMovement true)))

(event OnComponentEndOverlap(Box)
  (params (OverlappedComponent :type Primitive%20Component%20Object%20Reference) (OtherActor :type Actor%20Object%20Reference) (OtherComp :type Primitive%20Component%20Object%20Reference) (OtherBodyIndex :type Integer))
  (bind _asbp_main_character (Utilities|Casting|CastToBP_MainCharacter OtherActor))
  (if (Actor|ActorHasTag _asbp_main_character "Player")
    (if (Variables|Default|GetHaveMoved)
      (if (Variables|Default|GetFinishMovement)
        (Utilities|FlowControl|Delay 0.5)
        (Variables|Default|SetHaveMoved false)
        (Components|MoveComponentTo (Variables|Default|GetStaticMesh) (Variables|Default|GetPlatLocation1) "0, 0, 0" true true 1.0 false)
        (Variables|Default|SetFinishMovement false)))))

(event Custom|PlayerFall
  (if (Variables|Default|GetHaveMoved)
    (if (Variables|Default|GetFinishMovement)
      (Utilities|FlowControl|Delay 0.5)
      (Variables|Default|SetHaveMoved false)
      (Components|MoveComponentTo (Variables|Default|GetStaticMesh) (Variables|Default|GetPlatLocation1) "0, 0, 0" true true 1.0 false)
      (Variables|Default|SetFinishMovement false))))

(fn ConstructionScript)