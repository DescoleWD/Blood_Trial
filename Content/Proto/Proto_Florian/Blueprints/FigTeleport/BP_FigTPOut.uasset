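; Exit teleporter that sends the main character to the exit point of one of the numbered FigTPIn teleporters.
; On box overlap, a sequence checks each FigTeleportIn flag from GetInst, teleports the character to that entrance actor's ExitRef, then clears the flag.
; The branch for teleporter 3 does nothing, as its teleport logic is disconnected.
; The construction script positions this actor's Teleport and ExitRef components from variables.
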(event OnComponentBeginOverlap(Box)
  (params (OverlappedComponent :type Primitive%20Component%20Object%20Reference) (OtherActor :type Actor%20Object%20Reference) (OtherComp :type Primitive%20Component%20Object%20Reference) (OtherBodyIndex :type Integer) (bFromSweep :type Boolean) (SweepResult :type Hit%20Result%20Structure%20%28by%20ref%29))
  (bind _asbp_main_character (Utilities|Casting|CastToBP_MainCharacter OtherActor))
  (Utilities|FlowControl|Sequence
    (:then_0
      (if (Variables|/Game/Proto/Main/Blueprint/BloodTrial_GameInstance.BloodTrial_GameInstance_C|GetFigTeleportIn1 (CallFunction|GetInst))
        (bind _returnvalue (Actor|GetActorOfClass "/Game/Proto/Proto_Florian/Blueprints/FigTeleport/BP_FigTPIn1.BP_FigTPIn1_C"))
        (Transformation|Teleport _asbp_main_character (Transformation|GetWorldLocation (Variables|/Game/Proto/Proto_Florian/Blueprints/FigTeleport/BP_FigTPIn1.BP_FigTPIn1_C|GetExit%20Ref _returnvalue)) "0, 0, 0")
        (Variables|/Game/Proto/Main/Blueprint/BloodTrial_GameInstance.BloodTrial_GameInstance_C|SetFigTeleportIn1 (CallFunction|GetInst) false)))
    (:then_1
      (if (Variables|/Game/Proto/Main/Blueprint/BloodTrial_GameInstance.BloodTrial_GameInstance_C|GetFigTeleportIn2 (CallFunction|GetInst))
        (bind _returnvalue_2 (Actor|GetActorOfClass "/Game/Proto/Proto_Florian/Blueprints/FigTeleport/BP_FigTPIn2.BP_FigTPIn2_C"))
        (Transformation|Teleport _asbp_main_character (Transformation|GetWorldLocation (Variables|/Game/Proto/Proto_Florian/Blueprints/FigTeleport/BP_FigTPIn2.BP_FigTPIn2_C|GetExit%20Ref _returnvalue_2)) "0, 0, 0")
        (Variables|/Game/Proto/Main/Blueprint/BloodTrial_GameInstance.BloodTrial_GameInstance_C|SetFigTeleportIn2 (CallFunction|GetInst) false)))
    (:then_2
      (if (Variables|/Game/Proto/Main/Blueprint/BloodTrial_GameInstance.BloodTrial_GameInstance_C|GetFigTeleportIn3 (CallFunction|GetInst))
        _))
    (:then_3
      (if (Variables|/Game/Proto/Main/Blueprint/BloodTrial_GameInstance.BloodTrial_GameInstance_C|GetFigTeleportIn4 (CallFunction|GetInst))
        (bind _returnvalue_3 (Actor|GetActorOfClass "/Game/Proto/Proto_Florian/Blueprints/FigTeleport/BP_FigTPIn4.BP_FigTPIn4_C"))
        (Transformation|Teleport _asbp_main_character (Transformation|GetWorldLocation (Variables|/Game/Proto/Proto_Florian/Blueprints/FigTeleport/BP_FigTPIn4.BP_FigTPIn4_C|GetExit%20Ref _returnvalue_3)) "0, 0, 0")
        (Variables|/Game/Proto/Main/Blueprint/BloodTrial_GameInstance.BloodTrial_GameInstance_C|SetFigTeleportIn4 (CallFunction|GetInst) false)))
    (:then_4
      (if (Variables|/Game/Proto/Main/Blueprint/BloodTrial_GameInstance.BloodTrial_GameInstance_C|GetFigTeleportIn5 (CallFunction|GetInst))
        (bind _returnvalue_4 (Actor|GetActorOfClass "/Game/Proto/Proto_Florian/Blueprints/FigTeleport/BP_FigTPIn5.BP_FigTPIn5_C"))
        (Transformation|Teleport _asbp_main_character (Transformation|GetWorldLocation (Variables|/Game/Proto/Proto_Florian/Blueprints/FigTeleport/BP_FigTPIn5.BP_FigTPIn5_C|GetExit%20Ref _returnvalue_4)) "0, 0, 0")
        (Variables|/Game/Proto/Main/Blueprint/BloodTrial_GameInstance.BloodTrial_GameInstance_C|SetFigTeleportIn5 (CallFunction|GetInst) false)))
    (:then_5
      (if (Variables|/Game/Proto/Main/Blueprint/BloodTrial_GameInstance.BloodTrial_GameInstance_C|GetFigTeleportIn6 (CallFunction|GetInst))
        (bind _returnvalue_5 (Actor|GetActorOfClass "/Game/Proto/Proto_Florian/Blueprints/FigTeleport/BP_FigTPIn6.BP_FigTPIn6_C"))
        (Transformation|Teleport _asbp_main_character (Transformation|GetWorldLocation (Variables|/Game/Proto/Proto_Florian/Blueprints/FigTeleport/BP_FigTPIn6.BP_FigTPIn6_C|GetExit%20Ref _returnvalue_5)) "0, 0, 0")
        (Variables|/Game/Proto/Main/Blueprint/BloodTrial_GameInstance.BloodTrial_GameInstance_C|SetFigTeleportIn6 (CallFunction|GetInst) false)))
    (:then_6
      (if (Variables|/Game/Proto/Main/Blueprint/BloodTrial_GameInstance.BloodTrial_GameInstance_C|GetFigTeleportIn7 (CallFunction|GetInst))
        (bind _returnvalue_6 (Actor|GetActorOfClass "/Game/Proto/Proto_Florian/Blueprints/FigTeleport/BP_FigTPIn7.BP_FigTPIn7_C"))
        (Transformation|Teleport _asbp_main_character (Transformation|GetWorldLocation (Variables|/Game/Proto/Proto_Florian/Blueprints/FigTeleport/BP_FigTPIn7.BP_FigTPIn7_C|GetExit%20Ref _returnvalue_6)) "0, 0, 0")
        (Variables|/Game/Proto/Main/Blueprint/BloodTrial_GameInstance.BloodTrial_GameInstance_C|SetFigTeleportIn7 (CallFunction|GetInst) false)))))

(fn ConstructionScript
  ;[1 1 1] Set Enter And Exit Location
  (Transformation|SetRelativeTransform (Variables|Default|GetTeleport) (Variables|Default|GetTeleport%20Transform) false false)
  (Transformation|SetRelativeLocation (Variables|Default|GetExit%20Ref) (Variables|Default|GetExit%20Location) false false))